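; Spear projectile for TafaiFighter that turns toward the player, waits a warning delay, then flies forward on a looping timer.
; Each tick traces from actor to tip; hitting the player's Shield-tagged component plays a block sound, otherwise deals damage.
; Either hit stops the timer and hands the spear back to the enemy spawner for retrieval.
; In tutorial mode, launch shows the shield tutorial and pauses the game, and stopping hides it.
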(event Custom|InitilizeSpear
  (bind _spawnerennemiref (Variables|Reference|GetSpawnerEnnemiRef))
  (bind _wbp_tuto (Variables|/Game/04-TafaiFighter/Blueprints/BP_SpawnerEnnemi.BP_SpawnerEnnemi_C|GetWBP_Tuto _spawnerennemiref))
  ;[1 1 1] Set Rotation to the player, wait the warning delay and launch a spear
  (Transformation|SetActorRotation (Math|Rotator|FindLookatRotation (Transformation|GetActorLocation) (Math|Vector|MakeVector 0.0 0.0 1.5e+02)))
  (Utilities|FlowControl|Delay (Variables|Property|GetWarningDelay))
  (Movement|FLaunchSpear)
  ;[1 1 1] If it the tutorial. It's gonna launch the tuto of the spear
  (if (Variables|Property|GetbTuto?)
    (Utilities|FlowControl|Delay 0.2)
    (Class|WidgetSwitcher|SetActiveWidgetIndex (Variables|/Game/04-TafaiFighter/Widget/WBP_Tuto.WBP_Tuto_C|GetTutoSwitcher _wbp_tuto) 2)
    (Default|PlayTutoShield _wbp_tuto)
    (Game|SetGamePaused true)))

(fn ConstructionScript)

(fn FMoveSpear
  (Transformation|AddActorLocalOffset (Math|Vector|MakeVector (Variables|Movement|GetSpearSpeed) 0.0 0.0) false false) ; Move the spear
  ;[1 1 1] Search if he hit the player
  (bind _outhit (Collision|LineTraceByChannel (Transformation|GetActorLocation) (Transformation|GetWorldLocation (Variables|Default|GetPointe)) "TraceTypeQuery1" false 0 "None"))
  (bind _asbp_tafai_tafai_fighter (Utilities|Casting|CastToBP_Tafai_TafaiFighter (.HitActor (Collision|BreakHitResult _outhit))))
  (if (Components|ComponentHasTag (.HitComponent (Collision|BreakHitResult _outhit)) "Shield")
    (Audio|PlaySound2D "/Game/04-TafaiFighter/SFX/fighter/S_shield_hit.S_shield_hit" 1.67 1.0 0.0 0 0)
    (else
      (Default|RecieveDamage _asbp_tafai_tafai_fighter 1) ; If the player haven't shild apply damage to the player
    ))
  (Movement|FStopSpear)
  (return))

(fn FLaunchSpear
  (bind _returnvalue (Utilities|Time|SetTimerbyFunctionName self "F_MoveSpear" 0.01 true))
  (Variables|Timer|SetTimerMoveSpear _returnvalue)
  (return))

(fn FStopSpear
  (bind _spawnerennemiref (Variables|Reference|GetSpawnerEnnemiRef))
  (bind _wbp_tuto (Variables|/Game/04-TafaiFighter/Blueprints/BP_SpawnerEnnemi.BP_SpawnerEnnemi_C|GetWBP_Tuto _spawnerennemiref))
  ;[1 1 1] arrete la lance et la tp au point initial
  (Utilities|Time|ClearandInvalidateTimerbyHandle (Variables|Timer|GetTimerMoveSpear))
  (Default|FRetakeSpear (Variables|Reference|GetSpawnerEnnemiRef) self)
  ;[1 1 1] Désactive le widget tuto
  (if (Variables|Property|GetbTuto?)
    (Class|WidgetSwitcher|SetActiveWidgetIndex (Variables|/Game/04-TafaiFighter/Widget/WBP_Tuto.WBP_Tuto_C|GetTutoSwitcher _wbp_tuto))
    (Default|StopTutoShield _wbp_tuto)
    (return)
    (else
      (return))))