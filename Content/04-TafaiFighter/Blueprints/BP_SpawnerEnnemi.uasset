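; Spawner for the Tafai Fighter minigame that sends enemies and warned spears in from the left or right.
; Pre-spawns both off to the side as pools, which launches draw from and retake functions refill.
; Looping timers randomize side, enemy weak point and spear chance, and launches cease near game end.
; On first play, a scripted tutorial runs first, and the spear's return leads to a paused tip and the normal cycle.
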(event EventBeginPlay
  (StartSetting|FReference)
  (StartSetting|FSpawnEnnemi)
  (StartSetting|FSpawnSpear)
  ;[1 1 1] Is it the first time
  (Utilities|FlowControl|Delay 1.0) ; Delay of 1s for the fade in the loading map
  (if (Variables|Tuto|GetTuto?)
    (StartSetting|FLaunchTutorial)
    (else
      (Commande|FLaunchCycle))))

(fn ConstructionScript)

(fn IsNeertoEnd?
  (return (<= (Variables|/Game/04-TafaiFighter/Blueprints/GM_TafaiFighter.GM_TafaiFighter_C|GetTimeRemaining (Variables|Reference|GetGamemodeRef)) (Variables|Property|GetTimerBeforeStopSpawn))))

(fn FLaunchEnnemi
  (params (WeakPoint :type Enum_AttackType%20Enum :default "NewEnumerator0") (IsLeft? :type Boolean))
  ;[1 1 1] Cycle des ennemi
  (if (not (Check|IsNeertoEnd?)) ; Did the game is near to end?
    (if (> (Utilities|Array|Length (Variables|Ennemi|GetEnnemiArray)) 0) ; Is there a Something in the array
      (bind _output_get (Variables|Ennemi|SetEnnemiSelect (Utilities|Array|Get(acopy) (Variables|Ennemi|GetEnnemiArray)))) ; Take the ref of the ennemi Select
      (Variables|/Game/04-TafaiFighter/Blueprints/BP_Enemy.BP_Enemy_C|SetWeakPoint _output_get WeakPoint) ; Set he is weak point
      ;;[1 1 1] RandomSide
      (bind _output_get_2 (Variables|Ennemi|SetChosenSide (.x (Transformation|GetWorldLocation (select IsLeft? (Variables|Default|GetLeft) (Variables|Default|GetRight))))))
      (Transformation|SetActorLocation (Variables|Ennemi|GetEnnemiSelect) (Math|Vector|MakeVector _output_get_2 0.0 0.0) false false)
      (Default|FInitialize (Variables|Ennemi|GetEnnemiSelect))
      (Utilities|Array|Add (Variables|Ennemi|GetEnnemiInGameArray) (Variables|Ennemi|GetEnnemiSelect))
      (Utilities|Array|RemoveItem (Variables|Ennemi|GetEnnemiArray) (Variables|Ennemi|GetEnnemiSelect))
      (return))))

(fn FLaunchSpear
  (params (Random :type Boolean) (IsLeft? :type Boolean))
  (if (not (Check|IsNeertoEnd?))
    (if Random ; If it's true the spear gonna go
      (if (> (Utilities|Array|Length (Variables|Spear|GetSpearArray)) 0) ; Is there a reference of a spear in this array??
        (Variables|Spear|SetSpearSelect (Utilities|Array|Get(acopy) (Variables|Spear|GetSpearArray))) ; Take the reference of the first spear
        ;[1 1 1] Randomize the side where the spear come
        (Variables|Spear|SetSpearChosenSide (.x (Transformation|GetWorldLocation (select IsLeft? (Variables|Default|GetLeft) (Variables|Default|GetRight)))))
        (Default|FPlayWarning (Variables|Reference|GetWarningWidgetRef) IsLeft?)
        (Transformation|SetActorLocation (Variables|Spear|GetSpearSelect) (Math|Vector|MakeVector (Variables|Spear|GetSpearChosenSide) 0.0 1.5e+02) false false)
        (Default|InitilizeSpear (Variables|Spear|GetSpearSelect)) ; Start the movement of the spear
        (Utilities|Array|RemoveItem (Variables|Spear|GetSpearArray) (Variables|Spear|GetSpearSelect))
        (return)))))

(fn FReference
  (bind _asgm_tafai_fighter (Utilities|Casting|CastToGM_TafaiFighter (Game|GetGameMode)))
  (Variables|Reference|SetGamemodeRef _asgm_tafai_fighter)
  (bind _asgi_meta_game (Utilities|Casting|CastToGI_MetaGame (Game|GetGameInstance)))
  (Variables|Tuto|SetTuto? (Variables|/Game/MetaGame/Blueprints/GI_MetaGame.GI_MetaGame_C|GetbIsFirstTimeTafaiFighter _asgi_meta_game))
  ;[1 1 1] Creer le widget pour les prevention de la lance
  (bind _returnvalue (UserInterface|CreateWidget "/Game/04-TafaiFighter/Widget/WBP_Warning.WBP_Warning_C"))
  (Variables|Reference|SetWarningWidgetRef _returnvalue)
  (UserInterface|Viewport|AddtoViewport _returnvalue 0)
  (return))

(fn FSpawnEnnemi
  (for _index (range 0 (- (Variables|SpawnEnnemiParameter|GetEnnemiNumber) 1))
    (bind _returnvalue (Game|SpawnActorfromClass "/Game/04-TafaiFighter/Blueprints/BP_Enemy.BP_Enemy_C" (Math|Transform|MakeTransform "0,1000.000000, 0" "0, 0, 0" "1,1,1") "Undefined" self (Variables|Tuto|GetTuto?) 0))
    (Utilities|Array|Add (Variables|Ennemi|GetEnnemiArray) _returnvalue))
  (for _array_element (Variables|Ennemi|GetEnnemiArray)
    (Variables|/Game/04-TafaiFighter/Blueprints/BP_Enemy.BP_Enemy_C|SetActorEnnemi _array_element (Variables|Ennemi|GetEnnemiArray)) ; Give the reference of all ennemi for each ennemi for ignore when there use a line trace
  )
  (return))

(fn FSpawnSpear
  (for _index (range 0 (- (Variables|SpawnSpearParameter|GetNumberOfSpear) 1))
    (bind _returnvalue (Game|SpawnActorfromClass "/Game/04-TafaiFighter/Blueprints/BP_Spear.BP_Spear_C" (Math|Transform|MakeTransform "0,1000.000000,0.000000" "0, 0, 0" "1,1,1") "Undefined" 0 26.0 1.5 (Variables|Tuto|GetTuto?) self 0))
    (Utilities|Array|Add (Variables|Spear|GetSpearArray) _returnvalue)
    (return))
  (return))

(fn FLaunchCycle
  (Cycle|FStartTimerSpear)
  (Cycle|FStartTimerEnnemi)
  (Cycle|FStartTimer)
  (return))

(fn FLaunchTutorial
  ;[1 1 1] Start the tutorial
  (bind _returnvalue (UserInterface|CreateWidget "/Game/04-TafaiFighter/Widget/WBP_Tuto.WBP_Tuto_C"))
  (bind _output_get (Variables|Reference|SetWBP_Tuto _returnvalue))
  (UserInterface|Viewport|AddtoViewport _output_get 3)
  (StartSetting|FTuto)
  (return))

(fn FTuto
  (switch int (Variables|Tuto|GetTutoState) ; Ne pas oublier que le widget fonction avec cette ordre
    (:1
      (Utilities|FlowControl|DoOnce false
        (:Completed
          (Commande|FLaunchEnnemi "NewEnumerator1" true))))
    (:2
      (Utilities|FlowControl|DoOnce false
        (:Completed
          (Commande|FLaunchSpear true false))))))

(fn FStartTimer
  (Utilities|Time|SetTimerbyFunctionName self "F_Timer" 1.0 true)
  (return))

(fn FTimer
  (if (<= (Variables|/Game/04-TafaiFighter/Blueprints/GM_TafaiFighter.GM_TafaiFighter_C|GetTimeRemaining (Variables|Reference|GetGamemodeRef)) 0)
    (for _array_element (Variables|Ennemi|GetEnnemiArray)
      (Default|FEnnemiStopAll _array_element))
    (return)))

(fn FStartTimerEnnemi
  (bind _returnvalue (Utilities|Time|SetTimerbyFunctionName self "F_TimerEnnemi" (Variables|SpawnEnnemiParameter|GetEnnemiSpawnRate) true))
  (Variables|Ennemi|SetSpawnEnnemiHandle _returnvalue)
  (return))

(fn FTimerEnnemi
  (Commande|FLaunchEnnemi (Utilities|Enum|ByteToEnumEnum_AttackType (Math|Conversions|ToByte(Integer) (Math|Random|RandomIntegerinRange 0 2))) (Math|Random|RandomBool))
  (return))

(fn FStartTimerSpear
  (bind _returnvalue (Utilities|Time|SetTimerbyFunctionName self "F_TimerSpear" (Variables|SpawnSpearParameter|GetSpearSpawnRate) true (Math|Random|RandomFloatinRange 5.0 1e+01)))
  (Variables|Spear|SetSpawnSpearHandle _returnvalue)
  (return))

(fn FTimerSpear
  (Commande|FLaunchSpear (Math|Random|RandomBoolwithWeight 0.4) (Math|Random|RandomBool))
  (return))

(fn FRetakeEnnemi
  (params (Target :type BP%20Enemy%20Object%20Reference%20%28by%20ref%29))
  (Utilities|Array|Add (Variables|Ennemi|GetEnnemiArray) Target)
  (Utilities|Array|RemoveItem (Variables|Ennemi|GetEnnemiInGameArray) Target)
  (Transformation|AddActorWorldOffset Target "0,1500.000000,0.000000" false true)
  (return))

(fn FStopAllEnnemi
  (for _array_element (Variables|Ennemi|GetEnnemiInGameArray)
    (Default|FEnnemiStopAll _array_element))
  (Utilities|Time|ClearandInvalidateTimerbyHandle (Variables|Spear|GetSpawnSpearHandle))
  (Utilities|Time|ClearandInvalidateTimerbyHandle (Variables|Ennemi|GetSpawnEnnemiHandle))
  (return))

(fn FRetakeSpear
  (params (Target :type BP%20Spear%20Object%20Reference%20%28by%20ref%29))
  (Utilities|Array|Add (Variables|Spear|GetSpearArray) Target)
  (Transformation|AddActorWorldOffset Target "0,1500.000000,150.000000" false true)
  (if (Variables|Tuto|GetTuto?)
    (Utilities|Time|SetTimerbyFunctionName self "F_DisplayTuto" 2.0)
    (return)
    (else
      (return))))

(fn FDisplayTuto
  (bind _wbp_tuto (Variables|Reference|GetWBP_Tuto))
  (bind _gamemoderef (Variables|Reference|GetGamemodeRef))
  ;[1 1 1] Display Tuto
  (Class|WidgetSwitcher|SetActiveWidgetIndex (Variables|/Game/04-TafaiFighter/Widget/WBP_Tuto.WBP_Tuto_C|GetTutoSwitcher _wbp_tuto) 3)
  (Default|PlayTutoSensCritique _wbp_tuto)
  ;[1 1 1] Say to all ennemi than the tuto is display and pause the game
  (Variables|Tuto|SetTuto? false)
  (Default|LaunchAfterTuto _gamemoderef)
  (Variables|/Game/04-TafaiFighter/Blueprints/GM_TafaiFighter.GM_TafaiFighter_C|SetbFirstTime? _gamemoderef false)
  (Commande|FLaunchCycle)
  (for _array_element (Variables|Ennemi|GetEnnemiArray)
    (Variables|/Game/04-TafaiFighter/Blueprints/BP_Enemy.BP_Enemy_C|SetTuto? _array_element false))
  (for _array_element_2 (Variables|Spear|GetSpearArray)
    (Variables|/Game/04-TafaiFighter/Blueprints/BP_Spear.BP_Spear_C|SetbTuto? _array_element_2 false))
  (Game|SetGamePaused true)
  (return))