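; Pooled melee enemy for TafaiFighter that advances on the player, punches on a repeating timer and takes extra damage on its particle-marked weak point.
; Looping timers drive movement and attacks, with forward line traces detecting the player.
; Hits and shield pulses interrupt those timers and push it back through timelines before it resumes walking.
; Death returns it to BP_SpawnerEnnemi for reuse, and a Tuto flag drives tutorial prompts and pausing.
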(event Custom|DealEnnemiDamage
  (params (AttackType :type Enum_AttackType%20Enum :default "NewEnumerator0"))
  (bind _spawnerennemiref (Variables|Reference|GetSpawnerEnnemiRef))
  (bind _spawnerennemiref_2 (Variables|Reference|GetSpawnerEnnemiRef))
  (bind _wbp_tuto (Variables|/Game/04-TafaiFighter/Blueprints/BP_SpawnerEnnemi.BP_SpawnerEnnemi_C|GetWBP_Tuto _spawnerennemiref))
  ;[1 1 1] When receive any damage check if it's a crit or not and apply the adapt damage.
  (if (Utilities|Enum|Equal(Enum) AttackType (Variables|Property|GetWeakPoint)) ; Critique ?
    (VFX|FPlayHitFx true)
    (Variables|Property|SetLife (- (Variables|Property|GetLife) 2.0))
    (else
      (VFX|FPlayHitFx false)
      (Variables|Property|SetLife (- (Variables|Property|GetLife) 1.0))
      (Audio|PlaySound2D "/Game/04-TafaiFighter/SFX/fighter/S_take_damage.S_take_damage" 1.0 1.0 0.0 0 0)))
  (Rendering|Material|SetScalarParameterValue (Variables|Reference|GetCurrentMaterial) "HitIntensity" 1.0 :!class /Script/Engine.MaterialInstanceDynamic)
  (if (Variables|Tuto|GetTuto?)
    ;[1 1 1] Special code for the tutorial
    (Class|WidgetSwitcher|SetActiveWidgetIndex (Variables|/Game/04-TafaiFighter/Widget/WBP_Tuto.WBP_Tuto_C|GetTutoSwitcher _wbp_tuto))
    (Default|StopHitTutoAnim _wbp_tuto)
    (if (<= (Variables|Property|GetLife) 0.0)
      (Property|FDeath)
      (Utilities|FlowControl|Delay 0.15)
      (Audio|PlaySound2D "/Game/04-TafaiFighter/SFX/fighter/SC_damage_enemi.SC_damage_enemi" 1.0 1.0 0.0 0 0)
      (Utilities|FlowControl|Delay 0.15)
      (Variables|/Game/04-TafaiFighter/Blueprints/BP_SpawnerEnnemi.BP_SpawnerEnnemi_C|SetTutoState _spawnerennemiref_2 2)
      (Default|FTuto _spawnerennemiref_2)
      (Variables|Tuto|SetTuto? false)
      (Rendering|Material|SetScalarParameterValue (Variables|Reference|GetCurrentMaterial) "HitIntensity" 0.0 :!class /Script/Engine.MaterialInstanceDynamic)
      (else
        (CallFunction|KnockBack)
        (Rendering|Material|SetScalarParameterValue (Variables|Reference|GetCurrentMaterial) "HitIntensity" 0.0 :!class /Script/Engine.MaterialInstanceDynamic)))
    (elif (<= (Variables|Property|GetLife) 0.0)
      ;;[1 1 1] Too many delay I'm not gonna convert this in a function
      (Property|FDeath)
      (Utilities|FlowControl|Delay 0.15)
      (Audio|PlaySound2D "/Game/04-TafaiFighter/SFX/fighter/SC_damage_enemi.SC_damage_enemi" 1.0 1.0 0.0 0 0)
      (Utilities|FlowControl|Delay 0.15)
      (Audio|PlaySound2D "/Game/04-TafaiFighter/SFX/fighter/S_enemy_down.S_enemy_down" 0.65 1.0 0.0 0 0)
      (Rendering|Material|SetScalarParameterValue (Variables|Reference|GetCurrentMaterial) "HitIntensity" 0.0 :!class /Script/Engine.MaterialInstanceDynamic)
      (else
        (CallFunction|KnockBack)
        (Utilities|FlowControl|Delay 0.2)
        (Rendering|Material|SetScalarParameterValue (Variables|Reference|GetCurrentMaterial) "HitIntensity" 0.0 :!class /Script/Engine.MaterialInstanceDynamic)))))

(event Custom|Attack
  ;[1 1 1] Every time it call get if the player is still a live and punch him
  (bind _outhit (Collision|LineTraceByChannel (+ (Transformation|GetActorLocation) "0,0.000000,150.000000") (Transformation|GetWorldLocation (Variables|Default|GetFrontAim)) "TraceTypeQuery1" false (Variables|Reference|GetActorEnnemi) "None" true "(R=1.000000,G=0.000000,B=0.000000,A=1.000000)" "(R=0.000000,G=1.000000,B=0.000000,A=1.000000)" 0.2))
  (bind _asbp_tafai_tafai_fighter (Utilities|Casting|CastToBP_Tafai_TafaiFighter (.HitActor (Collision|BreakHitResult _outhit))))
  (if (Variables|/Game/04-TafaiFighter/Blueprints/BP_Tafai_TafaiFighter.BP_Tafai_TafaiFighter_C|GetbPlayerDead? _asbp_tafai_tafai_fighter)
    (Default|FStopAllEnnemi (Variables|Reference|GetSpawnerEnnemiRef) :!label _label)
    (Variables|AnimationBlueprint|SetbIsHitting? false)
    (else
      (Default|RecieveDamage _asbp_tafai_tafai_fighter 1)
      (Variables|AnimationBlueprint|SetbIsHitting? true)
      (Utilities|FlowControl|Delay 0.2)
      (Variables|AnimationBlueprint|SetbIsHitting? false)
      (if (Variables|/Game/04-TafaiFighter/Blueprints/BP_Tafai_TafaiFighter.BP_Tafai_TafaiFighter_C|GetbPlayerDead? _asbp_tafai_tafai_fighter)
        (goto _label)))))

(event Custom|PulsByShield
  ;[1 1 1] When the shield up repulsed the ennemi
  (Variables|AnimationBlueprint|SetbIsGettingRepulsed? true)
  (if (Variables|Timer|GetbIsAttacking?)
    (Utilities|Time|ClearandInvalidateTimerbyHandle (Variables|Timer|GetAttackHandle))
    (Timeline|ShinraTensei PlayFromStart ; Can't convert different Timeline
      (:Update
        (Transformation|AddActorLocalOffset "-3.000000, 0, 0" false false))
      (:Finished
        (Variables|Timer|SetbIsAttacking? false)
        (Variables|AnimationBlueprint|SetbIsGettingRepulsed? false)
        (Movement|FStartMove)))
    (else
      (Utilities|Time|ClearandInvalidateTimerbyHandle (Variables|Timer|GetMoveHandle))
      (Timeline|ShinraTensei PlayFromStart))))

(event Custom|KnockBack
  ;[1 1 1] Event when the ennemi is repulsed
  (Variables|AnimationBlueprint|SetbIsGettingRepulsed? true)
  (if (Variables|Timer|GetbIsAttacking?)
    (Utilities|Time|ClearandInvalidateTimerbyHandle (Variables|Timer|GetAttackHandle))
    (Timeline|Timeline_0 PlayFromStart ; Can't convert different Timeline
      (:Update
        (Transformation|AddActorLocalOffset "-10.000000, 0, 0" false false))
      (:Finished
        (Variables|Timer|SetbIsAttacking? false)
        (Variables|AnimationBlueprint|SetbIsGettingRepulsed? false)
        (Movement|FStartMove)))
    (else
      (Utilities|Time|ClearandInvalidateTimerbyHandle (Variables|Timer|GetMoveHandle))
      (Timeline|Timeline_0 PlayFromStart))))

(event EventBeginPlay
  ;[1 1 1] Get the reference of her spawner at the beginning
  (bind _asbp_spawner_ennemi (Utilities|Casting|CastToBP_SpawnerEnnemi (Components|GetOwner)))
  (Variables|Reference|SetSpawnerEnnemiRef _asbp_spawner_ennemi))

(fn ConstructionScript)

(fn FDestoyFX
  (Components|DestroyComponent (Variables|Default|GetImpactParticle))
  (Variables|Default|SetImpactParticle 0)
  (return))

(fn FPlayHitFx
  (params (IsCrit? :type Boolean))
  (bind _skeletalmesh (Variables|Default|GetSkeletalMesh))
  (bind _returnvalue (Effects|SpawnEmitteratLocation (select IsCrit? (LocalVariables|GetParticleCrit) (LocalVariables|GetParticleNormal)) (Transformation|GetSocketLocation _skeletalmesh "HitTorseSocket") (Transformation|GetSocketRotation _skeletalmesh "HitTorseSocket")))
  (Variables|Default|SetImpactParticle _returnvalue)
  (Utilities|Time|SetTimerbyFunctionName self "F_DestroyFX" 0.4)
  (return))

(fn FInitialize
  (bind _weakpoint (Variables|Property|GetWeakPoint))
  ;[1 1 1] Creat the dynamic texture
  (bind _returnvalue (Rendering|Material|CreateDynamicMaterialInstance (Utilities|Array|Get(acopy) (Variables|Reference|GetEnnemiMaterials) (Math|Random|RandomIntegerinRange 0 1)) "None" :!class /Script/Engine.KismetMaterialLibrary))
  (bind _output_get (Variables|Reference|SetCurrentMaterial _returnvalue))
  (Rendering|Material|SetMaterial (Variables|Default|GetSkeletalMesh) 0 _output_get)
  ;[1 1 1] Add FX depend on the weak spot
  (if (or (Utilities|Enum|Equal(Enum) _weakpoint "NewEnumerator0") (Utilities|Enum|Equal(Enum) _weakpoint "NewEnumerator1"))
    (bind _returnvalue_2 (Effects|SpawnEmitterAttached "/Game/04-TafaiFighter/ParticleSystems/PS_WeakSpot.PS_WeakSpot" (Variables|Default|GetSkeletalMesh) (Utilities|Select :Index _weakpoint :NewEnumerator0 "TeteSocket" :NewEnumerator1 "TorseSocket" :NewEnumerator2 "None") "0, 0, 0" "0, 0, 0" "0.200000,0.200000,0.500000"))
    (Variables|Default|SetParticule1 _returnvalue_2)
    (else
      (bind _returnvalue_3 (Effects|SpawnEmitterAttached "/Game/04-TafaiFighter/ParticleSystems/PS_WeakSpot.PS_WeakSpot" (Variables|Default|GetSkeletalMesh) "ChevilleGaucheSocket" "0, 0, 0" "0, 0, 0" "0.200000,0.200000,0.500000"))
      (Variables|Default|SetParticule1 _returnvalue_3)
      (bind _returnvalue_4 (Effects|SpawnEmitterAttached "/Game/04-TafaiFighter/ParticleSystems/PS_WeakSpot.PS_WeakSpot" (Variables|Default|GetSkeletalMesh) "ChevilleDroiteSocket" "0, 0, 0" "0, 0, 0" "0.200000,0.200000,0.500000"))
      (Variables|Default|SetParticule2 _returnvalue_4)))
  ;[1 1 1] Look at the direction of the player and start to move
  (Transformation|SetActorRotation (Math|Rotator|FindLookatRotation (Transformation|GetActorLocation) (Math|Vector|MakeVector 0.0 0.0 0.0)))
  (Movement|FStartMove)
  (return))

(fn FEnnemiStopAll
  ;[1 1 1] Stop le mouvement et les attaques
  (Utilities|Time|ClearandInvalidateTimerbyHandle (Variables|Timer|GetMoveHandle))
  (Utilities|Time|ClearandInvalidateTimerbyHandle (Variables|Timer|GetAttackHandle))
  ;[1 1 1] Permet de mettre l'anim BP en idle
  (Variables|AnimationBlueprint|SetbIsMoving? false)
  (Variables|Timer|SetbIsAttacking? true)
  (return))

(fn FRemoveWeakSpot
  (Utilities|IsValid (Variables|Default|GetParticule1)
    (:Is%20Valid
      (Components|DestroyComponent (Variables|Default|GetParticule1))
      (Variables|Default|SetParticule1 0))
    (:Is%20Not%20Valid
      _))
  (Utilities|IsValid (Variables|Default|GetParticule2)
    (:Is%20Valid
      (Components|DestroyComponent (Variables|Default|GetParticule2))
      (Variables|Default|SetParticule2 0)
      (return))
    (:Is%20Not%20Valid
      (return))))

(fn FStartMove
  (bind _returnvalue (Utilities|Time|SetTimerbyFunctionName self "F_Move" 0.01 true))
  (Variables|Timer|SetMoveHandle _returnvalue)
  (Variables|AnimationBlueprint|SetActivate true)
  (Variables|AnimationBlueprint|SetbIsMoving? true)
  (return))

(fn FMove
  (bind _spawnerennemiref (Variables|Reference|GetSpawnerEnnemiRef))
  (bind _wbp_tuto (Variables|/Game/04-TafaiFighter/Blueprints/BP_SpawnerEnnemi.BP_SpawnerEnnemi_C|GetWBP_Tuto _spawnerennemiref))
  ;[1 1 1] Bouge et verifi si le joueur est a porter
  (Transformation|AddActorLocalOffset "3.000000, 0, 0" false false)
  (bind _outhit (Collision|LineTraceByChannel (+ (Transformation|GetActorLocation) "0, 0,150.000000") (Transformation|GetWorldLocation (Variables|Default|GetFrontAim)) "TraceTypeQuery1" false (Variables|Reference|GetActorEnnemi) "None" true "(R=1.000000,G=0.000000,B=0.000000,A=1.000000)" "(R=0.000000,G=1.000000,B=0.000000,A=1.000000)" 0.02))
  (Utilities|Casting|CastToBP_Tafai_TafaiFighter (.HitActor (Collision|BreakHitResult _outhit)))
  (if (Components|ComponentHasTag (.HitComponent (Collision|BreakHitResult _outhit)) "Shield")
    (return)
    (else
      (if (Variables|Tuto|GetTuto?)
        ;[1 1 1] Lance le tuto des coup de point, si l'ennemi revien avec la motier de ses pv
        ; alors le joueur a deja donner un coup comme demander par le tuto alors on indique de donner un coup critique
        (Class|WidgetSwitcher|SetActiveWidgetIndex (Variables|/Game/04-TafaiFighter/Widget/WBP_Tuto.WBP_Tuto_C|GetTutoSwitcher _wbp_tuto) 1)
        (if (> (Variables|Property|GetLife) 1.0)
          (Default|PlayHitTutoAnim _wbp_tuto)
          (else
            (Default|PlayTutoCritique _wbp_tuto)))
        (Game|SetGamePaused true))
      ;[1 1 1] Passe en mode attack et attack toute les 1 sec
      (Variables|AnimationBlueprint|SetbIsMoving? false)
      (Variables|Timer|SetbIsAttacking? true)
      (Utilities|Time|ClearandInvalidateTimerbyHandle (Variables|Timer|GetMoveHandle))
      (bind _returnvalue (Utilities|Time|SetTimerbyFunctionName self "Attack" 1.0 true))
      (Variables|Timer|SetAttackHandle _returnvalue)
      (return))))

(fn FDeath
  (Utilities|Time|ClearandInvalidateTimerbyHandle (Variables|Timer|GetMoveHandle))
  (Utilities|Time|ClearandInvalidateTimerbyHandle (Variables|Timer|GetAttackHandle))
  (Variables|Property|SetLife 2.0)
  (Variables|AnimationBlueprint|SetActivate false)
  (Variables|Timer|SetbIsAttacking? false)
  (Utilities|Time|SetTimerbyFunctionName self "F_RecallEverything" 0.9)
  (return))

(fn FRecallEverything
  (Default|FRetakeEnnemi (Variables|Reference|GetSpawnerEnnemiRef) self)
  (VFX|FRemoveWeakSpot)
  (if (Variables|Tuto|GetTuto?)
    (Variables|Tuto|SetTuto? false)
    (return)
    (else
      (return))))