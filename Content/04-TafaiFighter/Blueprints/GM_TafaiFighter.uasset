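; Game mode for the TafaiFighter minigame, a timed survival round that is won when the countdown runs out.
; Play starts after a short fade delay, or on first launch once LaunchAfterTuto clears the GI_MetaGame first-time flag.
; Startup crossfades night audio into day, starts music, caches the player and daylight actors, and runs a one-second looping timer.
; At zero, it shows the victory widget scored by remaining life and stops timers and music.
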(event Custom|LaunchAfterTuto
  ;[1 1 1] Say if the tuto is done
  (Variables|/Game/MetaGame/Blueprints/GI_MetaGame.GI_MetaGame_C|SetbIsFirstTimeTafaiFighter (Variables|Reference|GetGameInstanceRef) false)
  (Utilities|FlowControl|Sequence
    (:then_0
      ;[1 1 1] Crossfade
      (Audio|Components|Audio|Play (Variables|Default|Getnight_time) 0.0)
      (Utilities|FlowControl|Delay 54.0)
      (Utilities|FlowControl|Sequence
        (:then_0
          (Audio|Components|Audio|FadeOut (Variables|Default|Getnight_time) 12.0 0.0 "Linear" :!class /Script/Engine.AudioComponent))
        (:then_1
          (Audio|Components|Audio|FadeIn (Variables|Default|Getday_time) 12.0 1.0 0.0 "Linear" :!class /Script/Engine.AudioComponent))))
    (:then_1
      (Start|FInitilialize))))

(event EventBeginPlay
  ;[1 1 1] Get if the player has play the the game before
  (bind _asgi_meta_game (Utilities|Casting|CastToGI_MetaGame (Game|GetGameInstance)))
  (Variables|Reference|SetGameInstanceRef _asgi_meta_game)
  (Variables|Property|SetbFirstTime? (Variables|/Game/MetaGame/Blueprints/GI_MetaGame.GI_MetaGame_C|GetbIsFirstTimeTafaiFighter _asgi_meta_game))
  (if (not (Variables|Property|GetbFirstTime?))
    (Utilities|FlowControl|Delay 1.0) ; Delay of 1 s for fade at the loading map
    (Utilities|FlowControl|Sequence
      (:then_0
        ;[1 1 1] Crossfade
        (Audio|Components|Audio|Play (Variables|Default|Getnight_time) 0.0)
        (Utilities|FlowControl|Delay 54.0)
        (Utilities|FlowControl|Sequence
          (:then_0
            (Audio|Components|Audio|FadeOut (Variables|Default|Getnight_time) 12.0 0.0 "Linear" :!class /Script/Engine.AudioComponent))
          (:then_1
            (Audio|Components|Audio|FadeIn (Variables|Default|Getday_time) 12.0 1.0 0.0 "Linear" :!class /Script/Engine.AudioComponent))))
      (:then_1
        (Start|FInitilialize)))))

(fn ConstructionScript)

(fn FEndGame
  (params (Score :type Integer))
  ;[1 1 1] Cree le wifget de fin
  (bind _returnvalue (UserInterface|CreateWidget "/Game/MetaGame/Widgets/WBP_MenuVictoire.WBP_MenuVictoire_C" (Game|GetPlayerController 0) Score 1 2 3 1.0))
  (UserInterface|Viewport|AddtoViewport _returnvalue 0)
  (Utilities|Time|ClearandInvalidateTimerbyHandle (Variables|/Game/04-TafaiFighter/Blueprints/BP_DayLight.BP_DayLight_C|GetSunRiserHandle (Variables|Reference|GetDayLightRef)))
  (Utilities|Time|ClearandInvalidateTimerbyHandle (Variables|Timer|GetTimerHandle))
  (Audio|Components|Audio|FadeOut (Variables|Default|Getmusic) 2.0 0.0 "Linear" :!class /Script/Engine.AudioComponent))

(fn FTimer
  (bind _result (Math|Integer|DecrementInt (Variables|Timer|GetTimeRemaining))
    (:%20%20
      (if (<= _result 0)
        (Utilities|Time|ClearandInvalidateTimerbyHandle (Variables|Timer|GetTimerHandle)) ; Stop the timer
        (Game|FEndGame (Variables|/Game/04-TafaiFighter/Blueprints/BP_Tafai_TafaiFighter.BP_Tafai_TafaiFighter_C|GetLife (Variables|Reference|GetBP_TafaiRef))) ; Launch the end of the game
        (Variables|/Game/04-TafaiFighter/Blueprints/BP_Tafai_TafaiFighter.BP_Tafai_TafaiFighter_C|SetbIsWinning? (Variables|Reference|GetBP_TafaiRef) true)
        (return)
        (else
          (return))))))

(fn FInitilialize
  ;[1 1 1] Start the music
  (Audio|Components|Audio|Play (Variables|Default|Getmusic) 0.0)
  ;[1 1 1] Initialize the timer
  (bind _returnvalue (Utilities|Time|SetTimerbyFunctionName self "F_Timer" 1.0 true))
  (Variables|Timer|SetTimerHandle _returnvalue)
  ;[1 1 1] Get the ref of the light and the player
  (bind _outactors (Actor|GetAllActorsOfClass "/Game/04-TafaiFighter/Blueprints/BP_DayLight.BP_DayLight_C"))
  (Variables|Reference|SetDayLightRef (Utilities|Array|Get(acopy) _outactors))
  (bind _outactors_2 (Actor|GetAllActorsOfClass "/Game/04-TafaiFighter/Blueprints/BP_Tafai_TafaiFighter.BP_Tafai_TafaiFighter_C"))
  (Variables|Reference|SetBP_TafaiRef (Utilities|Array|Get(acopy) _outactors_2))
  (return))