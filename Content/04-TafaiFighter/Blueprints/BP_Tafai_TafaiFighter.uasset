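; Player fighter for the TafaiFighter twin-stick minigame, striking enemies on either side.
; Each stick's direction picks an attack type and fires a side line trace that damages the enemy hit, or stuns the player on a miss.
; Pushing both sticks inward spends a timer-recharged shield charge, scaling a sphere that repulses enemies and blocks damage.
; BeginPlay creates HUD, pause and debug-shield widgets; death calls the GameMode's end game.
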(event OnComponentBeginOverlap(Sphere)
  (params (OverlappedComponent :type Primitive%20Component%20Object%20Reference) (OtherActor :type Actor%20Object%20Reference) (OtherComp :type Primitive%20Component%20Object%20Reference) (OtherBodyIndex :type Integer) (bFromSweep :type Boolean) (SweepResult :type Hit%20Result%20Structure%20%28by%20ref%29))
  ;[1 1 1] Repulse l'ennemi
  (bind _asbp_enemy (Utilities|Casting|CastToBP_Enemy OtherActor))
  (Default|PulsbyShield _asbp_enemy))

(event Custom|RecieveDamage
  (params (Damage :type Integer))
  ;[1 1 1] Recois des degats
  (if (not (Variables|PlayerState|GetbPlayerDead?))
    (if (not (Variables|Mechanic|GetbIsShieldUp?))
      (bind _output_get (Variables|PlayerState|SetLife (- (Variables|PlayerState|GetLife) Damage)))
      (Default|UpdateLifeWBP (Variables|Reference|GetWBP_HUD_Ref) _output_get)
      (if (== _output_get 0)
        (CallFunction|Death)
        (Audio|PlaySound2D "/Game/04-TafaiFighter/SFX/fighter/SC_damage_tafai.SC_damage_tafai" 1.0 1.0 0.0 0 0 :!label _label)
        (elif (> _output_get 0)
          (Variables|PlayerState|SetbPlayerTakeDamage? true)
          (Utilities|FlowControl|Delay 0.1)
          (Variables|PlayerState|SetbPlayerTakeDamage? false)
          (goto _label))))))

(event Custom|Death
  ;[1 1 1] Lors de la mort du joueur, active le EndGame du GM une fois
  (Utilities|FlowControl|DoOnce false
    (:Completed
      (Variables|PlayerState|SetbPlayerDead? true)
      (Variables|PlayerState|SetbIsWinning? false)
      (Utilities|FlowControl|Delay 0.2)
      (Default|FEndGame (Variables|Reference|GetGameModeRef) (Variables|PlayerState|GetLife)))))

(event Custom|ShieldReccuperation
  ;[1 1 1] Timer de reccuperation du Shield qui se desactive a son maximum
  (bind _returnvalue (Utilities|Time|SetTimerbyEvent (delegate Custom|AddShield) 5.0 true))
  (Variables|Timer|SetShieldRecover _returnvalue))

(event Custom|Shield
  ;[1 1 1] Systeme de shield
  (if (Variables|PlayerState|GetbTuto?)
    (Game|SetGamePaused false))
  (Variables|Mechanic|SetbIsShieldUp? true)
  (bind _scalevalue (Timeline|ScaleShield PlayFromStart)
    (:Update
      (Transformation|SetWorldScale3D (Variables|Default|GetSphere) (Math|Vector|MakeVector _scalevalue _scalevalue _scalevalue)))
    (:Finished
      (Transformation|SetWorldScale3D (Variables|Default|GetSphere) (Math|Vector|MakeVector 1.0 1.0 1.0))
      (Variables|Mechanic|SetbLeftInAction false)
      (Variables|Mechanic|SetbRightInAction false)
      (Variables|PlayerState|SetbPlayerDoSomeThing? false)
      (Variables|Mechanic|SetbCheatShield false)
      (Variables|Mechanic|SetbIsShieldUp? false))))

(event Custom|AddShield
  ;[1 1 1] Timer de reccuperation du Shield qui se desactive a son maximum
  (if (== (Variables|PlayerState|GetShieldNumber) 3)
    (Utilities|Time|ClearandInvalidateTimerbyHandle (Variables|Timer|GetShieldRecover) :!label _label)
    (else
      (bind _result (Math|Integer|IncrementInt (Variables|PlayerState|GetShieldNumber))
        (:%20%20
          (Default|UpdateShield (Variables|Reference|GetWBP_HUD_Ref) _result)
          (if (== _result 3)
            (goto _label)))))))

(event Custom|ResetShield
  ;[1 1 1] Joystaick
  (Utilities|FlowControl|DoOnce true) ; enters at Reset
)

(event Custom|CheatShield
  ;[1 1 1] Cheat shield for testing purposes
  (if (> (Variables|PlayerState|GetShieldNumber) 0)
    (Variables|Mechanic|SetbCheatShield true)
    ;[1 1 1] Joystaick
    (Variables|PlayerState|SetbPlayerDoSomeThing? true)
    (Utilities|FlowControl|DoOnce true
      (:Completed
        (CallFunction|Shield)
        (bind _result (Math|Integer|DecrementInt (Variables|PlayerState|GetShieldNumber))
          (:%20%20
            (Default|UpdateShield (Variables|Reference|GetWBP_HUD_Ref) _result)
            ;[1 1 1] Si le timer est out, le relance puisque un shield a ete utiliser
            (if (not (Utilities|Time|IsValidTimerHandle (Variables|Timer|GetShieldRecover)))
              (CallFunction|ShieldReccuperation))))))))

(event EventBeginPlay
  ;[0.4114 0.1027 1 1 30] Begin Play
  (Start|FStartGame))

(event Input|AxisEvents|InputAxisLeftAxisX
  (params (AxisValue :type Float%20%28single-precision%29))
  ;[1 1 1] Joystaick
  (Variables|JoystickDirection|SetLeftJoystickAxis (Math|Vector2D|MakeVector2D AxisValue (stale Input|AxisEvents|InputAxisLeftAxisY AxisValue)))
  (Utilities|CheckLeftJoystickDiplacement
    (:then
      (bind _hitactor (Mechanic|FLinetraceLeft))
      (if (Variables|Mechanic|GetbLeftHit?)
        (Audio|PlaySound2D "/Game/04-TafaiFighter/SFX/fighter/SC_whoosh.SC_whoosh" 1.0 1.0 0.0 0 0)
        (Default|DealEnnemiDamage _hitactor (Variables|Mechanic|GetAttackType))
        (Utilities|FlowControl|Delay 0.2)
        (else
          (Utilities|FlowControl|Delay 0.3)
          (Utilities|Stun (Variables|Stun|GetStunTime)
            (:Return
              _))))
      (Variables|Mechanic|SetbLeftInAction false)
      (Variables|PlayerState|SetbPlayerDoSomeThing? false))
    (:Shield
      (if (and (Utilities|Enum|Equal(Enum) (Variables|JoystickDirection|GetStateRightJoytisk) "NewEnumerator1") (> (Variables|PlayerState|GetShieldNumber) 0))
        (Variables|PlayerState|SetbPlayerDoSomeThing? true)
        (Utilities|FlowControl|DoOnce true
          (:Completed
            (CallFunction|Shield)
            (bind _result (Math|Integer|DecrementInt (Variables|PlayerState|GetShieldNumber))
              (:%20%20
                (Default|UpdateShield (Variables|Reference|GetWBP_HUD_Ref) _result)
                ;[1 1 1] Si le timer est out, le relance puisque un shield a ete utiliser
                (if (not (Utilities|Time|IsValidTimerHandle (Variables|Timer|GetShieldRecover)))
                  (CallFunction|ShieldReccuperation))))))))))

(event Input|AxisEvents|InputAxisLeftAxisY
  (params (AxisValue :type Float%20%28single-precision%29))
  ;[1 1 1] Joystaick
  (Variables|JoystickDirection|SetLeftJoystickAxis (Math|Vector2D|MakeVector2D (stale Input|AxisEvents|InputAxisLeftAxisX AxisValue) AxisValue))
  (Utilities|CheckLeftJoystickDiplacement
    (:then
      (bind _hitactor (Mechanic|FLinetraceLeft))
      (if (Variables|Mechanic|GetbLeftHit?)
        (Audio|PlaySound2D "/Game/04-TafaiFighter/SFX/fighter/SC_whoosh.SC_whoosh" 1.0 1.0 0.0 0 0)
        (Default|DealEnnemiDamage _hitactor (Variables|Mechanic|GetAttackType))
        (Utilities|FlowControl|Delay 0.2)
        (else
          (Utilities|FlowControl|Delay 0.3)
          (Utilities|Stun (Variables|Stun|GetStunTime)
            (:Return
              _))))
      (Variables|Mechanic|SetbLeftInAction false)
      (Variables|PlayerState|SetbPlayerDoSomeThing? false))
    (:Shield
      (if (and (Utilities|Enum|Equal(Enum) (Variables|JoystickDirection|GetStateRightJoytisk) "NewEnumerator1") (> (Variables|PlayerState|GetShieldNumber) 0))
        (Variables|PlayerState|SetbPlayerDoSomeThing? true)
        (Utilities|FlowControl|DoOnce true
          (:Completed
            (CallFunction|Shield)
            (bind _result (Math|Integer|DecrementInt (Variables|PlayerState|GetShieldNumber))
              (:%20%20
                (Default|UpdateShield (Variables|Reference|GetWBP_HUD_Ref) _result)
                ;[1 1 1] Si le timer est out, le relance puisque un shield a ete utiliser
                (if (not (Utilities|Time|IsValidTimerHandle (Variables|Timer|GetShieldRecover)))
                  (CallFunction|ShieldReccuperation))))))))))

(event Input|AxisEvents|InputAxisRightAxisX
  (params (AxisValue :type Float%20%28single-precision%29))
  ;[1 1 1] Joystaick
  (Variables|JoystickDirection|SetRightJoystickAxis (Math|Vector2D|MakeVector2D AxisValue (stale Input|AxisEvents|InputAxisRightAxisY AxisValue)))
  (Utilities|CheckRightJoystickDiplacement
    (:Shield
      (if (and (> (Variables|PlayerState|GetShieldNumber) 0) (Utilities|Enum|Equal(Enum) (Variables|JoystickDirection|GetStateLeftJoytisk) "NewEnumerator1"))
        (Variables|PlayerState|SetbPlayerDoSomeThing? true)
        (Utilities|FlowControl|DoOnce true
          (:Completed
            (CallFunction|Shield)
            (bind _result (Math|Integer|DecrementInt (Variables|PlayerState|GetShieldNumber))
              (:%20%20
                (Default|UpdateShield (Variables|Reference|GetWBP_HUD_Ref) _result)
                ;[1 1 1] Si le timer est out, le relance puisque un shield a ete utiliser
                (if (not (Utilities|Time|IsValidTimerHandle (Variables|Timer|GetShieldRecover)))
                  (CallFunction|ShieldReccuperation))))))))
    (:then
      (if (Variables|PlayerState|GetbTuto?)
        (Game|SetGamePaused false))
      (bind _hitactor (Mechanic|FLinetraceRight))
      (if (Variables|Mechanic|GetbRightHit?)
        (Audio|PlaySound2D "/Game/04-TafaiFighter/SFX/fighter/SC_whoosh.SC_whoosh" 1.0 1.0 0.0 0 0)
        (Default|DealEnnemiDamage _hitactor (Variables|Mechanic|GetAttackType))
        (Utilities|FlowControl|Delay 0.2)
        (else
          (Utilities|FlowControl|Delay 0.3)
          (Utilities|Stun (Variables|Stun|GetStunTime)
            (:Return
              _))))
      (Variables|Mechanic|SetbRightInAction false)
      (Variables|PlayerState|SetbPlayerDoSomeThing? false))))

(event Input|AxisEvents|InputAxisRightAxisY
  (params (AxisValue :type Float%20%28single-precision%29))
  ;[1 1 1] Joystaick
  (Variables|JoystickDirection|SetRightJoystickAxis (Math|Vector2D|MakeVector2D (stale Input|AxisEvents|InputAxisRightAxisX AxisValue) AxisValue))
  (Utilities|CheckRightJoystickDiplacement
    (:Shield
      (if (and (> (Variables|PlayerState|GetShieldNumber) 0) (Utilities|Enum|Equal(Enum) (Variables|JoystickDirection|GetStateLeftJoytisk) "NewEnumerator1"))
        (Variables|PlayerState|SetbPlayerDoSomeThing? true)
        (Utilities|FlowControl|DoOnce true
          (:Completed
            (CallFunction|Shield)
            (bind _result (Math|Integer|DecrementInt (Variables|PlayerState|GetShieldNumber))
              (:%20%20
                (Default|UpdateShield (Variables|Reference|GetWBP_HUD_Ref) _result)
                ;[1 1 1] Si le timer est out, le relance puisque un shield a ete utiliser
                (if (not (Utilities|Time|IsValidTimerHandle (Variables|Timer|GetShieldRecover)))
                  (CallFunction|ShieldReccuperation))))))))
    (:then
      (if (Variables|PlayerState|GetbTuto?)
        (Game|SetGamePaused false))
      (bind _hitactor (Mechanic|FLinetraceRight))
      (if (Variables|Mechanic|GetbRightHit?)
        (Audio|PlaySound2D "/Game/04-TafaiFighter/SFX/fighter/SC_whoosh.SC_whoosh" 1.0 1.0 0.0 0 0)
        (Default|DealEnnemiDamage _hitactor (Variables|Mechanic|GetAttackType))
        (Utilities|FlowControl|Delay 0.2)
        (else
          (Utilities|FlowControl|Delay 0.3)
          (Utilities|Stun (Variables|Stun|GetStunTime)
            (:Return
              _))))
      (Variables|Mechanic|SetbRightInAction false)
      (Variables|PlayerState|SetbPlayerDoSomeThing? false))))

(fn ConstructionScript)

(fn FLinetraceLeft
  (bind _returnvalue (Transformation|GetActorLocation))
  (bind (_outhit _returnvalue_2) (Collision|LineTraceByChannel (+ _returnvalue "0, 0,150.000000") (+ _returnvalue (Math|Vector|MakeVector (* (Variables|Mechanic|GetAttaqueRange) -1.0) 0.0 1.5e+02)) "TraceTypeQuery2" false 0 "None" true "(R=1.000000,G=0.000000,B=0.000000,A=1.000000)" "(R=0.000000,G=1.000000,B=0.000000,A=1.000000)" 1.0))
  (Variables|Mechanic|SetbLeftHit? _returnvalue_2)
  (bind _asbp_enemy (Utilities|Casting|CastToBP_Enemy (.HitActor (Collision|BreakHitResult _outhit)))
    (:then
      (return _asbp_enemy))
    (:CastFailed
      (return 0))))

(fn FLinetraceRight
  (bind _self self)
  (bind _returnvalue (Transformation|GetActorLocation _self))
  (bind (_outhit _returnvalue_2) (Collision|LineTraceByChannel (+ _returnvalue "0, 0,150.000000") (+ _returnvalue (Math|Vector|MakeVector (Variables|Mechanic|GetAttaqueRange) 0.0 1.5e+02)) "TraceTypeQuery2" false 0 "None" true "(R=1.000000,G=0.000000,B=0.000000,A=1.000000)" "(R=0.000000,G=1.000000,B=0.000000,A=1.000000)" 1.0))
  (Variables|Mechanic|SetbRightHit? _returnvalue_2)
  (bind _asbp_enemy (Utilities|Casting|CastToBP_Enemy (.HitActor (Collision|BreakHitResult _outhit)))
    (:then
      (return _asbp_enemy))
    (:CastFailed
      (return 0))))

(fn FStartGame
  ;[1 1 1] Get a Reference of the Current Gamemode
  (bind _asgm_tafai_fighter (Utilities|Casting|CastToGM_TafaiFighter (Game|GetGameMode)))
  (bind _output_get (Variables|Reference|SetGameModeRef _asgm_tafai_fighter))
  ;[1 1 1] If is the first Game Launch Tuto
  (Variables|PlayerState|SetbTuto? (Variables|/Game/04-TafaiFighter/Blueprints/GM_TafaiFighter.GM_TafaiFighter_C|GetbFirstTime? _output_get))
  ;[1 1 1] Creat the Current Widget Interface InGame / PreCreat The WidgetPause
  (bind _returnvalue (UserInterface|CreateWidget "/Game/04-TafaiFighter/Widget/WBP_HudTafaiFighter.WBP_HudTafaiFighter_C" (Game|GetPlayerController 0)))
  (Variables|Reference|SetWBP_HUD_Ref _returnvalue)
  (bind _returnvalue_2 (UserInterface|CreateWidget "/Game/MetaGame/Widgets/WPB_Hud.WPB_Hud_C" (Game|GetPlayerController 0)))
  (Variables|Reference|SetWBP_PauseRef _returnvalue_2)
  (Rendering|SetVisibility (Variables|Default|GetSM_Stun) false false) ; Set the FX_Stun Hidden
  (if true ; DBug or not?
    ;[1 1 1] DBug : Permet d'afficher un bouton pour le shield (que sur PC)
    (bind _returnvalue_3 (UserInterface|CreateWidget "/Game/04-TafaiFighter/Widget/WBP_CheatShield.WBP_CheatShield_C" 0 self))
    (UserInterface|Viewport|AddtoViewport (Variables|Reference|GetWBP_HUD_Ref) 0)
    (return)
    (else
      ;[1 1 1] Display Widget In Game/ Pause
      (UserInterface|Viewport|AddtoViewport (Variables|Reference|GetWBP_HUD_Ref) 0)
      (return))))