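; BP_DayLight is the sun and daylight controller for TafaiFighter, animating a sunrise after a delay from BeginPlay.
; A looping timer steps the RotatingPoint pitch by RotationRate until F_StopSunRise clears it, with no built-in end angle.
; Each step remaps the pitch into the TimeTransition scalar of MPC_TafaiFighter, letting materials follow the sun.
; The construction script applies the same mapping from the actor's pitch.
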(event EventBeginPlay
  (Utilities|Time|SetTimerbyFunctionName self "F_StartSunRise" 3e+01))

(fn ConstructionScript
  (Rendering|Material|SetScalarParameterValue "/Game/04-TafaiFighter/Materials/MPC_TafaiFighter.MPC_TafaiFighter" "TimeTransition" (Math|Float|Lerp -3.0 1.0 (Math|Float|NormalizetoRange (.pitch (Transformation|GetActorRotation)) 0.0 -9e+01)) :!class /Script/Engine.KismetMaterialLibrary))

(fn FStopSunRise
  (Utilities|Time|ClearandInvalidateTimerbyHandle (Variables|Timer|GetSunRiserHandle))
  (return))

(fn FStartSunRise
  (bind _returnvalue (Utilities|Time|SetTimerbyFunctionName self "F_SunRise" 0.01 true))
  (Variables|Timer|SetSunRiserHandle _returnvalue)
  (return))

(fn FSunRise
  (Variables|Property|SetActualRotation (- (Variables|Property|GetActualRotation) (Variables|Property|GetRotationRate)))
  (Transformation|SetRelativeRotation (Variables|Default|GetRotatingPoint) (Math|Rotator|MakeRotator 0.0 (Variables|Property|GetActualRotation) 0.0) false false)
  (Rendering|Material|SetScalarParameterValue "/Game/04-TafaiFighter/Materials/MPC_TafaiFighter.MPC_TafaiFighter" "TimeTransition" (Math|Float|Lerp -3.0 1.0 (Math|Float|NormalizetoRange (Variables|Property|GetActualRotation) 0.0 -9e+01)) :!class /Script/Engine.KismetMaterialLibrary)
  (return))