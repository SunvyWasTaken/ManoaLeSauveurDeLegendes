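; Game mode for the Ruahatu level that runs a two-phase timed challenge with star scoring, music and ambient sound.
; BeginPlay starts audio, enables touch and cursor, then after a delay shows onboarding and starts the first-phase countdown, which ends with zero score on timeout.
; StartSecondPhase swaps it for a count-up timer that lowers the star score as time passes.
; StopGame shows the victory menu with the given score and switches to UI-only input.
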(event Custom|StopGame
  (params (Score :type Integer))
  (Utilities|FlowControl|DoOnce (Variables|Default|GetbIsFirstPhases?)
    (:Completed
      ;[1 1 1] Stop le jeu et affiche le menu victoire.
      (bind _returnvalue (UserInterface|CreateWidget "/Game/00_Metajeu/Widgets/WBP_MenuVictoire4.WBP_MenuVictoire4_C" 0 Score 1 2 3))
      (UserInterface|Viewport|AddtoViewport _returnvalue 0)
      (Input|SetInputModeUIOnly (Game|GetPlayerController 0) _returnvalue "DoNotLock"))))

(event Custom|StartGame
  ;[1 1 1] Compte à rebour de la première phase.
  (bind _returnvalue (Utilities|Time|SetTimerbyEvent (delegate Custom|TimerFirstPhas) 1.0 true))
  (Variables|Default|SetHandlerFirstPhase _returnvalue))

(event Custom|TimerFirstPhas
  ;[1 1 1] Compte à rebour de la première phase.
  (bind _result (Math|Integer|DecrementInt (Variables|Default|GetTimeFirstPhase))
    (:%20%20
      (Class|BPIRuahatu|SetTimer(Message) (Variables|Default|GetBP_HUD_InGame) _result)
      (Class|BPIRuahatu|SetTimer(Message) (Variables|Default|GetOnboardHUD) _result)
      (if (<= _result 0)
        (Variables|Default|SetbIsFirstPhases? false)
        (CallFunction|StopGame)
        (Utilities|Time|ClearandInvalidateTimerbyHandle (Variables|Default|GetHandlerFirstPhase))))))

(event Custom|StartSecondPhase
  ;[1 1 1] Compteur de la seconde phase.
  (Utilities|Time|ClearandInvalidateTimerbyHandle (Variables|Default|GetHandlerFirstPhase))
  (bind _returnvalue (Utilities|Time|SetTimerbyEvent (delegate Custom|TimerSecondPhase) 1.0 true))
  (Variables|Default|SetHandlerSecondPhase _returnvalue))

(event Custom|TimerSecondPhase
  ;[1 1 1] Compteur de la seconde phase.
  (bind _result (Math|Integer|IncrementInt (Variables|Default|GetTimeSecondPhase))
    (:%20%20
      (Class|BPIRuahatu|SetTimer(Message) (Variables|Default|GetBP_HUD_InGame) _result)
      (if (< _result 25)
        (Variables|Default|SetScore 3)
        (elif (< _result 40)
          (Variables|Default|SetScore 2)
          (else
            (Variables|Default|SetScore 1)))))))

(event Custom|StopHandlerSecond
  ;[1 1 1] Stop le Compteur de la seconde phase
  (Utilities|Time|ClearandInvalidateTimerbyHandle (Variables|Default|GetHandlerSecondPhase)))

(event Custom|PlaySOundAmbiance
  ;[1 1 1] Play des sound
  (Utilities|FlowControl|Sequence
    (:then_0
      (Utilities|FlowControl|DoOnce false
        (:Completed
          (Audio|SpawnSound2D "/Game/02_Teura/Audio/S_Waves.S_Waves" 1.0 1.0 0.0 0)
          (Development|PrintString "NOOOOOOOOOOOOOOOOOOOOOOOOOOOOOOOOOOOOOON!"))))
    (:then_1
      (Audio|PlaySound2D "/Game/05_Ruahatu/Sound/S_Oiseaux1_Ruahatu_Cue.S_Oiseaux1_Ruahatu_Cue" 1.0 1.0 0.0 0 0)
      (Utilities|Time|SetTimerbyFunctionName 0 "PlaySOundAmbiance" 1e+01))))

(event EventBeginPlay
  (bind _returnvalue (Game|GetPlayerController 0))
  (Class|PlayerController|ActivateTouchInterface _returnvalue)
  (Variables|/Script/Engine.PlayerController|SetbShowMouseCursor _returnvalue true)
  (bind _returnvalue_2 (Audio|SpawnSound2D "/Game/05_Ruahatu/Sound/Tribal_Drum_Pattern_2_-_Rodincoil_No_Copyright_Music.Tribal_Drum_Pattern_2_-_Rodincoil_No_Copyright_Music" 1.0 1.0 0.0 0))
  (Variables|Default|SetMusicInGame _returnvalue_2)
  (CallFunction|PlaySOundAmbiance)
  (Utilities|FlowControl|Delay 4.0)
  (bind _returnvalue_3 (UserInterface|CreateWidget "/Game/05_Ruahatu/Widget/PopUp/WBP_Onboarding_Attrapper.WBP_Onboarding_Attrapper_C"))
  (bind _output_get (Variables|Default|SetOnboardHUD _returnvalue_3))
  (UserInterface|Viewport|AddtoViewport _output_get 0)
  (CallFunction|StartGame)
  (Variables|Default|SetbWaitOnBoarding false))

(fn ConstructionScript)