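; Player Blueprint for the Ruahatu fishing minigame: tap to throw a hook at the god Ruahatu, then reel him in.
; Hook overlap attaches him and starts phase two, where short drags lower LifePoint until victory.
; Random timed escapes pull him sideways until the player swipes the opposite way, guided by pop-up widgets.
; Tick positions the hook from interpolated LifePoint and escape alpha to smooth movement.
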(event OnComponentBeginOverlap(Sphere)
  (params (OverlappedComponent :type Primitive%20Component%20Object%20Reference) (OtherActor :type Actor%20Object%20Reference) (OtherComp :type Primitive%20Component%20Object%20Reference) (OtherBodyIndex :type Integer) (bFromSweep :type Boolean) (SweepResult :type Hit%20Result%20Structure%20%28by%20ref%29))
  (bind _gamemoderef (Variables|Ref|GetGamemodeRef))
  ;[1 0.9385 0 1 20] Lorsque la sphere de l'hamecon touche Ruahatu cela arrete l'animation du throw et change de phase.
  (bind _asbp_dieu_ruahatu (Utilities|Casting|CastToBP_Dieu_Ruahatu OtherActor))
  (Variables|Ref|SetRuahatuRef _asbp_dieu_ruahatu)
  (Transformation|AttachComponentToComponent OtherActor (Variables|Default|GetHamecon) "None" "SnapToTarget" "KeepWorld" "KeepRelative" false)
  (CallFunction|Gotcha)
  (Variables|/Game/05_Ruahatu/Blueprint/GM_Ruahatu.GM_Ruahatu_C|SetbIsFirstPhases? _gamemoderef false)
  (Default|StartSecondPhase _gamemoderef)
  (CallFunction|WanttoGoWay)
  (|TutoDrag))

(event Custom|Gotcha
  ;[0 1 0.3 1 25] Truc qui fait que l'hamecon part et s'accroche à Ruahatu à la fin
  (bind _alpha (Timeline|Throw Stop)
    (:Update
      (Transformation|SetWorldLocation (Variables|Default|GetHamecon) (Math|Vector|Lerp(Vector) (Variables|Default|GetOrigineLocationHam) (Transformation|GetActorLocation (Variables|Ref|GetControlRef)) _alpha) false false))
    (:Finished
      (Variables|Default|SetbIsThrowing false))))

(event Custom|SwipeLeft
  (params (Value :type Float%20%28single-precision%29))
  ;[0 0.3096 1 1 20] Permet de swipe d'un côte à l'autre en fonction de la ou se trouve Ruahatu.
  (if (and (Variables|Default|GetbIsTryToGetOut) (not (Variables|Default|GetIsGoLeft)))
    (CallFunction|FSetAlpha Value)
    (Audio|PlaySound2D "/Game/05_Ruahatu/Sound/S_TirerRuahatu_Ruahatu.S_TirerRuahatu_Ruahatu" 1.0 1.0 0.0 0 0)
    (else
      (Audio|PlaySound2D "/Game/05_Ruahatu/Sound/S_LancerRater_Ruahatu.S_LancerRater_Ruahatu" 1.0 1.0 0.0 0 0)
      (Default|WrongMove (Variables|Ref|GetWidgetRef)))))

(event Custom|SwipeRight
  (params (Value :type Float%20%28single-precision%29))
  ;[0 0.3096 1 1 20] Permet de swipe d'un côte à l'autre en fonction de la ou se trouve Ruahatu.
  (if (and (Variables|Default|GetbIsTryToGetOut) (Variables|Default|GetIsGoLeft))
    (CallFunction|FSetAlpha Value)
    (Audio|PlaySound2D "/Game/05_Ruahatu/Sound/S_TirerRuahatu_Ruahatu.S_TirerRuahatu_Ruahatu" 1.0 1.0 0.0 0 0)
    (else
      (Audio|PlaySound2D "/Game/05_Ruahatu/Sound/S_LancerRater_Ruahatu.S_LancerRater_Ruahatu" 1.0 1.0 0.0 0 0)
      (Default|WrongMove (Variables|Ref|GetWidgetRef)))))

(event Custom|Drag
  (params (Value :type Float%20%28single-precision%29))
  (bind _gamemoderef (Variables|Ref|GetGamemodeRef))
  (bind _pp_ramener (Variables|Default|GetPP_Ramener))
  (bind _pp_gauche (Variables|Default|GetPP_Gauche))
  (bind _pp_droite (Variables|Default|GetPP_Droite))
  (bind _limiteswipe (Variables|Default|GetLimiteSwipe))
  ;[0 0.9271 1 1 20] Event Reduit les life point donc ramène Ruahatu vers sois.
  (if (not (Variables|Default|GetbIsTryToGetOut))
    (Variables|Default|SetLifePoint (- (Variables|Default|GetLifePoint) (select (> Value _limiteswipe) _limiteswipe Value)))
    (Default|CorrectMove (Variables|Ref|GetWidgetRef))
    (Audio|PlaySound2D "/Game/05_Ruahatu/Sound/S_TirerRuahatu_Ruahatu.S_TirerRuahatu_Ruahatu" 1.0 1.0 0.2 0 0)
    (CallFunction|FSpawnSplash)
    (if (<= (Variables|Default|GetLifePoint) 5e+01)
      (Utilities|FlowControl|Sequence
        (:then_0
          (Variables|Default|SetbIsGameFinished true)
          (Default|StopGame _gamemoderef (Variables|/Game/05_Ruahatu/Blueprint/GM_Ruahatu.GM_Ruahatu_C|GetScore _gamemoderef))
          (Default|StopHandlerSecond _gamemoderef)
          (Utilities|IsValid _pp_ramener
            (:Is%20Valid
              (Widget|RemovefromParent _pp_ramener))
            (:Is%20Not%20Valid
              _))
          (Utilities|IsValid _pp_gauche
            (:Is%20Valid
              (Widget|RemovefromParent _pp_gauche))
            (:Is%20Not%20Valid
              _))
          (Utilities|IsValid _pp_droite
            (:Is%20Valid
              (Widget|RemovefromParent _pp_droite))))
        (:then_1
          (Audio|PlaySound2D "/Game/05_Ruahatu/Sound/S_VictoireRuahatu_Ruahatu.S_VictoireRuahatu_Ruahatu" 1.0 1.0 0.0 0 0))))))

(event Custom|WantToGoWay
  (bind _pp_ramener (Variables|Default|GetPP_Ramener))
  ;[0.401 0.1825 0.1665] Fait en sort que Ruahatu essais de s'échaper de droite à gauche à des moments différents.
  (Utilities|FlowControl|Delay (Math|Random|RandomFloatinRange 2.0 5.0)) ; Regler le delay entre chaque moment ou Ruahatu essais de s'échaper.
  (if (Variables|Default|GetbIsTryToGetOut)
    (CallFunction|WanttoGoWay)
    (else
      (Variables|Default|SetIsGoLeft (Math|Random|RandomBool))
      (Variables|Default|SetbIsTryToGetOut true)
      (Utilities|FlowControl|Sequence
        (:then_0
          (CallFunction|WanttoGoWay)
          ;;[1 1 1 0.5] Permet de faire une transient plus smooth
          (bind _returnvalue (Utilities|Time|SetTimerbyEvent (delegate Custom|GoOut) (Utilities|Time|GetWorldDeltaSeconds) true))
          (Utilities|FlowControl|Delay 0.2)
          (Utilities|Time|ClearandInvalidateTimerbyHandle _returnvalue)
          (Utilities|FlowControl|Delay 0.2)
          (CallFunction|FSpawnSplash))
        (:then_1
          (if (not (Variables|Default|GetbIsGameFinished))
            (Utilities|IsValid _pp_ramener
              (:Is%20Valid
                (Widget|RemovefromParent _pp_ramener))
              (:Is%20Not%20Valid
                _))
            (if (Variables|Default|GetIsGoLeft)
              (bind _returnvalue_2 (UserInterface|CreateWidget "/Game/05_Ruahatu/Widget/PopUp/WBP_PopUp_Droite.WBP_PopUp_Droite_C"))
              (bind _output_get (Variables|Default|SetPP_Droite _returnvalue_2))
              (Default|AnimationTirerDroite _output_get)
              (UserInterface|Viewport|AddtoViewport _output_get 0)
              (Utilities|IsValid (Variables|Default|GetPP_Gauche)
                (:Is%20Valid
                  (Widget|RemovefromParent (Variables|Default|GetPP_Gauche))))
              (else
                (bind _returnvalue_3 (UserInterface|CreateWidget "/Game/05_Ruahatu/Widget/PopUp/WBP_PopUp_Gauche.WBP_PopUp_Gauche_C"))
                (bind _output_get_2 (Variables|Default|SetPP_Gauche _returnvalue_3))
                (Default|AnimationTirerGauche _output_get_2)
                (UserInterface|Viewport|AddtoViewport _output_get_2 0)
                (Utilities|IsValid (Variables|Default|GetPP_Droite)
                  (:Is%20Valid
                    (Widget|RemovefromParent (Variables|Default|GetPP_Droite))))))
            (Audio|PlaySound2D "/Game/05_Ruahatu/Sound/S_ProieQuiSeDebatDansLeau_Ruahatu.S_ProieQuiSeDebatDansLeau_Ruahatu" 1.0 1.0 0.0 0 0)))))))

(event Custom|GoOut
  ;[0.401 0.1825 0.1665] Fait en sort que Ruahatu essais de s'échaper de droite à gauche à des moments différents.
  ;;[1 1 1 0.5] Permet de faire une transient plus smooth
  (Variables|Default|SetAlphGetOut (Math|Interpolation|FInterpTo (Variables|Default|GetAlphGetOut) 1.0 (Utilities|Time|GetWorldDeltaSeconds) 15.0))
  (CallFunction|FSpawnSplash))

(event EventTick
  (params (DeltaSeconds :type Float%20%28single-precision%29))
  ;[1 0 0 1 20] Tick qui Blend tous se qui fait que les déplacements soit smooth
  (if (not (Variables|/Game/05_Ruahatu/Blueprint/GM_Ruahatu.GM_Ruahatu_C|GetbIsFirstPhases? (Variables|Ref|GetGamemodeRef)))
    (Transformation|SetWorldLocation (Variables|Default|GetHamecon) (CallFunction|FSQJTEDV) false false)
    (Variables|Default|SetbIsDragging (not (select (Variables|Default|GetbIsTryToGetOut) (Math|Float|NearlyEqual(Float) (Variables|Default|GetAlphaTransi) (Variables|Default|GetAlphGetOut) 0.1) (Math|Float|NearlyEqual(Float) (Variables|Default|GetLifePoint) (Variables|Default|GetLifePointTransient) 0.1))))))

(event EventBeginPlay
  ;[1 1 1] Set toutes les references du gamemode au début
  (bind _returnvalue (UserInterface|CreateWidget "/Game/05_Ruahatu/Widget/WBP_InGame_Ruahatu.WBP_InGame_Ruahatu_C"))
  (bind _output_get (Variables|Ref|SetWidgetRef _returnvalue))
  (UserInterface|Viewport|AddtoViewport _output_get 0)
  (Input|SetInputModeGameandUI (Game|GetPlayerController 0) 0 "DoNotLock" false)
  (bind _asgm_ruahatu (Utilities|Casting|CastToGM_Ruahatu (Game|GetGameMode)))
  (Variables|Ref|SetGamemodeRef _asgm_ruahatu)
  (Variables|/Game/05_Ruahatu/Blueprint/GM_Ruahatu.GM_Ruahatu_C|SetBP_HUD_InGame _asgm_ruahatu (Variables|Ref|GetWidgetRef))
  (bind _returnvalue_2 (UserInterface|CreateWidget "/Game/05_Ruahatu/Widget/PopUp/WBP_PopUp_Ramener.WBP_PopUp_Ramener_C"))
  (bind _output_get_2 (Variables|Default|SetPP_Ramener _returnvalue_2))
  (UserInterface|Viewport|AddtoViewport _output_get_2 0)
  (Widget|SetVisibility _output_get_2 "Hidden"))

(event Input|TouchEvents|InputTouch
  (params (Location :type Vector) (FingerIndex :type ETouchIndex%20Enum))
  (:Pressed
    (Utilities|IsFirstPhase ; If it's true throw the hook\nfalse get the current location of the finger on the screen
      (:true
        (if (not (or (Variables|Default|GetbIsThrowing) (Variables|/Game/05_Ruahatu/Blueprint/GM_Ruahatu.GM_Ruahatu_C|GetbWaitOnBoarding (Variables|Ref|GetGamemodeRef)))) ; If the hook is already throw don't cast the rest
          (Variables|Default|SetbIsThrowing true)
          (Utilities|FlowControl|Sequence ; parce que j'avais la flemme de réfléchir et surtout que personne ne ressent la dif
            (:then_0
              ;[0 1 0.3 1 25] Truc qui fait que l'hamecon part et s'accroche à Ruahatu à la fin
              (bind _alpha (Timeline|Throw PlayFromStart)
                (:Update
                  (Transformation|SetWorldLocation (Variables|Default|GetHamecon) (Math|Vector|Lerp(Vector) (Variables|Default|GetOrigineLocationHam) (Transformation|GetActorLocation (Variables|Ref|GetControlRef)) _alpha) false false))
                (:Finished
                  (Variables|Default|SetbIsThrowing false))))
            (:then_1
              ;[1 1 1] Play un Son en fonction de si l'hamecon à toucher ou pas
              (Utilities|FlowControl|Delay 0.2)
              (Audio|PlaySound2D (select (Variables|/Game/05_Ruahatu/Blueprint/GM_Ruahatu.GM_Ruahatu_C|GetbIsFirstPhases? (Variables|Ref|GetGamemodeRef)) "/Game/05_Ruahatu/Sound/S_LancerRater_Ruahatu.S_LancerRater_Ruahatu" 0) 1.0 1.0 0.0 0 0)))))
      (:false
        (Variables|Default|SetStartLocationFinger (CallFunction|FFingerLocation)))))
  (:Released
    ;[1 0.03 0.8159 1 28] Calcule dans quel direction le doigth et swipe et appel la bonne fonction en retour.
    (Utilities|IsFirstPhase
      (:false
        (Variables|Default|SetEndLocationFinger (CallFunction|FFingerLocation))
        (if (or (<= (Math|Float|NormalizetoRange (.X (Math|Vector2D|BreakVector2D (- (Variables|Default|GetEndLocationFinger) (Variables|Default|GetStartLocationFinger)))) -5e+02 5e+02) 0.4) (>= (Math|Float|NormalizetoRange (.X (Math|Vector2D|BreakVector2D (- (Variables|Default|GetEndLocationFinger) (Variables|Default|GetStartLocationFinger)))) -5e+02 5e+02) 0.6)) ; Detecte si il swipe pour ramener au milieu ou si il drag
          (if (> (.X (Math|Vector2D|BreakVector2D (- (Variables|Default|GetEndLocationFinger) (Variables|Default|GetStartLocationFinger)))) 0.0)
            (CallFunction|SwipeRight (/ (Math|Vector2D|Vector2DLength (- (Variables|Default|GetEndLocationFinger) (Variables|Default|GetStartLocationFinger))) 1e+01))
            (else
              (CallFunction|SwipeLeft (/ (Math|Vector2D|Vector2DLength (- (Variables|Default|GetEndLocationFinger) (Variables|Default|GetStartLocationFinger))) 1e+01))))
          (else
            (CallFunction|Drag (/ (Math|Vector2D|Vector2DLength (- (Variables|Default|GetEndLocationFinger) (Variables|Default|GetStartLocationFinger))) 1e+01))))))))

(fn ConstructionScript
  (bind _lifepoint (Variables|Default|GetLifePoint))
  (Variables|Default|SetOrigineLocationHam (Transformation|GetWorldLocation (Variables|Default|GetHamecon)))
  (Variables|Default|SetLifePointMax _lifepoint)
  (Variables|Default|SetLifePointTransient _lifepoint))

(fn FFingerLocation
  (bind _returnvalue (Game|GetPlayerController 0))
  (bind (_locationx _locationy) (Class|PlayerController|GetInputTouchState _returnvalue "Touch1"))
  (return (Math|Vector2D|MakeVector2D _locationx _locationy)))

(fn FTCQGPEDC
  (params (Alpha :type Float%20%28single-precision%29))
  (return (select (Variables|Default|GetIsGoLeft) (Math|Float|Lerp (.Y (Math|Vector|BreakVector (Variables|Default|GetOrigineLocationHam))) (.Y (Math|Vector|BreakVector (Variables|/Game/05_Ruahatu/Blueprint/BP_Dieu_Ruahatu.BP_Dieu_Ruahatu_C|GetLeftPosition (Variables|Ref|GetRuahatuRef)))) Alpha) (Math|Float|Lerp (.Y (Math|Vector|BreakVector (Variables|Default|GetOrigineLocationHam))) (.Y (Math|Vector|BreakVector (Variables|/Game/05_Ruahatu/Blueprint/BP_Dieu_Ruahatu.BP_Dieu_Ruahatu_C|GetRightPosition (Variables|Ref|GetRuahatuRef)))) Alpha))))

(fn FSQJTEDV
  (bind _returnvalue (Utilities|Time|GetWorldDeltaSeconds))
  (Variables|Default|SetLifePointTransient (Math|Interpolation|FInterpTo (Variables|Default|GetLifePointTransient) (Variables|Default|GetLifePoint) _returnvalue 2.0))
  (Variables|Default|SetAlphaTransi (Math|Interpolation|FInterpTo (Variables|Default|GetAlphaTransi) (Variables|Default|GetAlphGetOut) _returnvalue 5.0))
  (return (Math|Vector|MakeVector (.X (Math|Vector|BreakVector (Math|Vector|Lerp(Vector) (Transformation|GetWorldLocation (Variables|Default|GetTargetPoint)) (Transformation|GetActorLocation (Variables|Ref|GetControlRef)) (Math|Float|NormalizetoRange (Math|Interpolation|FInterpTo (Variables|Default|GetLifePointTransient) (Variables|Default|GetLifePoint) _returnvalue 2.0) 0.0 (Variables|Default|GetLifePointMax))))) (Math|Float|Lerp (.Y (Math|Vector|BreakVector (Math|Vector|Lerp(Vector) (Transformation|GetWorldLocation (Variables|Default|GetTargetPoint)) (Transformation|GetActorLocation (Variables|Ref|GetControlRef)) (Math|Float|NormalizetoRange (Math|Interpolation|FInterpTo (Variables|Default|GetLifePointTransient) (Variables|Default|GetLifePoint) _returnvalue 2.0) 0.0 (Variables|Default|GetLifePointMax))))) (CallFunction|FTCQGPEDC (Math|Float|NormalizetoRange (Math|Interpolation|FInterpTo (Variables|Default|GetLifePointTransient) (Variables|Default|GetLifePoint) _returnvalue 2.0) 0.0 (Variables|Default|GetLifePointMax))) (Math|Interpolation|FInterpTo (Variables|Default|GetAlphaTransi) (Variables|Default|GetAlphGetOut) _returnvalue 5.0)) (.Z (Math|Vector|BreakVector (Math|Vector|Lerp(Vector) (Transformation|GetWorldLocation (Variables|Default|GetTargetPoint)) (Transformation|GetActorLocation (Variables|Ref|GetControlRef)) (Math|Float|NormalizetoRange (Math|Interpolation|FInterpTo (Variables|Default|GetLifePointTransient) (Variables|Default|GetLifePoint) _returnvalue 2.0) 0.0 (Variables|Default|GetLifePointMax))))))))

(fn FSpawnSplash
  (bind _ruahaturef (Variables|Ref|GetRuahatuRef))
  (bind _returnvalue (Transformation|GetActorLocation _ruahaturef))
  (Effects|SpawnEmitteratLocation "/Game/05_Ruahatu/FX_Splash/ParticleSystems/PS_Splash.PS_Splash" (Math|Vector|MakeVector (.x _returnvalue) (.y _returnvalue) (+ (.z _returnvalue) 1e+01)) "-10.000000, 0,0.000000" "0.250000,0.250000,0.250000"))

(fn FSetAlpha
  (params (Value :type Float%20%28single-precision%29))
  (bind _pp_gauche (Variables|Default|GetPP_Gauche))
  (bind _pp_droite (Variables|Default|GetPP_Droite))
  (bind _output_get (Variables|Default|SetAlphGetOut (- (Variables|Default|GetAlphGetOut) (Math|Float|NormalizetoRange Value 0.0 5e+02))))
  (Audio|PlaySound2D "/Game/05_Ruahatu/Sound/S_TirerRuahatu_Ruahatu.S_TirerRuahatu_Ruahatu" 1.0 1.0 0.2 0 0)
  (CallFunction|FSpawnSplash)
  (Default|CorrectMove (Variables|Ref|GetWidgetRef))
  (if (Math|Float|NearlyEqual(Float) _output_get 0.0 0.1)
    (Variables|Default|SetbIsTryToGetOut false)
    (CallFunction|FSpawnSplash)
    (bind _returnvalue (UserInterface|CreateWidget "/Game/05_Ruahatu/Widget/PopUp/WBP_PopUp_Ramener.WBP_PopUp_Ramener_C"))
    (bind _output_get_2 (Variables|Default|SetPP_Ramener _returnvalue))
    (Default|AnimationRamener _output_get_2)
    (UserInterface|Viewport|AddtoViewport _output_get_2 0)
    (Utilities|IsValid _pp_droite
      (:Is%20Valid
        (Widget|RemovefromParent _pp_droite))
      (:Is%20Not%20Valid
        _))
    (Utilities|IsValid _pp_gauche
      (:Is%20Valid
        (Widget|RemovefromParent _pp_gauche)))))