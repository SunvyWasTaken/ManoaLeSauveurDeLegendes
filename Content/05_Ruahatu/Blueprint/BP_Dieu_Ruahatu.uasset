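; BP_Dieu_Ruahatu is the Ruahatu god actor that darts between left and right positions until the player catches it.
; One timeline, played forward or reversed, lerps its location using one of three randomly chosen curves.
; Each pass starts with a struggling-in-water sound and ends with a splash, a curve re-roll and a short random delay before turning back.
; Player overlap stops the timeline, hides sprite and particles, and splashes.
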(event OnComponentBeginOverlap(BoxCollision)
  (params (OverlappedComponent :type Primitive%20Component%20Object%20Reference) (OtherActor :type Actor%20Object%20Reference) (OtherComp :type Primitive%20Component%20Object%20Reference) (OtherBodyIndex :type Integer) (bFromSweep :type Boolean) (SweepResult :type Hit%20Result%20Structure%20%28by%20ref%29))
  (bind _returnvalue (Transformation|GetActorLocation))
  (if (== (Utilities|GetClass OtherActor) "/Game/05_Ruahatu/Blueprint/BP_Player_Ruahatu.BP_Player_Ruahatu_C")
    (CallFunction|Catch)
    (Effects|SpawnEmitteratLocation "/Game/05_Ruahatu/FX_Splash/ParticleSystems/PS_Splash.PS_Splash" (Math|Vector|MakeVector (.x _returnvalue) (.y _returnvalue) (+ (.z _returnvalue) -25.0)) "-25.000000, 0,0.000000" "0.250000,0.250000,0.250000")
    (Development|SetHiddeninGame (Variables|Default|GetParticleSystem1) true false)))

(event Custom|Start
  (Variables|Default|SetChoice (CallFunction|FRandomSpeed))
  (if (Math|Random|RandomBool)
    (CallFunction|GoRight)
    (else
      (CallFunction|GoLeft))))

(event Custom|GoLeft
  (bind _returnvalue (Math|Random|RandomFloat))
  (bind _returnvalue_2 (Transformation|GetActorLocation))
  (bind _returnvalue_3 (* _returnvalue 1.2))
  (Audio|PlaySound2D "/Game/05_Ruahatu/Sound/S_ProieQuiSeDebatDansLeau_Ruahatu.S_ProieQuiSeDebatDansLeau_Ruahatu" 1.0 1.0 0.0 0 0)
  (bind (_direction _staight _slowstart _slowend) (Timeline|Timeline Reverse) ; J'ai fais 3 timeline différentes pour que la première partie soit un peu plus compliquer.\nSi tu veux changer la vitesse c'est ici qu'il faut le faire.\nPS Il faut aussi aller changer les curves dans le dossier Curve.
    (:Update
      ;[1 1 1] Set la location de Ruahatu en fonction de la timeline
      (Transformation|SetActorLocation (Math|Vector|Lerp(Vector) (Variables|Default|GetLeftPosition) (Variables|Default|GetRightPosition) (Utilities|Select :Index (Variables|Default|GetChoice) :NewEnumerator0 _staight :NewEnumerator1 _slowstart :NewEnumerator2 _slowend)) false false))
    (:Finished
      (Effects|SpawnEmitteratLocation "/Game/05_Ruahatu/FX_Splash/ParticleSystems/PS_Splash.PS_Splash" (Math|Vector|MakeVector (.x _returnvalue_2) (.y _returnvalue_2) (+ (.z _returnvalue_2) 5e+01)) "-10.000000, 0,0.000000" "0.120000,0.120000,0.120000")
      ;[1 1 1] Lorsque la timeline se termine lance automatiquement le reverse après un certain delay et une vitesse différente
      (Variables|Default|SetChoice (CallFunction|FRandomSpeed))
      (switch Utilities|FlowControl|Switch|SwitchonETimelineDirection _direction
        (:Forward
          (Utilities|FlowControl|Delay _returnvalue_3)
          (CallFunction|GoLeft))
        (:Backward
          (Utilities|FlowControl|Delay _returnvalue_3)
          (CallFunction|GoRight))))))

(event Custom|Catch
  (bind _returnvalue (Math|Random|RandomFloat))
  (bind _returnvalue_2 (Transformation|GetActorLocation))
  (bind _returnvalue_3 (* _returnvalue 1.2))
  (Rendering|SetVisibility (Variables|Default|GetPaperSprite) false false)
  (bind (_direction _staight _slowstart _slowend) (Timeline|Timeline Stop) ; J'ai fais 3 timeline différentes pour que la première partie soit un peu plus compliquer.\nSi tu veux changer la vitesse c'est ici qu'il faut le faire.\nPS Il faut aussi aller changer les curves dans le dossier Curve.
    (:Update
      ;[1 1 1] Set la location de Ruahatu en fonction de la timeline
      (Transformation|SetActorLocation (Math|Vector|Lerp(Vector) (Variables|Default|GetLeftPosition) (Variables|Default|GetRightPosition) (Utilities|Select :Index (Variables|Default|GetChoice) :NewEnumerator0 _staight :NewEnumerator1 _slowstart :NewEnumerator2 _slowend)) false false))
    (:Finished
      (Effects|SpawnEmitteratLocation "/Game/05_Ruahatu/FX_Splash/ParticleSystems/PS_Splash.PS_Splash" (Math|Vector|MakeVector (.x _returnvalue_2) (.y _returnvalue_2) (+ (.z _returnvalue_2) 5e+01)) "-10.000000, 0,0.000000" "0.120000,0.120000,0.120000")
      ;[1 1 1] Lorsque la timeline se termine lance automatiquement le reverse après un certain delay et une vitesse différente
      (Variables|Default|SetChoice (CallFunction|FRandomSpeed))
      (switch Utilities|FlowControl|Switch|SwitchonETimelineDirection _direction
        (:Forward
          (Utilities|FlowControl|Delay _returnvalue_3)
          (CallFunction|GoLeft))
        (:Backward
          (Utilities|FlowControl|Delay _returnvalue_3)
          (CallFunction|GoRight))))))

(event Custom|GoRight
  (bind _returnvalue (Math|Random|RandomFloat))
  (bind _returnvalue_2 (Transformation|GetActorLocation))
  (bind _returnvalue_3 (* _returnvalue 1.2))
  (Audio|PlaySound2D "/Game/05_Ruahatu/Sound/S_ProieQuiSeDebatDansLeau_Ruahatu.S_ProieQuiSeDebatDansLeau_Ruahatu" 1.0 1.0 0.0 0 0)
  (bind (_direction _staight _slowstart _slowend) (Timeline|Timeline Play) ; J'ai fais 3 timeline différentes pour que la première partie soit un peu plus compliquer.\nSi tu veux changer la vitesse c'est ici qu'il faut le faire.\nPS Il faut aussi aller changer les curves dans le dossier Curve.
    (:Update
      ;[1 1 1] Set la location de Ruahatu en fonction de la timeline
      (Transformation|SetActorLocation (Math|Vector|Lerp(Vector) (Variables|Default|GetLeftPosition) (Variables|Default|GetRightPosition) (Utilities|Select :Index (Variables|Default|GetChoice) :NewEnumerator0 _staight :NewEnumerator1 _slowstart :NewEnumerator2 _slowend)) false false))
    (:Finished
      (Effects|SpawnEmitteratLocation "/Game/05_Ruahatu/FX_Splash/ParticleSystems/PS_Splash.PS_Splash" (Math|Vector|MakeVector (.x _returnvalue_2) (.y _returnvalue_2) (+ (.z _returnvalue_2) 5e+01)) "-10.000000, 0,0.000000" "0.120000,0.120000,0.120000")
      ;[1 1 1] Lorsque la timeline se termine lance automatiquement le reverse après un certain delay et une vitesse différente
      (Variables|Default|SetChoice (CallFunction|FRandomSpeed))
      (switch Utilities|FlowControl|Switch|SwitchonETimelineDirection _direction
        (:Forward
          (Utilities|FlowControl|Delay _returnvalue_3)
          (CallFunction|GoLeft))
        (:Backward
          (Utilities|FlowControl|Delay _returnvalue_3)
          (CallFunction|GoRight))))))

(fn ConstructionScript)

(fn FRandomSpeed
  (switch int (Math|Random|RandomIntegerinRange 1 3)
    (:1
      (return "NewEnumerator0"))
    (:2
      (return "NewEnumerator1"))
    (:3
      (return "NewEnumerator2"))))