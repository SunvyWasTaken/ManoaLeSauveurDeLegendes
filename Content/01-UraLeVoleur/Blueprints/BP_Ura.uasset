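; BP_Ura is the feathered Ura character in the UraLeVoleur game, built on the SKZazou skeletal mesh.
; On BeginPlay it spawns a BP_Direction and a BP_Plume at each of six feather sockets, with pitch randomized around the socket's absolute roll.
; SpawnFeather gives each plume its slot index, base orientation and direction actor, then attaches it to the socket.
; HurtAnimation briefly plays a hurt animation before resuming the looping default.
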(event Custom|HurtAnimation
  (Components|Animation|PlayAnimation (Variables|Default|GetSK_Zazou) "/Game/01-UraLeVoleur/Animations/Anim_Hurt.Anim_Hurt" false)
  (Utilities|FlowControl|Delay 0.8)
  (Components|Animation|PlayAnimation (Variables|Default|GetSK_Zazou) "/Game/01-UraLeVoleur/Animations/Anim_Zazou.Anim_Zazou" true))

(event EventBeginPlay
  (for _index (range 0 5)
    (Variables|Default|SetSpotToTake _index)
    (Variables|Default|SetSocketToAttach (Utilities|Array|Get(acopy) (Variables|Default|GetSocketPlumes) _index))
    (bind _returnvalue (Game|SpawnActorfromClass "/Game/01-UraLeVoleur/Blueprints/BP_Direction.BP_Direction_C" (Math|Transform|MakeTransform (.location (Transformation|GetSocketTransform (Variables|Default|GetSK_Zazou) (Utilities|Array|Get(acopy) (Variables|Default|GetSocketPlumes) _index) "RTS_World")) (Math|Rotator|MakeRotator 0.0 (Math|Random|RandomFloatinRange (- (Math|Float|Absolute(Float) (.roll (.rotation (Transformation|GetSocketTransform (Variables|Default|GetSK_Zazou) (Utilities|Array|Get(acopy) (Variables|Default|GetSocketPlumes) _index) "RTS_World")))) 5e+01) (+ (Math|Float|Absolute(Float) (.roll (.rotation (Transformation|GetSocketTransform (Variables|Default|GetSK_Zazou) (Utilities|Array|Get(acopy) (Variables|Default|GetSocketPlumes) _index) "RTS_World")))) 5e+01)) 9e+01) "1,1,1") "Undefined" 0 0))
    (Transformation|AttachComponentToComponent 0 "None" "KeepWorld" "KeepWorld" "KeepWorld" true)
    (CallFunction|SpawnFeather (.location (Transformation|GetSocketTransform (Variables|Default|GetSK_Zazou) (Utilities|Array|Get(acopy) (Variables|Default|GetSocketPlumes) _index) "RTS_World")) (Math|Random|RandomFloatinRange (- (Math|Float|Absolute(Float) (.roll (.rotation (Transformation|GetSocketTransform (Variables|Default|GetSK_Zazou) (Utilities|Array|Get(acopy) (Variables|Default|GetSocketPlumes) _index) "RTS_World")))) 3e+01) (+ (Math|Float|Absolute(Float) (.roll (.rotation (Transformation|GetSocketTransform (Variables|Default|GetSK_Zazou) (Utilities|Array|Get(acopy) (Variables|Default|GetSocketPlumes) _index) "RTS_World")))) 3e+01)) (Math|Rotator|MakeRotator 0.0 (Math|Random|RandomFloatinRange (- (Math|Float|Absolute(Float) (.roll (.rotation (Transformation|GetSocketTransform (Variables|Default|GetSK_Zazou) (Utilities|Array|Get(acopy) (Variables|Default|GetSocketPlumes) _index) "RTS_World")))) 3e+01) (+ (Math|Float|Absolute(Float) (.roll (.rotation (Transformation|GetSocketTransform (Variables|Default|GetSK_Zazou) (Utilities|Array|Get(acopy) (Variables|Default|GetSocketPlumes) _index) "RTS_World")))) 3e+01)) 9e+01) _returnvalue)))

(fn ConstructionScript)

(fn SpawnFeather
  (params (SpawnTransform_Location :type Vector) (SpawnTransform_Rotation_Pitch :type Float%20%28single-precision%29) (BaseOrientation :type Rotator) (DirectionActor :type BP%20Direction%20Object%20Reference))
  (bind _returnvalue (Game|SpawnActorfromClass "/Game/01-UraLeVoleur/Blueprints/BP_Plume.BP_Plume_C" (Math|Transform|MakeTransform SpawnTransform_Location (Math|Rotator|MakeRotator 0.0 SpawnTransform_Rotation_Pitch 9e+01) (Variables|Default|GetFeatherSize)) "Undefined" self (Variables|Default|GetSpotToTake) BaseOrientation DirectionActor 0))
  (Transformation|AttachComponentToComponent _returnvalue (Variables|Default|GetSK_Zazou) (Variables|Default|GetSocketToAttach) "KeepWorld" "KeepWorld" "KeepWorld" true))