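; BP_Plume is a feather on the BP_Ura bird that is pulled off, scores points, then respawns.
; Setup rolls a weighted rarity that selects its look from StructPlumes, with golden feathers enabled only after a delay.
; Detaching swaps material or golden component, release enables physics, and select, unselect and hide calls toggle direction arrows.
; Reset optionally awards points through GM_Ura, rerolls rarity, and reattaches it to its bird socket facing a rerandomized direction.
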(event EventBeginPlay
  ;[1 1 1] Get All the needed reference when the game begins (GameMode and Owner)
  (bind _asbp_ura (Utilities|Casting|CastToBP_Ura (Components|GetOwner)))
  (Variables|References|SetUraOwnerRef _asbp_ura) ; Reference to the bird blueprint
  (bind _asgm_ura (Utilities|Casting|CastToGM_Ura (Game|GetGameMode)))
  (Variables|References|SetGMRef _asgm_ura) ; Reference to the game mode
  (Setup|FeathersSetup)
  (Utilities|FlowControl|Delay (Variables|GoldSpawn|GetDelayAvantSpawnGold))
  (Variables|GoldSpawn|SetShouldSpawnGold true))

(event EventResetFeather
  (params (ShouldAddToScore :type Boolean))
  (bind _structplumes (Variables|References|GetStructPlumes))
  (bind _nbrfeather (Variables|Variables|GetNbrFeather))
  (bind _output (Utilities|Array|Get(acopy) _structplumes _nbrfeather))
  (bind (_points _addscoresound) (Utilities|Struct|BreakStruct_Plumes _output))
  ;[1 1 1] Called when a Feather touches the ground or the Tree
  (Physics|SetSimulatePhysics (Variables|Components|GetFeatherPlane) false)
  (if ShouldAddToScore
    (Default|AddtoScore (Variables|References|GetGMRef) _points)
    (Audio|PlaySound2D _addscoresound 1.0 1.0 0.0 0 0))
  (Setup|FeathersSetup)
  (CallFunction|RespawnFeathers))

(fn ConstructionScript)

(fn FeatherRarityCalculator
  (LocalVariables|SetRareteTiree (Math|Random|RandomIntegerinRange 0 (select (Variables|GoldSpawn|GetShouldSpawnGold) 100 90)))
  (if (<= (LocalVariables|GetRareteTiree) 40)
    (return 0)
    (elif (and (<= (LocalVariables|GetRareteTiree) 65) (>= (LocalVariables|GetRareteTiree) 40))
      (return 1)
      (elif (and (<= (LocalVariables|GetRareteTiree) 75) (>= (LocalVariables|GetRareteTiree) 65))
        (return 2)
        (elif (and (<= (LocalVariables|GetRareteTiree) 90) (>= (LocalVariables|GetRareteTiree) 75))
          (return 3)
          (else
            (return 4)))))))

(fn FeathersSetup
  (Variables|Variables|SetNbrFeather (Setup|FeatherRarityCalculator))
  (if (== (Variables|Variables|GetNbrFeather) 4)
    (Development|SetHiddeninGame (Variables|Components|GetGoldenPlumeCut) false false)
    (Development|SetHiddeninGame (Variables|Components|GetGoldenPlumeFull) true false)
    (Development|SetHiddeninGame (Variables|Components|GetFeatherPlane) true false)
    (else
      (Development|SetHiddeninGame (Variables|Components|GetGoldenPlumeFull) true false)
      (Development|SetHiddeninGame (Variables|Components|GetFeatherPlane) false false)
      (Rendering|Material|SetMaterial (Variables|Components|GetFeatherPlane) 0 (Utilities|Struct|BreakStruct_Plumes (Utilities|Array|Get(acopy) (Variables|References|GetStructPlumes) (Variables|Variables|GetNbrFeather))))))
  (return))

(fn SelectFeathers
  (Default|ShoworHideArrow (Variables|References|GetDirectionActor) false)
  (return))

(fn UnselectFeathers
  (Default|ShoworHideArrow (Variables|References|GetDirectionActor) true)
  (return))

(fn DetachfromOwners
  (Transformation|DetachFromActor "KeepWorld" "KeepWorld" "KeepWorld")
  (if (== (Variables|Variables|GetNbrFeather) 4)
    (Development|SetHiddeninGame (Variables|Components|GetGoldenPlumeCut) true false)
    (Development|SetHiddeninGame (Variables|Components|GetGoldenPlumeFull) false false)
    (else
      (Rendering|Material|SetMaterial (Variables|Components|GetFeatherPlane) 0 (Utilities|Struct|BreakStruct_Plumes (Utilities|Array|Get(acopy) (Variables|References|GetStructPlumes) (Variables|Variables|GetNbrFeather)))))))

(fn HideDirections
  ;[1 1 1] Hide the direction when called
  (Development|SetHiddeninGame (Variables|Components|GetPullDirection) true false)
  (Default|ShoworHideArrow (Variables|References|GetDirectionActor) true)
  (return))

(fn ReleaseFeathers
  ;[1 1 1] Release the feather when called
  (Physics|SetSimulatePhysics (Variables|Components|GetFeatherPlane) true)
  (Default|ShoworHideArrow (Variables|References|GetDirectionActor) true)
  (return))

(fn RespawnFeathers
  (bind _returnvalue (Transformation|GetActorLocation))
  (bind _directionactor (Variables|References|GetDirectionActor))
  (bind _uraownerref (Variables|References|GetUraOwnerRef))
  (bind _spottaken (Variables|Variables|GetSpotTaken))
  (bind _uraownerref_2 (Variables|References|GetUraOwnerRef))
  (bind _sk_zazou (Variables|/Game/01-UraLeVoleur/Blueprints/BP_Ura.BP_Ura_C|GetSK_Zazou _uraownerref_2))
  (bind _socketplumes (Variables|/Game/01-UraLeVoleur/Blueprints/BP_Ura.BP_Ura_C|GetSocketPlumes _uraownerref))
  (bind _initialdirection (Variables|/Game/01-UraLeVoleur/Blueprints/BP_Direction.BP_Direction_C|GetInitialDirection _directionactor))
  (bind _returnvalue_2 (Transformation|GetWorldLocation _initialdirection))
  (bind _output (Utilities|Array|Get(acopy) _socketplumes _spottaken))
  (bind _returnvalue_3 (Math|Rotator|FindLookatRotation _returnvalue _returnvalue_2))
  (bind _returnvalue_4 (Transformation|GetSocketTransform _sk_zazou _output "RTS_World"))
  (Default|RandomRotwhenRespawn (Variables|References|GetDirectionActor))
  (Transformation|SetRelativeLocation (Variables|Components|GetFeatherPlane) (.location _returnvalue_4) false false)
  (Transformation|SetActorLocation (.location _returnvalue_4) false false)
  (Transformation|AttachComponentToComponent (Variables|Components|GetFeatherPlane) (Variables|Components|GetScene) "None" "KeepWorld" "KeepWorld" "KeepWorld" true)
  (Transformation|AttachComponentToComponent (Variables|Components|GetScene) (Variables|/Game/01-UraLeVoleur/Blueprints/BP_Ura.BP_Ura_C|GetSK_Zazou (Variables|References|GetUraOwnerRef)) (Utilities|Array|Get(acopy) (Variables|/Game/01-UraLeVoleur/Blueprints/BP_Ura.BP_Ura_C|GetSocketPlumes (Variables|References|GetUraOwnerRef)) (Variables|Variables|GetSpotTaken)) "KeepWorld" "KeepWorld" "KeepWorld" true)
  ;[1 1 1] Reset the feather to it's original rotation
  (Transformation|SetActorRotation (Math|Rotator|MakeRotator 0.0 (.pitch _returnvalue_3) (.yaw _returnvalue_3)))
  (return))