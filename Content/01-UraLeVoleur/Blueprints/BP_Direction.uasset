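; BP_Direction is a direction indicator with an arrow that can be shown or hidden and a randomly pitched Sphere component.
; GiveRandomRotation sets the Sphere's relative pitch within a small range around zero, while RandomRotWhenRespawn, not called here, randomizes it around the current pitch.
; The Show/HideArrow event forwards to ShowOrHideArrow, which toggles the Plane's hidden-in-game state without affecting its children.
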(event Custom|GiveRandomRotation
  (Transformation|SetRelativeRotation (Variables|Default|GetSphere) (Math|Rotator|MakeRotator 0.0 (Math|Random|RandomFloatinRange -15.0 15.0) 0.0) false false))

(event Custom|Show/Hide%20Arrow
  (params (Should%20Hide :type Boolean))
  (CallFunction|ShoworHideArrow Should%20Hide))

(fn ConstructionScript)

(fn RandomRotwhenRespawn
  (bind _sphere (Variables|Default|GetSphere))
  (bind _returnvalue (Transformation|GetRelativeTransform _sphere))
  (Transformation|SetRelativeRotation (Variables|Default|GetSphere) (Math|Rotator|MakeRotator 0.0 (Math|Random|RandomFloatinRange (- (.pitch (.rotation _returnvalue)) 15.0) (+ (.pitch (.rotation _returnvalue)) 15.0)) 0.0) false false)
  (return))

(fn ShoworHideArrow
  (params (ShouldHide :type Boolean))
  (Development|SetHiddeninGame (Variables|Default|GetPlane) ShouldHide false)
  (return))