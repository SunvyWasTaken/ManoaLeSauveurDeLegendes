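; BP_Sky is a sky actor for UraLeVoleur whose disc turns at a pace tied to the game timer.
; On BeginPlay it reads Timer from GM_Ura and sets a single-axis rate on its RotatingMovement component.
; RotationByTime derives that rate by dividing a defined rotation amount by the timer, so the component handles the motion without Tick logic.
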(event EventBeginPlay
  (bind _asgm_ura (Utilities|Casting|CastToGM_Ura (Game|GetGameMode)))
  (Variables|Default|SetTimer (Variables|/Game/01-UraLeVoleur/Blueprints/GM_Ura.GM_Ura_C|GetTimer _asgm_ura))
  (Variables|/Script/Engine.RotatingMovementComponent|SetRotationRate (Variables|Default|GetRotatingMovement) (Math|Rotator|MakeRotator (CallFunction|RotationbyTime) 0.0 0.0)))

(fn ConstructionScript)

(fn RotationbyTime
  (return (/ (Variables|Default|GetRotaionAmouht) (Math|Conversions|ToFloat(Integer) (Variables|Default|GetTimer)))))