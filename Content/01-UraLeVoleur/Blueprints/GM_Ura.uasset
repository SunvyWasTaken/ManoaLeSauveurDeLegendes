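; Game mode for the Ura le voleur game, running the countdown, score, pain meter, HUD and audio fades.
; TriggerGame starts looping timers for countdown and pain decay, then spawns onboarding through PC_Ura.
; Added pain past a threshold destroys feathers, plays the defeat sequence, docks score and shows the losing end screen; timeout shows the normal one.
; AddToScore clamps the score, updates the HUD and spawns per-value particles.
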(event Custom|Countdown
  (bind _returnvalue (Game|GetPlayerController 0))
  ;[1 1 1] Basic timer. Update the Timer widget at every tick
  (bind _output_get (Variables|Default|SetTimer (- (Variables|Default|GetTimer) 1)))
  (Default|UpdateWidgetHorloge (Variables|Default|GetHUDRef) _output_get)
  ;[1 1 1] If the timer is out, clear the timer and disable controller input while showing the EndGameHud
  (if (== (Variables|Default|GetTimer) 0)
    (Utilities|Time|ClearandInvalidateTimerbyHandle (Variables|Default|GetHandleTimer))
    (bind _returnvalue_2 (UserInterface|CreateWidget "/Game/MetaGame/Widgets/WBP_TimesUp.WBP_TimesUp_C" (Game|GetPlayerController 0) "GAME" (Variables|Score|GetScore) (Variables|Score|Get1star) (Variables|Score|Get2star) (Variables|Score|Get3star)))
    (UserInterface|Viewport|AddtoViewport _returnvalue_2 0)
    (Input|DisableInput _returnvalue _returnvalue)))

(event Custom|AddToScore
  (params (PointsGained :type Integer))
  ;[1 1 1] Add the points gained to the score and update the score widget
  (bind _output_get (Variables|Score|SetScore (Math|Integer|Clamp(Integer) (+ PointsGained (Variables|Score|GetScore)) 0 118218)))
  (Default|UpdateWidgetScore (Variables|Default|GetHUDRef) _output_get)
  ;[1 1 1] The unwanted child (spawn fx according to the score)
  (switch int PointsGained
    (:-5
      (Effects|SpawnEmitteratLocation "/Game/01-UraLeVoleur/ParticleSystems/PS_Score-5.PS_Score-5" (Variables|Default|GetScoreSpawnLocation)))
    (:1
      (Effects|SpawnEmitteratLocation "/Game/01-UraLeVoleur/ParticleSystems/PS_Score+1.PS_Score+1" (Variables|Default|GetScoreSpawnLocation)))
    (:3
      (Effects|SpawnEmitteratLocation "/Game/01-UraLeVoleur/ParticleSystems/PS_Score+3.PS_Score+3" (Variables|Default|GetScoreSpawnLocation)))
    (:5
      (Effects|SpawnEmitteratLocation "/Game/01-UraLeVoleur/ParticleSystems/PS_Score+5.PS_Score+5" (Variables|Default|GetScoreSpawnLocation)))
    (:10
      (Effects|SpawnEmitteratLocation "/Game/01-UraLeVoleur/ParticleSystems/PS_Score+10.PS_Score+10" (Variables|Default|GetScoreSpawnLocation)))))

(event Custom|TriggerGame
  ;[1 1 1] Starts the timer when called and tell everyone that the game is started
  (Variables|Default|SetbGameStarted true)
  (bind _returnvalue (Utilities|Time|SetTimerbyEvent (delegate Custom|Countdown) 1.0 true)) ; Décompte du minuteur
  (Variables|Default|SetHandleTimer _returnvalue)
  (CallFunction|TriggerDecrease)
  ;[1 1 1] SpawnTheOnboarding
  (bind _aspc_ura (Utilities|Casting|CastToPC_Ura (Game|GetPlayerController 0)))
  (Default|SpawnPlayableOnboarding _aspc_ura))

(event Custom|DouleurActuelle
  (params (Douleur :type Float%20%28single-precision%29))
  (bind _returnvalue (Game|GetPlayerController 0))
  ;[1 1 1] Calculate the actual level of pain when called. When the level of pain gets over a certain threshold, it will trigger the end game animation
  (bind _output_get (Variables|Default|SetDouleur (+ Douleur (Variables|Default|GetDouleur))))
  (if (>= _output_get 1e+02)
    (bind _outactors (Actor|GetAllActorsOfClass "/Game/01-UraLeVoleur/Blueprints/BP_Plume.BP_Plume_C"))
    (for _array_element _outactors
      (Actor|DestroyActor _array_element))
    (Audio|PlaySound2D "/Game/MetaGame/Sounds/S_defaite.S_defaite" 1.0 1.0 0.0 0 0)
    (Utilities|FlowControl|Delay 1.0)
    ;[1 1 1] Disable the player inputs, remove all the widgets and play the defeat animation before spawning the Final Score hud
    (Input|DisableInput _returnvalue _returnvalue)
    (Viewport|RemoveAllWidgets)
    (Sequencer|Player|CreateLevelSequencePlayer "/Game/01-UraLeVoleur/Sequences/seq_defaite_ura.seq_defaite_ura" (Utilities|Struct|MakeMovieSceneSequencePlaybackSettings true "(Value=0)" 1.0 0.0 false false false false false false false true))
    (Utilities|Time|ClearandInvalidateTimerbyHandle (Variables|Default|GetHandleTimer))
    (Variables|Score|SetScore (- (Variables|Score|GetScore) 20))
    (CallFunction|FadeOutAllSound)
    (Utilities|FlowControl|Delay 6.5)
    (bind _returnvalue_2 (UserInterface|CreateWidget "/Game/MetaGame/Widgets/WBP_TimesUp.WBP_TimesUp_C" (Game|GetPlayerController 0) "PERDU" (Math|Integer|Clamp(Integer) (Variables|Score|GetScore) 0 118218) (Variables|Score|Get1star) (Variables|Score|Get2star) (Variables|Score|Get3star)))
    (Variables|Default|SetbPerdu true)
    (UserInterface|Viewport|AddtoViewport _returnvalue_2 0)))

(event Custom|DecreaseDouleur
  ;[1 1 1] Decrease the amount of pain over time
  (if (<= 0.0 (Variables|Default|GetDouleur))
    (Variables|Default|SetDouleur (- (Variables|Default|GetDouleur) 0.08))))

(event Custom|TriggerDecrease
  ;[1 1 1] Decrease the amount of pain over time
  (Utilities|Time|SetTimerbyEvent (delegate Custom|DecreaseDouleur) 0.01 true) ; Décompte du minuteur pour Douleur
)

(event Custom|CreateHud
  ;[1 1 1] Create the default HUD when called and add it to the viewport
  (bind _returnvalue (UserInterface|CreateWidget "/Game/01-UraLeVoleur/Widgets/WPB_HudIngame.WPB_HudIngame_C"))
  (bind _output_get (Variables|Default|SetHUDRef _returnvalue))
  (UserInterface|Viewport|AddtoViewport _output_get 0))

(event Custom|TriggerAmbiance
  ;[1 1 1] Change the ambience when called from widget blueprint HUD
  (Utilities|FlowControl|Delay 0.5)
  (Audio|Components|Audio|FadeIn (Variables|Default|Getsleeping) 1.1 0.3 0.0 "Linear" :!class /Script/Engine.AudioComponent)
  (Audio|Components|Audio|FadeIn (Variables|Default|Getambiance) 1.1 0.3 0.0 "Linear" :!class /Script/Engine.AudioComponent)
  (Utilities|FlowControl|Delay 1.0)
  (Audio|Components|Audio|Play (Variables|Default|Getmusic) 0.0))

(event Custom|FadeOutAllSound
  ;[1 1 1] Fade out all the ingame sound and play the defeat sound
  (Audio|Components|Audio|FadeOut (Variables|Default|Getsleeping) 1.0 0.0 "Linear" :!class /Script/Engine.AudioComponent)
  (Audio|Components|Audio|FadeOut (Variables|Default|Getambiance) 1.0 0.0 "Linear" :!class /Script/Engine.AudioComponent)
  (Audio|Components|Audio|FadeOut (Variables|Default|Getmusic) 0.9 0.0 "Linear" :!class /Script/Engine.AudioComponent))

(fn ConstructionScript)