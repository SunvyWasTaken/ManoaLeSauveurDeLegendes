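; Player controller for a touch-based feather-plucking game, active once GM_Ura reports the game started.
; A touch trace grabs a BP_Plume, which rotates toward the finger until pulled past a distance limit, then detaches and follows it until released.
; Pull direction is checked against the feather's arrow: wrong pulls double the pain sent to GM_Ura and trigger hurt animation, with distinct sound and haptics.
; It also spawns the playable onboarding widget, removed upon releasing a feather.
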(event Custom|SpawnPlayableOnboarding
  ;[1 1 1] Spawn the playable onboarding when called
  (bind _returnvalue (UserInterface|CreateWidget "/Game/01-UraLeVoleur/Widgets/WBP_OnBoardingJouable.WBP_OnBoardingJouable_C" self))
  (Variables|Default|SetOnboardingRef _returnvalue)
  (UserInterface|Viewport|AddtoViewport _returnvalue 0))

(event EventBeginPlay
  ;[1 1 1] Get the game mode ref from the beginning
  (bind _asgm_ura (Utilities|Casting|CastToGM_Ura (Game|GetGameMode)))
  (Variables|Default|SetGamemodeRef _asgm_ura))

(event Input|TouchEvents|InputTouch
  (params (Location :type Vector) (FingerIndex :type ETouchIndex%20Enum))
  (bind _worldposition (CallFunction|ScreenTouchPosition))
  (bind _onboardingref (Variables|Default|GetOnboardingRef))
  (:Pressed
    ;[1 1 1] Linetrace to check if a feather is under the User's finger
    (Utilities|CheckGameStarted
      (:True
        (bind (_outhit _returnvalue) (Collision|LineTraceByChannel (CallFunction|ScreenTouchPosition) (Math|Vector|MakeVector (+ (.x _worldposition) 1.5e+03) (.y _worldposition) (.z _worldposition)) "TraceTypeQuery1" false 0 "Persistent"))
        (if _returnvalue
          (bind _asbp_plume (Utilities|Casting|CastToBP_Plume (.HitActor (Collision|BreakHitResult _outhit))))
          (Variables|Default|SetPlumeRef _asbp_plume) ; Store the reference of the feather if it's the feather
          ;[1 1 1] Track the feather's location in Vector Variables
          (bind _output_get (Variables|Default|SetDirectionActorArrow (Variables|/Game/01-UraLeVoleur/Blueprints/BP_Direction.BP_Direction_C|GetArrow (Variables|/Game/01-UraLeVoleur/Blueprints/BP_Plume.BP_Plume_C|GetDirectionActor (Variables|Default|GetPlumeRef)))))
          (Variables|Default|SetbIsGrab? true)
          (Variables|Default|SetPlumePosition (Transformation|GetActorLocation (Variables|Default|GetPlumeRef)))
          (Variables|Default|SetPlumeArrowPosition (Transformation|GetWorldLocation _output_get))
          (Default|SelectFeathers (Variables|Default|GetPlumeRef))))))
  (:Released
    ;[1 1 1] Set the feather when it's released
    (Utilities|CheckGameStarted
      (:True
        (Utilities|IsValid (Variables|Default|GetPlumeRef)
          (:Is%20Valid
            (Default|UnselectFeathers (Variables|Default|GetPlumeRef))
            (if (Variables|Default|GetbIsAttached?)
              _
              (else
                (Default|ReleaseFeathers (Variables|Default|GetPlumeRef))))
            (Variables|Default|SetPlumeRef 0)
            (Variables|Default|SetbIsGrab? false)
            (Variables|Default|SetbIsAttached? true)
            (Variables|Default|SetbIsActuallyPulled? false)
            (Utilities|IsValid _onboardingref
              (:Is%20Valid
                (Widget|RemovefromParent _onboardingref))))))))
  (:Moved
    ;[1 1 1] Update the feather's position when user's finger is moving
    (Utilities|CheckGameStarted
      (:True
        (|OnMoved)))))

(fn ConstructionScript)

(fn ScreenTouchPosition
  (bind (_locationx _locationy) (Class|PlayerController|GetInputTouchState "Touch1"))
  (return (.WorldPosition (Class|GameplayStatics|DeprojectScreentoWorld self (Math|Vector2D|MakeVector2D _locationx _locationy)))))

(fn FeatherLimit
  (bind _worldposition (CallFunction|ScreenTouchPosition))
  (bind _plumeposition (Variables|Default|GetPlumePosition))
  (return (>= (Math|Vector|VectorLength (- (Math|Vector|MakeVector (.x _worldposition) (.y _plumeposition) (.z _plumeposition)) (Math|Vector|MakeVector (.x _worldposition) (.y _worldposition) (.z _worldposition)))) 1e+02)))

(fn RotateFeathertoFinger
  (bind _worldposition (CallFunction|ScreenTouchPosition))
  (bind _plumeposition (Variables|Default|GetPlumePosition))
  (bind _returnvalue (Math|Vector|MakeVector (.x _plumeposition) (.y _plumeposition) (.z _plumeposition)))
  (bind _returnvalue_2 (Math|Vector|MakeVector (.x _plumeposition) (.y _worldposition) (.z _worldposition)))
  (bind _returnvalue_3 (Math|Rotator|FindLookatRotation _returnvalue _returnvalue_2))
  (Transformation|SetActorRotation (Variables|Default|GetPlumeRef) (Math|Rotator|MakeRotator 0.0 (.pitch _returnvalue_3) (.yaw _returnvalue_3))))