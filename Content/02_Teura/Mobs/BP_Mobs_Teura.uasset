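; Enemy mob of the Teura minigame: a spawner sends it walking down the screen, showing signs for which bee can attack it.
; F_StartWalking configures it and starts a looping timer that moves it, triggering the game mode's end animation and camera shake at the bottom.
; Each hit scores a point; a duo's first hit clears one sign and stuns it temporarily, otherwise the actor is parked off-play for reuse rather than destroyed.
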(event Custom|PlayerLoose
  ;[1 1 1] Arrive en bas de l'ecran, déclenché dans la fonction WalkTimer
  (bind _asgm_teura (Utilities|Casting|CastToGM_Teura (Game|GetGameMode)))
  (Default|PlayAnimeEnd _asgm_teura)
  (Camera|PlayWorldCameraShake "/Game/02_Teura/Level/Camera/CS_KillEnnemi_Teura.CS_KillEnnemi_Teura_C" (Transformation|GetActorLocation) 0.0 5e+06))

(event Custom|MobHit
  (params (Sign2Hit :type Boolean))
  ;[1 1 1] Hit et Stun
  (bind _asgm_teura (Utilities|Casting|CastToGM_Teura (Game|GetGameMode)))
  (Default|FAddScore _asgm_teura 1)
  (if (Variables|State|GetbIsDuo)
    (if Sign2Hit
      (Sprite|SetFlipbook (Variables|Default|GetPaperFlipbook) "/Game/02_Teura/Mobs/Art/Mob1/Stun/PFB_Mob1StunPlusFx.PFB_Mob1StunPlusFx")
      (CallFunction|MobStunned Sign2Hit)
      (Variables|References|SetSign2 4)
      (else
        (Sprite|SetFlipbook (Variables|Default|GetPaperFlipbook) "/Game/02_Teura/Mobs/Art/Mob2/Stun/PFB_Mob2StubPlusFx.PFB_Mob2StubPlusFx")
        (CallFunction|MobStunned false)
        (Variables|References|SetSign1 4)))
    (Variables|State|SetbIsDuo false)
    (References|FSetSignRender)
    (else
      (CallFunction|Reinitialize))))

(event Custom|Reinitialize
  ;[1 1 1] Reinitialiser apres defaite
  (Variables|References|SetSign1 4)
  (Variables|References|SetSign2 4)
  (References|FSetSignRender)
  (Variables|State|SetbIsAttacking false)
  (Utilities|Time|ClearTimerbyFunctionName 0 "F_WalkTimer")
  (Utilities|FlowControl|Delay 0.1)
  (Transformation|SetActorLocation "0,-800.000000,50.000000" false false))

(event Custom|MobStunned
  (params (Sign2Hit :type Boolean))
  ;[1 1 1] Hit et Stun
  (Audio|PlaySound2D "/Game/02_Teura/Mobs/SFX/S_Stun_Teura.S_Stun_Teura" 1.0 1.0 0.0 0 0)
  (Variables|State|SetbIsStunned true)
  (Utilities|Time|ClearTimerbyFunctionName 0 "F_WalkTimer")
  (Utilities|FlowControl|Delay (Variables|State|GetStunDelay))
  (if Sign2Hit
    (Sprite|SetFlipbook (Variables|Default|GetPaperFlipbook) "/Game/02_Teura/Mobs/Art/Mob1/Walk/PFB_Mobs1walking.PFB_Mobs1walking")
    (else
      (Sprite|SetFlipbook (Variables|Default|GetPaperFlipbook) "/Game/02_Teura/Mobs/Art/Mob2/Walk/PFB_Mobs2_Walking.PFB_Mobs2_Walking")))
  (if (Variables|State|GetbIsAttacking)
    (Utilities|Time|SetTimerbyFunctionName 0 "F_WalkTimer" 0.05 true)
    (Variables|State|SetbIsStunned false)))

(fn ConstructionScript)

(fn FWalkTimer
  ;[1 1 1] Timer du defilement de l'ennemi, s'active qd il est envoyé
  (if (>= (.y (Transformation|GetActorLocation)) 500.453766)
    (Utilities|Time|ClearTimerbyFunctionName 0 "F_WalkTimer")
    (CallFunction|PlayerLoose)
    (else
      (Transformation|AddActorWorldOffset (Math|Vector|MakeVector 0.0 (/ (Variables|Movements|GetWalkingSpeed) -1.0) 0.0))))
  (return))

(fn FSetSignRender
  ;[1 1 1] Defini le signe de l'abeille qui peut l'attaquer
  (Rendering|Components|Sprite|SetSprite (Variables|Default|GetPaperSprite) (Utilities|Array|Get(acopy) (Variables|References|GetArraySign) (Variables|References|GetSign1)))
  (Rendering|Components|Sprite|SetSprite (Variables|Default|GetPaperSprite1) (Utilities|Array|Get(acopy) (Variables|References|GetArraySign) (Variables|References|GetSign2)))
  (return))

(fn FStartWalking
  (params (NewLocation :type Vector) (NewFlipbook :type Paper%20Flipbook%20Object%20Reference) (Sign1 :type Integer) (Sign2 :type Integer) (bIsDuo :type Boolean) (WalkingSpeed :type Float%20%28single-precision%29) (EnnemyType :type Integer))
  ;[1 1 1] Est Declenché par le spawner qui a défini sa position, son type et son/ses signes
  (Transformation|SetActorLocation NewLocation false false)
  (Sprite|SetFlipbook (Variables|Default|GetPaperFlipbook) NewFlipbook)
  (Variables|Movements|SetWalkingSpeed WalkingSpeed)
  (Utilities|Time|SetTimerbyFunctionName 0 "F_WalkTimer" 0.05 true)
  (Variables|State|SetbIsAttacking true)
  (Variables|References|SetSign1 Sign1)
  (Variables|References|SetSign2 Sign2)
  (Variables|State|SetbIsDuo bIsDuo)
  (Variables|References|SetEnnemyType EnnemyType)
  (References|FSetSignRender)
  (return))