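; Enemy spawner for the Teura game that pre-spawns a pool of BP_Mobs_Teura on BeginPlay and hands it to GM_Teura.
; A looping timer, resettable with new delay and speed, cycles through the pool and launches each mob from a random X position.
; Each launch randomizes type, flipbook and signs, with the rarer duo type getting two different signs.
; FSpawnerEndGame stops the spawn timer and clears mob walk timers.
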(event Custom|SpawnEnnemy
  (bind _mobtogo (Variables|Initialization|GetMobToGo))
  (bind _mobarray (Variables|Ref|GetMobArray))
  (bind _output (Utilities|Array|Get(acopy) _mobarray _mobtogo))
  ;[1 1 1] Loop Qui spawn les ennemis
  (Utilities|SetEnnemytoGo
    (:End
      (Utilities|SetPosition
        (:End
          (Utilities|SetEnnemyType
            (:End
              (Variables|/Game/02_Teura/Mobs/BP_Mobs_Teura.BP_Mobs_Teura_C|SetbIsAttacking _output false)
              ;;[1 1 1] Declenche l'event du BP_Ennemy
              (Default|FStartWalking _output (Variables|Initialization|GetInitialLocation) (Variables|Initialization|GetMobFlipbook) (Variables|Initialization|GetSign1) (Variables|Initialization|GetSign2) (Variables|Initialization|GetbIsDuo) (Variables|Initialization|GetEnnemySpeed) (Variables|Initialization|GetMobType)))))))))

(event Custom|SetSpawnAndDifficulty
  (params (SpawnDelay :type Float%20%28single-precision%29) (EnnemySpeed :type Float%20%28single-precision%29))
  ;[1 1 1] Set les spawn et regle la difficulté si besoin
  (Utilities|Time|ClearandInvalidateTimerbyHandle (Variables|Timer|GetTimerHandle))
  (Variables|Timer|SetSpawnDelay SpawnDelay)
  (Variables|Initialization|SetEnnemySpeed EnnemySpeed)
  (bind _returnvalue (Utilities|Time|SetTimerbyEvent (delegate Custom|SpawnEnnemy) (Variables|Timer|GetSpawnDelay) true))
  (Variables|Timer|SetTimerHandle _returnvalue))

(event EventBeginPlay
  (bind _mobarray (Variables|Ref|GetMobArray))
  ;[1 1 1] BeginPlay
  ;;[1 1 1] Spawn les ennemis
  (for _index (range 0 (Variables|Ref|GetNumberOfMobs))
    (bind _returnvalue (Game|SpawnActorfromClass "/Game/02_Teura/Mobs/BP_Mobs_Teura.BP_Mobs_Teura_C" (Math|Transform|MakeTransform "0,0.000000,1600.000000" "0, 0, 0" "0.400000,0.400000,0.400000") "Undefined" 0 0))
    (Utilities|Array|Add _mobarray _returnvalue)
    (Variables|Ref|SetFirstEnnemi (Utilities|Array|Get(acopy) _mobarray)))
  (Variables|Initialization|SetMobToGo 0)
  (CallFunction|SetSpawnandDifficulty (Variables|Timer|GetSpawnDelay) (Variables|Initialization|GetEnnemySpeed))
  (Default|FArraytoBees (.AsGM%20Teura (Utilities|Casting|CastToGM_Teura (Game|GetGameMode))) (Variables|Ref|GetMobArray)))

(fn ConstructionScript)

(fn FSpawnerEndGame
  (Utilities|Time|ClearandInvalidateTimerbyHandle (Variables|Timer|GetTimerHandle))
  (for _array_element (Variables|Ref|GetMobArray)
    (Utilities|Time|ClearTimerbyFunctionName _array_element "F_WalkTimer")
    (return)))