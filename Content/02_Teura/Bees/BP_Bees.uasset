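; BP_Bees is a numbered bee in the Teura minigame that attacks enemies carrying its matching sign.
; Attaque loops through MobsArray, pausing on a Found flag while timer-driven Fly homes in on each attacking match.
; Impacts trigger effects, sounds, camera shake, brief slow motion, a death pop-up by enemy type and MobHit.
; The bee then returns to its start location, or heads toward InitialLocation when nothing matches.
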(event Custom|Attaque
  (params (Numero :type Integer))
  ;[1 1 1] Loop special
  (if (Math|Boolean|ANDBoolean (== Numero (Variables|Referencement|GetNumberBee)) (not (Variables|State|GetbIsAttacking)) (not (Variables|State|GetbIsDead)))
    (Default|SigneJ (Variables|/Game/02_Teura/Gamemode/GM_Teura.GM_Teura_C|GetHud_InGame (Variables|Gamemode|GetTeuraGamemode)) Numero)
    (CallFunction|PlaySoundAtk)
    (Variables|Movements|SetSpeed 5e+01)
    (Variables|Mobs|SetCurrentIndex 0) ; A chaque début reset l'index
    (Variables|State|SetbHasAttacked false)
    (Utilities|FlowControl|Delay 0.4)
    (if (< (Variables|Mobs|GetCurrentIndex) (Utilities|Array|Length (Variables|Mobs|GetMobsArray))) :!label _label ; Continue tant que l'index n'est pas supérieur à la longueur de l'array
      (Utilities|FlowControl|Sequence
        (:then_0
          (bind _output_get (Variables|Mobs|SetTargetedMob (Utilities|Array|Get(acopy) (Variables|Mobs|GetMobsArray) (Variables|Mobs|GetCurrentIndex))))
          ;[1 1 1] Check si l'ennemie ne porte pas le symbole et si il attaque
          (if (and (== (Variables|/Game/02_Teura/Mobs/BP_Mobs_Teura.BP_Mobs_Teura_C|GetSign1 _output_get) (Variables|Referencement|GetNumberBee)) (Variables|/Game/02_Teura/Mobs/BP_Mobs_Teura.BP_Mobs_Teura_C|GetbIsAttacking _output_get))
            (Variables|State|SetbIsAttackingSecondMob false)
            ;[1 1 1] Si un ennemi est possède le symbole et qu'il attaque met en pause la loop. Puis lance le déplacement de l'abeille et cette ça rotation
            (Variables|State|SetbFound true :!label _label_2)
            (bind _returnvalue (Utilities|Time|SetTimerbyEvent (delegate Custom|Fly) 0.01 true))
            (Variables|Movements|SetHandlerFly _returnvalue)
            (Variables|State|SetbIsAttacking true)
            (Transformation|SetActorRotation (Math|Rotator|FindLookatRotation (Transformation|GetActorLocation self) (Transformation|GetActorLocation (Variables|Mobs|GetTargetedMob))))
            (Variables|State|SetbHasAttacked true)
            (elif (and (== (Variables|/Game/02_Teura/Mobs/BP_Mobs_Teura.BP_Mobs_Teura_C|GetSign2 _output_get) (Variables|Referencement|GetNumberBee)) (Variables|/Game/02_Teura/Mobs/BP_Mobs_Teura.BP_Mobs_Teura_C|GetbIsAttacking _output_get))
              (Variables|State|SetbIsAttackingSecondMob true)
              (goto _label_2))))
        (:then_1
          (Math|Integer|IncrementInt (Variables|Mobs|GetCurrentIndex) ; Increas l'index
            (:%20%20
              (if (Variables|State|GetbFound) :!label _label_3 ; Tant qu'un ennemie est found il attaque met en pause la loop
                (Utilities|FlowControl|Delay (Utilities|Time|GetWorldDeltaSeconds))
                (goto _label_3)
                (else
                  (goto _label)))))))
      (else
        (CallFunction|EndCheckAllEnnemi)))))

(event Custom|Fly
  (bind _returnvalue (Transformation|GetActorLocation))
  (bind _returnvalue_2 (Transformation|GetActorLocation))
  (bind _self self)
  (bind _targetedmob (Variables|Mobs|GetTargetedMob))
  (bind _targetedmob_2 (Variables|Mobs|GetTargetedMob))
  (bind _returnvalue_3 (Transformation|GetActorLocation _targetedmob))
  (bind _returnvalue_4 (Transformation|GetActorLocation _self))
  (bind _ennemytype (Variables|/Game/02_Teura/Mobs/BP_Mobs_Teura.BP_Mobs_Teura_C|GetEnnemyType _targetedmob_2))
  ;[1 1 1] L'abeille se déplace jusqu'à l'ennemi et active la fonction toucher
  (Transformation|AddActorWorldOffset self (* (Class|KismetMathLibrary|VectorNormalUnsafe (- _returnvalue_3 _returnvalue_4)) (Variables|Movements|GetSpeed)))
  (if (Math|Vector|Equal(Vector) _returnvalue_3 _returnvalue_4 5e+01)
    (Variables|State|SetbFound false)
    (Utilities|Time|ClearandInvalidateTimerbyHandle (Variables|Movements|GetHandlerFly))
    (Effects|SpawnEmitteratLocation "/Game/02_Teura/FX/VFX/PS_BeesHit_Teura.PS_BeesHit_Teura" _returnvalue)
    (CallFunction|SlowMo 0.01 0.1)
    (Camera|PlayWorldCameraShake "/Game/02_Teura/Level/Camera/CS_KillEnnemi_Teura.CS_KillEnnemi_Teura_C" _returnvalue 0.0 1e+03 0.25)
    (Audio|PlaySound2D "/Game/02_Teura/Bees/SFX/SC_BeeHit1_Teura.SC_BeeHit1_Teura" 1.0 1.0 0.0 0 0)
    (Audio|PlaySound2D "/Game/02_Teura/Mobs/SFX/SC_DeathMob_Teura__1__Cue.SC_DeathMob_Teura__1__Cue" 1.0 1.0 0.0 0 0)
    (if (== _ennemytype 0)
      (Game|SpawnActorfromClass "/Game/02_Teura/Mobs/BP_PopUpDeathFat_Teura.BP_PopUpDeathFat_Teura_C" (Math|Transform|MakeTransform _returnvalue_2 "0, 0, 0" "1,1,1") "Undefined" 0 0 :!label _label)
      (Default|MobHit _targetedmob_2 (Variables|State|GetbIsAttackingSecondMob) :!label _label_2)
      (elif (== _ennemytype 1)
        (Game|SpawnActorfromClass "/Game/02_Teura/Mobs/BP_PopUpDeathSmall_Teura.BP_PopUpDeathSmall_Teura_C" (Math|Transform|MakeTransform _returnvalue_2 "0, 0, 0" "1,1,1") "Undefined" 0 0 :!label _label_3)
        (goto _label_2)
        (elif (== _ennemytype 2)
          (if (Variables|State|GetbIsAttackingSecondMob)
            (goto _label_3)
            (else
              (goto _label))))))))

(event Custom|SlowMo
  (params (Duration :type Float%20%28single-precision%29) (TimeDilation :type Float%20%28single-precision%29))
  ;[1 1 1] SlowMotion
  (Utilities|Time|SetGlobalTimeDilation TimeDilation)
  (Utilities|FlowControl|Delay Duration)
  (Utilities|Time|SetGlobalTimeDilation 1.0))

(event Custom|EndCheckAllEnnemi
  ;[1 1 1] Check si il a attack un ennemi ou pas
  (if (not (Variables|State|GetbHasAttacked))
    (CallFunction|HItNothing)
    (else
      ;[1 1 1] movement permetant à l'abeille de revenir
      (bind _returnvalue (Utilities|Time|SetTimerbyEvent (delegate Custom|BackToHome) 0.01 true))
      (Transformation|SetActorRotation "0,-90.000000, 0")
      (Variables|Movements|SetHandlerReturn _returnvalue)
      (Variables|Movements|SetSpeed 25.0))))

(event Custom|HItNothing
  ;[1 1 1] lorsque l'abeille n'a rien à hit
  (bind _returnvalue (Utilities|Time|SetTimerbyEvent (delegate Custom|GoToTargetPoint) 0.01 true))
  (Variables|Movements|SetHandlerTargetPoint _returnvalue)
  (Variables|State|SetbIsAttacking true))

(event Custom|GoToTargetPoint
  (bind _self self)
  (bind _initiallocation (Variables|Movements|GetInitialLocation))
  (bind _returnvalue (Transformation|GetActorLocation _self))
  ;[1 1 1] lorsque l'abeille n'a rien à hit
  (Transformation|AddActorWorldOffset self (* (Class|KismetMathLibrary|VectorNormalUnsafe (- _initiallocation _returnvalue)) (Variables|Movements|GetSpeed)))
  (if (Math|Vector|Equal(Vector) _initiallocation _returnvalue 5e+01)
    (Utilities|Time|ClearandInvalidateTimerbyHandle (Variables|Movements|GetHandlerTargetPoint))
    (Variables|State|SetbHasAttacked true)
    (CallFunction|EndCheckAllEnnemi)
    (else
      (CallFunction|EndCheckAllEnnemi))))

(event Custom|BackToHome
  (bind _self self)
  (bind _startlocation (Variables|Movements|GetStartLocation))
  (bind _returnvalue (Transformation|GetActorLocation _self))
  ;[1 1 1] movement permetant à l'abeille de revenir
  (Transformation|AddActorWorldOffset self (/ (* (Class|KismetMathLibrary|VectorNormalUnsafe (- _startlocation _returnvalue)) (Variables|Movements|GetSpeed)) 4.0))
  (if (Math|Vector|Equal(Vector) _startlocation _returnvalue 5.0)
    (Utilities|Time|ClearandInvalidateTimerbyHandle (Variables|Movements|GetHandlerReturn))
    (Variables|State|SetbIsAttacking false)
    (Variables|State|SetbHasAttacked false)))

(event Custom|PlaySoundAtk
  ;[1 1 1] Comment
  (Audio|PlaySound2D "/Game/02_Teura/Bees/SFX/S_BeesFast_Teura.S_BeesFast_Teura" 1.0 (Math|Random|RandomFloatinRange 0.7 1.0) 0.0 0 0)
  (Audio|PlaySound2D "/Game/02_Teura/Bees/SFX/S_BeeIdle1_Teura.S_BeeIdle1_Teura" 1.0 1.0 0.0 0 0))

(event EventBeginPlay
  ;[1 1 1] BeginPlay
  (bind _asgm_teura (Utilities|Casting|CastToGM_Teura (Game|GetGameMode)))
  (Variables|Gamemode|SetTeuraGamemode _asgm_teura)
  (Utilities|FlowControl|Delay 0.1)
  (Rendering|Components|Sprite|SetSprite (Variables|Default|GetT_Signe03_Teura_Sprite) (Utilities|Array|Get(acopy) (Variables|Mobs|GetSigneArraySprite) (Variables|Referencement|GetNumberBee)))
  (Variables|Movements|SetStartLocation (Transformation|GetActorLocation)))

(fn ConstructionScript)