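; Game mode for the Teura minigame, in which signs made by the player send bees to attack spawned enemies.
; BeginPlay starts audio, the enemy spawner and HUD, then shows a delayed onboarding widget in slow motion.
; Four bees spawn at tagged points, share the enemy array and attack by sign index.
; Score thresholds adjust spawn delay and enemy speed; a one-shot ending kills bees, stops spawning and shows victory.
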(event Custom|PlayerMadeSign
  (params (SignMade :type Integer))
  ;[1 1 1] Quand le pc a effectue le signe, declenche l'event de l'abeille qui lui fait check l'Array du spawner
  (Default|Attaque (Utilities|Array|Get(acopy) (Variables|Bees|GetBeesArray) SignMade) SignMade))

(event Custom|PlayAnimeEnd
  ;[1 1 1] EndGameAnimation
  (Utilities|FlowControl|DoOnce false
    (:Completed
      (Audio|PlaySound2D "/Game/02_Teura/Gamemode/SFX/S_EndGame_Blow_Teura.S_EndGame_Blow_Teura" 1.0 1.0 0.0 0 0)
      (Audio|PlaySound2D "/Game/02_Teura/Gamemode/SFX/S_Music_EndGame_Teura.S_Music_EndGame_Teura" 1.0 1.0 0.0 0 0)
      (Audio|PlaySound2D "/Game/02_Teura/Gamemode/SFX/S_EndGame_Teura.S_EndGame_Teura" 1.0 1.0 0.0 0 0)
      (Audio|Components|Audio|Stop (Variables|Default|GetMusiqueTeura))
      (bind _returnvalue (UserInterface|CreateWidget "/Game/02_Teura/UI/EndGame/WBP_EndGame_Teura.WBP_EndGame_Teura_C"))
      (UserInterface|Viewport|AddtoViewport _returnvalue 0)
      (for _array_element (Variables|Bees|GetBeesArray)
        (Variables|/Game/02_Teura/Bees/BP_Bees.BP_Bees_C|SetbIsDead _array_element true))
      (Utilities|FlowControl|Delay 1.0)
      (EndGame|FEndGame)
      (Default|FSpawnerEndGame (Variables|Mobs|GetSpawner)))))

(event Custom|Onboarding
  (params (Delay :type Float%20%28single-precision%29))
  ;[1 1 1] Onboarding
  (Utilities|FlowControl|Delay Delay)
  (Utilities|Time|SetGlobalTimeDilation 0.2)
  (bind _returnvalue (UserInterface|CreateWidget "/Game/02_Teura/UI/Onboarding/WBP_Onboarding_Teura.WBP_Onboarding_Teura_C"))
  (bind _output_get (Variables|UI|SetHud_Onboarding _returnvalue))
  (UserInterface|Viewport|AddtoViewport _output_get 0))

(event EventBeginPlay
  ;[1 1 1] BeginPlay, set les variables de base
  (bind _returnvalue (Audio|SpawnSound2D "/Game/02_Teura/Gamemode/SFX/S_MainMenu_Teura.S_MainMenu_Teura" 1.0 1.0 0.0 0))
  (Variables|Default|SetMusiqueTeura _returnvalue)
  (Audio|PlaySound2D "/Game/02_Teura/Level/Background/Terrain/S_Waves.S_Waves" 1.0 1.0 0.0 0 0)
  (Bees|FGetSpawnPoint)
  (Variables|/Script/Engine.PlayerController|SetbShowMouseCursor (Game|GetPlayerController 0) true)
  (bind _returnvalue_2 (Game|SpawnActorfromClass "/Game/02_Teura/Mobs/BP_SpawnerMobs_Teura.BP_SpawnerMobs_Teura_C" (Math|Transform|MakeTransform "0, 0, 0" "0, 0, 0" "1,1,1") "Undefined" 0 0))
  (Variables|Mobs|SetSpawner _returnvalue_2)
  (bind _returnvalue_3 (UserInterface|CreateWidget "/Game/02_Teura/UI/HUD/WBP_InGame_Teura.WBP_InGame_Teura_C"))
  (bind _output_get (Variables|UI|SetHud_InGame _returnvalue_3))
  (UserInterface|Viewport|AddtoViewport _output_get 0)
  (CallFunction|Onboarding 3.0)
  (Input|SetInputModeGameandUI (Game|GetPlayerController 0) _returnvalue_3 "DoNotLock" false))

(fn ConstructionScript)

(fn FEndGame
  (bind _score (Variables|Scoring&Difficulty|GetScore))
  (bind _returnvalue (UserInterface|CreateWidget "/Game/00_Metajeu/Widgets/WBP_MenuVictoire1.WBP_MenuVictoire1_C" 0 _score 10 20 30 0.05))
  (Development|PrintString (Utilities|String|ToString(Integer) _score) true true "(R=1.000000,G=0.886320,B=0.000000,A=1.000000)")
  (UserInterface|Viewport|AddtoViewport _returnvalue 0)
  (return))

(fn FGetSpawnPoint
  (bind _outactors (Actor|GetAllActorswithTag "Bee"))
  (Variables|Bees|SetBeeSpawnPointArray _outactors)
  (return))

(fn FSetDifficulty
  (params (Palier01 :type Integer) (Palier02 :type Integer) (Palier03 :type Integer) (PalierBonus :type Integer) (TryHarder :type Integer) (TryHarder++ :type Integer))
  (bind _score (Variables|Scoring&Difficulty|GetScore))
  (if (Math|Boolean|ORBoolean (== _score Palier01) (== _score Palier02) (== _score Palier03))
    (Variables|Scoring&Difficulty|SetSpawnDelay (- (Variables|Scoring&Difficulty|GetSpawnDelay) 1.5))
    (Variables|Scoring&Difficulty|SetEnnemySpeed (- (Variables|Scoring&Difficulty|GetEnnemySpeed) 2.5))
    (Default|SetSpawnandDifficulty (Variables|Mobs|GetSpawner) (Variables|Scoring&Difficulty|GetSpawnDelay) (Variables|Scoring&Difficulty|GetEnnemySpeed))
    (return)
    (elif (== _score PalierBonus)
      (Variables|Scoring&Difficulty|SetSpawnDelay 1.5)
      (Variables|Scoring&Difficulty|SetEnnemySpeed (- (Variables|Scoring&Difficulty|GetEnnemySpeed) 1.5))
      (Default|SetSpawnandDifficulty (Variables|Mobs|GetSpawner) (Variables|Scoring&Difficulty|GetSpawnDelay) (Variables|Scoring&Difficulty|GetEnnemySpeed))
      (return)
      (elif (== TryHarder _score)
        (Variables|Scoring&Difficulty|SetSpawnDelay 1.0)
        (Variables|Scoring&Difficulty|SetEnnemySpeed (- (Variables|Scoring&Difficulty|GetEnnemySpeed) 1.5))
        (Default|SetSpawnandDifficulty (Variables|Mobs|GetSpawner) (Variables|Scoring&Difficulty|GetSpawnDelay) (Variables|Scoring&Difficulty|GetEnnemySpeed))
        (return)
        (elif (== TryHarder++ _score)
          (Variables|Scoring&Difficulty|SetSpawnDelay 0.75)
          (Variables|Scoring&Difficulty|SetEnnemySpeed (- (Variables|Scoring&Difficulty|GetEnnemySpeed) 1.5))
          (Default|SetSpawnandDifficulty (Variables|Mobs|GetSpawner) (Variables|Scoring&Difficulty|GetSpawnDelay) (Variables|Scoring&Difficulty|GetEnnemySpeed))
          (return))))))

(fn FAddScore
  (params (ScoreAdded :type Integer))
  ;[1 1 1] Ennemi ajoute un point au score qd touché
  (Variables|Scoring&Difficulty|SetScore (+ ScoreAdded (Variables|Scoring&Difficulty|GetScore)))
  (Scoring&Difficulty|FSetDifficulty 5 10 15 20 50 70)
  (Default|EventPlayAnimation (Variables|UI|GetHud_InGame))
  (return))

(fn FArraytoBees
  (params (MobsArray :type Array%20of%20BP%20Mobs%20Teura%20Object%20References))
  (bind _beespawnpointarray (Variables|Bees|GetBeeSpawnPointArray))
  (bind _indexspawnpoint (Variables|Bees|GetIndexSpawnPoint))
  (bind _output (Utilities|Array|Get(acopy) _beespawnpointarray _indexspawnpoint))
  ;[1 1 1] Cree les abeilles et les range dans un array
  (for _index (range 0 3)
    (bind _returnvalue (Game|SpawnActorfromClass "/Game/02_Teura/Bees/BP_Bees.BP_Bees_C" (Math|Transform|MakeTransform (Transformation|GetActorLocation _output) (Transformation|GetActorRotation _output) "1,1,1") "Undefined" 0 MobsArray 0 0))
    (Variables|/Game/02_Teura/Bees/BP_Bees.BP_Bees_C|SetNumberBee _returnvalue _index)
    (Math|Integer|IncrementInt (Variables|Bees|GetIndexSpawnPoint)
      (:%20%20
        (Utilities|Array|Add (Variables|Bees|GetBeesArray) _returnvalue))))
  (return))