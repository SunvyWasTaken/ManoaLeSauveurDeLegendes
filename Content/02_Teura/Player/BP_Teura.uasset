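; Player Blueprint for Teura that recognizes touch-drawn shapes and triggers the matching Attaque on every bee in the game mode's BeesArray.
; Touch movement records viewport points and redraws a WBP_Draw_Teura trail widget.
; On release, the stroke becomes four normalized segment directions, tested with tolerance-based compass checks against four shapes, each accepting two drawing directions.
; All shapes except the straight vertical line require over 20 points; unmatched long strokes play a failure sound.
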(event Custom|SimplifyComplex
  (bind _arraypoint (Variables|Drawing|GetArrayPoint))
  (bind _returnvalue (Utilities|Array|LastIndex _arraypoint))
  (bind _returnvalue_2 (/ _returnvalue 4))
  (bind _returnvalue_3 (+ _returnvalue_2 _returnvalue_2))
  (bind _returnvalue_4 (+ _returnvalue_3 _returnvalue_2))
  ;[1 1 1] Simply toute les coordonnées en 4 vector plus simple à comparé.
  (Utilities|Array|SetArrayElem (Variables|Drawing|GetArrayCompar) 0 (Signs|FNormalizeHomeMade (Utilities|Array|Get(acopy) _arraypoint) (Utilities|Array|Get(acopy) _arraypoint _returnvalue_2)) true)
  (Utilities|Array|SetArrayElem (Variables|Drawing|GetArrayCompar) 1 (Signs|FNormalizeHomeMade (Utilities|Array|Get(acopy) _arraypoint _returnvalue_2) (Utilities|Array|Get(acopy) _arraypoint _returnvalue_3)) true)
  (Utilities|Array|SetArrayElem (Variables|Drawing|GetArrayCompar) 2 (Signs|FNormalizeHomeMade (Utilities|Array|Get(acopy) _arraypoint _returnvalue_3) (Utilities|Array|Get(acopy) _arraypoint _returnvalue_4)) true)
  (Utilities|Array|SetArrayElem (Variables|Drawing|GetArrayCompar) 3 (Signs|FNormalizeHomeMade (Utilities|Array|Get(acopy) _arraypoint _returnvalue_4) (Utilities|Array|Get(acopy) _arraypoint _returnvalue)) true)
  ;[1 1 1] Mettre toute les formes qui seront disponible
  (Signs|FForme2)
  (if (> (Utilities|Array|Length (Variables|Drawing|GetArrayPoint)) 20)
    (Signs|FForme0)
    (Signs|FForme1)
    (Signs|FForme3)
    (if (Variables|State|GetbBadSound)
      (Audio|PlaySound2D "/Game/05_Ruahatu/Sound/S_LancerRater_Ruahatu.S_LancerRater_Ruahatu" 1.0 1.0 0.0 0 0))))

(event EventBeginPlay
  (Class|PlayerController|ActivateTouchInterface (Game|GetPlayerController 0))
  (bind _asgm_teura (Utilities|Casting|CastToGM_Teura (Game|GetGameMode)))
  (Variables|Refs|SetGM_Ref _asgm_teura))

(event Input|TouchEvents|InputTouch
  (params (Location :type Vector) (FingerIndex :type ETouchIndex%20Enum))
  (bind _returnvalue (Game|GetPlayerController 0))
  (bind (_locationx _locationy) (Class|PlayerController|GetInputTouchState _returnvalue FingerIndex))
  (:Pressed
    (Utilities|Array|Clear (Variables|Drawing|GetArrayPoint)) ; clear le precedent array
    (Variables|State|SetbBadSound true))
  (:Released
    (Widget|RemovefromParent (Variables|Refs|GetCurrentWidget)) ; retire le dernier widget
    (CallFunction|SimplifyComplex)
    (Input|SetInputModeGameandUI (Game|GetPlayerController 0) (Variables|/Game/02_Teura/Gamemode/GM_Teura.GM_Teura_C|GetHud_InGame (Variables|Refs|GetGM_Ref)) "DoNotLock" false))
  (:Moved
    (Widget|RemovefromParent (Variables|Refs|GetCurrentWidget)) ; remove le precedent widget
    (if (Utilities|Enum|Equal(Enum) FingerIndex "Touch1")
      (Class|PlayerController|SetMouseLocation _returnvalue (Math|Float|Truncate _locationx) (Math|Float|Truncate _locationy))
      (bind _returnvalue_2 (Class|WidgetLayoutLibrary|GetMousePositiononViewport))
      (Utilities|Array|Add (Variables|Drawing|GetArrayPoint) _returnvalue_2) ; ajout la position de l'input à chaque nouveau tracer.
      ;[1 1 1] Create un nouveau widget à chaque tracer
      (bind _returnvalue_3 (UserInterface|CreateWidget "/Game/02_Teura/UI/HUD/WBP_Draw_Teura.WBP_Draw_Teura_C" 0 (Variables|Drawing|GetArrayPoint)))
      (bind _output_get (Variables|Refs|SetCurrentWidget _returnvalue_3))
      (UserInterface|Viewport|AddtoViewport _output_get -1))))

(fn ConstructionScript)

(fn FNormalizeHomeMade
  (params (Start :type Vector%202D%20Structure) (End :type Vector%202D%20Structure))
  (return (Math|Vector2D|Normalize2D (- End Start))))

(fn FSouth
  (params (InVec :type Vector%202D%20Structure))
  (bind (_x _y) (Math|Vector2D|BreakVector2D InVec))
  (bind _tolerance (Variables|Drawing|GetTolerance))
  (return (and (Math|Float|NearlyEqual(Float) _x 0.0 _tolerance) (Math|Float|NearlyEqual(Float) _y 1.0 _tolerance))))

(fn FEast
  (params (InVec :type Vector%202D%20Structure))
  (bind (_x _y) (Math|Vector2D|BreakVector2D InVec))
  (bind _tolerance (Variables|Drawing|GetTolerance))
  (return (and (Math|Float|NearlyEqual(Float) _x 1.0 _tolerance) (Math|Float|NearlyEqual(Float) _y 0.0 _tolerance))))

(fn FNorth
  (params (InVec :type Vector%202D%20Structure))
  (bind (_x _y) (Math|Vector2D|BreakVector2D InVec))
  (bind _tolerance (Variables|Drawing|GetTolerance))
  (return (and (Math|Float|NearlyEqual(Float) _x 0.0 _tolerance) (Math|Float|NearlyEqual(Float) _y -1.0 _tolerance))))

(fn FWest
  (params (InVec :type Vector%202D%20Structure))
  (bind (_x _y) (Math|Vector2D|BreakVector2D InVec))
  (bind _tolerance (Variables|Drawing|GetTolerance))
  (return (and (Math|Float|NearlyEqual(Float) _x -1.0 _tolerance) (Math|Float|NearlyEqual(Float) _y 0.0 _tolerance))))

(fn FNW
  (params (InVec :type Vector%202D%20Structure))
  (bind (_x _y) (Math|Vector2D|BreakVector2D InVec))
  (bind _tolerance (Variables|Drawing|GetTolerance))
  (return (and (Math|Float|NearlyEqual(Float) _x -0.8 _tolerance) (Math|Float|NearlyEqual(Float) _y -0.5 _tolerance))))

(fn FSW
  (params (InVec :type Vector%202D%20Structure))
  (bind (_x _y) (Math|Vector2D|BreakVector2D InVec))
  (bind _tolerance (Variables|Drawing|GetTolerance))
  (return (and (Math|Float|NearlyEqual(Float) _x -0.7 _tolerance) (Math|Float|NearlyEqual(Float) _y 0.5 _tolerance))))

(fn FNE
  (params (InVec :type Vector%202D%20Structure))
  (bind (_x _y) (Math|Vector2D|BreakVector2D InVec))
  (bind _tolerance (Variables|Drawing|GetTolerance))
  (return (and (Math|Float|NearlyEqual(Float) _x 0.5 _tolerance) (Math|Float|NearlyEqual(Float) _y -0.7 _tolerance))))

(fn FSE
  (params (InVec :type Vector%202D%20Structure))
  (bind (_x _y) (Math|Vector2D|BreakVector2D InVec))
  (bind _tolerance (Variables|Drawing|GetTolerance))
  (return (and (Math|Float|NearlyEqual(Float) _x 0.6 _tolerance) (Math|Float|NearlyEqual(Float) _y 0.7 _tolerance))))

(fn FForme0
  (bind _arraycompar (Variables|Drawing|GetArrayCompar))
  (bind _arraycompar_2 (Variables|Drawing|GetArrayCompar))
  (if (or (Math|Boolean|ANDBoolean (Direction|FSouth (Utilities|Array|Get(acopy) _arraycompar)) (or (Direction|FSouth (Utilities|Array|Get(acopy) _arraycompar 1)) (Direction|FSouth (Utilities|Array|Get(acopy) _arraycompar 2))) (Direction|FNW (Utilities|Array|Get(acopy) _arraycompar 3))) (Math|Boolean|ANDBoolean (Direction|FSE (Utilities|Array|Get(acopy) _arraycompar_2)) (or (Direction|FNorth (Utilities|Array|Get(acopy) _arraycompar_2 1)) (Direction|FNorth (Utilities|Array|Get(acopy) _arraycompar_2 2))) (Direction|FNorth (Utilities|Array|Get(acopy) _arraycompar_2 3))))
    (for _array_element (Variables|/Game/02_Teura/Gamemode/GM_Teura.GM_Teura_C|GetBeesArray (Variables|Refs|GetGM_Ref))
      (bind _asbp_bees (Utilities|Casting|CastToBP_Bees _array_element))
      (Default|Attaque _asbp_bees))
    (Audio|PlaySound2D "/Game/02_Teura/Player/Signs/SFX/SC_SignNice2_Teura.SC_SignNice2_Teura" 1.0 1.0 0.0 0 0)
    (Variables|State|SetbBadSound false)
    (return)
    (else
      (return))))

(fn FForme1
  (bind _arraycompar (Variables|Drawing|GetArrayCompar))
  (bind _arraycompar_2 (Variables|Drawing|GetArrayCompar))
  (if (or (Math|Boolean|ANDBoolean (Direction|FEast (Utilities|Array|Get(acopy) _arraycompar)) (Direction|FEast (Utilities|Array|Get(acopy) _arraycompar 1)) (Direction|FSouth (Utilities|Array|Get(acopy) _arraycompar 2)) (Direction|FSouth (Utilities|Array|Get(acopy) _arraycompar 3))) (Math|Boolean|ANDBoolean (Direction|FNorth (Utilities|Array|Get(acopy) _arraycompar_2)) (Direction|FNorth (Utilities|Array|Get(acopy) _arraycompar_2 1)) (Direction|FWest (Utilities|Array|Get(acopy) _arraycompar_2 2)) (Direction|FWest (Utilities|Array|Get(acopy) _arraycompar_2 3))))
    (for _array_element (Variables|/Game/02_Teura/Gamemode/GM_Teura.GM_Teura_C|GetBeesArray (Variables|Refs|GetGM_Ref))
      (bind _asbp_bees (Utilities|Casting|CastToBP_Bees _array_element))
      (Default|Attaque _asbp_bees 1))
    (Audio|PlaySound2D "/Game/02_Teura/Player/Signs/SFX/SC_SignNice2_Teura.SC_SignNice2_Teura" 1.0 1.0 0.0 0 0)
    (Variables|State|SetbBadSound false)
    (return)
    (else
      (return))))

(fn FForme2
  (bind _arraycompar (Variables|Drawing|GetArrayCompar))
  (bind _arraycompar_2 (Variables|Drawing|GetArrayCompar))
  (if (or (Math|Boolean|ANDBoolean (Direction|FSouth (Utilities|Array|Get(acopy) _arraycompar)) (Direction|FSouth (Utilities|Array|Get(acopy) _arraycompar 1)) (Direction|FSouth (Utilities|Array|Get(acopy) _arraycompar 2)) (Direction|FSouth (Utilities|Array|Get(acopy) _arraycompar 3))) (Math|Boolean|ANDBoolean (Direction|FNorth (Utilities|Array|Get(acopy) _arraycompar_2)) (Direction|FNorth (Utilities|Array|Get(acopy) _arraycompar_2 1)) (Direction|FNorth (Utilities|Array|Get(acopy) _arraycompar_2 2)) (Direction|FNorth (Utilities|Array|Get(acopy) _arraycompar_2 3))))
    (for _array_element (Variables|/Game/02_Teura/Gamemode/GM_Teura.GM_Teura_C|GetBeesArray (Variables|Refs|GetGM_Ref))
      (bind _asbp_bees (Utilities|Casting|CastToBP_Bees _array_element))
      (Default|Attaque _asbp_bees 2))
    (Audio|PlaySound2D "/Game/02_Teura/Player/Signs/SFX/SC_SignNice2_Teura.SC_SignNice2_Teura" 1.0 1.0 0.0 0 0)
    (Variables|State|SetbBadSound false)
    (return)
    (else
      (return))))

(fn FForme3
  (bind _arraycompar (Variables|Drawing|GetArrayCompar))
  (bind _arraycompar_2 (Variables|Drawing|GetArrayCompar))
  (if (or (Math|Boolean|ANDBoolean (Direction|FSW (Utilities|Array|Get(acopy) _arraycompar)) (Direction|FSW (Utilities|Array|Get(acopy) _arraycompar 1)) (Direction|FSE (Utilities|Array|Get(acopy) _arraycompar 2)) (Direction|FSE (Utilities|Array|Get(acopy) _arraycompar 3))) (Math|Boolean|ANDBoolean (Direction|FNW (Utilities|Array|Get(acopy) _arraycompar_2)) (Direction|FNW (Utilities|Array|Get(acopy) _arraycompar_2 1)) (Direction|FNE (Utilities|Array|Get(acopy) _arraycompar_2 2)) (Direction|FNE (Utilities|Array|Get(acopy) _arraycompar_2 3))))
    (for _array_element (Variables|/Game/02_Teura/Gamemode/GM_Teura.GM_Teura_C|GetBeesArray (Variables|Refs|GetGM_Ref))
      (bind _asbp_bees (Utilities|Casting|CastToBP_Bees _array_element))
      (Default|Attaque _asbp_bees 3))
    (Audio|PlaySound2D "/Game/02_Teura/Player/Signs/SFX/SC_SignNice2_Teura.SC_SignNice2_Teura" 1.0 1.0 0.0 0 0)
    (Variables|State|SetbBadSound false)
    (return)
    (else
      (return))))