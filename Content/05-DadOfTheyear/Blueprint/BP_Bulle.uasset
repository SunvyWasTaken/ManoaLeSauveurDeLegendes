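; BP_Bulle is a draggable bubble in DadOfTheYear that refills a kid's (BP_SaleGosse) oxygen when released over one.
; When activated, a looping timer raises it until it passes a height limit and returns to its spawner's spawn point.
; Touch stops the rise, and Tick maps the finger's screen position linearly onto world Y/Z.
; On release, it refills any overlapped kid, then returns to spawn without a pop effect (TODO).
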(event OnComponentBeginOverlap(GosseDetector)
  (params (OverlappedComponent :type Primitive%20Component%20Object%20Reference) (OtherActor :type Actor%20Object%20Reference) (OtherComp :type Primitive%20Component%20Object%20Reference) (OtherBodyIndex :type Integer) (bFromSweep :type Boolean) (SweepResult :type Hit%20Result%20Structure%20%28by%20ref%29))
  (bind _asbp_sale_gosse (Utilities|Casting|CastToBP_SaleGosse OtherActor))
  (Variables|Default|SetBP_SaleGosseRef _asbp_sale_gosse))

(event OnComponentEndOverlap(GosseDetector)
  (params (OverlappedComponent :type Primitive%20Component%20Object%20Reference) (OtherActor :type Actor%20Object%20Reference) (OtherComp :type Primitive%20Component%20Object%20Reference) (OtherBodyIndex :type Integer))
  (Variables|Default|SetBP_SaleGosseRef 0))

(event OnInputTouchBegin(TemporarrySphere)
  (params (FingerIndex :type ETouchIndex%20Enum :default "Touch1") (TouchedComponent :type Primitive%20Component%20Object%20Reference))
  ;[1 1 1] Quand le joueur touche la bulle, stop la monté et dit que la bulle est touché.
  (Variables|Default|SetFIngerIndex FingerIndex)
  (CallFunction|StopMonteBulle)
  (Variables|Default|SetbIsTouched true)
  (Audio|PlaySound2D "/Game/05-DadOfTheyear/SFX/dolphin/S_bubble_touch.S_bubble_touch" 0.8 0.9 0.0 0 0))

(event OnInputTouchEnd(TemporarrySphere)
  (params (FingerIndex :type ETouchIndex%20Enum :default "Touch1") (TouchedComponent :type Primitive%20Component%20Object%20Reference))
  ;[1 1 1] Si le joueur lache la bulle, fait stopper le mouvement de la bulle
  (Variables|Default|SetbIsTouched false)
  ;[1 1 1] Si à ce moment la, y'à un gamin, sur la bulle, lui donne de l'oxygène
  (Utilities|IsValid (Variables|Default|GetBP_SaleGosseRef)
    (:Is%20Valid
      (Default|RefillOxygen (Variables|Default|GetBP_SaleGosseRef) (Variables|Default|GetOxygenToFill))
      (Variables|Default|SetBP_SaleGosseRef 0)
      (Audio|PlaySound2D "/Game/05-DadOfTheyear/SFX/dolphin/SC_oxygenUP.SC_oxygenUP" 1.33 1.0 0.0 0 0))
    (:Is%20Not%20Valid
      _))
  (CallFunction|EclateBulle))

(event Custom|MonteBulle
  ;[1 1 1] Fait monter les bulles quand appelé
  (Transformation|AddActorWorldOffset "0.000000, 0,5.000000")
  (if (> (.z (Transformation|GetActorLocation)) 1.1e+03)
    (CallFunction|StopMonteBulle)
    (Transformation|SetActorLocation (Transformation|GetWorldLocation (Variables|/Game/05-DadOfTheyear/Blueprint/BP_Spawner.BP_Spawner_C|GetSpawnPoint (Variables|Default|GetBulleSpawnerRef))) false false)))

(event Custom|ActivateMonteBulle
  ;[1 1 1] Fait monter les bulles quand appelé
  (bind _returnvalue (Utilities|Time|SetTimerbyEvent (delegate Custom|MonteBulle) 0.01 true))
  (Variables|Default|SetMonteBulleHandle _returnvalue))

(event Custom|StopMonteBulle
  ;[1 1 1] Fait monter les bulles quand appelé
  (Utilities|Time|ClearandInvalidateTimerbyHandle (Variables|Default|GetMonteBulleHandle)))

(event Custom|EclateBulle
  ;[1 1 1] Rammène la bulle au point de spawn quand le joueur lache la bulle (TODO : Effet éclatement)
  (Transformation|SetActorLocation (Transformation|GetWorldLocation (Variables|/Game/05-DadOfTheyear/Blueprint/BP_Spawner.BP_Spawner_C|GetSpawnPoint (Variables|Default|GetBulleSpawnerRef))) false false))

(event EventBeginPlay
  (bind _aspc_dad_of_the_year (Utilities|Casting|CastToPC_DadOfTheYear (Game|GetPlayerController 0)))
  (Variables|Default|SetPlayerControllerRef _aspc_dad_of_the_year)
  ;[1 1 1] Récupère la résolution de l'écran
  (bind _returnvalue (Settings|GetGameUserSettings))
  (Variables|Default|SetScreenResX (.x (Class|GameUserSettings|GetScreenResolution _returnvalue)))
  (Variables|Default|SetScreenResY (.y (Class|GameUserSettings|GetScreenResolution _returnvalue))))

(event EventTick
  (params (DeltaSeconds :type Float%20%28single-precision%29))
  (bind _playercontrollerref (Variables|Default|GetPlayerControllerRef))
  (bind _fingerindex (Variables|Default|GetFIngerIndex))
  (bind (_locationx _locationy) (Class|PlayerController|GetInputTouchState _playercontrollerref _fingerindex))
  ;[1 1 1] Fait suivre le doigt du joueur lorsque celui ci à touché la bulle.
  (if (Variables|Default|GetbIsTouched)
    (Transformation|SetActorLocation (Math|Vector|MakeVector 0.0 (Math|Float|Lerp -9.6e+02 9.6e+02 (/ _locationx (Math|Conversions|ToFloat(Integer) (Variables|Default|GetScreenResX)))) (Math|Float|Lerp 8.6e+02 -1e+02 (/ _locationy (Math|Conversions|ToFloat(Integer) (Variables|Default|GetScreenResY))))) false false)))

(fn ConstructionScript)