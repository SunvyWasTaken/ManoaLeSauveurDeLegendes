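; Game mode for the Dad of the Year game, handling first-time tutorial state, HUD creation and the underwater soundscape.
; BeginPlay reads the first-time flag from GI_MetaGame, and TutoDone clears it on both.
; GameBegin shows the HUD, fades in ambiance, starts music, then starts a self-calling loop of randomly timed whale sounds placed around the camera.
; Fadeout clears Available to end that loop and fades all audio.
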(event Custom|Fade%20out
  ;[1 1 1] ambiance & music
  (Variables|Default|SetAvailable false)
  (Audio|Components|Audio|FadeOut (Variables|Default|Getmusic) 2.0 0.0 "Linear" :!class /Script/Engine.AudioComponent)
  (Audio|Components|Audio|FadeOut (Variables|Default|Getwhales) 2.5 0.0 "Linear" :!class /Script/Engine.AudioComponent)
  (Audio|Components|Audio|FadeOut (Variables|Default|GetUW_ambiance) 2.5 0.0 "Linear" :!class /Script/Engine.AudioComponent))

(event Custom|PlayWhaleSound
  (bind _returnvalue (Game|GetPlayerCameraManager 0))
  (bind _whales (Variables|Default|Getwhales))
  (bind _returnvalue_2 (Camera|GetCameraLocation _returnvalue))
  (bind (_x _y _z) (Math|Vector|BreakVector _returnvalue_2))
  ;[1 1 1] ambiance & music
  (if (Variables|Default|GetAvailable)
    (Utilities|FlowControl|Delay (Math|Random|RandomFloatinRange 5.0 8.0))
    (Audio|Components|Audio|Play _whales 0.0)
    (Transformation|SetRelativeLocation _whales (Math|Vector|MakeVector (+ _x (Math|Random|RandomFloatinRange -6e+02 6e+02)) (+ _y (Math|Random|RandomFloatinRange -6e+02 6e+02)) _z) false false)
    (CallFunction|PlayWhaleSound)))

(event Custom|GameBegin
  (bind _returnvalue (UserInterface|CreateWidget "/Game/MetaGame/Widgets/WPB_Hud.WPB_Hud_C" (Game|GetPlayerController 0)))
  (UserInterface|Viewport|AddtoViewport _returnvalue 0)
  ;[1 1 1] ambiance & music
  (Audio|Components|Audio|FadeIn (Variables|Default|GetUW_ambiance) 2.0 1.0 0.0 "Linear" :!class /Script/Engine.AudioComponent)
  (Utilities|FlowControl|Delay 2.0)
  (Audio|Components|Audio|Play (Variables|Default|Getmusic) 0.0)
  (CallFunction|PlayWhaleSound))

(event Custom|TutoDone
  (Variables|/Game/MetaGame/Blueprints/GI_MetaGame.GI_MetaGame_C|SetbIsFirstTimeDadOfTheYear (Variables|Default|GetGameInstance) false)
  (Variables|Default|SetbIsFirstTime? false))

(event EventBeginPlay
  (bind _asgi_meta_game (Utilities|Casting|CastToGI_MetaGame (Game|GetGameInstance)))
  (Variables|Default|SetGameInstance _asgi_meta_game)
  (Variables|Default|SetbIsFirstTime? (Variables|/Game/MetaGame/Blueprints/GI_MetaGame.GI_MetaGame_C|GetbIsFirstTimeDadOfTheYear _asgi_meta_game)))

(fn ConstructionScript)