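; Fish actor for the DadOfTheYear game that swims in a straight line until it passes an end position, then is handed back to its owner, BP_GerantPoissonDadOfTheYear.
; ChangeForm randomizes its plane's material and scale.
; Avance starts a looping timer that nudges it along local Y.
; Crossing the world-Y limit, compared according to that limit's sign, clears the timer and calls RecupPoisson on the owner.
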(event Custom|Avance
  (bind _returnvalue (Utilities|Time|SetTimerbyEvent (delegate Custom|AddLocation) 0.03 true))
  (Variables|Default|SetMoveHandle _returnvalue))

(event Custom|AddLocation
  (Transformation|AddActorLocalOffset "0,3.000000, 0" false false)
  (if (< (Variables|Default|GetEndToReach) 0.0)
    (if (< (.y (Transformation|GetActorLocation)) (Variables|Default|GetEndToReach))
      (CallFunction|StopMoving :!label _label))
    (elif (> (.y (Transformation|GetActorLocation)) (Variables|Default|GetEndToReach))
      (goto _label))))

(event Custom|StopMoving
  (Utilities|Time|ClearandInvalidateTimerbyHandle (Variables|Default|GetMoveHandle))
  (Default|RecupPoisson (Variables|Default|GetOwnerRef) self))

(event Custom|ChangeForm
  (Rendering|Material|SetMaterial (Variables|Default|GetPlane) 0 (Utilities|Array|Get(acopy) (Variables|Default|GetMaterial) (Math|Random|RandomIntegerinRange 0 2)))
  (Transformation|SetRelativeScale3D (Variables|Default|GetPlane) (* (* (Variables|Default|GetBaseScaleValue) 1.5) (Math|Random|RandomIntegerinRange 1 2))))

(event Custom|SetEndToReach
  (params (EndLocation :type Float%20%28single-precision%29))
  (Variables|Default|SetEndToReach EndLocation))

(event EventBeginPlay
  (bind _asbp_gerant_poisson_dad_of_the_year (Utilities|Casting|CastToBP_GerantPoissonDadOfTheYear (Components|GetOwner)))
  (Variables|Default|SetOwnerRef _asbp_gerant_poisson_dad_of_the_year))

(event Collision|EventActorBeginOverlap
  (params (OtherActor :type Actor%20Object%20Reference)))

(fn ConstructionScript)