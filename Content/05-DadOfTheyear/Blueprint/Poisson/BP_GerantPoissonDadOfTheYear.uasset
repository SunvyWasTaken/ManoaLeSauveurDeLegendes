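; Fish manager for the DadOfTheYear minigame that pools and launches fish swimming across the play area.
; On BeginPlay it spawns a pool of fish hidden below itself and starts a looping timer.
; Each tick of the timer takes the first pooled fish, places it at a random depth and height on a random side, and sends it toward the opposite limit.
; RecupPoisson returns fish to the hidden pool.
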(event Custom|SpawnPoisson
  (bind _limiteleft (Variables|Default|GetLimiteLeft))
  (bind _limiteright (Variables|Default|GetLimiteRight))
  (bind _returnvalue (Transformation|GetWorldLocation _limiteright))
  (bind _returnvalue_2 (Transformation|GetWorldLocation _limiteleft))
  (Variables|Default|SetPoissonSelectRef (Utilities|Array|Get(acopy) (Variables|Default|GetListPoisson)))
  (if (Math|Random|RandomBoolwithWeight 0.5)
    (Variables|Default|SetSideLocation (.y _returnvalue_2))
    (Variables|Default|SetSideToStop (.y _returnvalue))
    (Variables|Default|SetPoissonRotation "0, 0, 0")
    (else
      (Variables|Default|SetSideLocation (.y _returnvalue))
      (Variables|Default|SetSideToStop (.y _returnvalue_2))
      (Variables|Default|SetPoissonRotation "0,180.000000,0.000000")))
  (Transformation|SetActorTransform (Variables|Default|GetPoissonSelectRef) (Math|Transform|MakeTransform (Math|Vector|MakeVector (Math|Random|RandomFloatinRange 1387.0 1.6e+03) (Variables|Default|GetSideLocation) (Math|Random|RandomFloatinRange 0.0 7e+02)) (Variables|Default|GetPoissonRotation) "1,1,1"))
  (Default|SetEndtoReach (Variables|Default|GetPoissonSelectRef) (Variables|Default|GetSideToStop))
  (Default|ChangeForm (Variables|Default|GetPoissonSelectRef))
  (Default|Avance (Variables|Default|GetPoissonSelectRef))
  (Utilities|Array|RemoveItem (Variables|Default|GetListPoisson) (Variables|Default|GetPoissonSelectRef)))

(event Custom|RecupPoisson
  (params (PoissonRef :type BP%20Poisson%20Dad%20Of%20the%20Year%20Object%20Reference))
  (Utilities|Array|Add (Variables|Default|GetListPoisson) PoissonRef)
  (Transformation|SetActorLocation PoissonRef (- (Transformation|GetActorLocation) "0, 0,500.000000") false false))

(event EventBeginPlay
  (for _index (range 0 19)
    (bind _returnvalue (Game|SpawnActorfromClass "/Game/05-DadOfTheyear/Blueprint/Poisson/BP_PoissonDadOfTheYear.BP_PoissonDadOfTheYear_C" (Math|Transform|MakeTransform (- (Transformation|GetActorLocation) "0, 0,500.000000") "0, 0, 0" "1,1,1") "Undefined" self 0))
    (Utilities|Array|Add (Variables|Default|GetListPoisson) _returnvalue))
  (bind _returnvalue_2 (Utilities|Time|SetTimerbyEvent (delegate Custom|SpawnPoisson) 1.0 true))
  (Variables|Default|SetSpawnPoissonHandle _returnvalue_2))

(event Collision|EventActorBeginOverlap
  (params (OtherActor :type Actor%20Object%20Reference)))

(event EventTick
  (params (DeltaSeconds :type Float%20%28single-precision%29)))

(fn ConstructionScript)