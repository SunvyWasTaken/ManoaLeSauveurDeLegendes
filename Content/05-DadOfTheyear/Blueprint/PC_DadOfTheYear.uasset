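; Player controller for the DadOfTheYear level that tracks touch input, with helpers for detecting a downward swipe.
; Touch press stores the start position and a touch flag, and release clears that flag and the swipe-done flag.
; ScreenTouchPosition derives direction and length from the start point, and SwipeVersLeBas tolerance-checks that direction against downward.
; The chain combining these with a minimum length to mark the swipe done is unconnected, so it never runs.
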(event EventBeginPlay)

(event EventTick
  (params (DeltaSeconds :type Float%20%28single-precision%29)))

(event Input|TouchEvents|InputTouch
  (params (Location :type Vector) (FingerIndex :type ETouchIndex%20Enum))
  (:Pressed
    (Variables|Default|SetbIsTouchScreen? true)
    (Variables|Default|SetFirstPosition (.ScreenPosition (CallFunction|ScreenTouchPosition))))
  (:Released
    (Variables|Default|SetbIsTouchScreen? false)
    (Variables|Default|SetbDoneSwip? false)))

(fn ConstructionScript)

(fn ScreenTouchPosition
  (bind (_locationx _locationy) (Class|PlayerController|GetInputTouchState "Touch1"))
  (bind _firstposition (Variables|Default|GetFirstPosition))
  (bind _returnvalue (Math|Vector2D|MakeVector2D _locationx _locationy))
  (bind _returnvalue_2 (- _returnvalue _firstposition))
  (bind (_outdir _outlength) (Class|KismetMathLibrary|ToDirectionandLength2D _returnvalue_2))
  (return (.WorldPosition (Class|GameplayStatics|DeprojectScreentoWorld self _returnvalue)) _returnvalue _outdir _outlength))

(fn SwipeVersLeBas?
  (params (Direction2DVector :type Vector%202D%20Structure))
  (bind (_x _y) (Math|Vector2D|BreakVector2D Direction2DVector))
  (return (and (Math|Float|NearlyEqual(Float) _x 0.0 0.2) (Math|Float|NearlyEqual(Float) _y 0.9 0.2))))