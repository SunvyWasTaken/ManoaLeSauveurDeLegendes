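; Underwater child actor for the DadOfTheYear minigame that dives in, loses oxygen and gradually transforms body part by body part.
; A looping timer drains oxygen, triggering agitation, then panic with warning FX, then EndGame on the spawner at zero; RefillOxygen adds air.
; A randomly delayed recursive loop swaps random part sprites, with variant and score depending on oxygen, and calls spawner Victory when complete.
; The Spawn timeline drives the dive and reverses for despawn.
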(event Custom|RefillOxygen
  (params (OxygenToFill :type Integer))
  (bind _output_get (Variables|Default|SetOxygenLevel (+ OxygenToFill (Variables|Default|GetOxygenLevel))))
  (if (>= _output_get 6)
    (CallFunction|StopPANIC))
  (if (< _output_get 10)
    (CallFunction|RunningOutOfOxygen)
    (elif (>= _output_get 10)
      (CallFunction|StopAgitationAnim))))

(event Custom|StopAgitationAnim
  (bind _rotation (Timeline|NoyadeLOL Stop)
    (:Update
      (Transformation|SetActorRelativeRotation (Math|Rotator|MakeRotator _rotation 0.0 0.0)))
    (:Finished
      (Transformation|SetActorRelativeRotation (Math|Rotator|MakeRotator 0.0 0.0 0.0)))))

(event Custom|Transformation
  (bind _head (Variables|Default|GetHead))
  (bind _hair (Variables|Default|GetHair))
  (bind _arms (Variables|Default|GetArms))
  (bind _legs (Variables|Default|GetLegs))
  (bind _bodypartstotransform (Variables|Default|GetBodyPartsToTransform))
  (Audio|PlaySound2D "/Game/05-DadOfTheyear/SFX/dolphin/S_body_part.S_body_part" 0.71 0.88 0.0 0 0)
  (if (<= (Variables|Default|GetOxygenLevel) 5)
    (Variables|Default|SetbGudTransform? false)
    (else
      (Variables|Default|SetbGudTransform? true)))
  (bind _output_get (Variables|Default|SetRandomSelectedPart (Utilities|Array|Get(acopy) (Variables|Default|GetBodyPartsToTransform) (Math|Random|RandomIntegerinRange 0 (Utilities|Array|Length (Variables|Default|GetBodyPartsToTransform))))))
  (Utilities|SwitchonParts _output_get
    (:Hair
      (if (Variables|Default|GetbGudTransform?)
        (Rendering|Components|Sprite|SetSprite _hair "/Game/05-DadOfTheyear/Textures/Gamin/T_Hair3.T_Hair3")
        (Math|Integer|IncrementInt (Variables|Default|GetScore) :!label _label
          (:%20%20
            _))
        (else
          (Rendering|Components|Sprite|SetSprite _hair "/Game/05-DadOfTheyear/Textures/Gamin/T_Hair2.T_Hair2"))))
    (:Body
      (Rendering|Components|Sprite|SetSprite (Variables|Default|GetBody) "/Game/05-DadOfTheyear/Textures/Gamin/T_Body2.T_Body2")
      (goto _label))
    (:Arm
      (if (Variables|Default|GetbGudTransform?)
        (Rendering|Components|Sprite|SetSprite _arms "/Game/05-DadOfTheyear/Textures/Gamin/T_Arm3.T_Arm3")
        (goto _label)
        (else
          (Rendering|Components|Sprite|SetSprite _arms "/Game/05-DadOfTheyear/Textures/Gamin/T_Arm2.T_Arm2"))))
    (:Legs
      (if (Variables|Default|GetbGudTransform?)
        (Rendering|Components|Sprite|SetSprite _legs "/Game/05-DadOfTheyear/Textures/Gamin/T_Leg3.T_Leg3")
        (goto _label)
        (else
          (Rendering|Components|Sprite|SetSprite _legs "/Game/05-DadOfTheyear/Textures/Gamin/T_Leg2.T_Leg2"))))
    (:Head
      (if (Variables|Default|GetbGudTransform?)
        (Rendering|Components|Sprite|SetSprite _head "/Game/05-DadOfTheyear/Textures/Gamin/T_Head3.T_Head3")
        (Audio|PlaySound2D "/Game/05-DadOfTheyear/SFX/dolphin/SC_dolphins.SC_dolphins" 0.67 1.0 0.0 0 0)
        (goto _label)
        (else
          (Rendering|Components|Sprite|SetSprite _head "/Game/05-DadOfTheyear/Textures/Gamin/T_Head2.T_Head2")))))
  (Utilities|Array|RemoveItem _bodypartstotransform (Variables|Default|GetRandomSelectedPart))
  (if (== (Utilities|Array|Length _bodypartstotransform) 0)
    (Variables|Default|SetIsTransformed true)
    (Utilities|Time|ClearandInvalidateTimerbyHandle (Variables|Default|GetTimerHandle))
    (Default|Victory? (Variables|Default|GetSpawnerRef))
    (Audio|PlaySound2D "/Game/05-DadOfTheyear/SFX/dolphin/S_transfo_completed.S_transfo_completed" 0.9 1.0 0.0 0 0)
    (CallFunction|StopPANIC)
    (CallFunction|StopAgitationAnim)))

(event Custom|TransformationRate
  (if (not (Variables|Default|GetIsTransformed))
    (Utilities|FlowControl|Delay (Math|Random|RandomFloatinRange 8.0 12.0))
    (CallFunction|Transformation)
    (CallFunction|TransformationRate)))

(event Custom|StopPANIC
  (CallFunction|DespawnWarningFX)
  (bind _rotation (Timeline|PANIC Stop)
    (:Update
      (Transformation|SetActorRelativeRotation (Math|Rotator|MakeRotator _rotation 0.0 0.0)))
    (:Finished
      (Transformation|SetActorRelativeRotation (Math|Rotator|MakeRotator 0.0 0.0 0.0)))))

(event Custom|DangerZone
  (bind _returnvalue (Effects|SpawnEmitteratLocation "/Game/05-DadOfTheyear/ParticleSystems/PS_WarningOxygen.PS_WarningOxygen" (+ (Transformation|GetActorLocation) "0, 0,150.000000") "0, 0, 0" "0.800000,0.800000,0.800000"))
  (Variables|Default|SetParticleWarningRef _returnvalue)
  (bind _rotation (Timeline|PANIC Play)
    (:Update
      (Transformation|SetActorRelativeRotation (Math|Rotator|MakeRotator _rotation 0.0 0.0)))
    (:Finished
      (Transformation|SetActorRelativeRotation (Math|Rotator|MakeRotator 0.0 0.0 0.0)))))

(event Custom|StartTimer
  (bind _returnvalue (Utilities|Time|SetTimerbyEvent (delegate Custom|OxygenCountdown) 1.0 true))
  (Variables|Default|SetTimerHandle _returnvalue))

(event Custom|OxygenCountdown
  (Math|Integer|DecrementInt (Variables|Default|GetOxygenLevel)
    (:%20%20
      (switch int (Variables|Default|GetOxygenLevel)
        (:0
          (if (not (Variables|Default|GetbIsDed))
            (CallFunction|OutOfOxygen)))
        (:5
          (CallFunction|StopAgitationAnim)
          (CallFunction|DangerZone)
          (Audio|PlaySound2D "/Game/05-DadOfTheyear/SFX/dolphin/SC_chokes.SC_chokes" 0.91 1.0 0.0 0 0))
        (:10
          (CallFunction|RunningOutOfOxygen)
          (Audio|PlaySound2D "/Game/05-DadOfTheyear/SFX/dolphin/SC_bubbles_UW.SC_bubbles_UW" 1.0 1.0 0.0 0 0))))))

(event Custom|OutOfOxygen
  ;[1 1 1] Prévient le spawner que un des gosses n'a plus d'oxygène
  (CallFunction|InstaKill)
  (Default|EndGame (Variables|Default|GetSpawnerRef) self)
  (Variables|Default|SetbIsDed true)
  (Utilities|Time|ClearandInvalidateTimerbyHandle (Variables|Default|GetTimerHandle))
  (Development|PrintString "Congratulations, tu l'a noyed lol"))

(event Custom|RunningOutOfOxygen
  (bind _rotation (Timeline|NoyadeLOL Play)
    (:Update
      (Transformation|SetActorRelativeRotation (Math|Rotator|MakeRotator _rotation 0.0 0.0)))
    (:Finished
      (Transformation|SetActorRelativeRotation (Math|Rotator|MakeRotator 0.0 0.0 0.0)))))

(event Custom|SpawnGosse
  (Audio|PlaySound2D "/Game/05-DadOfTheyear/SFX/dolphin/S_immersion.S_immersion" 0.75 0.78 0.0 0 0)
  (Utilities|FlowControl|Delay (Math|Random|RandomFloatinRange 0.01 1.0))
  (Effects|SpawnEmitteratLocation "/Game/05-DadOfTheyear/ParticleSystems/PS_Plongeon.PS_Plongeon" (Math|Vector|MakeVector (- (.x (Transformation|GetActorLocation)) 3e+02) (+ (Variables|Default|GetRandomSpawnLocation) 1e+02) (+ (Variables|Default|GetRandomSpawnDepth) 1.1e+03)) "0, 0, 0" "0.500000,0.500000,0.500000")
  (bind _alpha (Timeline|Spawn Play)
    (:Update
      (Transformation|SetActorLocation (Math|Vector|MakeVector 0.0 (Variables|Default|GetRandomSpawnLocation) (Math|Float|Lerp 1.2e+03 (Variables|Default|GetRandomSpawnDepth) _alpha)) false false))
    (:Finished
      (Effects|SpawnEmitterAttached "/Game/05-DadOfTheyear/ParticleSystems/PS_BullesNormales.PS_BullesNormales" (Variables|Default|GetDefaultSceneRoot) "None"))))

(event Custom|DespawnGosse
  (Variables|Default|SetIsTransformed true) ; Arrete la transformation
  (CallFunction|DespawnWarningFX)
  ;[1 1 1] Possibilité de mettre un son de remonté à la surface ici
  (Utilities|FlowControl|Delay (Math|Random|RandomFloatinRange 2.0 3.0))
  (Development|PrintString "Despawn sale gosse after delay" true true "(R=1.000000,G=0.403122,B=0.000000,A=1.000000)")
  (bind _alpha (Timeline|Spawn ReverseFromEnd)
    (:Update
      (Transformation|SetActorLocation (Math|Vector|MakeVector 0.0 (Variables|Default|GetRandomSpawnLocation) (Math|Float|Lerp 1.2e+03 (Variables|Default|GetRandomSpawnDepth) _alpha)) false false))
    (:Finished
      (Effects|SpawnEmitterAttached "/Game/05-DadOfTheyear/ParticleSystems/PS_BullesNormales.PS_BullesNormales" (Variables|Default|GetDefaultSceneRoot) "None"))))

(event Custom|InstaKill
  (Development|PrintString "InstaKill" true true "(R=1.000000,G=0.036430,B=0.000000,A=1.000000)")
  (CallFunction|DespawnWarningFX)
  (bind _alpha (Timeline|Spawn ReverseFromEnd)
    (:Update
      (Transformation|SetActorLocation (Math|Vector|MakeVector 0.0 (Variables|Default|GetRandomSpawnLocation) (Math|Float|Lerp 1.2e+03 (Variables|Default|GetRandomSpawnDepth) _alpha)) false false))
    (:Finished
      (Effects|SpawnEmitterAttached "/Game/05-DadOfTheyear/ParticleSystems/PS_BullesNormales.PS_BullesNormales" (Variables|Default|GetDefaultSceneRoot) "None"))))

(event EventBeginPlay
  (bind _asgm_dad_of_the_year (Utilities|Casting|CastToGM_DadOfTheYear (Game|GetGameMode)))
  (Variables|Default|SetGamemodeRef _asgm_dad_of_the_year)
  (Variables|Default|SetOxygenLevel (Math|Random|RandomIntegerinRange 15 25))
  (Variables|Default|SetRandomSpawnDepth (Math|Random|RandomFloatinRange 2e+02 7e+02))
  (Variables|Default|SetBodyPartsToTransform (Utilities|Array|MakeArray (Variables|Default|GetHair) (Variables|Default|GetBody) (Variables|Default|GetArms) (Variables|Default|GetLegs) (Variables|Default|GetHead)))
  (Utilities|FlowControl|Delay 3.0)
  (CallFunction|TransformationRate))

(fn ConstructionScript)

(fn DespawnWarningFX
  (Utilities|IsValid (Variables|Default|GetParticleWarningRef)
    (:Is%20Valid
      (Components|DestroyComponent (Variables|Default|GetParticleWarningRef))
      (Variables|Default|SetParticleWarningRef 0))
    (:Is%20Not%20Valid)))