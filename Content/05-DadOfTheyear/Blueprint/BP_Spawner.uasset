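; Spawner and round manager for the DadOfTheYear minigame, handling bubbles, kids (BP_SaleGosse) and win/loss screens.
; BeginPlay pre-spawns both pools, starts the kids after a delay, then shows a pausing tutorial on first play.
; A looping timer recycles parked bubbles, launching them at random Y within construction-time limits.
; EndGame pops bubbles and despawns remaining kids, while Victory? totals scores once every kid is transformed.
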(event Custom|LaunchBulles
  ;[1 1 1] Lance les bulles toutes les 2 à 5 secondes
  (bind _returnvalue (Utilities|Time|SetTimerbyEvent (delegate Custom|Bubbling) 1.0 true))
  (Variables|Default|SetLaunchBullesHandle _returnvalue))

(event Custom|Bubbling
  (bind _limitright (Variables|Default|GetLimitRight))
  (if (< (Variables|Default|GetBullesLaunched) (Utilities|Array|Length (Variables|Default|GetBulleArray)))
    ;[1 1 1] Si la bulle qu'on souhaite lancer ne se trouve pas au spawn, on passe à la suivante
    (if (Math|Vector|Equal(Vector) (Transformation|GetActorLocation (Utilities|Array|Get(acopy) (Variables|Default|GetBulleArray) (Variables|Default|GetBullesLaunched))) (Transformation|GetWorldLocation (Variables|Default|GetSpawnPoint)) 1.0)
      ;[1 1 1] Lance la bulle et active sa flotaison
      (Transformation|SetActorLocation (Utilities|Array|Get(acopy) (Variables|Default|GetBulleArray) (Variables|Default|GetBullesLaunched)) (Math|Vector|MakeVector 0.0 (Math|Random|RandomFloatinRange (.y (Variables|Default|GetLimitLeft)) (.y _limitright)) (.z _limitright)) false false)
      (Default|ActivateMonteBulle (Utilities|Array|Get(acopy) (Variables|Default|GetBulleArray) (Variables|Default|GetBullesLaunched)))
      ;[1 1 1] Incrémente pour lancer la prochaine bulle
      (Math|Integer|IncrementInt (Variables|Default|GetBullesLaunched))
      (else
        (Math|Integer|IncrementInt (Variables|Default|GetBullesLaunched)
          (:%20%20
            (CallFunction|Bubbling)))))
    (else
      (Variables|Default|SetBullesLaunched 0))))

(event Custom|EndGame
  (params (FirstNoyer :type BP%20Sale%20Gosse%20Object%20Reference))
  (Utilities|Array|RemoveItem (Variables|Default|GetGossesArray) FirstNoyer)
  (Utilities|FlowControl|DoOnce false
    (:Completed
      (CallFunction|StopBulles)
      (for _array_element (Variables|Default|GetGossesArray)
        (Utilities|Time|ClearandInvalidateTimerbyHandle (Variables|/Game/05-DadOfTheyear/Blueprint/BP_SaleGosse.BP_SaleGosse_C|GetTimerHandle _array_element))
        (Default|DespawnGosse _array_element))
      (Utilities|FlowControl|Delay 3.0)
      (bind _returnvalue (UserInterface|CreateWidget "/Game/MetaGame/Widgets/WBP_TimesUp.WBP_TimesUp_C" 0 "Dommage" 0 10 20 30))
      (UserInterface|Viewport|AddtoViewport _returnvalue 0)
      (Default|FadeOut (Variables|Default|GetGamemodeRef)))))

(event Custom|StopBulles
  ;[1 1 1] Comment
  (Utilities|Time|ClearandInvalidateTimerbyHandle (Variables|Default|GetLaunchBullesHandle))
  (for _array_element (Variables|Default|GetBulleArray)
    (Utilities|FlowControl|Delay (Math|Random|RandomFloatinRange 0.01 0.2))
    (Default|EclateBulle _array_element)))

(event Custom|Victory?
  (bind _array_element (Utilities|Array|ForEachLoopwithBreak (Variables|Default|GetGossesArray) :!label _label)
    (:LoopBody
      (if (Variables|/Game/05-DadOfTheyear/Blueprint/BP_SaleGosse.BP_SaleGosse_C|GetIsTransformed _array_element)
        (Variables|Default|SetGlobalScore (+ (Variables|Default|GetGlobalScore) (Variables|/Game/05-DadOfTheyear/Blueprint/BP_SaleGosse.BP_SaleGosse_C|GetScore _array_element)))
        (Variables|Default|SetEveryoneIsTransform? true)
        (else
          (Variables|Default|SetGlobalScore 0)
          (Variables|Default|SetEveryoneIsTransform? false)
          (goto _label Break))))
    (:Completed
      (if (Variables|Default|GetEveryoneIsTransform?)
        (Default|FadeOut (Variables|Default|GetGamemodeRef))
        (Utilities|FlowControl|Delay 2.0)
        (bind _returnvalue (UserInterface|CreateWidget "/Game/MetaGame/Widgets/WBP_TimesUp.WBP_TimesUp_C" 0 " " (Variables|Default|GetGlobalScore) 10 20 30))
        (UserInterface|Viewport|AddtoViewport _returnvalue 0)))))

(event EventBeginPlay
  (bind _asgm_dad_of_the_year (Utilities|Casting|CastToGM_DadOfTheYear (Game|GetGameMode)))
  (Variables|Default|SetGameModeRef _asgm_dad_of_the_year)
  (if (Variables|/Game/05-DadOfTheyear/Blueprint/GM_DadOfTheYear.GM_DadOfTheYear_C|GetbIsFirstTime? (Variables|Default|GetGameModeRef))
    (bind _returnvalue (UserInterface|CreateWidget "/Game/05-DadOfTheyear/Widget/WBP_TutoDadOdTheYear.WBP_TutoDadOdTheYear_C" (Game|GetPlayerController 0) self))
    (Variables|Default|SetWBP_Tuto _returnvalue))
  ;[1 1 1] Fait spawn toutes les bulles au début du jeu.
  (for _index (range 0 (Variables|Default|GetNumberOfSpawnBulle))
    (bind _returnvalue_2 (Game|SpawnActorfromClass "/Game/05-DadOfTheyear/Blueprint/BP_Bulle.BP_Bulle_C" (Math|Transform|MakeTransform (Transformation|GetWorldLocation (Variables|Default|GetSpawnPoint)) "0, 0, 0" "1,1,1") "AlwaysSpawn" 0 self 0))
    (Utilities|Array|Add (Variables|Default|GetBulleArray) _returnvalue_2))
  (for _index_2 (range 0 5)
    (bind _returnvalue_3 (Game|SpawnActorfromClass "/Game/05-DadOfTheyear/Blueprint/BP_SaleGosse.BP_SaleGosse_C" (Math|Transform|MakeTransform (Transformation|GetWorldLocation (Variables|Default|GetSpawnPoint)) "0, 0, 0" "1,1,1") "Undefined" 0 (Math|Conversions|ToFloat(Integer) (Utilities|Array|Get(acopy) (Variables|Default|GetPredefinitLocation) _index_2)) self 0))
    (Utilities|Array|Add (Variables|Default|GetGossesArray) _returnvalue_3))
  (Utilities|FlowControl|Delay 4.0)
  (for _array_element (Variables|Default|GetGossesArray)
    (Default|SpawnGosse _array_element)
    (Default|StartTimer _array_element))
  (Utilities|FlowControl|Delay 3.0)
  (CallFunction|LaunchBulles)
  (if (Variables|/Game/05-DadOfTheyear/Blueprint/GM_DadOfTheYear.GM_DadOfTheYear_C|GetbIsFirstTime? (Variables|Default|GetGameModeRef))
    (UserInterface|Viewport|AddtoViewport (Variables|Default|GetWBP_Tuto) 0)
    (Default|TutoDone (Variables|Default|GetGameModeRef))
    (Game|SetGamePaused true)))

(fn ConstructionScript
  (Variables|Default|SetLimitLeft (Transformation|GetWorldLocation (Variables|Default|GetSpawnLimitLeft)))
  (Variables|Default|SetLimitRight (Transformation|GetWorldLocation (Variables|Default|GetSpawnLimitRight))))