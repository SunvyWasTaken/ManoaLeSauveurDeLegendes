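; BP_PopUpScore_Coco is a short-lived floating score pop-up actor for the coconut (Coco) part of the Vaihiria game section.
; On BeginPlay a looping timer calls F_Move to shift it along world Z by Speed, and the actor destroys itself after a one-second delay.
; F_PopUpParameter writes the given integer to a text render and tints both text components Yellow or Nice depending on a condition.
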(event EventBeginPlay
  ;[1 1 1] Active le FX le temps du flipbook
  (Utilities|Time|SetTimerbyFunctionName 0 "F_Move" 0.03 true)
  (Utilities|FlowControl|Delay 1.0)
  (Actor|DestroyActor))

(fn ConstructionScript)

(fn FMove
  (Transformation|AddActorWorldOffset (Math|Vector|MakeVector 0.0 0.0 (* (Variables|Stuff|GetSpeed) 1.0))))

(fn FPopUpParameter
  (params (Condition :type Boolean) (Value :type Integer))
  (bind _score (Variables|Default|GetScore))
  (bind __ (Variables|Default|Get+))
  (Rendering|Components|TextRender|SetText (Variables|Default|Get+) (Utilities|Text|ToText(Integer) Value))
  (if Condition
    (Rendering|Components|TextRender|SetTextRenderColor __ (Variables|Stuff|GetYellow))
    (Rendering|Components|TextRender|SetTextRenderColor _score (Variables|Stuff|GetYellow))
    (else
      (Rendering|Components|TextRender|SetTextRenderColor __ (Variables|Stuff|GetNice))
      (Rendering|Components|TextRender|SetTextRenderColor _score (Variables|Stuff|GetNice)))))