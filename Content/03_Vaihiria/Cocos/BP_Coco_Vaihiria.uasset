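; Falling coconut (Normal, Gold or Multicolor) in the Vaihiria minigame, launched by its spawner and scored when touched as Perfect or Nice.
; A looping timer moves it downward or toward intersection targets, where turns are random and Multicolors split through the spawner.
; Overlapping coconuts merge, combining score multipliers up to 5 and keeping the higher type.
; Fever time slows it, and touched or absorbed coconuts reset to their initial position for reuse.
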(event OnComponentBeginOverlap(Box1)
  (params (OverlappedComponent :type Primitive%20Component%20Object%20Reference) (OtherActor :type Actor%20Object%20Reference) (OtherComp :type Primitive%20Component%20Object%20Reference) (OtherBodyIndex :type Integer) (bFromSweep :type Boolean) (SweepResult :type Hit%20Result%20Structure%20%28by%20ref%29))
  ;[1 1 1] Coco Spawned
  (bind _asbp_coco_vaihiria (Utilities|Casting|CastToBP_Coco_Vaihiria OtherActor))
  (if (and (Variables|State|GetbIsFalling) (not (Variables|State|GetbHasJustSpawned)))
    (if (> (.z (Transformation|GetActorLocation)) (.z (Transformation|GetActorLocation _asbp_coco_vaihiria)))
      (Utilities|MacroSetCocoMerging _asbp_coco_vaihiria
        (:End
          (Audio|SpawnSound2D "/Game/03_Vaihiria/Cocos/SFX/S_CocoPoofReverse_Coco.S_CocoPoofReverse_Coco" 1.0 1.0 0.0 0))))))

(event EventCocoReinitialize
  ;[1 1 1] Réinitialise coco
  (Variables|State|SetbHasJustSpawned false)
  (Variables|State|SetbIsFalling false)
  (Variables|State|SetbIsTurning false)
  (Variables|State|SetbFeverTime false)
  (Variables|Scoring|SetScoreMultiplier 1)
  (bind _returnvalue (Effects|SpawnEmitteratLocation "/Game/02_Teura/FX/VFX/PS_BeesHit_Teura.PS_BeesHit_Teura" (Transformation|GetActorLocation) "0, 0, 0" "5.000000,5.000000,5.000000"))
  (Rendering|SetTranslucentSortPriority _returnvalue 25)
  (Development|SetHiddeninGame (Variables|Default|GetFeverTimed) true false)
  (Utilities|Time|ClearTimerbyFunctionName 0 "FallTimer")
  (Transformation|SetActorLocation (Variables|Movements|GetInitialLocation) false false))

(event EventSpawnerFeverTime
  ;[1 1 1] FeverTime
  (Variables|State|SetbFeverTime true)
  (Variables|Movements|SetSpeed (/ (Variables|Movements|GetSpeed) (Variables|State|GetFeverDenominateur)))
  (Development|SetHiddeninGame (Variables|Default|GetFeverTimed) false false)
  (Default|AnimeFeverTimer (Variables|/Game/03_Vaihiria/Gamemode/GM_Vaihiria.GM_Vaihiria_C|GetHUD_inGame (Variables|Refs|GetGameode)))
  (Audio|SpawnSound2D "/Game/03_Vaihiria/Gamemode/SFX/S_FreezeTime.S_FreezeTime" 1.0 1.0 0.0 0)
  (Audio|Components|Audio|SetPitchMultiplier (Variables|/Game/03_Vaihiria/Gamemode/GM_Vaihiria.GM_Vaihiria_C|GetMusique (Variables|Refs|GetGameode)) 0.5)
  (Utilities|FlowControl|Delay 1.0)
  (Audio|SpawnSound2D "/Game/03_Vaihiria/Gamemode/SFX/S_FreezeTime.S_FreezeTime" 1.0 1.0 0.0 0)
  (Utilities|FlowControl|Delay 1.0)
  (Audio|Components|Audio|SetPitchMultiplier (Variables|/Game/03_Vaihiria/Gamemode/GM_Vaihiria.GM_Vaihiria_C|GetMusique (Variables|Refs|GetGameode)) 1.0))

(event EventCocoTouchCoco
  (params (Perfect :type Boolean))
  ;[1 1 1] CocoCliqué
  (Scoring|FCocoTouched Perfect))

(event EventCocoCrossIntersection
  (params (TargetLocation :type Vector :default "0, 0, 0") (IntersectionCrossed :type Actor%20Object%20Reference))
  ;[1 1 1] Set la direction qd arrivé a l'intersection
  (Variables|Movements|SetTargetLocation TargetLocation)
  (if (Utilities|Enum|Equal(Enum) (Variables|Initialize|GetCocoType) "NewEnumerator2")
    (CallFunction|SpawnerandCocoSplitCoco (Transformation|GetActorLocation) (Variables|Movements|GetTargetLocation) false)
    (Class|BPIVaihiria|IntersectionSetifCrossed(Message) IntersectionCrossed true)
    (Audio|SpawnSound2D "/Game/03_Vaihiria/Cocos/SFX/S_WooshMoveCoco_Coco.S_WooshMoveCoco_Coco" 1.0 (Math|Random|RandomFloatinRange 1.0 1.3) 0.15 0)
    (Audio|SpawnSound2D "/Game/03_Vaihiria/Cocos/SFX/S_CocoPoof_Coco.S_CocoPoof_Coco" 1.0 1.0 0.0 0)
    (elif (Variables|State|GetbIsTurning)
      (Variables|State|SetbIsTurning false)
      (Class|BPIVaihiria|IntersectionSetifCrossed(Message) IntersectionCrossed false)
      (elif (Math|Random|RandomBool)
        (Variables|State|SetbIsTurning true)
        (Class|BPIVaihiria|IntersectionSetifCrossed(Message) IntersectionCrossed true)
        (Audio|SpawnSound2D "/Game/03_Vaihiria/Cocos/SFX/S_WooshMoveCoco_Coco.S_WooshMoveCoco_Coco" 1.0 (Math|Random|RandomFloatinRange 1.0 1.3) 0.15 0)))))

(event EventSpawnerandCocoSplitCoco
  (params (StartPosition :type Vector :default "0, 0, 0") (TargetLocation :type Vector :default "0, 0, 0") (FeverTime :type Boolean) (Multiplier :type Integer))
  (bind _returnvalue (Transformation|GetActorLocation))
  (bind _scoremultiplier (Variables|Scoring|GetScoreMultiplier))
  (bind _bfevertime (Variables|State|GetbFeverTime))
  ;[1 1 1] Multicolore est splité
  (Class|BPIVaihiria|SpawnerandCocoSplitCoco(Message) (Components|GetOwner) _returnvalue TargetLocation _bfevertime _scoremultiplier)
  (CallFunction|CocoGo _returnvalue (Utilities|Select :Index (Math|Random|RandomIntegerinRange 0 9) :Option%200 "NewEnumerator0" :Option%201 "NewEnumerator0" :Option%202 "NewEnumerator0" :Option%203 "NewEnumerator0" :Option%204 "NewEnumerator0" :Option%205 "NewEnumerator0" :Option%206 "NewEnumerator0" :Option%207 "NewEnumerator0" :Option%208 "NewEnumerator0" :Option%209 "NewEnumerator1") false _bfevertime "0, 0, 0" _scoremultiplier))

(event EventCocoGo
  (params (StartPosition :type Vector :default "0, 0, 0") (CocoType :type E_CocoType_Vaihiria%20Enum :default "NewEnumerator0") (IsTurning :type Boolean) (FeverTime :type Boolean) (TargetLocation :type Vector :default "0, 0, 0") (Multiplier :type Integer))
  ;[1 1 1] Set la position, le type de coco et active le timer de la chute. Déclenché depuis le Spawner
  (Utilities|Time|ClearTimerbyFunctionName 0 "FallTimer")
  (Variables|State|SetbHasJustSpawned true)
  (Variables|State|SetbIsFalling true)
  (Transformation|SetActorLocation StartPosition false false)
  (Variables|Initialize|SetCocoType CocoType)
  (Variables|State|SetbIsTurning IsTurning)
  (Variables|State|SetbFeverTime FeverTime)
  (Variables|Movements|SetTargetLocation TargetLocation)
  (Variables|Scoring|SetScoreMultiplier Multiplier)
  (Scoring|FSetMultiplierSprite)
  (Rendering|Components|Sprite|SetSprite (Variables|Default|GetPaperSprite) (Utilities|Select :Index (Variables|Initialize|GetCocoType) :NewEnumerator0 "/Game/03_Vaihiria/Cocos/Art/SP_CocoNormal_Vaihiria.SP_CocoNormal_Vaihiria" :NewEnumerator1 "/Game/03_Vaihiria/Cocos/Art/SP_CocoGold_Vaihiria.SP_CocoGold_Vaihiria" :NewEnumerator2 "/Game/03_Vaihiria/Cocos/Art/SP_CocoRainbow_Vaihiria.SP_CocoRainbow_Vaihiria"))
  (if (Variables|State|GetbFeverTime)
    (Variables|Movements|SetSpeed (/ (Utilities|Select :Index (Variables|Initialize|GetCocoType) :NewEnumerator0 15.0 :NewEnumerator1 2e+01 :NewEnumerator2 17.0) (Variables|State|GetFeverDenominateur)))
    (else
      (Variables|Movements|SetSpeed (Utilities|Select :Index (Variables|Initialize|GetCocoType) :NewEnumerator0 15.0 :NewEnumerator1 2e+01 :NewEnumerator2 17.0))))
  (Utilities|Time|SetTimerbyFunctionName 0 "FallTimer" 0.03 true)
  (Utilities|FlowControl|Delay 0.5)
  (Variables|State|SetbHasJustSpawned false))

(event EventBeginPlay
  ;[1 1 1] BeginPlay: Set GM
  (bind _asgm_vaihiria (Utilities|Casting|CastToGM_Vaihiria (Game|GetGameMode)))
  (Variables|Refs|SetGameode _asgm_vaihiria))

(fn ConstructionScript
  (Variables|Movements|SetInitialLocation (Transformation|GetActorLocation))
  (Variables|State|SetFeverDenominateur 2.0)
  (Development|SetHiddeninGame (Variables|Default|GetFeverTimed) true false))

(fn FallTimer
  (if (Variables|State|GetbIsTurning)
    ;[1 1 1] Si le coco tourne, va dans la direction du boxcomponent dans BP_Intersection
    (Transformation|AddActorWorldOffset (* (Math|Vector|Normalize (- (Variables|Movements|GetTargetLocation) (Transformation|GetActorLocation))) (Variables|Movements|GetSpeed)))
    (else
      ;[1 1 1] Sinon se contente de tomber (vitesse x-1 car le coco chute en -Z chez moi)
      (Transformation|AddActorWorldOffset (Math|Vector|MakeVector 0.0 0.0 (* (Variables|Movements|GetSpeed) -1.0)))))
  (return))

(fn FPopUpScore
  (params (Score :type Integer%20%28by%20ref%29) (isPerfect :type Boolean))
  (bind _returnvalue (Game|SpawnActorfromClass "/Game/03_Vaihiria/Cocos/BP_PopUpScore_Coco.BP_PopUpScore_Coco_C" (Math|Transform|MakeTransform (Transformation|GetActorLocation) "0, 0, 0" "1,1,1") "Undefined" 0 0))
  (Default|FPopUpParameter _returnvalue isPerfect Score)
  (return))

(fn FCocoTouched
  (params (IsPerfect :type Boolean))
  (bind _returnvalue (Transformation|GetActorLocation))
  (bind _returnvalue_2 (Transformation|GetActorLocation))
  (bind _gameode (Variables|Refs|GetGameode))
  (bind _gameode_2 (Variables|Refs|GetGameode))
  (bind _cocotype (Variables|Initialize|GetCocoType))
  (bind _scoremultiplier (Variables|Scoring|GetScoreMultiplier))
  (bind _scoremultiplier_2 (Variables|Scoring|GetScoreMultiplier))
  (bind _cocotype_2 (Variables|Initialize|GetCocoType))
  (bind _returnvalue_3 (Utilities|Select :Index _cocotype :NewEnumerator0 22 :NewEnumerator1 55 :NewEnumerator2 44))
  (bind _returnvalue_4 (Utilities|Select :Index _cocotype_2 :NewEnumerator0 20 :NewEnumerator1 50 :NewEnumerator2 40))
  (bind _hud_ingame (Variables|/Game/03_Vaihiria/Gamemode/GM_Vaihiria.GM_Vaihiria_C|GetHUD_inGame _gameode_2))
  (bind _hud_ingame_2 (Variables|/Game/03_Vaihiria/Gamemode/GM_Vaihiria.GM_Vaihiria_C|GetHUD_inGame _gameode))
  (bind _returnvalue_5 (* _returnvalue_4 _scoremultiplier))
  (bind _returnvalue_6 (* _returnvalue_3 _scoremultiplier_2))
  ;[1 1 1] CocoCliqué
  (if (Variables|State|GetbCanTouchCoco)
    (if IsPerfect
      (Class|BPIVaihiria|GMAddScore(Message) (Game|GetGameMode) _returnvalue_6 true (Components|GetOwner))
      (Variables|/Game/03_Vaihiria/Gamemode/GM_Vaihiria.GM_Vaihiria_C|SetTouchedPopUp _gameode_2 0)
      (Default|EventTextAnimScorePerfect _hud_ingame)
      (Default|IncreasePerfectCount _hud_ingame)
      (Scoring|FPopUpScore _returnvalue_6 true)
      (bind _returnvalue_7 (Game|SpawnActorfromClass "/Game/03_Vaihiria/Cocos/BP_FxCocoDestroy.BP_FxCocoDestroy_C" (Math|Transform|MakeTransform (Math|Vector|MakeVector (.x _returnvalue_2) (.y _returnvalue_2) (.z _returnvalue_2)) (Transformation|GetActorRotation) "0.500000,0.500000,0.500000") "Undefined" 0 0))
      (Default|SetFlipbook _returnvalue_7 (Utilities|Select :Index (Variables|Initialize|GetCocoType) :NewEnumerator0 "/Game/03_Vaihiria/Cocos/Art/FX/PFB_CocoNormal_Vaihiria.PFB_CocoNormal_Vaihiria" :NewEnumerator1 "/Game/03_Vaihiria/Cocos/Art/FX/PFB_CocoGold_Vaihiria.PFB_CocoGold_Vaihiria" :NewEnumerator2 "/Game/03_Vaihiria/Cocos/Art/FX/PFB_CocoRainbow_Vaihiria.PFB_CocoRainbow_Vaihiria"))
      (Audio|SpawnSound2D "/Game/03_Vaihiria/Cocos/SFX/S_TouchPerfect_Coco.S_TouchPerfect_Coco" 1.0 1.0 0.0 0)
      (else
        (Class|BPIVaihiria|GMAddScore(Message) (Game|GetGameMode) _returnvalue_5 false (Components|GetOwner))
        (Variables|/Game/03_Vaihiria/Gamemode/GM_Vaihiria.GM_Vaihiria_C|SetTouchedPopUp (Variables|Refs|GetGameode) 1)
        (Default|EventTextAnimScoreNice _hud_ingame_2)
        (Default|ResetCount _hud_ingame_2)
        (Scoring|FPopUpScore _returnvalue_5 false)
        (bind _returnvalue_8 (Game|SpawnActorfromClass "/Game/03_Vaihiria/Cocos/BP_FxCocoDestroy.BP_FxCocoDestroy_C" (Math|Transform|MakeTransform (Math|Vector|MakeVector (.x _returnvalue) (.y _returnvalue) (.z _returnvalue)) "0, 0, 0" "0.500000,0.500000,0.500000") "Undefined" 0 0))
        (Default|SetFlipbook _returnvalue_8 (Utilities|Select :Index (Variables|Initialize|GetCocoType) :NewEnumerator0 "/Game/03_Vaihiria/Cocos/Art/FX/PFB_CocoNormal_Vaihiria.PFB_CocoNormal_Vaihiria" :NewEnumerator1 "/Game/03_Vaihiria/Cocos/Art/FX/PFB_CocoGold_Vaihiria.PFB_CocoGold_Vaihiria" :NewEnumerator2 "/Game/03_Vaihiria/Cocos/Art/FX/PFB_CocoRainbow_Vaihiria.PFB_CocoRainbow_Vaihiria"))
        (Audio|SpawnSound2D "/Game/03_Vaihiria/Cocos/SFX/S_TouchNice_Coco.S_TouchNice_Coco" 1.0 1.0 0.0 0)))
    (Audio|SpawnSound2D "/Game/03_Vaihiria/Cocos/SFX/S_CocoPoofReverse_Coco.S_CocoPoofReverse_Coco" 1.0 0.8 0.0 0)
    (CallFunction|CocoReinitialize)
    (return)))

(fn FSetMultiplierSprite
  (Rendering|Components|Sprite|SetSprite (Variables|Default|GetMultiplier) (Utilities|Select :Index (- (Variables|Scoring|GetScoreMultiplier) 1) :Option%200 0 :Option%201 "/Game/03_Vaihiria/UI/MainMenu/Texture/SP_Multiplicateur2_Vaihiria.SP_Multiplicateur2_Vaihiria" :Option%202 "/Game/03_Vaihiria/UI/MainMenu/Texture/SP_Multiplicateur3_Vaihiria.SP_Multiplicateur3_Vaihiria" :Option%203 "/Game/03_Vaihiria/UI/MainMenu/Texture/SP_Multiplicateur4_Vaihiria.SP_Multiplicateur4_Vaihiria" :Option%204 "/Game/03_Vaihiria/UI/MainMenu/Texture/SP_Multiplicateur5_Vaihiria.SP_Multiplicateur5_Vaihiria"))
  (return))

(fn FShowHidePerfectTiming
  (params (Hide :type Boolean))
  (Development|SetHiddeninGame (Variables|Default|GetPerfectTimed) Hide false)
  (return))