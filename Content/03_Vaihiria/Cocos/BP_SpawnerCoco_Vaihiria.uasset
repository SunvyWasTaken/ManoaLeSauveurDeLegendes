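; Coconut spawner for the Vaihiria game that pre-spawns a pool of BP_Coco_Vaihiria actors on BeginPlay.
; A looping timer sends the first non-falling coco from one of three random start positions with a weighted random type.
; Split requests send another pooled coco turning toward a target.
; Difficulty events shorten the spawn delay, fever time is forwarded to falling cocos, and EndGame clears the spawn and fall timers.
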(event Custom|SpawnCoco
  ;[1 1 1] Timer qui spawn les cocos
  (bind (_whichcoco _startposition _cocotype) (Utilities|SetCoco)
    (:End
      (Class|BPIVaihiria|CocoGo(Message) (Utilities|Array|Get(acopy) (Variables|Ref|GetCocoArray) _whichcoco) _startposition _cocotype false false "0, 0, 0" 1))))

(event Custom|SetSpawnerCoco
  ;[1 1 1] Relance le timer du spawner avec le delay désiré)
  (Utilities|Time|ClearandInvalidateTimerbyHandle (Variables|Timer|GetTimerHandle))
  (bind _returnvalue (Utilities|Time|SetTimerbyEvent (delegate Custom|SpawnCoco) (Variables|Timer|GetSpawnDelay) true))
  (Variables|Timer|SetTimerHandle _returnvalue))

(event EventBeginPlay
  ;[1 1 1] BeginPlay: Spawn les cocos et les range dans un array
  (for _index (range 0 (Variables|Timer|GetCocoSpawned))
    (bind _returnvalue (Game|SpawnActorfromClass "/Game/03_Vaihiria/Cocos/BP_Coco_Vaihiria.BP_Coco_Vaihiria_C" (Math|Transform|MakeTransform (Utilities|Array|Get(acopy) (Variables|Movements|GetStartPosition) 1) "0,90.000000, 0" "1,1,1") "Undefined" self 0))
    (Utilities|Array|Add (Variables|Ref|GetCocoArray) _returnvalue))
  ;[1 1 1] Lance le Spawn
  (CallFunction|SetSpawnerCoco))

(event EventEndGame
  (params (Spawner :type Actor%20Object%20Reference))
  ;[1 1 1] EndGame
  (Utilities|Time|ClearandInvalidateTimerbyHandle (Variables|Timer|GetTimerHandle))
  (for _array_element (Variables|Ref|GetCocoArray)
    (Utilities|Time|ClearTimerbyFunctionName _array_element "FallTimer")))

(event EventSpawnerSetDifficulty
  ;[1 1 1] SetDifficulty
  ;;[1 1 1] 3.5
  (Variables|Timer|SetSpawnDelay (- (Variables|Timer|GetSpawnDelay) (Variables|Timer|GetSpawnDelayReduction)))
  (CallFunction|SetSpawnerCoco))

(event EventSpawnerFeverTime
  ;[1 1 1] FeverTime
  (Development|PrintString "FeverTimeSpawnerrrrr" true true "(R=1.000000,G=0.000000,B=0.056943,A=1.000000)")
  (for _array_element (Variables|Ref|GetCocoArray)
    (if (Variables|/Game/03_Vaihiria/Cocos/BP_Coco_Vaihiria.BP_Coco_Vaihiria_C|GetbIsFalling _array_element)
      (Default|SpawnerFeverTime _array_element))))

(event EventSpawnerandCocoSplitCoco
  (params (StartPosition :type Vector :default "0, 0, 0") (TargetLocation :type Vector :default "0, 0, 0") (FeverTime :type Boolean) (Multiplier :type Integer))
  ;[1 1 1] Qd un coco multicolore est a une intersection, spawn un deuxieme coco
  (bind _whichcoco (Utilities|SetWhichCoco)
    (:End
      (Class|BPIVaihiria|CocoGo(Message) (Utilities|Array|Get(acopy) (Variables|Ref|GetCocoArray) _whichcoco) StartPosition (Utilities|Select :Index (Math|Random|RandomIntegerinRange 0 9) :Option%200 "NewEnumerator0" :Option%201 "NewEnumerator0" :Option%202 "NewEnumerator0" :Option%203 "NewEnumerator0" :Option%204 "NewEnumerator0" :Option%205 "NewEnumerator0" :Option%206 "NewEnumerator0" :Option%207 "NewEnumerator0" :Option%208 "NewEnumerator0" :Option%209 "NewEnumerator1") true FeverTime TargetLocation Multiplier))))

(fn ConstructionScript)