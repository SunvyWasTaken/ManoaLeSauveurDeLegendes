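; Game mode for the Vaihiria coconut mini-game, handling score, misses, audio, HUD and game end.
; Score thresholds trigger the SetDifficulty macro, which raises spawner difficulty up to a cap and toggles the track intersections.
; A perfect-hit streak triggers the spawner's fever time, while missed coconuts drain three HUD hearts.
; Reaching the top score or losing the last heart stops the spawner and shows the star-rated end menu.
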(event EventEndGame
  (params (Spawner :type Actor%20Object%20Reference))
  ;[1 1 1] Compte le nombre de cocos loupés
  (Class|BPIVaihiria|EndGame(Message) Spawner)
  (Components|Activation|Deactivate (Variables|Default|GetMusique))
  (Audio|SpawnSound2D "/Game/02_Teura/Gamemode/SFX/S_Music_EndGame_Teura.S_Music_EndGame_Teura" 1.0 1.0 0.0 0)
  (bind _returnvalue (UserInterface|CreateWidget "/Game/00_Metajeu/Widgets/WBP_MenuVictoire2.WBP_MenuVictoire2_C" 0 (Variables|Scoring&Difficulty|GetScore) 1000 2000 3000 0.00018))
  (UserInterface|Viewport|AddtoViewport _returnvalue 0))

(event EventBeginPlay
  ;[1 1 1] BeginPlay
  (bind _returnvalue (Audio|SpawnSound2D "/Game/03_Vaihiria/Gamemode/SFX/S_Theme_Vaihiria.S_Theme_Vaihiria" 1.0 1.0 0.0 0))
  (Variables|Default|SetMusique _returnvalue)
  (Audio|SpawnSound2D "/Game/02_Teura/Level/Background/Terrain/S_Waves.S_Waves" 0.6 1.0 0.0 0)
  (Audio|SpawnSound2D "/Game/03_Vaihiria/Gamemode/SFX/S_WindCoco.S_WindCoco" 1.0 1.0 0.0 0)
  (Class|PlayerController|ActivateTouchInterface (Game|GetPlayerController 0))
  (Variables|Scoring&Difficulty|SetLevel (Variables|Scoring&Difficulty|GetLevelAdded))
  (bind _returnvalue_2 (UserInterface|CreateWidget "/Game/03_Vaihiria/UI/InGame/WBP_HUD_InGame.WBP_HUD_InGame_C"))
  (bind _output_get (Variables|UI|SetHUD_inGame _returnvalue_2))
  (UserInterface|Viewport|AddtoViewport _output_get 0)
  ;;[1 0 0] A remplacer si possible
  (bind _outactors (Actor|GetAllActorsOfClass "/Game/03_Vaihiria/Level/Intersections/BP_SwitchIntersection_Vaihiria.BP_SwitchIntersection_Vaihiria_C"))
  (Utilities|FlowControl|Delay 1.0)
  (bind _output_get_2 (Variables|Refs|SetIntersections _outactors))
  (for _array_element _output_get_2
    (Class|BPIVaihiria|SwitchIntersectionSwitch(Message) _array_element)))

(event EventGMAddScore
  (params (ScoreAdded :type Integer) (Perfect :type Boolean) (Spawner :type Actor%20Object%20Reference))
  ;[1 1 1] AddScore
  (Variables|Scoring&Difficulty|SetScore (+ ScoreAdded (Variables|Scoring&Difficulty|GetScore)))
  (Default|EventComboAnim (Variables|UI|GetHUD_inGame))
  (if (>= (Variables|Scoring&Difficulty|GetScore) (Variables|Scoring&Difficulty|GetLevel))
    (if (>= (Variables|Scoring&Difficulty|GetScore) 3000)
      (Utilities|FlowControl|DoOnce false
        (:Completed
          (CallFunction|EndGame Spawner)))
      (else
        (Utilities|SetDifficulty Spawner
          (:else
            (Development|PrintString (Utilities|String|ToString(Integer) (Variables|Scoring&Difficulty|GetPerfectCounter)))
            (Math|Integer|IncrementInt (Variables|Scoring&Difficulty|GetPerfectCounter) :!label _label
              (:%20%20
                (if (== (Variables|Scoring&Difficulty|GetPerfectCounter) 5)
                  (Utilities|FlowControl|Delay 0.5)
                  (Class|BPIVaihiria|SpawnerFeverTime(Message) Spawner)
                  (Variables|Scoring&Difficulty|SetPerfectCounter 0))))))))
    (elif Perfect
      (goto _label)
      (else
        (Variables|Scoring&Difficulty|SetPerfectCounter 0)))))

(event EventGMCocoLost
  (params (Spawner :type Actor%20Object%20Reference))
  (bind _hud_ingame (Variables|UI|GetHUD_inGame))
  (bind _hud_ingame_2 (Variables|UI|GetHUD_inGame))
  ;[1 1 1] Compte le nombre de cocos loupés
  (Audio|SpawnSound2D "/Game/03_Vaihiria/Gamemode/SFX/S_TooBad_Coco.S_TooBad_Coco" 1.0 1.0 0.0 0)
  (Variables|EndGame|SetCocoMissed (+ (Variables|EndGame|GetCocoMissed) 1))
  (Variables|Refs|SetTouchedPopUp 2)
  (Default|EventComboAnim (Variables|UI|GetHUD_inGame))
  (if (== (Variables|EndGame|GetCocoMissed) 0)
    (Variables|Scoring&Difficulty|SetPerfectCounter 0)
    (Default|ResetCount (Variables|UI|GetHUD_inGame))
    (elif (== (Variables|EndGame|GetCocoMissed) 2)
      (Variables|Scoring&Difficulty|SetPerfectCounter 0)
      (Default|ResetCount _hud_ingame)
      (Default|AnimeCoeur01 _hud_ingame)
      (elif (== (Variables|EndGame|GetCocoMissed) 4)
        (Variables|Scoring&Difficulty|SetPerfectCounter 0)
        (Default|ResetCount _hud_ingame_2)
        (Default|AnimeCoeur2 _hud_ingame_2)
        (elif (== (Variables|EndGame|GetCocoMissed) 6)
          (Utilities|FlowControl|DoOnce false
            (:Completed
              (Default|AnimeCoeur3 (Variables|UI|GetHUD_inGame))
              (CallFunction|EndGame Spawner))))))))

(fn ConstructionScript)