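; End zone for the Vaihiria level's timing mini-game, where the player taps or clicks the sprite as a coco arrives.
; Nested overlap spheres grade the tap as normal or perfect, scaling the sprite during the perfect window and briefly dimming it afterwards.
; The first coco to reach any perfect zone registers with GM_Vaihiria and opens the objective widget.
; A LooseBox overlap reinitializes missed cocos, notifies the game mode and shakes the camera.
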(event OnComponentBeginOverlap(Sphere)
  (params (OverlappedComponent :type Primitive%20Component%20Object%20Reference) (OtherActor :type Actor%20Object%20Reference) (OtherComp :type Primitive%20Component%20Object%20Reference) (OtherBodyIndex :type Integer) (bFromSweep :type Boolean) (SweepResult :type Hit%20Result%20Structure%20%28by%20ref%29))
  ;[1 1 1] Coco arrive a portée et peut etre cliqué
  (if (== (Utilities|GetClass OtherActor) "/Game/03_Vaihiria/Cocos/BP_Coco_Vaihiria.BP_Coco_Vaihiria_C")
    (Variables|State|SetbIsCocoAtRange true)
    (Variables|Ref|SetCoco OtherActor)))

(event OnClicked(PaperSprite)
  (params (TouchedComponent :type Primitive%20Component%20Object%20Reference) (ButtonPressed :type Key%20Structure :default "None"))
  ;[1 1 1] Touch
  (if (Variables|State|GetbIsCocoAtRange)
    (if (Variables|State|GetbCocoAtPerfectRange)
      (Class|BPIVaihiria|CocoTouchCoco(Message) (Variables|Ref|GetCoco) true)
      (else
        (Class|BPIVaihiria|CocoTouchCoco(Message) (Variables|Ref|GetCoco) false)))
    (Variables|State|SetbIsCocoAtRange false)
    (Variables|State|SetbCocoAtPerfectRange false)))

(event OnComponentBeginOverlap(SpherePerfect)
  (params (OverlappedComponent :type Primitive%20Component%20Object%20Reference) (OtherActor :type Actor%20Object%20Reference) (OtherComp :type Primitive%20Component%20Object%20Reference) (OtherBodyIndex :type Integer) (bFromSweep :type Boolean) (SweepResult :type Hit%20Result%20Structure%20%28by%20ref%29))
  ;[1 1 1] Coco est a portée pr faire un perfect
  (if (== (Utilities|GetClass OtherActor) "/Game/03_Vaihiria/Cocos/BP_Coco_Vaihiria.BP_Coco_Vaihiria_C")
    (if (Variables|State|GetbFirstCoco)
      (Utilities|FlowControl|DoOnce false
        (:Completed
          (Variables|State|SetbCocoAtPerfectRange true)
          (bind _asbp_coco_vaihiria (Utilities|Casting|CastToBP_Coco_Vaihiria OtherActor))
          (Default|FShowHidePerfectTiming _asbp_coco_vaihiria false)
          (CallFunction|FScalePaperSprite)
          (bind _asgm_vaihiria (Utilities|Casting|CastToGM_Vaihiria (Game|GetGameMode)))
          (bind _output_get (Variables|Ref|SetFirstCoco _asbp_coco_vaihiria))
          (Variables|/Game/03_Vaihiria/Gamemode/GM_Vaihiria.GM_Vaihiria_C|SetFirstCoco_Ref _asgm_vaihiria _output_get)
          (bind _outactors (Actor|GetAllActorsOfClass "BP_EndZone_Vaihiria_C"))
          (for _array_element _outactors
            (Variables|BP_EndZone_Vaihiria_C|SetbFirstCoco _array_element false))
          (Utilities|FlowControl|Delay 0.05)
          (bind _returnvalue (UserInterface|CreateWidget "/Game/03_Vaihiria/UI/Onboarding/WBP_Objectif_Vaihiria.WBP_Objectif_Vaihiria_C"))
          (UserInterface|Viewport|AddtoViewport _returnvalue 0)))
      (else
        (Variables|State|SetbCocoAtPerfectRange true)
        (bind _asbp_coco_vaihiria_2 (Utilities|Casting|CastToBP_Coco_Vaihiria OtherActor))
        (Default|FShowHidePerfectTiming _asbp_coco_vaihiria_2 false)
        (CallFunction|FScalePaperSprite)))))

(event OnComponentEndOverlap(SpherePerfect)
  (params (OverlappedComponent :type Primitive%20Component%20Object%20Reference) (OtherActor :type Actor%20Object%20Reference) (OtherComp :type Primitive%20Component%20Object%20Reference) (OtherBodyIndex :type Integer))
  (bind _scalebase (Variables|Effect|GetScaleBase))
  ;[1 1 1] On ne peut plus faire de perfect
  (if (== (Utilities|GetClass OtherActor) "/Game/03_Vaihiria/Cocos/BP_Coco_Vaihiria.BP_Coco_Vaihiria_C")
    (Variables|State|SetbCocoAtPerfectRange false)
    (bind _asbp_coco_vaihiria (Utilities|Casting|CastToBP_Coco_Vaihiria OtherActor))
    (Default|FShowHidePerfectTiming _asbp_coco_vaihiria true)
    (Transformation|SetRelativeScale3D (Variables|Default|GetPaperSprite) (Math|Vector|MakeVector _scalebase _scalebase _scalebase))
    (Variables|/Game/03_Vaihiria/Cocos/BP_Coco_Vaihiria.BP_Coco_Vaihiria_C|SetbCanTouchCoco _asbp_coco_vaihiria false)
    (Sprite|SetSpriteColor (Variables|Default|GetPaperSprite) "(R=0.000000,G=0.000000,B=0.000000,A=0.744000)")
    (Utilities|FlowControl|Delay 0.4)
    (Variables|/Game/03_Vaihiria/Cocos/BP_Coco_Vaihiria.BP_Coco_Vaihiria_C|SetbCanTouchCoco _asbp_coco_vaihiria true)
    (Sprite|SetSpriteColor (Variables|Default|GetPaperSprite) "(R=1.000000,G=1.000000,B=1.000000,A=1.000000)")))

(event OnComponentBeginOverlap(LooseBox)
  (params (OverlappedComponent :type Primitive%20Component%20Object%20Reference) (OtherActor :type Actor%20Object%20Reference) (OtherComp :type Primitive%20Component%20Object%20Reference) (OtherBodyIndex :type Integer) (bFromSweep :type Boolean) (SweepResult :type Hit%20Result%20Structure%20%28by%20ref%29))
  ;[1 1 1] On a raté le coco, qui se reinitialise
  (if (== (Utilities|GetClass OtherActor) "/Game/03_Vaihiria/Cocos/BP_Coco_Vaihiria.BP_Coco_Vaihiria_C")
    (Variables|Ref|SetCoco 0)
    (Variables|State|SetbIsCocoAtRange false)
    (Variables|State|SetbCocoAtPerfectRange false)
    (Utilities|FlowControl|Delay 0.2)
    (Class|BPIVaihiria|CocoReinitialize(Message) OtherActor)
    (Class|BPIVaihiria|GMCocoLost(Message) (Game|GetGameMode))
    (Camera|PlayWorldCameraShake "/Game/02_Teura/Level/Camera/CS_KillEnnemi_Teura.CS_KillEnnemi_Teura_C" (Transformation|GetActorLocation) 0.0 5e+06)
    (Class|BPIVaihiria|GMCocoLost(Message) (Game|GetGameMode) (Components|GetOwner OtherActor))))

(event OnInputTouchBegin(PaperSprite)
  (params (FingerIndex :type ETouchIndex%20Enum :default "Touch1") (TouchedComponent :type Primitive%20Component%20Object%20Reference))
  ;[1 1 1] Touch
  (if (Variables|State|GetbIsCocoAtRange)
    (if (Variables|State|GetbCocoAtPerfectRange)
      (Class|BPIVaihiria|CocoTouchCoco(Message) (Variables|Ref|GetCoco) true)
      (else
        (Class|BPIVaihiria|CocoTouchCoco(Message) (Variables|Ref|GetCoco) false)))
    (Variables|State|SetbIsCocoAtRange false)
    (Variables|State|SetbCocoAtPerfectRange false)))

(fn ConstructionScript)

(fn FScalePaperSprite
  (bind _scalemax (Variables|Effect|GetScaleMax))
  ;[1 1 1] Changer taille coco
  (Transformation|SetRelativeScale3D (Variables|Default|GetPaperSprite) (Math|Vector|MakeVector _scalemax _scalemax _scalemax))
  (return))