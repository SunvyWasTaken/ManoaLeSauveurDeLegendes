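; Intersection for the Vaihiria level that sends a BP_Coco_Vaihiria across when it overlaps either end.
; Each side box messages the coco with the opposite box's location and the intersection's parent actor.
; Activation randomly picks one of two sprite tilts, but only one branch also shows the sprite and enables box collision.
; Deactivation hides the sprite and disables both boxes.
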(event OnComponentBeginOverlap(RightBox)
  (params (OverlappedComponent :type Primitive%20Component%20Object%20Reference) (OtherActor :type Actor%20Object%20Reference) (OtherComp :type Primitive%20Component%20Object%20Reference) (OtherBodyIndex :type Integer) (bFromSweep :type Boolean) (SweepResult :type Hit%20Result%20Structure%20%28by%20ref%29))
  ;[1 1 1] Si le coco touche box de droite, va a box de gauche
  (if (== (Utilities|GetClass OtherActor) "/Game/03_Vaihiria/Cocos/BP_Coco_Vaihiria.BP_Coco_Vaihiria_C")
    (Class|BPIVaihiria|CocoCrossIntersection(Message) OtherActor (Transformation|GetWorldLocation (Variables|Default|GetLeftBox)) (Actor|GetParentActor))))

(event OnComponentBeginOverlap(LeftBox)
  (params (OverlappedComponent :type Primitive%20Component%20Object%20Reference) (OtherActor :type Actor%20Object%20Reference) (OtherComp :type Primitive%20Component%20Object%20Reference) (OtherBodyIndex :type Integer) (bFromSweep :type Boolean) (SweepResult :type Hit%20Result%20Structure%20%28by%20ref%29))
  ;[1 1 1] Si le coco touche box de gauche, va a box de droite
  (if (== (Utilities|GetClass OtherActor) "/Game/03_Vaihiria/Cocos/BP_Coco_Vaihiria.BP_Coco_Vaihiria_C")
    (Class|BPIVaihiria|CocoCrossIntersection(Message) OtherActor (Transformation|GetWorldLocation (Variables|Default|GetRightBox)) (Actor|GetParentActor))))

(event EventIntersectionActivate
  ;[1 1 1] Intersection est changée
  ;;[1 1 1] Active la visibilité
  (if (Math|Random|RandomBool)
    (Transformation|SetRelativeRotation (Variables|Default|GetPaperSprite) "20.000000,90.000000,0.000000" false false)
    (Rendering|SetVisibility (Variables|Default|GetPaperSprite) true false)
    (Collision|SetCollisionEnabled (Variables|Default|GetLeftBox) "QueryOnly")
    (Collision|SetCollisionEnabled (Variables|Default|GetRightBox) "QueryOnly")
    (else
      (Transformation|SetRelativeRotation (Variables|Default|GetPaperSprite) "-20.000000,90.000000,0.000000" false false))))

(event EventIntersectionDeactivate
  ;[1 1 1] Intersection est changée
  ;;[1 1 1] Desactive la visibilité
  (Rendering|SetVisibility (Variables|Default|GetPaperSprite) false false)
  (Collision|SetCollisionEnabled (Variables|Default|GetLeftBox) "NoCollision")
  (Collision|SetCollisionEnabled (Variables|Default|GetRightBox) "NoCollision"))

(fn ConstructionScript)