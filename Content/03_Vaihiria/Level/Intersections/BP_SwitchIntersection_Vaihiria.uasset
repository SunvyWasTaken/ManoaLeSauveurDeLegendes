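; Vaihiria level actor that randomly switches between two intersections, held as child actors of BP_Intersection_Vaihiria.
; A switch call activates one and deactivates the other at random, and is ignored while IsCrossed flags a coco crossing.
; After the first switch, each call, even one repicking the same side, plays a HUD animation and map-change sound while briefly hiding the red path.
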(event EventBeginPlay
  (bind _asgm_vaihiria (Utilities|Casting|CastToGM_Vaihiria (Game|GetGameMode)))
  (bind _output_get (Variables|Refs|SetGamemode _asgm_vaihiria))
  (Variables|Refs|SetHud_InGame (Variables|/Game/03_Vaihiria/Gamemode/GM_Vaihiria.GM_Vaihiria_C|GetHUD_inGame _output_get)))

(event EventIntersectionSetifCrossed
  (params (Crossed :type Boolean))
  ;[1 1 1] Empeche le switch si un coco traverse une intersection
  (Variables|States|SetbIsCrossed Crossed))

(event EventSwitchIntersectionSwitch
  (bind _cheminrouge_ref (Variables|Refs|GetCheminRouge_Ref))
  ;[1 1 1] Randomizer
  (if (not (Variables|States|GetbIsCrossed))
    (if (Math|Random|RandomBool)
      (Class|BPIVaihiria|IntersectionActivate(Message) (Variables|/Script/Engine.ChildActorComponent|GetChildActor (Variables|Default|Get01)))
      (Class|BPIVaihiria|IntersectionDeactivate(Message) (Variables|/Script/Engine.ChildActorComponent|GetChildActor (Variables|Default|Get02)))
      (else
        (Class|BPIVaihiria|IntersectionDeactivate(Message) (Variables|/Script/Engine.ChildActorComponent|GetChildActor (Variables|Default|Get01)))
        (Class|BPIVaihiria|IntersectionActivate(Message) (Variables|/Script/Engine.ChildActorComponent|GetChildActor (Variables|Default|Get02)))))
    (if (Variables|States|GetFirstTime)
      (Variables|States|SetFirstTime false)
      (else
        (Default|Anime500 (Variables|/Game/03_Vaihiria/Gamemode/GM_Vaihiria.GM_Vaihiria_C|GetHUD_inGame (Variables|Refs|GetGamemode)))
        (Utilities|FlowControl|Delay 0.75)
        (Default|FShowHideRedPath _cheminrouge_ref false)
        (Audio|SpawnSound2D "/Game/03_Vaihiria/Level/Intersections/SFX/S_MapChange4_Coco.S_MapChange4_Coco" 1.0 1.0 0.0 0)
        (Utilities|FlowControl|Delay 1.0)
        (Default|FShowHideRedPath _cheminrouge_ref true)))))

(fn ConstructionScript
  (ChildActorComponent|SetChildActorClass (Variables|Default|Get01) "/Game/03_Vaihiria/Level/Intersections/BP_Intersection_Vaihiria.BP_Intersection_Vaihiria_C"))