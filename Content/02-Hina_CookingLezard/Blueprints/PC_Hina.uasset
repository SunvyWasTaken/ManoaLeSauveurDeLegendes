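; Player controller for the Hina lizard-cooking game, routing touch drags to whichever of three minigames is active.
; Minigame 1 moves the procedural cutter.
; Minigame 2 moves the palm and turns vertical swipe reversals, detected against a timer-sampled offset, into HUD temperature increases scaled by swipe length.
; Minigame 3 derives circular stirring direction from the yaw of a detector actor spawned at screen-center pixel coordinates in world space, aimed at the finger.
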(event Custom|IncreaseFire
  (params (IncrementRate :type Float%20%28single-precision%29))
  (Default|IncreaseTemperature (Variables|/Game/02-Hina_CookingLezard/Blueprints/GM_Hina.GM_Hina_C|GetHudRef (Variables|Default|GetGM_HinaRef)) IncrementRate))

(event Custom|AssignLoc
  (bind (_locationx _locationy) (Class|PlayerController|GetInputTouchState "Touch1"))
  ;[1 1 1] Required for Minigame 2 (If deleted Minigame 2 won't update temperature)
  (Variables|Default|SetPreviousLocalisation (.Y (Math|Vector2D|BreakVector2D (- (Variables|Default|GetTouchStart2D) (Math|Vector2D|MakeVector2D _locationx _locationy))))))

(event Custom|MiniGame3
  (bind _rotationdetectorref (Variables|Default|GetRotationDetectorRef))
  (bind _returnvalue (CallFunction|FindALookatTouch _rotationdetectorref))
  ;[1 1 1] MiniGame 3
  ;;[1 1 1] Update l'orientation
  (Variables|Default|SetActualYaw (.yaw _returnvalue))
  (Transformation|SetActorRotation (Variables|Default|GetRotationDetectorRef) (Math|Rotator|MakeRotator 0.0 0.0 (.yaw _returnvalue)))
  (Variables|Default|SetbTourne? true) ; on move, ça tourne
  ;;[1 1 1] Compare l'angle actuel et l'ancien angle de l'acteur rotation pour voir dans quel sens il tourne
  (if (> (.yaw (Transformation|GetActorRotation (Variables|Default|GetRotationDetectorRef))) (Variables|Default|GetAncienYaw))
    (Variables|Default|SetTourneADroite true)
    (else
      (Variables|Default|SetTourneADroite false)))
  (Variables|Default|SetAncienYaw (.yaw (Transformation|GetActorRotation (Variables|Default|GetRotationDetectorRef))))
  (Audio|PlaySound2D "/Game/02-Hina_CookingLezard/SFX/SC_whip.SC_whip" 1.0 1.0 0.0 0 0))

(event Custom|Minigame2
  (bind (_locationx _locationy) (Class|PlayerController|GetInputTouchState "Touch1"))
  (bind _returnvalue (Math|Vector2D|MakeVector2D _locationx _locationy))
  ;[1 1 1] MiniGame 2 Check position
  (if (> (Math|Vector2D|Vector2DLength (- (Variables|Default|GetTouchStart2D) _returnvalue)) 5e+01)
    (if (not (> (Math|Float|Absolute(Float) (.X (Math|Vector2D|BreakVector2D (- (Variables|Default|GetTouchStart2D) _returnvalue)))) (Math|Float|Absolute(Float) (.Y (Math|Vector2D|BreakVector2D (- (Variables|Default|GetTouchStart2D) _returnvalue))))))
      (Variables|Default|SetLocalisationY (.Y (Math|Vector2D|BreakVector2D (- (Variables|Default|GetTouchStart2D) _returnvalue))))
      (if (Variables|Default|GetbIsSwipingUp)
        ;[1 1 1] DetectionSwiping Up
        (if (> (Variables|Default|GetPreviousLocalisation) (Variables|Default|GetLocalisationY))
          (Variables|Default|SetbIsSwipingUp false)
          (Utilities|FlowControl|Sequence
            (:then_0
              (Utilities|FlowControl|DoOnce false :!label _label
                (:Completed
                  (Variables|Default|SetTouchEnd2D _returnvalue)
                  ;[1 1 1] Increase temperature depending on the movement
                  (CallFunction|IncreaseFire (/ (Math|Float|Absolute(Float) (Math|Vector2D|Vector2DLength (- (Variables|Default|GetTouchStart2D) (Variables|Default|GetTouchEnd2D)))) 1e+04))
                  (Variables|Default|SetTouchStart2D (Variables|Default|GetTouchEnd2D) :!label _label_2))))
            (:then_1
              (goto _label_3 Reset))))
        (else
          ;[1 1 1] Detection swiping Down
          (if (> (Variables|Default|GetLocalisationY) (Variables|Default|GetPreviousLocalisation))
            (Variables|Default|SetbIsSwipingUp true)
            (Utilities|FlowControl|Sequence
              (:then_0
                (Utilities|FlowControl|DoOnce false :!label _label_3
                  (:Completed
                    (Variables|Default|SetTouchEnd2D _returnvalue)
                    (CallFunction|IncreaseFire (/ (Math|Float|Absolute(Float) (Math|Vector2D|Vector2DLength (- (Variables|Default|GetTouchStart2D) (Variables|Default|GetTouchEnd2D)))) 1e+04))
                    (goto _label_2))))
              (:then_1
                (goto _label Reset)))))))))

(event EventBeginPlay
  (bind _outactors (Actor|GetAllActorsOfClass "/Game/02-Hina_CookingLezard/Blueprints/CuttingMiniGame/BP_ProceduralCutter.BP_ProceduralCutter_C"))
  (Variables|Default|SetProceduralCutterRef (Utilities|Array|Get(acopy) _outactors))
  (bind _asgm_hina (Utilities|Casting|CastToGM_Hina (Game|GetGameMode)))
  (Variables|Default|SetGM_HinaRef _asgm_hina)
  (bind _outactors_2 (Actor|GetAllActorsOfClass "/Game/02-Hina_CookingLezard/Blueprints/FireMiniGame/BP_Palme.BP_Palme_C"))
  (Variables|Default|SetBP_PalmeRef (Utilities|Array|Get(acopy) _outactors_2))
  ;[1 1 1] Prend la resolution de l'écran du joueur
  (bind _returnvalue (Settings|GetGameUserSettings))
  (bind _output_get (Variables|Default|SetScreenResolution (Class|GameUserSettings|GetScreenResolution _returnvalue)))
  ;[1 1 1] Spawn un actor en fonction de la resolution de l'écran pour que ses coordonée in world corespondent au coordoner de l'écran
  (bind _returnvalue_2 (Game|SpawnActorfromClass "/Game/02-Hina_CookingLezard/Blueprints/MixMiniGame/BP_RotationDetector_Hina.BP_RotationDetector_Hina_C" (Math|Transform|MakeTransform (Math|Vector|MakeVector (Math|Conversions|ToFloat(Integer) (/ (.x _output_get) 2)) (Math|Conversions|ToFloat(Integer) (/ (.y _output_get) 2)) 4e+03) "0, 0, 0" "1,1,1") "Undefined" self 0))
  (Variables|Default|SetRotationDetectorRef _returnvalue_2))

(event Input|TouchEvents|InputTouch
  (params (Location :type Vector) (FingerIndex :type ETouchIndex%20Enum))
  ;[1 1 1] Send the touch movement to the procedural cutter
  (:Pressed
    (Variables|Default|SetTouchStart2D (Math|Vector2D|MakeVector2D (.x Location) (.y Location))))
  (:Moved
    (Variables|Default|SetFingerLoc (Math|Vector2D|MakeVector2D (.x Location) (.y Location)))
    (if (Variables|Default|GetbCanPlay)
      (switch int (Variables|/Game/02-Hina_CookingLezard/Blueprints/GM_Hina.GM_Hina_C|GetActualMiniGame (Variables|Default|GetGM_HinaRef))
        (:1
          (Default|MoveCutter (Variables|Default|GetProceduralCutterRef) (Math|Vector2D|MakeVector2D (.x (Variables|Default|GetFingerLoc)) (.y (Variables|Default|GetFingerLoc)))))
        (:2
          (CallFunction|Minigame2)
          (Default|MovePalme (Variables|Default|GetBP_PalmeRef))
          ;[1 1 1] Required for Minigame 2 (If deleted Minigame 2 won't update temperature)
          (Utilities|FlowControl|DoOnce false
            (:Completed
              (Utilities|Time|SetTimerbyEvent (delegate Custom|AssignLoc) 0.02 true))))
        (:3
          (CallFunction|MiniGame3))))))

(fn ConstructionScript)

(fn FindALookatTouch
  (params (Target :type Actor%20Object%20Reference))
  (bind _returnvalue (Transformation|GetActorLocation Target))
  (bind (_locationx _locationy) (Class|PlayerController|GetInputTouchState "Touch1"))
  (return (Math|Rotator|FindLookatRotation (Math|Vector|MakeVector (.x _returnvalue) (.y _returnvalue) 0.0) (Math|Vector|MakeVector _locationx _locationy 0.0))))