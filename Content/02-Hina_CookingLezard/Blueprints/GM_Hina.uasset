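; Game mode for Hina's cooking game, chaining three timed minigames: food cutting, a BP_Palme time-in-zone challenge and pot stirring.
; LaunchGame caches scene actors and creates onboarding and HUD widgets, while StartMinigame runs the countdown and per-second timer.
; SwitchMinigame blends cameras and HUD pages between stages, and a looping timer scores stirring in the required direction.
; ScoreCalculator awards one star per threshold beaten, shown on the final victory menu.
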(event Custom|DoesItInTheRightSens
  ;[1 1 1] Score Minigame 3
  ;;[1 1 1] Verifie si le joueur est entrain tourner et qu'il le fait dans le bon sens
  (bind _aspc_hina (Utilities|Casting|CastToPC_Hina (Game|GetPlayerController 0)))
  (if (Variables|/Game/02-Hina_CookingLezard/Blueprints/PC_Hina.PC_Hina_C|GetbTourne? _aspc_hina)
    (if (Math|Boolean|Equal(Boolean) (Variables|/Game/02-Hina_CookingLezard/Blueprints/PC_Hina.PC_Hina_C|GetTourneADroite _aspc_hina) (Variables|Default|GetSensASuivre))
      ;;[1 1 1] Ajoute du temps en fontion du rafraichisement du timer by event
      (bind _output_get (Variables|Default|SetTempsDeBonTouillage (+ (Variables|Default|GetTempsDeBonTouillage) (Variables|Default|GetRefreshRate))))
      (Variables|Score|SetScoreMiniGame3 (Math|Float|Truncate _output_get))
      (Default|UpdateHUDTempsDeTouille (Variables|Default|GetHudRef) _output_get))))

(event Custom|StartMinigame
  (Utilities|FlowControl|Delay 1.0)
  (bind _returnvalue (UserInterface|CreateWidget "/Game/02-Hina_CookingLezard/Widgets/WBP_CountDown.WBP_CountDown_C" (Game|GetPlayerController 0)))
  (UserInterface|Viewport|AddtoViewport _returnvalue 0)
  (Utilities|FlowControl|Delay 4.0)
  (Variables|/Game/02-Hina_CookingLezard/Blueprints/PC_Hina.PC_Hina_C|SetbCanPlay (Variables|Default|GetPC_HinaRef) true)
  (switch int (Variables|Default|GetActualMiniGame)
    (:1
      (Variables|Timer|SetTimeRemaining (Variables|Timer|GetMaxTimeMiniGame1))
      (Default|TriggerFoodMovement (Variables|Default|GetFoodSelectorRef))
      (Audio|Components|Audio|Play (Variables|Default|Getmusic) 0.0))
    (:2
      (Variables|Timer|SetTimeRemaining (Variables|Timer|GetMaxTimeMiniGame2)))
    (:3
      (Variables|Timer|SetTimeRemaining (Variables|Timer|GetMaxTimeMiniGame3))
      (CallFunction|CalculeScoreMiniGame3)))
  (Default|Timer (Variables|Default|GetHudRef) (Variables|Timer|GetTimeRemaining))
  (bind _returnvalue_2 (Utilities|Time|SetTimerbyEvent (delegate Custom|Timer) 1.0 true))
  (Variables|Timer|SetTimerHandle _returnvalue_2))

(event Custom|PlayWidgetAnims
  (params (AnimToPlay :type Integer))
  (Default|PlayAnim (Variables|Default|GetOnboardingRef) AnimToPlay))

(event Custom|DegageCaillouOnBoard
  (Default|TriggerFoodMovement (Variables|Default|GetFoodSelectorOnboardRef)))

(event Custom|CouteauClick
  (Default|CouteauClicked (Variables|Default|GetOnboardingRef)))

(event Custom|Timer
  (bind _result (Math|Integer|DecrementInt (Variables|Timer|GetTimeRemaining))
    (:%20%20
      (Default|Timer (Variables|Default|GetHudRef) _result)
      (if (< (Variables|Timer|GetTimeRemaining) 1)
        (Utilities|Time|ClearandInvalidateTimerbyHandle (Variables|Timer|GetTimerHandle))
        (Default|PlayAnim (Variables|Default|GetOnboardingRef) 2)
        (Variables|/Game/02-Hina_CookingLezard/Blueprints/PC_Hina.PC_Hina_C|SetbCanPlay (Variables|Default|GetPC_HinaRef) false)
        (Utilities|FlowControl|Delay 3.0)
        (CallFunction|ScoreCalculator)
        (Math|Integer|IncrementInt (Variables|Default|GetActualMiniGame))))))

(event Custom|Switch%20Minigame
  (if (< (Variables|Default|GetActualMiniGame) 4)
    (switch int (Variables|Default|GetActualMiniGame)
      (:1
        (Class|WidgetSwitcher|SetActiveWidgetIndex (Variables|/Game/02-Hina_CookingLezard/Widgets/WBP_IGHUD.WBP_IGHUD_C|GetHUDWidgetSwitcher (Variables|Default|GetHudRef))))
      (:2
        (Variables|/Game/02-Hina_CookingLezard/Blueprints/CuttingMiniGame/BP_ProceduralCutter.BP_ProceduralCutter_C|SetbCanCut (Variables|/Game/02-Hina_CookingLezard/Blueprints/PC_Hina.PC_Hina_C|GetProceduralCutterRef (Variables|Default|GetPC_HinaRef)) false)
        (Game|Player|SetViewTargetwithBlend (Game|GetPlayerController 0) (Variables|Default|GetBP_PalmeRef) 1.0 "VTBlend_Linear" 0.0 false)
        (Class|WidgetSwitcher|SetActiveWidgetIndex (Variables|/Game/02-Hina_CookingLezard/Widgets/WBP_IGHUD.WBP_IGHUD_C|GetHUDWidgetSwitcher (Variables|Default|GetHudRef)) 2)
        (Utilities|FlowControl|Delay 1.0)
        (Default|PlayAnim (Variables|Default|GetOnboardingRef) 3)
        (CallFunction|MoveRandomFoodatLocation)
        (Variables|Timer|SetTimeRemaining (Variables|Timer|GetMaxTimeMiniGame2))
        (Default|Timer (Variables|Default|GetHudRef) (Variables|Timer|GetTimeRemaining)))
      (:3
        (Game|Player|SetViewTargetwithBlend (Game|GetPlayerController 0) (Variables|Default|GetCameraMiniGame3) 1.0 "VTBlend_Linear" 0.0 false)
        (Class|WidgetSwitcher|SetActiveWidgetIndex (Variables|/Game/02-Hina_CookingLezard/Widgets/WBP_IGHUD.WBP_IGHUD_C|GetHUDWidgetSwitcher (Variables|Default|GetHudRef)) 3)
        (Utilities|FlowControl|Delay 1.0)
        (Default|InitilizeRandomRotation (Variables|Default|GetBP_SensDeTouilleRef))
        (Default|PlayAnim (Variables|Default|GetOnboardingRef) 4)
        (Variables|Timer|SetTimeRemaining (Variables|Timer|GetMaxTimeMiniGame3))
        (Default|Timer (Variables|Default|GetHudRef) (Variables|Timer|GetTimeRemaining))))
    (else
      (Viewport|RemoveAllWidgets)
      (bind _returnvalue (UserInterface|CreateWidget "/Game/MetaGame/Widgets/WBP_MenuVictoire.WBP_MenuVictoire_C" 0 (Variables|Score|GetScoreTotal) 1 2 3 1.0))
      (UserInterface|Viewport|AddtoViewport _returnvalue 0))))

(event Custom|MoveRandomFoodAtLocation
  ;[1 1 1] When called, move some randomly selected procedural cutted food over the cooking pot
  (for _index (range 0 10)
    (Utilities|IsValid (Utilities|Array|Get(acopy) (Variables|Default|GetProcMeshRef) _index)
      (:Is%20Valid
        (Transformation|SetWorldLocation (Utilities|Array|Get(acopy) (Variables|Default|GetProcMeshRef) _index) "2894.521240,-162.707886,979.430908" false true)))))

(event Custom|AddToScore
  (params (TimeSpentInGoodZone :type Float%20%28single-precision%29))
  ;[1 1 1] Score for the second minigame
  (Variables|Default|SetTimeSpentInGoodZone (+ TimeSpentInGoodZone (Variables|Default|GetTimeSpentInGoodZone))))

(event Custom|CalculeScoreMiniGame3
  ;[1 1 1] Score Minigame 3
  (Utilities|FlowControl|DoOnce false
    (:Completed
      (bind _returnvalue (Utilities|Time|SetTimerbyEvent (delegate Custom|DoesItInTheRightSens) (Variables|Default|GetRefreshRate) true))
      (Variables|Default|SetMiniGame3ScoreTimer _returnvalue))))

(event Custom|LaunchGame
  (bind _aspc_hina (Utilities|Casting|CastToPC_Hina (Game|GetPlayerController 0)))
  (Variables|Default|SetPC_HinaRef _aspc_hina)
  (Variables|Default|SetActualMiniGame 1)
  (bind _outactors (Actor|GetAllActorsOfClasswithTag "/Script/Engine.CameraActor" "MiniGame3"))
  (Variables|Default|SetCameraMiniGame3 (Utilities|Array|Get(acopy) _outactors))
  (bind _outactors_2 (Actor|GetAllActorsOfClass "/Game/02-Hina_CookingLezard/Blueprints/FireMiniGame/BP_Palme.BP_Palme_C"))
  (Variables|Default|SetBP_PalmeRef (Utilities|Array|Get(acopy) _outactors_2))
  (bind _outactors_3 (Actor|GetAllActorsOfClass "/Game/02-Hina_CookingLezard/Blueprints/MixMiniGame/BP_SensDeTouille_Hina.BP_SensDeTouille_Hina_C"))
  (Variables|Default|SetBP_SensDeTouilleRef (Utilities|Array|Get(acopy) _outactors_3))
  (bind _outactors_4 (Actor|GetAllActorsOfClass "/Game/02-Hina_CookingLezard/Blueprints/CuttingMiniGame/BP_FoodSelector.BP_FoodSelector_C"))
  (Variables|Default|SetFoodSelectorRef (Utilities|Array|Get(acopy) _outactors_4))
  (bind _outactors_5 (Actor|GetAllActorsOfClass "/Game/02-Hina_CookingLezard/Blueprints/CuttingMiniGame/BP_FoodSelectorOnBoard.BP_FoodSelectorOnBoard_C"))
  (bind _output_get (Variables|Default|SetFoodSelectorOnboardRef (Utilities|Array|Get(acopy) _outactors_5)))
  (bind _returnvalue (UserInterface|CreateWidget "/Game/02-Hina_CookingLezard/Widgets/WBP_OnBoardingJouable.WBP_OnBoardingJouable_C" (Game|GetPlayerController 0) _output_get))
  (bind _output_get_2 (Variables|Default|SetOnboardingRef _returnvalue))
  (UserInterface|Viewport|AddtoViewport _returnvalue 0)
  (bind _returnvalue_2 (UserInterface|CreateWidget "/Game/02-Hina_CookingLezard/Widgets/WBP_IGHUD.WBP_IGHUD_C" (Game|GetPlayerController 0)))
  (bind _output_get_3 (Variables|Default|SetHudRef _returnvalue_2))
  (UserInterface|Viewport|AddtoViewport _output_get_3 0))

(event Custom|OnBoardCanPlay
  ;[1 1 1] Set Can Play for Onboardings
  (Variables|/Game/02-Hina_CookingLezard/Blueprints/PC_Hina.PC_Hina_C|SetbCanPlay (Variables|Default|GetPC_HinaRef) true))

(event Custom|ClearAnims
  (Default|ClearCurrentAnim (Variables|Default|GetOnboardingRef)))

(event EventBeginPlay)

(fn ConstructionScript)

(fn ScoreCalculator
  (switch int (Variables|Default|GetActualMiniGame)
    (:1
      (if (> (Variables|Score|GetScoreMiniGame1) (Variables|Score|GetScoreMinimumG1))
        (Variables|Score|SetScoreTotal (+ 1 (Variables|Score|GetScoreTotal)))))
    (:2
      (if (> (Variables|Default|GetTimeSpentInGoodZone) (Variables|Default|GetTempsMinimumG2))
        (Variables|Score|SetScoreTotal (+ 1 (Variables|Score|GetScoreTotal)))))
    (:3
      (if (> (Variables|Score|GetScoreMiniGame3) (Variables|Score|GetTempsAFaire))
        (Variables|Score|SetScoreTotal (+ 1 (Variables|Score|GetScoreTotal)))))))