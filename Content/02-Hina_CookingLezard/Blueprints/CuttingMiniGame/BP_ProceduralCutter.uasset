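; Player-controlled knife for Hina's cutting minigame, slicing procedural objects it touches.
; MoveCutter maps touch position to clamped-range location and tilt by lerping over viewport size, notifying GM_Hina on the first move.
; Box overlap sends ProceduralCutMessage through BPI_Hina to the hit actor, gated by a DoOnce that resets on end overlap.
; Stun plays a sound, snaps the knife to a raised pose, flags MPC_Hina and blocks movement temporarily.
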(event OnComponentBeginOverlap(Box)
  (params (OverlappedComponent :type Primitive%20Component%20Object%20Reference) (OtherActor :type Actor%20Object%20Reference) (OtherComp :type Primitive%20Component%20Object%20Reference) (OtherBodyIndex :type Integer) (bFromSweep :type Boolean) (SweepResult :type Hit%20Result%20Structure%20%28by%20ref%29))
  ;[1 1 1] Linetrace du noob
  ;[1 1 1] Check if has interface
  (if (Utilities|DoesObjectImplementInterface OtherActor "/Game/02-Hina_CookingLezard/Blueprints/BPI_Hina.BPI_Hina_C")
    ;[1 1 1] Call the procedural object blueprint to make a cut
    (Utilities|FlowControl|DoOnce false
      (:Completed
        (Class|BPIHina|ProceduralCut(Message) OtherActor (Transformation|GetWorldLocation (Variables|Default|GetBox)) self)))))

(event OnComponentEndOverlap(Box)
  (params (OverlappedComponent :type Primitive%20Component%20Object%20Reference) (OtherActor :type Actor%20Object%20Reference) (OtherComp :type Primitive%20Component%20Object%20Reference) (OtherBodyIndex :type Integer))
  ;[1 1 1] If the object left the knife's perimeter, re-enable the cut
  (CallFunction|Reset))

(event Custom|Reset
  ;[1 1 1] Call the procedural object blueprint to make a cut
  (Utilities|FlowControl|DoOnce false) ; enters at Reset
)

(event Custom|Stun
  (bind _returnvalue (Transformation|GetActorLocation))
  ;[1 1 1] Stun the knife : Disable it's movement for 2 seconds
  (Audio|PlaySound2D "/Game/02-Hina_CookingLezard/SFX/S_stunt.S_stunt" 0.7 1.0 0.0 0 0)
  (Variables|Default|SetbIsStun? true)
  (Utilities|FlowControl|Delay 0.1)
  (Transformation|SetActorLocationAndRotation (Math|Vector|MakeVector (.x _returnvalue) (.y _returnvalue) 4.4e+02) "0, 0,60.000000")
  (Rendering|Material|SetScalarParameterValue "/Game/02-Hina_CookingLezard/Materials/MPC_Hina.MPC_Hina" "Stun" 1.0 :!class /Script/Engine.KismetMaterialLibrary)
  (Utilities|FlowControl|Delay 2.5)
  (Rendering|Material|SetScalarParameterValue "/Game/02-Hina_CookingLezard/Materials/MPC_Hina.MPC_Hina" "Stun" 0.0 :!class /Script/Engine.KismetMaterialLibrary)
  (Variables|Default|SetbIsStun? false))

(event Custom|MoveCutter
  (params (FingerPosition :type Vector%202D%20Structure))
  (bind (_x _y) (Math|Vector2D|BreakVector2D FingerPosition))
  (bind _returnvalue (Viewport|GetViewportSize))
  (bind _returnvalue_2 (/ _y (.y _returnvalue)))
  ;[1 1 1] This event control the knife's movement
  (if (not (Variables|Default|GetbIsStun?))
    ;;[1 1 1] Knife Movement based on touch input (From PC_Hina) and it's position on screen
    (Transformation|SetActorLocation (Math|Vector|MakeVector (Math|Float|Lerp 1124.0 1412.0 (/ _x (.x _returnvalue))) (.y (Transformation|GetActorLocation)) (Math|Float|Lerp 4.8e+02 364.0 _returnvalue_2)) false false)
    (Transformation|SetActorRotation (Math|Rotator|MakeRotator (Math|Float|Lerp 75.0 -2e+01 _returnvalue_2) 0.0 0.0))
    (Utilities|FlowControl|DoOnce false
      (:Completed
        (bind _asgm_hina (Utilities|Casting|CastToGM_Hina (Game|GetGameMode)))
        (Default|CouteauClick _asgm_hina)))))

(event EventBeginPlay
  ;[1 1 1] Store the screen's resolution
  (bind _returnvalue (Settings|GetGameUserSettings))
  (Variables|Default|SetScreenResolution (Class|GameUserSettings|GetScreenResolution _returnvalue)))

(fn ConstructionScript)