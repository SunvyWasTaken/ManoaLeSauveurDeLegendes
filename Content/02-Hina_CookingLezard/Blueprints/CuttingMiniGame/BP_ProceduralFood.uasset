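; Procedural food piece for Hina's cutting minigame, moved along a path by a looping timer and sliced where the knife hits.
; The construction script copies a configurable static mesh into a procedural mesh, which is cut into two capped, physics-driven halves.
; Cailloux (rock) items stun the cutter instead.
; Cuts either notify the food selector board when unboarding or show and add a score favoring centered cuts, with a penalty for Rori items.
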(event Custom|MoveAlongDeathPath
  ;[1 1 1] Move the food at the initial position and move it along a death march lol
  (Utilities|FlowControl|FlipFlop
    (:A
      (Transformation|SetActorLocation "778.338867,288.000000,386.916046" false false))
    (:B
      (Variables|Default|SetbIsUnboarding false)))
  (bind _returnvalue (Utilities|Time|SetTimerbyEvent (delegate Custom|Move) 0.01 true))
  (Variables|Movement|SetTimerHandle _returnvalue))

(event Custom|Move
  (bind _foodselectorref (Variables|Default|GetFoodSelectorRef))
  ;[1 1 1] As long as it hasn't reached the end, move towards it
  (if (< (.x (Transformation|GetActorLocation)) (select (Variables|Default|GetbIsUnboarding) 1.25e+03 1.7e+03))
    (Transformation|AddActorWorldOffset "3.000000, 0, 0")
    (elif (Variables|Default|GetbIsUnboarding)
      ;[1 1 1] Set it's location to a safe space and stop it's movement
      (CallFunction|StopMoving)
      (Utilities|IsValid _foodselectorref
        (:Is%20Valid
          (Default|ShowonBoard _foodselectorref)))
      (else
        (Transformation|SetActorLocation "1700.000000,288.000000,1500.000000" false false)
        (CallFunction|StopMoving)))))

(event Custom|Cut
  ;[1 1 1] Cut the procedural mesh at a specific place when called
  (bind _outotherhalfprocmesh (Class|KismetProceduralMeshLibrary|SliceProceduralMesh (Variables|Default|GetProceduralMesh) (Variables|Default|GetKnifePosition) "-1.000000,0.000000,0.000000" true "CreateNewSectionForCap" (Variables|ProceduralParameters|GetFaceCutMaterial)))
  (Audio|PlaySound2D "/Game/02-Hina_CookingLezard/SFX/SC_knife.SC_knife" 1.1 1.0 0.0 0 0)
  (Utilities|Array|Add (Variables|/Game/02-Hina_CookingLezard/Blueprints/GM_Hina.GM_Hina_C|GetProcMeshRef (Variables|Default|GetGM_HinaRef)) _outotherhalfprocmesh)
  (Physics|SetSimulatePhysics _outotherhalfprocmesh true)
  (Physics|AddImpulse _outotherhalfprocmesh "0, 0,10.000000" "None" true)
  (Collision|SetCollisionObjectType _outotherhalfprocmesh "ECC_WorldDynamic")
  (Utilities|FlowControl|RetriggerableDelay 2.0)
  (Transformation|SetWorldLocation _outotherhalfprocmesh "6027.671875,1512.937744,721.501831" false false))

(event Custom|StopMoving
  ;[1 1 1] Stop the food movement when called
  (Utilities|Time|ClearandInvalidateTimerbyHandle (Variables|Movement|GetTimerHandle)))

(event Custom|Calculate%20Score
  (bind _returnvalue (Transformation|GetActorLocation))
  (bind _knifeposition (Variables|Default|GetKnifePosition))
  (bind _gm_hinaref (Variables|Default|GetGM_HinaRef))
  (bind _bisrori_ (Variables|Default|GetbIsRori?))
  (bind _returnvalue_2 (- (.x _knifeposition) (.x _returnvalue)))
  (bind _returnvalue_3 (Math|Float|NormalizetoRange _returnvalue_2 -1e+02 1e+02))
  (bind _returnvalue_4 (> _returnvalue_3 0.5))
  (bind _returnvalue_5 (- 1.0 _returnvalue_3))
  (bind _returnvalue_6 (select _returnvalue_4 _returnvalue_5 _returnvalue_3))
  (bind _returnvalue_7 (* _returnvalue_6 2.0))
  (bind _returnvalue_8 (Math|Float|Lerp 1.0 1e+01 _returnvalue_7))
  (bind _returnvalue_9 (Math|Float|Truncate _returnvalue_8))
  (bind _returnvalue_10 (select _bisrori_ -10 _returnvalue_9))
  ;[1 1 1] Calculate the score based on the position of the knife and the food when called
  (Variables|/Game/02-Hina_CookingLezard/Blueprints/GM_Hina.GM_Hina_C|SetScoreMiniGame1 _gm_hinaref (+ (Variables|/Game/02-Hina_CookingLezard/Blueprints/GM_Hina.GM_Hina_C|GetScoreMiniGame1 _gm_hinaref) _returnvalue_10))
  (Rendering|Components|TextRender|SetText (Variables|Default|GetScore) (Utilities|Text|ToText(Integer) _returnvalue_10))
  (Rendering|Components|TextRender|SetTextRenderColor (Variables|Default|GetScore) (select (Variables|Default|GetbIsRori?) (Math|Color|MakeColor 0 0 1) (Math|Color|MakeColor 0 1 0)))
  (Development|SetHiddeninGame (Variables|Default|GetScore) false false)
  (Utilities|FlowControl|Delay 1.0)
  (Development|SetHiddeninGame (Variables|Default|GetScore) true false))

(event EventProceduralCut
  (params (WorldPosition :type Vector :default "0, 0, 0") (ProceduralCutterRef :type BP%20Procedural%20Cutter%20Object%20Reference))
  (bind _foodselectorref (Variables|Default|GetFoodSelectorRef))
  ;[1 1 1] Check if it's cailloux or not
  (Variables|Default|SetKnifePosition WorldPosition)
  (if (Variables|Default|GetbIsCailloux?)
    ;[1 1 1] If Cailloux, stun
    (Default|Stun ProceduralCutterRef)
    (Audio|PlaySound2D "/Game/02-Hina_CookingLezard/SFX/S_rock1.S_rock1" 1.68 1.0 0.0 0 0)
    (else
      ;[1 1 1] If Not Cailloux, Cut
      (Utilities|FlowControl|DoOnce false
        (:Completed
          (CallFunction|Cut)
          (if (Variables|Default|GetbIsUnboarding)
            (Utilities|IsValid _foodselectorref
              (:Is%20Valid
                (Default|FoodCutted _foodselectorref)))
            (else
              (CallFunction|CalculateScore))))))))

(event EventBeginPlay
  ;[1 1 1] Get the Gamemode's reference
  (bind _asgm_hina (Utilities|Casting|CastToGM_Hina (Game|GetGameMode)))
  (Variables|Default|SetGM_HinaRef _asgm_hina)
  (bind _asbp_food_selector_on_board (Utilities|Casting|CastToBP_FoodSelectorOnBoard (Components|GetOwner)))
  (Variables|Default|SetFoodSelectorRef _asbp_food_selector_on_board))

(fn ConstructionScript
  ;[1 1 1] Initialize the mesh for easy edit in instanced blueprint
  (Transformation|SetWorldScale3D (Variables|Default|GetStaticMesh) (Variables|Default|GetWorldScale))
  (Components|StaticMesh|SetStaticMesh (Variables|Default|GetStaticMesh) (Variables|ProceduralParameters|GetMesh))
  (Class|KismetProceduralMeshLibrary|CopyProceduralMeshfromStaticMeshComponent (Variables|Default|GetStaticMesh) 0 (Variables|Default|GetProceduralMesh) true))