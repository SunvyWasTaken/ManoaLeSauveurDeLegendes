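; Food selector for the board in Hina's cutting minigame, supplying the food to cut and tracking how many are cut.
; BeginPlay pre-spawns all food from a class list into an array.
; Each cut increments the count, clears GM_Hina's animations and sends the indexed food along its death path, with that index advancing only from 0 to 1.
; ShowOnBoard passes the cut count to GM_Hina to play widget animations.
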(event Custom|TriggerFoodMovement
  (bind _actualfoodmoving (Variables|Default|GetActualFoodMoving))
  ;[1 1 1] Make every food from the array move until they all moved then stop.
  (Default|MoveAlongDeathPath (Utilities|Array|Get(acopy) (Variables|Default|GetCuttableFoodArray) (Variables|Default|GetActualFoodMoving)))
  (if (== _actualfoodmoving 0)
    (Math|Integer|IncrementInt _actualfoodmoving)))

(event Custom|FoodCutted
  (Math|Integer|IncrementInt (Variables|Default|GetFoodCuttedVar)
    (:%20%20
      (Default|ClearAnims (Variables|Default|GetGMRef))
      (CallFunction|TriggerFoodMovement))))

(event Custom|ShowOnBoard
  (Default|PlayWidgetAnims (Variables|Default|GetGMRef) (Variables|Default|GetFoodCuttedVar)))

(event Custom|RefillFood
  (params (FoodSpawnNumber :type Integer))
  ;[1 1 1] Spawn procedural food when called and adds it to an array
  (bind _returnvalue (Game|SpawnActorfromClass (Utilities|Array|Get(acopy) (Variables|Default|GetProcFoodSpawnable) FoodSpawnNumber) (Math|Transform|MakeTransform (Variables|Default|GetTempSpawnLocation) "270.000000,-90.000000,0.000000" "1,1,1") "AlwaysSpawn" self true 0))
  (Utilities|Array|Add (Variables|Default|GetCuttableFoodArray) _returnvalue))

(event EventBeginPlay
  ;[1 1 1] Spawn all the needed food for the whole game
  (for _index (range 0 (Variables|Default|GetNumberOfFoodToSpawn))
    (CallFunction|RefillFood _index))
  (bind _asgm_hina (Utilities|Casting|CastToGM_Hina (Game|GetGameMode)))
  (Variables|Default|SetGMRef _asgm_hina))

(fn ConstructionScript)