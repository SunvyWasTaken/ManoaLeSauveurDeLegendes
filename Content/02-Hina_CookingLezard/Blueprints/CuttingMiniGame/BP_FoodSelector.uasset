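; Food spawner for the cutting minigame that creates all the food for the game on BeginPlay.
; RefillFood spawns random classes from ProcFoodSpawnable at a temporary location and stores them in CuttableFoodArray.
; TriggerFoodMovement starts a looping timer that sends each stored food along its death path in turn, one per second, clearing itself at the end.
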(event Custom|TriggerFoodMovement
  ;[1 1 1] Trigger Movement
  (bind _returnvalue (Utilities|Time|SetTimerbyEvent (delegate Custom|MoveForward) 1.0 true))
  (Variables|Default|SetTimerHandle _returnvalue))

(event Custom|MoveForward
  ;[1 1 1] Make every food from the array move until they all moved then stop.
  (Default|MoveAlongDeathPath (Utilities|Array|Get(acopy) (Variables|Default|GetCuttableFoodArray) (Variables|Default|GetActualFoodMoving)))
  (if (< (Variables|Default|GetActualFoodMoving) (Variables|Default|GetNumberOfFoodToSpawn))
    (Math|Integer|IncrementInt (Variables|Default|GetActualFoodMoving))
    (else
      (Utilities|Time|ClearandInvalidateTimerbyHandle (Variables|Default|GetTimerHandle)))))

(event Custom|RefillFood
  (params (FoodSpawnNumber :type Integer))
  ;[1 1 1] Spawn procedural food when called and adds it to an array
  (bind _returnvalue (Game|SpawnActorfromClass (Utilities|Array|Get(acopy) (Variables|Default|GetProcFoodSpawnable) (Math|Random|RandomIntegerinRange 0 8)) (Math|Transform|MakeTransform (Variables|Default|GetTempSpawnLocation) "270.000000,-90.000000,0.000000" "1,1,1") "AlwaysSpawn" 0 false 0))
  (Utilities|Array|Add (Variables|Default|GetCuttableFoodArray) _returnvalue))

(event EventBeginPlay
  ;[1 1 1] Spawn all the needed food for the whole game
  (for _index (range 0 (Variables|Default|GetNumberOfFoodToSpawn))
    (CallFunction|RefillFood _index)))

(fn ConstructionScript)