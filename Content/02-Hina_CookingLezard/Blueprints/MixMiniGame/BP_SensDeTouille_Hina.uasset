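; Stirring-direction indicator for Hina's mixing minigame, showing which way to rotate.
; It stays hidden until InitilizeRandomRotation reveals it and starts a looping three-second timer that re-rolls the direction at 50/50 odds.
; Each roll toggles the two arrow components, sets the RotatingMovement spin to match, and writes the required direction to GM_Hina's SensASuivre.
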(event Custom|RandomChoose
  (bind _rotatingmovement (Variables|Default|GetRotatingMovement))
  ;[1 1 1] 50% de chance que le sens soit a gauche ou a droite
  (if (== (Math|Random|RandomIntegerinRange 0 1) 0)
    (Variables|Default|SetbDroite? true)
    ;[1 1 1] Affiche le sens
    (Rendering|SetVisibility (Variables|Default|GetFlecheDroite) false false)
    (Variables|/Script/Engine.RotatingMovementComponent|SetRotationRate _rotatingmovement "0,40.000000, 0")
    (Rendering|SetVisibility (Variables|Default|GetFlecheGauche) true false)
    (else
      (Variables|Default|SetbDroite? false)
      (Rendering|SetVisibility (Variables|Default|GetFlecheGauche) false false)
      (Variables|/Script/Engine.RotatingMovementComponent|SetRotationRate _rotatingmovement "0,-40.000000, 0")
      (Rendering|SetVisibility (Variables|Default|GetFlecheDroite) true false)))
  ;[1 1 1] renvoie le sens demander au GameMode
  (bind _asgm_hina (Utilities|Casting|CastToGM_Hina (Game|GetGameMode)))
  (Variables|/Game/02-Hina_CookingLezard/Blueprints/GM_Hina.GM_Hina_C|SetSensASuivre _asgm_hina (Variables|Default|GetbDroite?)))

(event Custom|ActiveRandom
  ;[1 1 1] Toute les trois seconde, il est possible que le sens change
  (CallFunction|RandomChoose))

(event Custom|InitilizeRandomRotation
  ;[1 1 1] Toute les trois seconde, il est possible que le sens change
  (CallFunction|RandomChoose)
  (Utilities|Time|SetTimerbyEvent (delegate Custom|ActiveRandom) 3.0 true)
  (Rendering|SetActorHiddenInGame false))

(event EventBeginPlay
  (Rendering|SetActorHiddenInGame true))

(fn ConstructionScript)