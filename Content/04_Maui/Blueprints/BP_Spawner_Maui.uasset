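; Spawner for the Maui level that sends clouds, hoops, birds and collectibles along left, middle and right paths.
; BeginPlay registers it with the gamemode and pre-spawns actor pools, whose idle members are reused for each launch.
; Looping timers scaled to path length and game speed launch side clouds, random obstacles under a shared cooldown, and lane-wandering collectibles.
; Birds use random delays, while events handle scripted onboarding, timer resets and end-game shutdown.
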(event Custom|LaunchBlanc
  (params (Location :type Vector) (End :type Vector) (IsLeft :type Boolean))
  ;[0 1 1] Gère toute la partie avec les nuages
  ;;[1 1 1] Event qui permet de lancer un nuage specifique au bon endroit
  (bind _array_element (Utilities|Array|ForEachLoopwithBreak (Variables|Ref|GetNuageBlancArray) :!label _label)
    (:LoopBody
      (if (not (Variables|/Game/04_Maui/Blueprints/BP_Parent_Maui.BP_Parent_Maui_C|GetbIsMoving _array_element))
        (Default|GoStarting _array_element "0, 0, 0")
        (Transformation|SetActorLocation _array_element Location false true)
        (Default|FEndLocation _array_element End)
        (if IsLeft
          (Transformation|SetActorRotation _array_element "0, 0,180.000000")
          (goto _label Break)
          (else
            (Transformation|SetActorRotation _array_element)
            (goto _label Break)))))))

(event Custom|LaunchVert
  (params (Location :type Vector) (End :type Vector) (IsLeft :type Boolean))
  ;[0 1 1] Gère toute la partie avec les nuages
  ;;[1 1 1] Event qui permet de lancer un nuage specifique au bon endroit
  (bind _array_element (Utilities|Array|ForEachLoopwithBreak (Variables|Ref|GetNuageVertArray) :!label _label)
    (:LoopBody
      (if (not (Variables|/Game/04_Maui/Blueprints/BP_Parent_Maui.BP_Parent_Maui_C|GetbIsMoving _array_element))
        (Default|GoStarting _array_element "0, 0, 0")
        (Transformation|SetActorLocation _array_element Location false true)
        (Default|FEndLocation _array_element End)
        (if IsLeft
          (Transformation|SetActorRotation _array_element "0, 0,180.000000")
          (goto _label Break)
          (else
            (Transformation|SetActorRotation _array_element)
            (goto _label Break)))))))

(event Custom|EventAttack
  ;[0 1 1] Gère toute la partie avec les nuages
  ;;[1 1 1] Delay qui permet déviter qu'un obstacle ne sois pas impossible.
  (|DelayBtwAttack
    (:Completed
      (Variables|Default|SetbCanAttack false))))

(event Custom|LaunchCerceau
  ;[0 1 1] Gère toute la partie avec les nuages
  ;;[1 1 1] Event qui permet de lancer un nuage specifique au bon endroit
  (bind _array_element (Utilities|Array|ForEachLoopwithBreak (Variables|Default|GetCerceauxArray) :!label _label)
    (:LoopBody
      (if (not (Variables|/Game/04_Maui/Blueprints/BP_Parent_Maui.BP_Parent_Maui_C|GetbIsMoving _array_element))
        (Default|GoStarting _array_element "0, 0, 0")
        (Transformation|SetActorLocation _array_element (Transformation|GetWorldLocation (Variables|Default|GetStartMid)) false true)
        (Default|FEndLocation _array_element (Transformation|GetWorldLocation (Variables|Default|GetEndMid)))
        (goto _label Break)))))

(event Custom|LaunchCollectible
  (params (Location :type Vector) (End :type Vector))
  ;[1 1 1] Lance Collectibles
  (bind _array_element (Utilities|Array|ForEachLoopwithBreak (Variables|Default|GetCollectible) :!label _label)
    (:LoopBody
      (if (not (Variables|/Game/04_Maui/Blueprints/BP_Parent_Maui.BP_Parent_Maui_C|GetbIsMoving _array_element))
        (Default|GoStarting _array_element Location)
        (Default|FEndLocation _array_element End)
        (goto _label Break)))))

(event Custom|SpawnBird
  ;[1 1 1] Set oiseaux
  (if (Variables|Default|GetbCanSpawnObstacles)
    (if (Math|Random|RandomBool)
      (CallFunction|LaunchBird (Transformation|GetWorldLocation (Variables|Default|GetS_Utility_Left)) (Transformation|GetWorldLocation (Variables|Default|GetE_Utility_Left)) true)
      (else
        (CallFunction|LaunchBird (Transformation|GetWorldLocation (Variables|Default|GetS_Utility_Right)) (Transformation|GetWorldLocation (Variables|Default|GetE_Utility_Right)) false)))))

(event Custom|TriggerBird
  ;[1 1 1] Set oiseaux
  (Utilities|FlowControl|Delay (Math|Random|RandomFloatinRange (Variables|Default|GetMinTimeBird) (Variables|Default|GetMaxTimeBird)))
  (if (Variables|Default|GetbCanSpawnBird)
    (if (<= (Math|Random|RandomFloat) (Variables|Default|GetChanceBird))
      (CallFunction|SpawnBird))
    (CallFunction|TriggerBird)))

(event Custom|PresetCollectible
  ;[1 1 1] Setup la partie collectible
  ;;[0.5 0 1] Begin Play
  (Utilities|FlowControl|Sequence
    (:then_0
      (CallFunction|TriggerCollectible)
      (Variables|Default|SetbCanSpawnBird true)
      (CallFunction|TriggerBird))
    (:then_1
      (for _index (range 0 (Variables|NbrUtility|GetNbrCollectible))
        (bind _returnvalue (Game|SpawnActorfromClass "/Game/04_Maui/Blueprints/BPChildren/BPC_Collectible_Maui.BPC_Collectible_Maui_C" (Transformation|GetWorldTransform (Variables|Default|GetSpawnPoint)) "Undefined" 0 0))
        (Utilities|Array|Add (Variables|Default|GetCollectible) _returnvalue))
      (for _index_2 (range 0 (Variables|NbrUtility|GetNbrBird))
        (bind _returnvalue_2 (Game|SpawnActorfromClass "/Game/04_Maui/Blueprints/BPChildren/BPC_Bird_Maui.BPC_Bird_Maui_C" (Transformation|GetWorldTransform (Variables|Default|GetSpawnPoint)) "Undefined" 0 0))
        (Utilities|Array|Add (Variables|Default|GetBirdArray) _returnvalue_2)))))

(event Custom|LaunchNoir
  (params (StartLocation :type Vector) (EndLocation :type Vector) (isLeft :type Boolean))
  ;[0 1 1] Gère toute la partie avec les nuages
  ;;[1 1 1] Event qui permet de lancer un nuage specifique au bon endroit
  (bind _array_element (Utilities|Array|ForEachLoopwithBreak (Variables|Ref|GetNuageNoirArray) :!label _label)
    (:LoopBody
      (if (not (Variables|/Game/04_Maui/Blueprints/BP_Parent_Maui.BP_Parent_Maui_C|GetbIsMoving _array_element))
        (Default|GoStarting _array_element "0, 0, 0")
        (Transformation|SetActorLocation _array_element StartLocation false true)
        (Default|FEndLocation _array_element EndLocation)
        (if isLeft
          (Transformation|SetActorRotation _array_element "0, 0,180.000000")
          (goto _label Break)
          (else
            (Transformation|SetActorRotation _array_element)
            (goto _label Break)))))))

(event Custom|LaunchJaune
  (params (Location :type Vector) (End :type Vector) (IsLeft :type Boolean))
  ;[0 1 1] Gère toute la partie avec les nuages
  ;;[1 1 1] Event qui permet de lancer un nuage specifique au bon endroit
  (bind _array_element (Utilities|Array|ForEachLoopwithBreak (Variables|Ref|GetNuageJauneArray) :!label _label)
    (:LoopBody
      (if (not (Variables|/Game/04_Maui/Blueprints/BP_Parent_Maui.BP_Parent_Maui_C|GetbIsMoving _array_element))
        (Default|GoStarting _array_element "0, 0, 0")
        (Transformation|SetActorLocation _array_element Location false true)
        (Default|FEndLocation _array_element End)
        (if IsLeft
          (Transformation|SetActorRotation _array_element "0, 0,180.000000")
          (goto _label Break)
          (else
            (Transformation|SetActorRotation _array_element)
            (goto _label Break)))))))

(event Custom|Start%28L%29
  ;[0 1 1] Gère toute la partie avec les nuages
  ;;[1 1 1] Timer permettant de lancer les nuages de gauche
  (bind _returnvalue (Utilities|Time|SetTimerbyEvent (delegate Custom|CallLaunch%28L%29) (CallFunction|FDelayCall "NewEnumerator0" (Variables|NbrNuage|GetNbrTiles)) true))
  (Variables|Default|SetTimerLeft _returnvalue))

(event Custom|CallLaunch%28L%29
  (bind _endleft (Variables|Default|GetEndLeft))
  (bind _startleft (Variables|Default|GetStartLeft))
  (bind _returnvalue (Transformation|GetWorldLocation _startleft))
  (bind _returnvalue_2 (Transformation|GetWorldLocation _endleft))
  ;[0 1 1] Gère toute la partie avec les nuages
  ;;[1 1 1] Timer permettant de lancer les nuages de gauche
  (if (Variables|Default|GetbCanSpawnObstacles)
    (Utilities|CheckSpawnCerceaux true
      (:False
        (if (and (<= (Math|Random|RandomFloat) (Variables|NbrNuage|GetChanceBlack)) (not (Variables|Default|GetbCanAttack)))
          (Variables|Default|SetbCanAttack true)
          (CallFunction|LaunchBlanc _returnvalue _returnvalue_2 true)
          (CallFunction|LaunchNoir (Transformation|GetWorldLocation (Variables|Default|GetS_Utility_Left)) (Transformation|GetWorldLocation (Variables|Default|GetE_Utility_Left)) true)
          (CallFunction|EventAttack)
          (elif (and (<= (Math|Random|RandomFloat) (Variables|NbrNuage|GetChanceGray)) (not (Variables|Default|GetbCanAttack)))
            (Variables|Default|SetbCanAttack true)
            (CallFunction|LaunchJaune _returnvalue _returnvalue_2 true)
            (CallFunction|EventAttack)
            (else
              (CallFunction|LaunchBlanc _returnvalue _returnvalue_2 true))))))
    (else
      (CallFunction|LaunchBlanc (Transformation|GetWorldLocation (Variables|Default|GetStartLeft)) (Transformation|GetWorldLocation (Variables|Default|GetEndLeft)) true))))

(event Custom|TriggerCollectible
  ;[1 1 1] Lance les Projectiles
  (bind _returnvalue (Utilities|Time|SetTimerbyEvent (delegate Custom|SpawnCollectible) (CallFunction|FDelayCall "NewEnumerator1" (Variables|Default|GetNbrTiles_Collectible)) true))
  (Variables|Default|SetTimerCollectible _returnvalue))

(event Custom|SpawnCollectible
  ;[1 1 1] Lance les Projectiles
  (if (Variables|Default|GetbCanSpawnObstacles)
    (if (Variables|Default|GetbCanAttack)
      (|RandomWay_2)
      (CallFunction|LaunchCollectible (Transformation|GetWorldLocation (Utilities|Select :Index (Variables|Default|GetWay) :NewEnumerator0 (Variables|Default|GetS_Utility_Left) :NewEnumerator1 (Variables|Default|GetStartMid) :NewEnumerator2 (Variables|Default|GetS_Utility_Right))) (Transformation|GetWorldLocation (Utilities|Select :Index (Variables|Default|GetWay) :NewEnumerator0 (Variables|Default|GetE_Utility_Left) :NewEnumerator1 (Variables|Default|GetEndMid) :NewEnumerator2 (Variables|Default|GetE_Utility_Right)))))))

(event Custom|Start%28R%29
  ;[0 1 1] Gère toute la partie avec les nuages
  ;;[1 1 1] Timer permettant de lancer des nuages à droite.
  (bind _returnvalue (Utilities|Time|SetTimerbyEvent (delegate Custom|CallLaunch) (CallFunction|FDelayCall "NewEnumerator2" (Variables|NbrNuage|GetNbrTiles)) true))
  (Variables|Default|SetTimerRight _returnvalue))

(event Custom|CallLaunch
  (bind _startright (Variables|Default|GetStartRight))
  (bind _endright (Variables|Default|GetEndRight))
  (bind _returnvalue (Transformation|GetWorldLocation _startright))
  (bind _returnvalue_2 (Transformation|GetWorldLocation _endright))
  ;[0 1 1] Gère toute la partie avec les nuages
  ;;[1 1 1] Timer permettant de lancer des nuages à droite.
  (if (Variables|Default|GetbCanSpawnObstacles)
    (Utilities|CheckSpawnCerceaux false
      (:False
        (if (and (<= (Math|Random|RandomFloat) (Variables|NbrNuage|GetChanceBlack)) (not (Variables|Default|GetbCanAttack)))
          (Variables|Default|SetbCanAttack true)
          (CallFunction|LaunchBlanc _returnvalue _returnvalue_2 false)
          (CallFunction|LaunchNoir (Transformation|GetWorldLocation (Variables|Default|GetS_Utility_Right)) (Transformation|GetWorldLocation (Variables|Default|GetE_Utility_Right)) false)
          (CallFunction|EventAttack)
          (elif (and (<= (Math|Random|RandomFloat) (Variables|NbrNuage|GetChanceGray)) (not (Variables|Default|GetbCanAttack)))
            (Variables|Default|SetbCanAttack true)
            (CallFunction|LaunchJaune _returnvalue _returnvalue_2 false)
            (CallFunction|EventAttack)
            (else
              (CallFunction|LaunchBlanc _returnvalue _returnvalue_2 false))))))
    (else
      (CallFunction|LaunchBlanc (Transformation|GetWorldLocation (Variables|Default|GetStartRight)) (Transformation|GetWorldLocation (Variables|Default|GetEndRight)) false))))

(event Custom|LaunchBird
  (params (Location :type Vector) (End :type Vector) (IsLeft :type Boolean))
  ;[1 1 1] Lance oiseaux
  (bind _array_element (Utilities|Array|ForEachLoopwithBreak (Variables|Default|GetBirdArray) :!label _label)
    (:LoopBody
      (if (not (Variables|/Game/04_Maui/Blueprints/BP_Parent_Maui.BP_Parent_Maui_C|GetbIsMoving _array_element))
        (Default|GoStarting _array_element Location)
        (Default|FEndLocation _array_element End)
        (if IsLeft
          (Transformation|SetActorRotation _array_element "0, 0,180.000000")
          (goto _label Break)
          (else
            (Transformation|SetActorRotation _array_element)
            (goto _label Break)))))))

(event EventBeginPlay
  ;[0 1 1] Gère toute la partie avec les nuages
  ;;[1 1 1] Set Le Début
  ;;;[0.5 0 1] Begin Play
  (Utilities|FlowControl|Sequence
    (:then_0
      ;;;[1 1 1] Set la Reference du Gamemode
      (bind _asbp_gamemode_maui (Utilities|Casting|CastToBP_Gamemode_Maui (Game|GetGameMode)))
      (bind _output_get (Variables|Ref|SetGamemodeRef _asbp_gamemode_maui))
      (Variables|/Game/04_Maui/Blueprints/BP_Gamemode_Maui.BP_Gamemode_Maui_C|SetSpawner _output_get self)
      (CallFunction|Start(R))
      (CallFunction|Start(L)))
    (:then_1
      ;;;[1 1 1] PreSpawn Tous les nuages qui seront Réutiliser.
      (for _index (range 0 (Variables|NbrNuage|GetNbrNuageBlanc))
        (bind _returnvalue (Game|SpawnActorfromClass "/Game/04_Maui/Blueprints/BPChildren/BPC_NuageBlanc_Maui.BPC_NuageBlanc_Maui_C" (Transformation|GetWorldTransform (Variables|Default|GetSpawnPoint)) "Undefined" 0 0))
        (Utilities|Array|Add (Variables|Ref|GetNuageBlancArray) _returnvalue))
      (for _index_2 (range 0 (Variables|NbrNuage|GetNbrNuageVert))
        (bind _returnvalue_2 (Game|SpawnActorfromClass "/Game/04_Maui/Blueprints/BPChildren/BPC_NuageVert_Maui.BPC_NuageVert_Maui_C" (Transformation|GetWorldTransform (Variables|Default|GetSpawnPoint)) "Undefined" 0 0))
        (Utilities|Array|Add (Variables|Ref|GetNuageVertArray) _returnvalue_2))
      (for _index_3 (range 0 (Variables|NbrNuage|GetNbrNuageJaune))
        (bind _returnvalue_3 (Game|SpawnActorfromClass "/Game/04_Maui/Blueprints/BPChildren/BPC_NuageSeemless_Maui.BPC_NuageSeemless_Maui_C" (Transformation|GetWorldTransform (Variables|Default|GetSpawnPoint)) "Undefined" 0 0))
        (Utilities|Array|Add (Variables|Ref|GetNuageJauneArray) _returnvalue_3))
      (for _index_4 (range 0 (Variables|NbrNuage|GetNbrNuageNoir))
        (bind _returnvalue_4 (Game|SpawnActorfromClass "/Game/04_Maui/Blueprints/BPChildren/BPC_NuageNoir_Maui.BPC_NuageNoir_Maui_C" (Transformation|GetWorldTransform (Variables|Default|GetSpawnPoint)) "Undefined" 0 0))
        (Utilities|Array|Add (Variables|Ref|GetNuageNoirArray) _returnvalue_4))
      (for _index_5 (range 0 (Variables|Default|GetNbrCerceaux))
        (bind _returnvalue_5 (Game|SpawnActorfromClass "/Game/04_Maui/Blueprints/BPChildren/BPC_Cerceau_Maui.BPC_Cerceau_Maui_C" (Transformation|GetWorldTransform (Variables|Default|GetSpawnPoint)) "Undefined" 0 0))
        (Utilities|Array|Add (Variables|Default|GetCerceauxArray) _returnvalue_5)))
    (:then_2
      (CallFunction|PresetCollectible))))

(event EventSpawnerEndGame
  ;[0 1 1] Gère toute la partie avec les nuages
  ;;[1 0 0.5804] ENDGAME
  (Utilities|Time|ClearandInvalidateTimerbyHandle (Variables|Default|GetTimerLeft))
  (Utilities|Time|ClearandInvalidateTimerbyHandle (Variables|Default|GetTimerRight))
  (Utilities|Time|ClearandInvalidateTimerbyHandle (Variables|Default|GetTimerCollectible))
  (Variables|Default|SetbCanSpawnBird false)
  (for _array_element (Variables|Ref|GetNuageBlancArray)
    (Default|EndGame _array_element))
  (for _array_element_2 (Variables|Ref|GetNuageVertArray)
    (Default|EndGame _array_element_2))
  (for _array_element_3 (Variables|Ref|GetNuageJauneArray)
    (Default|EndGame _array_element_3))
  (for _array_element_4 (Variables|Ref|GetNuageNoirArray)
    (Default|EndGame _array_element_4))
  (for _array_element_5 (Variables|Default|GetCollectible)
    (Default|EndGame _array_element_5))
  (for _array_element_6 (Variables|Default|GetBirdArray)
    (Default|EndGame _array_element_6))
  (for _array_element_7 (Variables|Default|GetCerceauxArray)
    (Default|EndGame _array_element_7)))

(event EventSpawnerResetTimer
  ;[0 1 1] Gère toute la partie avec les nuages
  ;;[1 0 0.5804] Clean puis relance le Timer du spawn des nuages sur les côtes. Parce que sinon la vitesse va bien changer mais pas le rythme de Spawn
  (Utilities|Time|ClearandInvalidateTimerbyHandle (Variables|Default|GetTimerRight))
  (Utilities|Time|ClearandInvalidateTimerbyHandle (Variables|Default|GetTimerLeft))
  (CallFunction|Start(R))
  (CallFunction|Start(L)))

(event EventSpawnerCanSpawnObstacles
  ;[1 0 0.5804] CanSpawnObstacles
  (Variables|Default|SetbCanSpawnObstacles true))

(event EventSpawnerScriptedOnboarding
  (params (Step :type Integer))
  ;[1 1 1] OnboardingScript
  (if (== Step 0)
    (CallFunction|LaunchBird (Transformation|GetWorldLocation (Variables|Default|GetS_Utility_Right)) (Transformation|GetWorldLocation (Variables|Default|GetE_Utility_Right)) false)
    (elif (== Step 1)
      (CallFunction|LaunchVert (Transformation|GetWorldLocation (Variables|Default|GetS_Utility_Left)) (Transformation|GetWorldLocation (Variables|Default|GetE_Utility_Left)) true)
      (elif (== Step 2)
        (CallFunction|LaunchCerceau)
        (elif (== Step 3)
          (CallFunction|LaunchCollectible (Transformation|GetWorldLocation (Variables|Default|GetStartMid)) (Transformation|GetWorldLocation (Variables|Default|GetEndMid)))
          (elif (== Step 4)
            (CallFunction|LaunchNoir (Transformation|GetWorldLocation (Variables|Default|GetStartMid)) (Transformation|GetWorldLocation (Variables|Default|GetEndMid)) true)))))))

(fn ConstructionScript
  (Rendering|Components|TextRender|SetText (Variables|Default|GetTextRender%28SR%29) (Utilities|Text|ToText(String) (Utilities|GetObjectName (Variables|Default|GetStartRight))))
  (Rendering|Components|TextRender|SetText (Variables|Default|GetTextRender%28SL%29) (Utilities|Text|ToText(String) (Utilities|GetObjectName (Variables|Default|GetStartLeft))))
  (Rendering|Components|TextRender|SetText (Variables|Default|GetTextRender%28ER%29) (Utilities|Text|ToText(String) (Utilities|GetObjectName (Variables|Default|GetEndRight))))
  (Rendering|Components|TextRender|SetText (Variables|Default|GetTextRender%28EL%29) (Utilities|Text|ToText(String) (Utilities|GetObjectName (Variables|Default|GetEndLeft))))
  (Rendering|Components|TextRender|SetText (Variables|Default|GetTextRender%28SM%29) (Utilities|Text|ToText(String) (Utilities|GetObjectName (Variables|Default|GetStartMid))))
  (Rendering|Components|TextRender|SetText (Variables|Default|GetTextRender%28EM%29) (Utilities|Text|ToText(String) (Utilities|GetObjectName (Variables|Default|GetEndMid))))
  (Rendering|Components|TextRender|SetText (Variables|Default|GetTextRender%28SUL%29) (Utilities|Text|ToText(String) (Utilities|GetObjectName (Variables|Default|GetS_Utility_Left))))
  (Rendering|Components|TextRender|SetText (Variables|Default|GetTextRender%28SUR%29) (Utilities|Text|ToText(String) (Utilities|GetObjectName (Variables|Default|GetS_Utility_Right))))
  (Rendering|Components|TextRender|SetText (Variables|Default|GetTextRender%28EUL%29) (Utilities|Text|ToText(String) (Utilities|GetObjectName (Variables|Default|GetE_Utility_Left))))
  (Rendering|Components|TextRender|SetText (Variables|Default|GetTextRender%28EUR%29) (Utilities|Text|ToText(String) (Utilities|GetObjectName (Variables|Default|GetE_Utility_Right)))))

(fn FDelayCall
  (params (Index :type Enum_Lane%20Enum :default "NewEnumerator0") (Frequency :type Float%20%28single-precision%29))
  (return (/ (/ (Math|Vector|VectorLength (- (Transformation|GetWorldLocation (Utilities|Select :Index Index :NewEnumerator0 (Variables|Default|GetEndLeft) :NewEnumerator1 (Variables|Default|GetEndMid) :NewEnumerator2 (Variables|Default|GetEndRight))) (Transformation|GetWorldLocation (Utilities|Select :Index Index :NewEnumerator0 (Variables|Default|GetStartLeft) :NewEnumerator1 (Variables|Default|GetStartMid) :NewEnumerator2 (Variables|Default|GetStartRight))))) Frequency) (Variables|/Game/04_Maui/Blueprints/BP_Gamemode_Maui.BP_Gamemode_Maui_C|GetSpeed (Variables|Ref|GetGamemodeRef)))))