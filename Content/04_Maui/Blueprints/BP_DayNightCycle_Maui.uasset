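; Day/night cycle actor for the Maui level that scrolls two background roots and registers itself with the Maui gamemode.
; A looping timer moves both roots in X and leapfrogs them at a threshold, randomly toggling each one's rainbow.
; Player overlaps with day, twilight and night triggers set the current time of day.
; They also start looping timers that gradually blend the sky scalars in a Material Parameter Collection.
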(event OnComponentBeginOverlap(BG1Daytime)
  (params (OverlappedComponent :type Primitive%20Component%20Object%20Reference) (OtherActor :type Actor%20Object%20Reference) (OtherComp :type Primitive%20Component%20Object%20Reference) (OtherBodyIndex :type Integer) (bFromSweep :type Boolean) (SweepResult :type Hit%20Result%20Structure%20%28by%20ref%29))
  (if (== (Utilities|GetClass OtherActor) "/Game/04_Maui/Blueprints/BP_PlayerPawn_Maui.BP_PlayerPawn_Maui_C")
    (Utilities|Time|SetTimerbyFunctionName 0 "DayTimer" (Variables|Default|GetTimerSpeed) true)
    (Variables|Default|SetWhatTimeIsIt 0)))

(event OnComponentBeginOverlap(BG2Daytime)
  (params (OverlappedComponent :type Primitive%20Component%20Object%20Reference) (OtherActor :type Actor%20Object%20Reference) (OtherComp :type Primitive%20Component%20Object%20Reference) (OtherBodyIndex :type Integer) (bFromSweep :type Boolean) (SweepResult :type Hit%20Result%20Structure%20%28by%20ref%29))
  (if (== (Utilities|GetClass OtherActor) "/Game/04_Maui/Blueprints/BP_PlayerPawn_Maui.BP_PlayerPawn_Maui_C")
    (Utilities|Time|SetTimerbyFunctionName 0 "DayTimer" (Variables|Default|GetTimerSpeed) true)
    (Variables|Default|SetWhatTimeIsIt 0)))

(event OnComponentBeginOverlap(BG1Sunset)
  (params (OverlappedComponent :type Primitive%20Component%20Object%20Reference) (OtherActor :type Actor%20Object%20Reference) (OtherComp :type Primitive%20Component%20Object%20Reference) (OtherBodyIndex :type Integer) (bFromSweep :type Boolean) (SweepResult :type Hit%20Result%20Structure%20%28by%20ref%29))
  (if (== (Utilities|GetClass OtherActor) "/Game/04_Maui/Blueprints/BP_PlayerPawn_Maui.BP_PlayerPawn_Maui_C")
    (Utilities|Time|SetTimerbyFunctionName 0 "CrepusculeTimer" (Variables|Default|GetTimerSpeed) true)
    (Variables|Default|SetWhatTimeIsIt 1)))

(event OnComponentBeginOverlap(BG1Sunshine)
  (params (OverlappedComponent :type Primitive%20Component%20Object%20Reference) (OtherActor :type Actor%20Object%20Reference) (OtherComp :type Primitive%20Component%20Object%20Reference) (OtherBodyIndex :type Integer) (bFromSweep :type Boolean) (SweepResult :type Hit%20Result%20Structure%20%28by%20ref%29))
  (if (== (Utilities|GetClass OtherActor) "/Game/04_Maui/Blueprints/BP_PlayerPawn_Maui.BP_PlayerPawn_Maui_C")
    (Utilities|Time|SetTimerbyFunctionName 0 "CrepusculeTimer" (Variables|Default|GetTimerSpeed) true)
    (Variables|Default|SetWhatTimeIsIt 1)))

(event OnComponentBeginOverlap(BG2Sunset)
  (params (OverlappedComponent :type Primitive%20Component%20Object%20Reference) (OtherActor :type Actor%20Object%20Reference) (OtherComp :type Primitive%20Component%20Object%20Reference) (OtherBodyIndex :type Integer) (bFromSweep :type Boolean) (SweepResult :type Hit%20Result%20Structure%20%28by%20ref%29))
  (if (== (Utilities|GetClass OtherActor) "/Game/04_Maui/Blueprints/BP_PlayerPawn_Maui.BP_PlayerPawn_Maui_C")
    (Utilities|Time|SetTimerbyFunctionName 0 "CrepusculeTimer" (Variables|Default|GetTimerSpeed) true)
    (Variables|Default|SetWhatTimeIsIt 1)))

(event OnComponentBeginOverlap(BG2Sunshine)
  (params (OverlappedComponent :type Primitive%20Component%20Object%20Reference) (OtherActor :type Actor%20Object%20Reference) (OtherComp :type Primitive%20Component%20Object%20Reference) (OtherBodyIndex :type Integer) (bFromSweep :type Boolean) (SweepResult :type Hit%20Result%20Structure%20%28by%20ref%29))
  (if (== (Utilities|GetClass OtherActor) "/Game/04_Maui/Blueprints/BP_PlayerPawn_Maui.BP_PlayerPawn_Maui_C")
    (Utilities|Time|SetTimerbyFunctionName 0 "CrepusculeTimer" (Variables|Default|GetTimerSpeed) true)
    (Variables|Default|SetWhatTimeIsIt 1)))

(event OnComponentBeginOverlap(BG1NightTime)
  (params (OverlappedComponent :type Primitive%20Component%20Object%20Reference) (OtherActor :type Actor%20Object%20Reference) (OtherComp :type Primitive%20Component%20Object%20Reference) (OtherBodyIndex :type Integer) (bFromSweep :type Boolean) (SweepResult :type Hit%20Result%20Structure%20%28by%20ref%29))
  (if (== (Utilities|GetClass OtherActor) "/Game/04_Maui/Blueprints/BP_PlayerPawn_Maui.BP_PlayerPawn_Maui_C")
    (Utilities|Time|SetTimerbyFunctionName 0 "NightTimer" (Variables|Default|GetTimerSpeed) true)
    (Variables|Default|SetWhatTimeIsIt 2)))

(event OnComponentBeginOverlap(BG2NightTime)
  (params (OverlappedComponent :type Primitive%20Component%20Object%20Reference) (OtherActor :type Actor%20Object%20Reference) (OtherComp :type Primitive%20Component%20Object%20Reference) (OtherBodyIndex :type Integer) (bFromSweep :type Boolean) (SweepResult :type Hit%20Result%20Structure%20%28by%20ref%29))
  (if (== (Utilities|GetClass OtherActor) "/Game/04_Maui/Blueprints/BP_PlayerPawn_Maui.BP_PlayerPawn_Maui_C")
    (Utilities|Time|SetTimerbyFunctionName 0 "NightTimer" (Variables|Default|GetTimerSpeed) true)
    (Variables|Default|SetWhatTimeIsIt 2)))

(event Custom|CycleTimer
  (Transformation|AddRelativeLocation (Variables|Default|GetBG1Root) (Math|Vector|MakeVector (Variables|Default|GetSpeed) 0.0 0.0) false false)
  (Transformation|AddRelativeLocation (Variables|Default|GetBG2Root) (Math|Vector|MakeVector (Variables|Default|GetSpeed) 0.0 0.0) false false)
  (if (<= (.x (Variables|/Script/Engine.SceneComponent|GetRelativeLocation (Variables|Default|GetBG1Root))) -1e+03)
    (Transformation|SetWorldTransform (Variables|Default|GetBG1Root) (Transformation|GetWorldTransform (Variables|Default|GetEndBG2)) false false)
    (Rendering|SetVisibility (Variables|Default|GetRainbowbg1) (Math|Random|RandomBool) false)
    (elif (<= (.x (Variables|/Script/Engine.SceneComponent|GetRelativeLocation (Variables|Default|GetBG2Root))) -1e+03)
      (Transformation|SetWorldTransform (Variables|Default|GetBG2Root) (Transformation|GetWorldTransform (Variables|Default|GetEndBG1)) false false)
      (Rendering|SetVisibility (Variables|Default|GetRainbowbg2) (Math|Random|RandomBool) false))))

(event EventBeginPlay
  (bind _returnvalue (Utilities|Time|SetTimerbyEvent (delegate Custom|CycleTimer) 0.04 true))
  (Variables|Default|SetTimerKey _returnvalue)
  (bind _asbp_gamemode_maui (Utilities|Casting|CastToBP_Gamemode_Maui (Game|GetGameMode)))
  (Variables|/Game/04_Maui/Blueprints/BP_Gamemode_Maui.BP_Gamemode_Maui_C|SetDayNightCycle _asbp_gamemode_maui self))

(event Collision|EventActorBeginOverlap
  (params (OtherActor :type Actor%20Object%20Reference)))

(event EventSpawnerEndGame
  (Utilities|Time|ClearandInvalidateTimerbyHandle (Variables|Default|GetTimerKey)))

(fn ConstructionScript)

(fn DayTimer
  (if (Math|Boolean|ANDBoolean (>= (Variables|Default|GetDayScalar) 1.0) (<= (Variables|Default|GetNightScalar) 0.0) (<= (Variables|Default|GetCrepusculeScalar) 0.0))
    (Variables|Default|SetDayScalar 1.0)
    (Variables|Default|SetNightScalar 0.0)
    (Variables|Default|SetCrepusculeScalar 0.0)
    (Rendering|Material|SetScalarParameterValue "/Game/04_Maui/Asset2D/MPC_CycleJourNuit_Maui.MPC_CycleJourNuit_Maui" "Day" (Variables|Default|GetDayScalar) :!class /Script/Engine.KismetMaterialLibrary)
    (Rendering|Material|SetScalarParameterValue "/Game/04_Maui/Asset2D/MPC_CycleJourNuit_Maui.MPC_CycleJourNuit_Maui" "Night" (Variables|Default|GetNightScalar) :!class /Script/Engine.KismetMaterialLibrary)
    (Rendering|Material|SetScalarParameterValue "/Game/04_Maui/Asset2D/MPC_CycleJourNuit_Maui.MPC_CycleJourNuit_Maui" "Crepuscule" (Variables|Default|GetCrepusculeScalar) :!class /Script/Engine.KismetMaterialLibrary)
    (Utilities|Time|ClearTimerbyFunctionName 0 "DayTimer")
    (else
      (Utilities|FlowControl|Sequence
        (:then_0
          (if (< (Variables|Default|GetDayScalar) 1.0)
            (bind _output_get (Variables|Default|SetDayScalar (+ (Variables|Default|GetDayScalar) (Variables|Default|GetScalarModifier))))
            (Rendering|Material|SetScalarParameterValue "/Game/04_Maui/Asset2D/MPC_CycleJourNuit_Maui.MPC_CycleJourNuit_Maui" "Day" _output_get :!class /Script/Engine.KismetMaterialLibrary)))
        (:then_1
          (if (> (Variables|Default|GetNightScalar) 0.0)
            (bind _output_get_2 (Variables|Default|SetNightScalar (- (Variables|Default|GetNightScalar) (Variables|Default|GetScalarModifier))))
            (Rendering|Material|SetScalarParameterValue "/Game/04_Maui/Asset2D/MPC_CycleJourNuit_Maui.MPC_CycleJourNuit_Maui" "Night" _output_get_2 :!class /Script/Engine.KismetMaterialLibrary)))
        (:then_2
          (if (> (Variables|Default|GetCrepusculeScalar) 0.0)
            (bind _output_get_3 (Variables|Default|SetCrepusculeScalar (- (Variables|Default|GetCrepusculeScalar) (Variables|Default|GetScalarModifier))))
            (Rendering|Material|SetScalarParameterValue "/Game/04_Maui/Asset2D/MPC_CycleJourNuit_Maui.MPC_CycleJourNuit_Maui" "Crepuscule" _output_get_3 :!class /Script/Engine.KismetMaterialLibrary)))))))

(fn NightTimer
  (if (Math|Boolean|ANDBoolean (>= (Variables|Default|GetNightScalar) 1.0) (<= (Variables|Default|GetDayScalar) 0.5) (<= (Variables|Default|GetCrepusculeScalar) 0.0))
    (Variables|Default|SetDayScalar 0.5)
    (Variables|Default|SetNightScalar 1.0)
    (Variables|Default|SetCrepusculeScalar 0.0)
    (Rendering|Material|SetScalarParameterValue "/Game/04_Maui/Asset2D/MPC_CycleJourNuit_Maui.MPC_CycleJourNuit_Maui" "Day" (Variables|Default|GetDayScalar) :!class /Script/Engine.KismetMaterialLibrary)
    (Rendering|Material|SetScalarParameterValue "/Game/04_Maui/Asset2D/MPC_CycleJourNuit_Maui.MPC_CycleJourNuit_Maui" "Night" (Variables|Default|GetNightScalar) :!class /Script/Engine.KismetMaterialLibrary)
    (Rendering|Material|SetScalarParameterValue "/Game/04_Maui/Asset2D/MPC_CycleJourNuit_Maui.MPC_CycleJourNuit_Maui" "Crepuscule" (Variables|Default|GetCrepusculeScalar) :!class /Script/Engine.KismetMaterialLibrary)
    (Utilities|Time|ClearTimerbyFunctionName 0 "NightTimer")
    (else
      (Utilities|FlowControl|Sequence
        (:then_0
          (if (< (Variables|Default|GetNightScalar) 1.0)
            (bind _output_get (Variables|Default|SetNightScalar (+ (Variables|Default|GetNightScalar) (Variables|Default|GetScalarModifier))))
            (Rendering|Material|SetScalarParameterValue "/Game/04_Maui/Asset2D/MPC_CycleJourNuit_Maui.MPC_CycleJourNuit_Maui" "Night" _output_get :!class /Script/Engine.KismetMaterialLibrary)))
        (:then_1
          (if (> (Variables|Default|GetDayScalar) 0.5)
            (bind _output_get_2 (Variables|Default|SetDayScalar (- (Variables|Default|GetDayScalar) (Variables|Default|GetScalarModifier))))
            (Rendering|Material|SetScalarParameterValue "/Game/04_Maui/Asset2D/MPC_CycleJourNuit_Maui.MPC_CycleJourNuit_Maui" "Day" _output_get_2 :!class /Script/Engine.KismetMaterialLibrary)))
        (:then_2
          (if (> (Variables|Default|GetCrepusculeScalar) 0.0)
            (bind _output_get_3 (Variables|Default|SetCrepusculeScalar (- (Variables|Default|GetCrepusculeScalar) (Variables|Default|GetScalarModifier))))
            (Rendering|Material|SetScalarParameterValue "/Game/04_Maui/Asset2D/MPC_CycleJourNuit_Maui.MPC_CycleJourNuit_Maui" "Crepuscule" _output_get_3 :!class /Script/Engine.KismetMaterialLibrary)))))))

(fn CrepusculeTimer
  (if (Math|Boolean|ANDBoolean (>= (Variables|Default|GetCrepusculeScalar) 1.0) (<= (Variables|Default|GetDayScalar) 0.5) (<= (Variables|Default|GetNightScalar) 0.0))
    (Variables|Default|SetDayScalar 0.5)
    (Variables|Default|SetNightScalar 0.0)
    (Variables|Default|SetCrepusculeScalar 1.0)
    (Rendering|Material|SetScalarParameterValue "/Game/04_Maui/Asset2D/MPC_CycleJourNuit_Maui.MPC_CycleJourNuit_Maui" "Day" (Variables|Default|GetDayScalar) :!class /Script/Engine.KismetMaterialLibrary)
    (Rendering|Material|SetScalarParameterValue "/Game/04_Maui/Asset2D/MPC_CycleJourNuit_Maui.MPC_CycleJourNuit_Maui" "Night" (Variables|Default|GetNightScalar) :!class /Script/Engine.KismetMaterialLibrary)
    (Rendering|Material|SetScalarParameterValue "/Game/04_Maui/Asset2D/MPC_CycleJourNuit_Maui.MPC_CycleJourNuit_Maui" "Crepuscule" (Variables|Default|GetCrepusculeScalar) :!class /Script/Engine.KismetMaterialLibrary)
    (Utilities|Time|ClearTimerbyFunctionName 0 "CrepusculeTimer")
    (else
      (Utilities|FlowControl|Sequence
        (:then_0
          (if (< (Variables|Default|GetCrepusculeScalar) 1.0)
            (bind _output_get (Variables|Default|SetCrepusculeScalar (+ (Variables|Default|GetCrepusculeScalar) (Variables|Default|GetScalarModifier))))
            (Rendering|Material|SetScalarParameterValue "/Game/04_Maui/Asset2D/MPC_CycleJourNuit_Maui.MPC_CycleJourNuit_Maui" "Crepuscule" _output_get :!class /Script/Engine.KismetMaterialLibrary)))
        (:then_1
          (if (> (Variables|Default|GetDayScalar) 0.5)
            (bind _output_get_2 (Variables|Default|SetDayScalar (- (Variables|Default|GetDayScalar) (Variables|Default|GetScalarModifier))))
            (Rendering|Material|SetScalarParameterValue "/Game/04_Maui/Asset2D/MPC_CycleJourNuit_Maui.MPC_CycleJourNuit_Maui" "Day" _output_get_2 :!class /Script/Engine.KismetMaterialLibrary)))
        (:then_2
          (if (> (Variables|Default|GetNightScalar) 0.0)
            (bind _output_get_3 (Variables|Default|SetNightScalar (- (Variables|Default|GetNightScalar) (Variables|Default|GetScalarModifier))))
            (Rendering|Material|SetScalarParameterValue "/Game/04_Maui/Asset2D/MPC_CycleJourNuit_Maui.MPC_CycleJourNuit_Maui" "Night" _output_get_3 :!class /Script/Engine.KismetMaterialLibrary)))))))