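; Parent Blueprint for moving objects in the Maui game, such as birds, that travel along X to an end location and then return to their construction-time origin for reuse.
; GoStarting teleports the actor and opens a Tick gate that moves it using game mode speed and Nitro, until Finish or EndGame closes it.
; SwitchSide mirrors the target Z and rotates the actor 180 degrees, adding diagonal movement until it reaches the other side.
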(event Custom|Finish
  ;[1 1 1] Reinitialiser
  (Variables|Default|SetbIsMoving false)
  (Transformation|SetActorLocation (Variables|Default|GetOriginLocation) false true)
  ;[1 1 1] Tick
  (Utilities|FlowControl|Gate true) ; enters at Close
)

(event Custom|EndGame
  ;[1 1 1] EndGame
  ;[1 1 1] Tick
  (Utilities|FlowControl|Gate true) ; enters at Close
)

(event Custom|SwitchSide
  ;[1 1 1] Oiseau change de cote
  (Variables|Default|SetEndLocation (Math|Vector|MakeVector (.x (Variables|Default|GetEndLocation)) (.y (Variables|Default|GetEndLocation)) (* (.z (Transformation|GetActorLocation)) -1.0)))
  (Variables|Default|SetbIsCrossing true)
  (Transformation|AddActorLocalRotation "0, 0,180.000000" false false))

(event Custom|GoStarting
  (params (Location :type Vector))
  ;[1 1 1] Go
  (Variables|Default|SetbIsMoving true)
  (Transformation|SetActorLocation Location false true)
  ;[1 1 1] Tick
  (Utilities|FlowControl|Gate true) ; enters at Open
)

(event EventTick
  (params (DeltaSeconds :type Float%20%28single-precision%29))
  (bind _returnvalue (Utilities|CalculateSpeed DeltaSeconds))
  ;[1 1 1] Tick
  (Utilities|FlowControl|Gate true
    (:Exit
      (if (Variables|Default|GetbIsCrossing)
        (Transformation|AddActorWorldOffset (Math|Vector|MakeVector _returnvalue 0.0 (select (> (.z (Variables|Default|GetEndLocation)) 0.0) (* _returnvalue -1.0) _returnvalue)))
        (if (Math|Float|NearlyEqual(Float) (.z (Transformation|GetActorLocation)) (.z (Variables|Default|GetEndLocation)) (Variables|/Game/04_Maui/Blueprints/BP_Gamemode_Maui.BP_Gamemode_Maui_C|GetTolerance (Variables|Default|GetGameModeRef)))
          (Variables|Default|SetbIsCrossing false))
        (else
          (Transformation|AddActorWorldOffset (Math|Vector|MakeVector (Utilities|CalculateSpeed DeltaSeconds) 0.0 0.0))))
      (if (Math|Vector|Equal(Vector) (Transformation|GetActorLocation) (Variables|Default|GetEndLocation) (Variables|/Game/04_Maui/Blueprints/BP_Gamemode_Maui.BP_Gamemode_Maui_C|GetTolerance (Variables|Default|GetGameModeRef)))
        (CallFunction|Finish)))))

(event EventBeginPlay
  ;[1 1 1] Game Mode Ref
  (bind _asbp_gamemode_maui (Utilities|Casting|CastToBP_Gamemode_Maui (Game|GetGameMode)))
  (Variables|Default|SetGameModeRef _asbp_gamemode_maui))

(fn ConstructionScript
  (Variables|Default|SetOriginLocation (Transformation|GetActorLocation)))

(fn FEndLocation
  (params (EndLocation :type Vector))
  (Variables|Default|SetEndLocation EndLocation))