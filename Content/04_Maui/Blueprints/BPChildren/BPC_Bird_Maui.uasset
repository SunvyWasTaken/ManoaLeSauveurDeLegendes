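; Bird hazard in the Maui game, a child Blueprint that sets its own Nitro value and kills the player pawn on contact.
; A box overlap with the player plays damage sound, impact flipbooks and camera shake, then sends the pawn a bird-death message.
; A brief global time-dilation dip creates hit-stop before Finish is called and the flipbooks are cleared.
; FxImpactBird drives four flipbook components, tinting two yellow.
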(event OnComponentBeginOverlap(BoxCollision)
  (params (OverlappedComponent :type Primitive%20Component%20Object%20Reference) (OtherActor :type Actor%20Object%20Reference) (OtherComp :type Primitive%20Component%20Object%20Reference) (OtherBodyIndex :type Integer) (bFromSweep :type Boolean) (SweepResult :type Hit%20Result%20Structure%20%28by%20ref%29))
  ;[1 1 1] PlayerCollision
  (if (== (Utilities|GetClass OtherActor) "/Game/04_Maui/Blueprints/BP_PlayerPawn_Maui.BP_PlayerPawn_Maui_C")
    (Audio|PlaySound2D "/Game/04_Maui/Sound/IG/S_MauiDamage_Maui.S_MauiDamage_Maui" 1.0 1.0 0.0 0 0)
    (CallFunction|FxImpactBird "/Game/04_Maui/Asset2D/Fx/Fx_Impact_Bird1_Maui1.Fx_Impact_Bird1_Maui1" "/Game/04_Maui/Asset2D/Fx/Fx_Impact_Bird3_Maui2.Fx_Impact_Bird3_Maui2")
    (Camera|PlayWorldCameraShake "/Game/02_Teura/Blueprint/CameraShake/CS_KillEnnemi_Teura.CS_KillEnnemi_Teura_C" (Transformation|GetActorLocation) 0.0 5e+06)
    (Class|BPIMaui|PawnDeathBird(Message) OtherActor)
    (Utilities|FlowControl|Delay 0.05)
    (Utilities|Time|SetGlobalTimeDilation 0.05)
    (Utilities|FlowControl|Delay 0.02)
    (Utilities|Time|SetGlobalTimeDilation 1.0)
    (CallFunction|Finish)
    (Utilities|FlowControl|Delay 0.1)
    (CallFunction|FxImpactBird)))

(event EventBeginPlay
  (|CallParentFunction)
  (Variables|Default|SetNitro? 1.5))

(event Collision|EventActorBeginOverlap
  (params (OtherActor :type Actor%20Object%20Reference))
  (|CallParentFunction OtherActor))

(event EventTick
  (params (DeltaSeconds :type Float%20%28single-precision%29))
  (|CallParentFunction DeltaSeconds) ; This node is disabled and will not be called.\nDrag off pins to build functionality.
)

(fn ConstructionScript
  (|CallParentFunction))

(fn FxImpactBird
  (params (NewFlipbook :type Paper%20Flipbook%20Object%20Reference) (NewFlipbook1 :type Paper%20Flipbook%20Object%20Reference))
  (bind _paperflipbook1 (Variables|Default|GetPaperFlipbook1))
  (bind _paperflipbook4 (Variables|Default|GetPaperFlipbook4))
  (Sprite|SetFlipbook _paperflipbook1 NewFlipbook)
  (Sprite|SetFlipbook (Variables|Default|GetPaperFlipbook3) NewFlipbook)
  (Sprite|SetSpriteColor _paperflipbook4 "(R=1.000000,G=1.000000,B=0.000000,A=1.000000)")
  (Sprite|SetFlipbook _paperflipbook4 NewFlipbook1)
  (Sprite|SetFlipbook (Variables|Default|GetPaperFlipbook5) NewFlipbook1)
  (Audio|Components|Audio|Play _paperflipbook1)
  (Components|Timeline|SetLooping _paperflipbook1 false))