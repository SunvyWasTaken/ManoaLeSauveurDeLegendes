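; Black cloud hazard for the Maui game, a child Blueprint with a lightning-cloud flipbook that kills the player on contact.
; Its box collision sends the player pawn a black-cloud death message on overlap.
; NuageNoirDestroyed plays the death flipbook for its length, calls Finish, then restores the normal cloud, plays a damage sound and prints a debug string.
; A second custom event runs a fixed-delay death variant; some leftover nodes are unconnected.
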(event OnComponentBeginOverlap(BoxCollision)
  (params (OverlappedComponent :type Primitive%20Component%20Object%20Reference) (OtherActor :type Actor%20Object%20Reference) (OtherComp :type Primitive%20Component%20Object%20Reference) (OtherBodyIndex :type Integer) (bFromSweep :type Boolean) (SweepResult :type Hit%20Result%20Structure%20%28by%20ref%29))
  ;[1 1 1] Player Collision
  (if (== (Utilities|GetClass OtherActor) "/Game/04_Maui/Blueprints/BP_PlayerPawn_Maui.BP_PlayerPawn_Maui_C")
    (Class|BPIMaui|PawnDeathBlackCloud(Message) OtherActor self)))

(event Custom|CustomEvent_0
  (bind _pfb_nuageeclairs_maui1 (Variables|Default|GetPFB_NuageEclairs_Maui1))
  (Sprite|SetFlipbook _pfb_nuageeclairs_maui1 "/Game/04_Maui/Asset2D/Animation/Decors/PFB_NuageNoirDeath_Maui1.PFB_NuageNoirDeath_Maui1")
  (Audio|Components|Audio|Play _pfb_nuageeclairs_maui1)
  (Components|Timeline|SetLooping _pfb_nuageeclairs_maui1 false)
  (Utilities|FlowControl|Delay 0.4)
  (CallFunction|Finish))

(event EventBeginPlay
  (|CallParentFunction) ; This node is disabled and will not be called.\nDrag off pins to build functionality.
)

(event Collision|EventActorBeginOverlap
  (params (OtherActor :type Actor%20Object%20Reference))
  (|CallParentFunction OtherActor))

(event EventTick
  (params (DeltaSeconds :type Float%20%28single-precision%29))
  (|CallParentFunction DeltaSeconds) ; This node is disabled and will not be called.\nDrag off pins to build functionality.
)

(event EventNuageNoirDestroyed
  (bind _pfb_nuageeclairs_maui1 (Variables|Default|GetPFB_NuageEclairs_Maui1))
  ;[1 1 1] Nuage detruit
  (Sprite|SetFlipbook _pfb_nuageeclairs_maui1 "/Game/04_Maui/Asset2D/Animation/Decors/PFB_NuageNoirDeath_Maui1.PFB_NuageNoirDeath_Maui1")
  (Utilities|FlowControl|Delay (Class|PaperFlipbookComponent|GetFlipbookLength _pfb_nuageeclairs_maui1))
  (CallFunction|Finish)
  (Sprite|SetFlipbook _pfb_nuageeclairs_maui1 "/Game/04_Maui/Asset2D/Animation/Decors/Texture/FBP_NuageNoir.FBP_NuageNoir")
  (Audio|PlaySound2D "/Game/04_Maui/Sound/IG/S_MauiDamage_Maui.S_MauiDamage_Maui" 1.0 1.0 0.0 0 0)
  (Development|PrintString " !!!!!!!!!!!!!!!!!!!!!!!!!!!!!!!!!!!!!!!!!!!!!!!!!!!!!!!!!!!!!!!!!!!!!!!!!!!!!!!!!!!!!!!!!!" true true "(R=1.000000,G=1.000000,B=1.000000,A=1.000000)"))

(fn ConstructionScript
  (|CallParentFunction))