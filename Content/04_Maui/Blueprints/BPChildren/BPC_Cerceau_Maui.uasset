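; Maui-level child Blueprint of a hoop (cerceau) that reacts when the player pawn passes into it.
; On overlap it runs the parent handler, then checks that the other actor's class is exactly BP_PlayerPawn_Maui.
; For that pawn it triggers FxDestroy, sends PawnFlyingMessage and calls Finish on itself.
; BeginPlay, Tick and the construction script add no logic of their own.
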(event EventBeginPlay
  (|CallParentFunction) ; This node is disabled and will not be called.\nDrag off pins to build functionality.
)

(event Collision|EventActorBeginOverlap
  (params (OtherActor :type Actor%20Object%20Reference))
  ;[1 1 1] Player Collision
  (|CallParentFunction OtherActor)
  (if (== (Utilities|GetClass OtherActor) "/Game/04_Maui/Blueprints/BP_PlayerPawn_Maui.BP_PlayerPawn_Maui_C")
    (bind _asbp_player_pawn_maui (Utilities|Casting|CastToBP_PlayerPawn_Maui OtherActor))
    (Default|FxDestroy _asbp_player_pawn_maui)
    (Class|BPIMaui|PawnFlying(Message) OtherActor)
    (CallFunction|Finish)))

(event EventTick
  (params (DeltaSeconds :type Float%20%28single-precision%29))
  (|CallParentFunction DeltaSeconds) ; This node is disabled and will not be called.\nDrag off pins to build functionality.
)

(fn ConstructionScript
  (|CallParentFunction))