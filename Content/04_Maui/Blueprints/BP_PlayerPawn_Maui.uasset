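; Player pawn for the Maui level: a Paper2D character that swipes between left and right lanes, with a timed kite power-up for free flight.
; Looping timers drive crossing, touch-following flight, the countdown with low-time warning flipbooks, and falls.
; Hazard events end flight, destroy black clouds or trigger death, depending on flying and invincibility.
; Score, speed and game-over exchange messages with the GameMode.
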(event Custom|PLumeFx
  (bind _plume1 (Variables|Default|GetPlume1))
  ;[1 0 0] Stuffs
  (Audio|PlaySound2D "/Game/04_Maui/Sound/IG/S_WingGetProp2_Maui.S_WingGetProp2_Maui" 0.6 1.0 0.0 0 0)
  (Sprite|SetFlipbook _plume1 "/Game/04_Maui/Asset2D/Fx/PFB_SparklesPlumeFX_Maui2.PFB_SparklesPlumeFX_Maui2")
  (Sprite|SetSpriteColor _plume1 "(R=0.460541,G=0.910018,B=1.000000,A=1.000000)")
  (Audio|Components|Audio|Play _plume1)
  (Components|Timeline|SetLooping _plume1 false)
  (Utilities|FlowControl|Delay (Class|PaperFlipbookComponent|GetFlipbookLength _plume1))
  (Sprite|SetFlipbook _plume1))

(event Custom|CheckActualTouchLocation
  ;[1 1 1] Inputs
  (if (Variables|Default|GetNoInput)
    (Variables|Default|SetbIsTouched false)
    (Utilities|Time|ClearandInvalidateTimerbyHandle (Variables|Default|GetCheckSwipingKey))
    (else
      (Variables|Default|SetActualTouchLocation (.WorldLocation (Game|Player|ConvertMouseLocationToWorldSpace (Game|GetPlayerController 0))))
      (if (Math|Boolean|NORBoolean (Variables|Default|GetbIsFlying) (Variables|Default|GetbIsCrossing))
        (if (Variables|Default|GetbOnLeftSide)
          (if (< (.z (Variables|Default|GetActualTouchLocation)) (- (.z (Variables|Default|GetInitialTouchLocation)) 1e+01))
            (Utilities|Crossing
              (:End
                (Audio|PlaySound2D "/Game/04_Maui/Sound/IG/S_SonRandom_Maui.S_SonRandom_Maui" 1.0 1.0 0.0 0 0))))
          (elif (> (.z (Variables|Default|GetActualTouchLocation)) (+ (.z (Variables|Default|GetInitialTouchLocation)) 1e+01))
            (Utilities|Crossing
              (:End
                (Audio|PlaySound2D "/Game/04_Maui/Sound/IG/S_SonRandom_Maui.S_SonRandom_Maui" 1.0 1.0 0.0 0 0)))))))))

(event Custom|EndFlying
  ;[1 1 1] Flying
  (if (not (Variables|Default|GetNoInput))
    (Utilities|StopFlying)))

(event Custom|UpdateAnimation
  (params (State :type E_PlayerStateMachine%20Enum :default "NewEnumerator0"))
  ;[1 1 1] StateMachine
  (Sprite|SetFlipbook (Variables|Default|GetCharaRecto) (Utilities|Select :Index State :NewEnumerator0 "/Game/04_Maui/Asset2D/Animation/Maui/PFB_Running_Maui.PFB_Running_Maui" :NewEnumerator1 "/Game/04_Maui/Asset2D/Animation/Maui/PFB_CerfVolantFlying_Maui1.PFB_CerfVolantFlying_Maui1" :NewEnumerator2 "/Game/04_Maui/Asset2D/Animation/Maui/PFB_CerfVolantFlying_Maui1.PFB_CerfVolantFlying_Maui1" :NewEnumerator3 "/Game/04_Maui/Asset2D/Animation/Maui/PFB_Falling_Maui.PFB_Falling_Maui" :NewEnumerator4 "/Game/04_Maui/Asset2D/Animation/Maui/Electrocution/PFB_MauiElectrocution_Maui1.PFB_MauiElectrocution_Maui1" :NewEnumerator5 "/Game/04_Maui/Asset2D/Animation/Maui/PoweredUp/Sprite/PFB_CerfVolant_Maui1.PFB_CerfVolant_Maui1" :NewEnumerator6 "/Game/04_Maui/Asset2D/Animation/Maui/Flying/FX_EndCerfVolantJaune1.FX_EndCerfVolantJaune1" :NewEnumerator7 "/Game/04_Maui/Asset2D/Animation/Maui/Flying/FX_EndCerfVolantRouge1.FX_EndCerfVolantRouge1")))

(event Custom|FxDestroy
  (bind _cerceaufx (Variables|Default|GetCerceauFx))
  ;[1 0 0] Stuffs
  (Audio|PlaySound2D "/Game/04_Maui/Sound/IG/S_BonusCerceauProp2_Maui.S_BonusCerceauProp2_Maui" 0.8 1.0 0.0 0 0)
  (Sprite|SetFlipbook (Variables|Default|GetPlume) "/Game/04_Maui/Asset2D/Fx/PFB_SparklesPlumeFX_Maui1.PFB_SparklesPlumeFX_Maui1")
  (Sprite|SetFlipbook _cerceaufx "/Game/04_Maui/Asset2D/Fx/PFB_SparklesCerceauFX_Maui1.PFB_SparklesCerceauFX_Maui1")
  (Audio|Components|Audio|Play _cerceaufx)
  (Components|Timeline|SetLooping _cerceaufx false)
  (Utilities|FlowControl|Delay (Class|PaperFlipbookComponent|GetFlipbookLength _cerceaufx))
  (Sprite|SetFlipbook (Variables|Default|GetCerceauFx))
  (Sprite|SetFlipbook (Variables|Default|GetPlume)))

(event EventBeginPlay
  ;[1 1 1] BeginPlay
  (Variables|/Script/Engine.PlayerController|SetbShowMouseCursor (Game|GetPlayerController 0) true)
  (Variables|Default|SetNoInput true)
  (Variables|Default|SetLeftLocation (Transformation|GetWorldLocation (Variables|Default|GetLeftPoint)))
  (Variables|Default|SetRightLocation (Transformation|GetWorldLocation (Variables|Default|GetRightPoint)))
  (Variables|Default|SetSpeed (Variables|Default|GetInitialSpeed))
  (Collision|SetCollisionEnabled (Variables|Default|GetHitBox) "NoCollision")
  (Utilities|Time|SetTimerbyFunctionName 0 "FlyTimer" (Variables|Default|GetTimerDelay) true))

(event EventPawnFlying
  ;[1 1 1] Flying
  (if (Variables|Default|GetbIsFlying)
    (Variables|Default|SetTimerCoundown (Variables|Default|GetFlyDelay))
    (CallFunction|UpdateAnimation "NewEnumerator2")
    (else
      (Utilities|StartFlying))))

(event EventPawnScriptedCrossing
  (params (Cross :type Boolean))
  ;[1 1 1] Scripted Onboarding
  (if Cross
    (Utilities|Crossing
      (:End
        (Audio|PlaySound2D "/Game/04_Maui/Sound/IG/S_SonRandom_Maui.S_SonRandom_Maui" 1.0 1.0 0.0 0 0)))))

(event EventPawnAddScore
  ;[1 1 1] AddScore
  (bind _result (Math|Integer|IncrementInt (Variables|Default|GetScore))
    (:%20%20
      (Class|BPIMaui|GMAddScore(Message) (Game|GetGameMode) _result))))

(event EventPawnStartOnboarding
  ;[1 1 1] BeginPlay
  (if (not (Variables|Default|GetbGameHasStarted))
    (Variables|Default|SetbGameHasStarted true)
    (Collision|SetCollisionEnabled (Variables|Default|GetCloudDetection) "NoCollision")
    (Collision|SetCollisionEnabled (Variables|Default|GetHitBox) "QueryAndPhysics")
    (Class|BPIMaui|GMLaunchOnboarding(Message) (Game|GetGameMode))
    (Utilities|StopFlying)))

(event EventPawnDeathGreyCloud
  ;[1 1 1] Death
  (if (not (Variables|Default|GetbIsInvicible))
    (if (not (Variables|Default|GetbIsFlying))
      (Class|BPIMaui|GMEndGame(Message) (Game|GetGameMode))
      (Utilities|ClearTimers)
      (CallFunction|UpdateAnimation "NewEnumerator3")
      (Utilities|Time|SetTimerbyFunctionName 0 "FallHorizontally" (Variables|Default|GetTimerDelay) true)
      (Transformation|SetRelativeRotation (Variables|Default|GetCharaRoot) "0, 0, 0" false false))))

(event EventPawnDeathBird
  (params (Bird :type Actor%20Object%20Reference))
  ;[1 1 1] Death
  (if (not (Variables|Default|GetbIsInvicible))
    (if (Variables|Default|GetbIsFlying)
      (Utilities|StopFlying)
      (else
        (Class|BPIMaui|GMEndGame(Message) (Game|GetGameMode))
        (Utilities|ClearTimers)
        (CallFunction|UpdateAnimation "NewEnumerator3")
        (Utilities|Time|SetTimerbyFunctionName 0 "FallVertically" (Variables|Default|GetTimerDelay) true)
        (Transformation|SetRelativeRotation (Variables|Default|GetCharaRoot) "0, 0, 0" false false)))))

(event EventPawnDeathBlackCloud
  (params (Actor :type Actor%20Object%20Reference))
  ;[1 1 1] Death
  (if (or (Variables|Default|GetbIsInvicible) (Variables|Default|GetbIsFlying))
    (Utilities|IsValid Actor
      (:Is%20Valid
        (Class|BPIMaui|NuageNoirDestroyed(Message) Actor)))
    (else
      (Class|BPIMaui|GMEndGame(Message) (Game|GetGameMode))
      (Utilities|ClearTimers)
      (CallFunction|UpdateAnimation "NewEnumerator4")
      (Transformation|SetRelativeRotation (Variables|Default|GetCharaRoot) "0, 0, 0" false false)
      (Utilities|FlowControl|Delay 1.0)
      (CallFunction|UpdateAnimation "NewEnumerator3")
      (Utilities|Time|SetTimerbyFunctionName 0 "FallVertically" (Variables|Default|GetTimerDelay) true)
      (Transformation|SetRelativeRotation (Variables|Default|GetCharaRoot) "0, 0, 0" false false))))

(event EventPawnSetDifficulty
  (params (GMSpeed :type Float%20%28single-precision%29))
  (bind _returnvalue (/ GMSpeed 4.0))
  (bind _initialspeed (Variables|Default|GetInitialSpeed))
  (bind _returnvalue_2 (+ _returnvalue _initialspeed))
  ;[0 0.7428 1] SetCrossingSpeed
  (if (> _returnvalue_2 25.0)
    (Variables|Default|SetSpeed 25.0)
    (else
      (Variables|Default|SetSpeed _returnvalue_2))))

(event EventPawnStartGame
  ;[1 1 1] BeginPlay
  (Variables|Default|SetNoInput false)
  (Utilities|StopFlying))

(event EventPawnDeathSafeZone
  ;[1 1 1] Death
  (if (not (Variables|Default|GetbIsInvicible))
    (if (not (Variables|Default|GetbIsFlying))
      (Class|BPIMaui|GMEndGame(Message) (Game|GetGameMode))
      (Utilities|ClearTimers)
      (CallFunction|UpdateAnimation "NewEnumerator3")
      (Utilities|Time|SetTimerbyFunctionName 0 "FallHorizontally" (Variables|Default|GetTimerDelay) true)
      (Transformation|SetRelativeRotation (Variables|Default|GetCharaRoot) "0, 0, 0" false false))))

(event Input|ActionEvents|InputActionTouched
  (params (Key :type Key%20Structure))
  ;[1 1 1] Inputs
  (:Pressed
    (if (not (Variables|Default|GetNoInput))
      (Variables|Default|SetbIsTouched true)
      (Variables|Default|SetInitialTouchLocation (.WorldLocation (Game|Player|ConvertMouseLocationToWorldSpace (Game|GetPlayerController 0))))
      (bind _returnvalue (Utilities|Time|SetTimerbyEvent (delegate Custom|CheckActualTouchLocation) (Variables|Default|GetTimerDelay) true))
      (Variables|Default|SetCheckSwipingKey _returnvalue)))
  (:Released
    (Variables|Default|SetbIsTouched false)
    (Utilities|Time|ClearandInvalidateTimerbyHandle (Variables|Default|GetCheckSwipingKey))))

(event Input|KeyboardEvents|Z
  (params (Key :type Key%20Structure))
  ;[1 1 1] TestAddScore
  (:Pressed
    (CallFunction|PawnAddScore)))

(event Input|KeyboardEvents|W
  (params (Key :type Key%20Structure))
  ;[1 1 1] Inputs
  (:Pressed
    (if (not (Variables|Default|GetNoInput))
      (Variables|Default|SetbIsTouched true)
      (Variables|Default|SetInitialTouchLocation (.WorldLocation (Game|Player|ConvertMouseLocationToWorldSpace (Game|GetPlayerController 0))))
      (bind _returnvalue (Utilities|Time|SetTimerbyEvent (delegate Custom|CheckActualTouchLocation) (Variables|Default|GetTimerDelay) true))
      (Variables|Default|SetCheckSwipingKey _returnvalue)))
  (:Released
    (Variables|Default|SetbIsTouched false)
    (Utilities|Time|ClearandInvalidateTimerbyHandle (Variables|Default|GetCheckSwipingKey))))

(fn ConstructionScript)

(fn CrossTimer
  (if (Variables|Default|GetbOnLeftSide)
    (if (Math|Vector|Equal(Vector) (Transformation|GetWorldLocation (Variables|Default|GetCharaRoot)) (Variables|Default|GetLeftLocation) (Variables|Default|GetTolerance))
      (Transformation|SetWorldLocation (Variables|Default|GetCharaRoot) (Variables|Default|GetLeftLocation) false false)
      (Utilities|Time|ClearTimerbyFunctionName 0 "CrossTimer")
      (Variables|Default|SetbIsCrossing false)
      (Transformation|SetRelativeRotation (Variables|Default|GetCharaRoot) "0, 0,180.000000" false false)
      (CallFunction|UpdateAnimation "NewEnumerator0")
      (else
        (Transformation|AddWorldOffset (Variables|Default|GetCharaRoot) (* (Math|Vector|Normalize (- (Variables|Default|GetLeftLocation) (Transformation|GetWorldLocation (Variables|Default|GetCharaRoot))) 0.1) (Variables|Default|GetSpeed)) false false)
        (Transformation|AddRelativeRotation (Variables|Default|GetCharaRoot) "0, 0,20.000000" false false)))
    (elif (Math|Vector|Equal(Vector) (Transformation|GetWorldLocation (Variables|Default|GetCharaRoot)) (Variables|Default|GetRightLocation) (Variables|Default|GetTolerance))
      (Transformation|SetWorldLocation (Variables|Default|GetCharaRoot) (Variables|Default|GetRightLocation) false false)
      (Utilities|Time|ClearTimerbyFunctionName 0 "CrossTimer")
      (Variables|Default|SetbIsCrossing false)
      (Transformation|SetRelativeRotation (Variables|Default|GetCharaRoot) "0, 0, 0" false false)
      (CallFunction|UpdateAnimation "NewEnumerator0")
      (else
        (Transformation|AddWorldOffset (Variables|Default|GetCharaRoot) (* (Math|Vector|Normalize (- (Variables|Default|GetRightLocation) (Transformation|GetWorldLocation (Variables|Default|GetCharaRoot))) 0.1) (Variables|Default|GetSpeed)) false false)
        (Transformation|AddRelativeRotation (Variables|Default|GetCharaRoot) "0, 0,-20.000000" false false)))))

(fn FlyTimer
  (bind _speed (Variables|Default|GetSpeed))
  (bind _actualtouchlocation (Variables|Default|GetActualTouchLocation))
  (bind _chararoot (Variables|Default|GetCharaRoot))
  (bind _returnvalue (Transformation|GetWorldLocation _chararoot))
  (bind _returnvalue_2 (- _actualtouchlocation _returnvalue))
  (bind _returnvalue_3 (Math|Vector|Normalize _returnvalue_2 0.1))
  (bind _returnvalue_4 (* _returnvalue_3 _speed))
  (if (>= (.x (Transformation|GetWorldLocation (Variables|Default|GetCharaRoot))) -2e+01)
    _
    (else
      _))
  (if (Variables|Default|GetbIsTouched)
    (Transformation|AddWorldOffset (Variables|Default|GetCharaRoot) (Math|Vector|MakeVector 0.0 0.0 (.z _returnvalue_4)) false false)
    (if (> (.z _returnvalue_4) 0.0)
      (Transformation|SetRelativeRotation (Variables|Default|GetCharaRoot) "0, 0,60.000000" false false)
      (else
        (Transformation|SetRelativeRotation (Variables|Default|GetCharaRoot) "0, 0,-60.000000" false false)))
    (else
      (Transformation|SetRelativeRotation (Variables|Default|GetCharaRoot) "0, 0, 0" false false))))

(fn FallHorizontally
  (if (Variables|Default|GetbOnLeftSide)
    (if (> 0.0 (.z (Transformation|GetWorldLocation (Variables|Default|GetCharaRoot))))
      (Utilities|Time|ClearTimerbyFunctionName 0 "FallHorizontally")
      (else
        (Transformation|AddWorldOffset (Variables|Default|GetCharaRoot) "0.000000, 0,4.000000" false false)))
    (elif (< (.z (Transformation|GetWorldLocation (Variables|Default|GetCharaRoot))) -3e+02)
      (Utilities|Time|ClearTimerbyFunctionName 0 "FallHorizontally")
      (else
        (Transformation|AddWorldOffset (Variables|Default|GetCharaRoot) "0.000000, 0,-4.000000" false false)))))

(fn FallVertically
  (if (< (.x (Transformation|GetWorldLocation (Variables|Default|GetCharaRoot))) -3.5e+02)
    (Utilities|Time|ClearTimerbyFunctionName 0 "FallHorizontally")
    (else
      (Transformation|AddWorldOffset (Variables|Default|GetCharaRoot) "-4.000000, 0, 0" false false))))

(fn FlyTimerCountdown
  (bind _timercoundown (Variables|Default|GetTimerCoundown))
  (Math|Integer|DecrementInt _timercoundown
    (:%20%20
      (if (> _timercoundown 0)
        (if (== (Variables|Default|GetTimerCoundown) 3)
          (CallFunction|UpdateAnimation "NewEnumerator6")
          (elif (== (Variables|Default|GetTimerCoundown) 1)
            (CallFunction|UpdateAnimation "NewEnumerator7")))
        (else
          (CallFunction|EndFlying))))))