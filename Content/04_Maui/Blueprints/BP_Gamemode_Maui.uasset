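; Game mode for the Maui mini-game, running music, HUD, onboarding, score, difficulty and game over.
; Score and flying-state changes recompute Speed from game time, score and a flying bonus, capped at a maximum.
; Below the cap, it also resets the spawner timer and passes difficulty to the pawn.
; Game end stops music, disables input, notifies spawner, day-night cycle and clouds, then shows a star-rated result menu.
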(event Custom|SetDifficulty
  (bind _returnvalue (Utilities|Time|GetGameTimeinSeconds))
  (bind _initialspeed (Variables|Default|GetInitialSpeed))
  (bind _bisplayerflying (Variables|Default|GetbIsPlayerFlying))
  (bind _score (Variables|Default|GetScore))
  (bind _returnvalue_2 (Math|Conversions|ToFloat(Integer) _score))
  (bind _returnvalue_3 (select _bisplayerflying 5e+01 0.0))
  (bind _returnvalue_4 (/ _returnvalue_2 8.0))
  (bind _returnvalue_5 (* _returnvalue _returnvalue_4))
  (bind _returnvalue_6 (+ _initialspeed _returnvalue_5 _returnvalue_3))
  ;[1 0 0.0169] Keanu SetScale Difficulty
  (if (> _returnvalue_6 5e+02)
    (bind _output_get (Variables|Default|SetSpeed 5e+02))
    (Variables|Default|SetTolerance (- _output_get 2e+02))
    (else
      (bind _output_get_2 (Variables|Default|SetSpeed _returnvalue_6))
      (Variables|Default|SetTolerance (- _output_get_2 2e+02))
      (Class|BPIMaui|SpawnerResetTimer(Message) (Variables|Default|GetSpawner))
      (Class|BPIMaui|PawnSetDifficulty(Message) (Game|Player|GetPlayerPawn 0) _returnvalue_5))))

(event EventGMSetFlyingSpeed
  (params (bIsFlying :type Boolean))
  ;[1 1 1] FlyingSpeed
  (Variables|Default|SetbIsPlayerFlying bIsFlying)
  (CallFunction|SetDifficulty))

(event EventGMLaunchOnboarding
  ;[1 1 1] Obscales On
  (bind _returnvalue (UserInterface|CreateWidget "/Game/04_Maui/Widget/OnBoarding/WBP_Onboarding_Maui.WBP_Onboarding_Maui_C"))
  (Variables|Default|SetOnboarding _returnvalue)
  (Variables|/Game/04_Maui/Widget/OnBoarding/WBP_Onboarding_Maui.WBP_Onboarding_Maui_C|SetSpawner (Variables|Default|GetOnboarding) (Variables|Default|GetSpawner))
  (UserInterface|Viewport|AddtoViewport (Variables|Default|GetOnboarding) 0))

(event EventGMAddScore
  (params (Score :type Integer))
  ;[1 1 1] AddScore
  (bind _output_get (Variables|Default|SetScore Score))
  (Class|BPIMaui|HUDAddScore(Message) (Variables|Default|GetHUD) _output_get)
  ;;[1 0 0.05902] Comment
  (CallFunction|SetDifficulty))

(event EventGMEndGame
  ;[1 1 1] EndGame
  (Audio|Components|Audio|Stop (Variables|Default|GetMusicIG))
  (Audio|PlaySound2D "/Game/04_Maui/Sound/IG/S_MauiDamage_Maui.S_MauiDamage_Maui" 1.0 1.0 0.0 0 0)
  (Utilities|FlowControl|Delay 0.15)
  (Audio|PlaySound2D "/Game/04_Maui/Sound/IG/S_MauiDeath_Maui.S_MauiDeath_Maui" 1.0 1.0 0.0 0 0)
  (Class|BPIMaui|SpawnerEndGame(Message) (Variables|Default|GetSpawner))
  (Input|DisableInput (Game|Player|GetPlayerPawn 0) (Game|GetPlayerController 0))
  (Class|BPIMaui|SpawnerEndGame(Message) (Variables|Default|GetDayNightCycle))
  (for _array_element (Variables|Default|GetCloudsBG)
    (Class|BPIMaui|SpawnerEndGame(Message) _array_element))
  ;;[1 1 1] HUd EndGame
  (Utilities|FlowControl|Delay 1.0)
  (bind _returnvalue (UserInterface|CreateWidget "/Game/00_Metajeu/Widgets/WBP_MenuVictoire3.WBP_MenuVictoire3_C" 0 (Variables|Default|GetScore) 10 30 60))
  (UserInterface|Viewport|AddtoViewport _returnvalue 0)
  (Class|BPIMaui|SpawnerEndGame(Message) (Variables|Default|GetSpawner)))

(event EventBeginPlay
  ;[1 1 1] BeginPlay
  (bind _returnvalue (Audio|SpawnSound2D "/Game/04_Maui/Sound/S_MusicEcranTitreProp.S_MusicEcranTitreProp" 1.0 1.0 0.0 0))
  (Variables|Default|SetMusicIG _returnvalue)
  (Class|PlayerController|ActivateTouchInterface (Game|GetPlayerController 0))
  (bind _returnvalue_2 (UserInterface|CreateWidget "/Game/04_Maui/Widget/HUDEnvolDeMaui/HUD/WBP_InGame.WBP_InGame_C"))
  (bind _output_get (Variables|Default|SetHUD _returnvalue_2))
  (UserInterface|Viewport|AddtoViewport _output_get 0)
  (Variables|Default|SetSpeed (Variables|Default|GetInitialSpeed)))

(event EventTick
  (params (DeltaSeconds :type Float%20%28single-precision%29)))

(fn ConstructionScript)