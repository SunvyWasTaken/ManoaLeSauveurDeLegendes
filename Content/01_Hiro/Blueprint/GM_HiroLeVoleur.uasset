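; Game mode for the Hiro Le Voleur level, running the star score, countdown and end of game, and enabling the mobile touch interface.
; A looping one-second timer starts on PartyStart and ends the game at zero.
; Each score gain spawns a guard through the passed spawner to raise difficulty, and reaching three stars shows the victory widget with sound.
; DestroyBlocus removes the first BP_blocus found in the map.
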(event Custom|EventTimer
  ;[0 1 0.2078] Timer
  (bind _output_get (Variables|Timer|SetTimer (- (Variables|Timer|GetTimer) 1)))
  (if (<= _output_get 0)
    (GamePlay|FEndGame)))

(event Custom|PartyStart
  ;[0 1 0.2078] Timer
  (bind _returnvalue (Utilities|Time|SetTimerbyEvent (delegate Custom|EventTimer) 1.0 true))
  (Variables|Timer|SetHandlerTimer _returnvalue)
  (Development|PrintString "Party started!"))

(event Custom|DestroyBlocus
  ;[1 1 1] I know EXACTLY why it's here, but there IS another way... unfortunately, that would require to redo the WHOLE level
  ;;[1 1 1] Get all the blocus on the map and delete it when called
  (bind _outactors (Actor|GetAllActorsOfClass "/Game/01_Hiro/Blueprint/BP_blocus.BP_blocus_C"))
  (Actor|DestroyActor (Utilities|Array|Get(acopy) _outactors)))

(event EventBeginPlay
  ;[1 1 1] Show the mobile interface when game starts
  (Class|PlayerController|ActivateTouchInterface (Game|GetPlayerController 0) "/Game/01_Hiro/Blueprint/TI_HiroLeVoleur.TI_HiroLeVoleur"))

(fn ConstructionScript)

(fn FAddScore
  (params (GardeSpawnerRef :type BP%20Spawner%20Garde%20Object%20Reference%20%28by%20ref%29) (Value :type Integer))
  ;[1 1 1] Add to score when called (apparently) and then spawn another guard to higher up the difficulty
  (bind _output_get (Variables|Score|SetNbrOfEtoile (+ (Variables|Score|GetNbrOfEtoile) Value)))
  (Default|SpawnGarde GardeSpawnerRef _output_get)
  (Score|FScoring)
  (return))

(fn FEndGame
  ;[1 1 1] Stop the timer and finish the game when called (Accesoirly play a victory sound)
  (Utilities|Time|ClearandInvalidateTimerbyHandle (Variables|Timer|GetHandlerTimer))
  (Audio|PlaySound2D "/Game/01_Hiro/Sound/Wav/S_Victoire.S_Victoire" 1.0 1.0 0.0 0 0)
  (bind _returnvalue (UserInterface|CreateWidget "/Game/00_Metajeu/Widgets/WBP_MenuVictoire.WBP_MenuVictoire_C" 0 (Variables|Score|GetNbrOfEtoile) 1 2 3 1.0))
  (UserInterface|Viewport|AddtoViewport _returnvalue 0)
  (return))

(fn FScoring
  ;[1 1 1] Check if the player score when called. If the score is more or equal to 3, end the game.
  (if (>= (Variables|Score|GetNbrOfEtoile) 3)
    (Audio|PlaySound2D "/Game/01_Hiro/Sound/Wav/S_Victoire.S_Victoire" 1.0 1.0 0.0 0 0) ; Victory Sound
    (GamePlay|FEndGame)
    (return)))