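; Guard AI for BP_LeVoleur stealth: patrols between two target points with random pauses, then chases and arrests the detected player.
; Cone overlap starts a looping timer that fills a spotted meter, reset on exit; at threshold an alert emitter spawns and the chase begins.
; Hear overlap triggers the faster chase immediately, calling FSpotted, then FArrested on arrival.
; MakeSound diverts the guard to a given location before patrol resumes.
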(event OnComponentEndOverlap(Cone)
  (params (OverlappedComponent :type Primitive%20Component%20Object%20Reference) (OtherActor :type Actor%20Object%20Reference) (OtherComp :type Primitive%20Component%20Object%20Reference) (OtherBodyIndex :type Integer))
  ;[1 1 1] Lorsque Hiro sort de la zone de detection désative le timer et reste la marche.
  (if (and (== OtherActor (Variables|PlayerInteraction|GetPlayerRef)) (not (Variables|PlayerInteraction|GetArrest)))
    (Variables|AI|SetPercentSpotted 0.0)
    (Utilities|Time|ClearandInvalidateTimerbyHandle (Variables|AI|GetTimerSpotted))
    (CallFunction|Walk (Variables|AI|GetCurrentPoint))))

(event OnComponentBeginOverlap(Cone)
  (params (OverlappedComponent :type Primitive%20Component%20Object%20Reference) (OtherActor :type Actor%20Object%20Reference) (OtherComp :type Primitive%20Component%20Object%20Reference) (OtherBodyIndex :type Integer) (bFromSweep :type Boolean) (SweepResult :type Hit%20Result%20Structure%20%28by%20ref%29))
  ;[1 1 1] Detecte la colision avec le player
  (bind _asbp_le_voleur (Utilities|Casting|CastToBP_LeVoleur OtherActor))
  (Variables|PlayerInteraction|SetPlayerRef _asbp_le_voleur)
  (if (not (and (Variables|/Game/01_Hiro/Blueprint/BP_LeVoleur.BP_LeVoleur_C|GetbIsInSafeZone _asbp_le_voleur) (Variables|PlayerInteraction|GetArrest)))
    (CallFunction|PlayerDetected)))

(event OnComponentBeginOverlap(Hear)
  (params (OverlappedComponent :type Primitive%20Component%20Object%20Reference) (OtherActor :type Actor%20Object%20Reference) (OtherComp :type Primitive%20Component%20Object%20Reference) (OtherBodyIndex :type Integer) (bFromSweep :type Boolean) (SweepResult :type Hit%20Result%20Structure%20%28by%20ref%29))
  ;[1 1 1] Detecte la colision avec le player
  (bind _asbp_le_voleur (Utilities|Casting|CastToBP_LeVoleur OtherActor))
  (Variables|PlayerInteraction|SetPlayerRef _asbp_le_voleur)
  (if (not (and (Variables|/Game/01_Hiro/Blueprint/BP_LeVoleur.BP_LeVoleur_C|GetbIsInSafeZone _asbp_le_voleur) (Variables|PlayerInteraction|GetArrest)))
    (CallFunction|TheUnwantedChild)))

(event Custom|Walk
  (params (Index :type Integer))
  (bind _targetpoint (Variables|AI|GetTargetPoint))
  (bind _output (Utilities|Array|Get(acopy) _targetpoint 1))
  (bind _output_2 (Utilities|Array|Get(acopy) _targetpoint))
  (bind _returnvalue (Utilities|Select :Index Index :Option%200 _output :Option%201 _output_2))
  ;[1 1 1] Patrouille du garde
  (AI|AIMoveTo self "0, 0, 0" _returnvalue 5.0 true
    (:OnSuccess
      (Variables|AI|SetCurrentPoint (Utilities|Array|FindItem _targetpoint _returnvalue))
      (Utilities|FlowControl|Delay (Math|Random|RandomFloatinRange 0.5 2.0))
      (if (not (Variables|PlayerInteraction|GetArrest))
        (CallFunction|Walk (Variables|AI|GetCurrentPoint))))))

(event Custom|EventSpotted
  (bind _returnvalue (Transformation|GetActorLocation))
  (bind _playerref (Variables|PlayerInteraction|GetPlayerRef))
  ;[1 1 1] Timer lorsque le time est == à 1s lance le spotted puis arrest lorsqu'il atteind Hiro
  (bind _output_get (Variables|AI|SetPercentSpotted (+ (Variables|AI|GetPercentSpotted) 0.1)))
  (if (>= _output_get 0.6)
    (Utilities|Time|ClearandInvalidateTimerbyHandle (Variables|AI|GetTimerSpotted))
    (Effects|SpawnEmitteratLocation "/Game/01_Hiro/VFX/FX/P_AlertGarde.P_AlertGarde" (Math|Vector|MakeVector (.x _returnvalue) (.y _returnvalue) (+ (.z _returnvalue) 5e+01)))
    (Default|FSpotted _playerref)
    (Variables|/Script/Engine.CharacterMovementComponent|SetMaxWalkSpeed (Variables|Character|GetCharacterMovement) 3e+02) ; Speed Run
    (Variables|PlayerInteraction|SetArrest true)
    (AI|AIMoveTo self "0, 0, 0" _playerref 5.0 false
      (:OnSuccess
        (Default|FArrested _playerref)))))

(event Custom|PlayerDetected
  ;[1 1 1] Lorsque le garde detecte Hiro il se dirige vers lui
  (if (not (Variables|PlayerInteraction|GetArrest))
    (bind _returnvalue (Utilities|Time|SetTimerbyEvent (delegate Custom|EventSpotted) 0.1 true))
    (Variables|AI|SetTimerSpotted _returnvalue)))

(event Custom|TheUnwantedChild
  (bind _playerref (Variables|PlayerInteraction|GetPlayerRef))
  ;[1 1 1] Timer lorsque le time est == à 1s lance le spotted puis arrest lorsqu'il atteind Hiro
  (Default|FSpotted _playerref)
  (Variables|/Script/Engine.CharacterMovementComponent|SetMaxWalkSpeed (Variables|Character|GetCharacterMovement) 3e+02) ; Speed Run
  (Variables|PlayerInteraction|SetArrest true)
  (AI|AIMoveTo self "0, 0, 0" _playerref 5.0 false
    (:OnSuccess
      (Default|FArrested _playerref))))

(event EventBeginPlay
  (CallFunction|Walk))

(event EventMakeSound
  (params (Location :type Vector :default "0, 0, 0"))
  ;[1 1 1] Make a sound when called
  (Components|Movement|StopMovementImmediately (Variables|Character|GetCharacterMovement))
  (AI|AIMoveTo self Location 0 5.0 true
    (:OnSuccess
      (Utilities|FlowControl|Delay (Math|Random|RandomFloatinRange 0.5 2.0))
      (CallFunction|Walk (Variables|AI|GetCurrentPoint)))))

(fn ConstructionScript)