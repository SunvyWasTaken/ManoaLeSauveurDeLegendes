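; Safe zone actor where Hiro (BP_LeVoleur) is flagged as safe and shown pig pickup feedback.
; Box overlap sets the thief's safe-zone flag and toggles the pickup display; exit also notifies the in-game HUD through CallHim.
; The first entry adds a WBP_DropCochon_Hiro widget to the viewport.
; Two cubes act as the zone decal, hidden on BeginPlay and toggled by show/hide functions.
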(event OnComponentBeginOverlap(Box)
  (params (OverlappedComponent :type Primitive%20Component%20Object%20Reference) (OtherActor :type Actor%20Object%20Reference) (OtherComp :type Primitive%20Component%20Object%20Reference) (OtherBodyIndex :type Integer) (bFromSweep :type Boolean) (SweepResult :type Hit%20Result%20Structure%20%28by%20ref%29))
  ;[1 1 1] Check if Hiro's entering the SafeZone
  (bind _asbp_le_voleur (Utilities|Casting|CastToBP_LeVoleur OtherActor))
  (if (Variables|Boolean|GetbIsFirstTime) ; Check if it's the first time the player enter this zone
    ;[1 1 1] Notify Hiro that he's in a safe zone and show the PickUp FX
    (Variables|Boolean|SetbIsFirstTime false)
    (Variables|/Game/01_Hiro/Blueprint/BP_LeVoleur.BP_LeVoleur_C|SetbIsInSafeZone _asbp_le_voleur true)
    (Default|FShowPickup _asbp_le_voleur)
    (bind _returnvalue (UserInterface|CreateWidget "/Game/01_Hiro/HUD/WBP_DropCochon_Hiro.WBP_DropCochon_Hiro_C"))
    (UserInterface|Viewport|AddtoViewport _returnvalue 0)
    (else
      ;[1 1 1] Comment
      (Variables|/Game/01_Hiro/Blueprint/BP_LeVoleur.BP_LeVoleur_C|SetbIsInSafeZone _asbp_le_voleur true)
      (Default|FShowPickup _asbp_le_voleur))))

(event OnComponentEndOverlap(Box)
  (params (OverlappedComponent :type Primitive%20Component%20Object%20Reference) (OtherActor :type Actor%20Object%20Reference) (OtherComp :type Primitive%20Component%20Object%20Reference) (OtherBodyIndex :type Integer))
  ;[1 1 1] When the player leaves the safe zone, notify it he's out and "disable" the ability to pick up pigs
  (bind _asbp_le_voleur (Utilities|Casting|CastToBP_LeVoleur OtherActor))
  (Variables|/Game/01_Hiro/Blueprint/BP_LeVoleur.BP_LeVoleur_C|SetbIsInSafeZone _asbp_le_voleur false)
  (Default|FHidePickUp _asbp_le_voleur)
  (Default|CallHim (Variables|/Game/01_Hiro/Blueprint/BP_LeVoleur.BP_LeVoleur_C|GetHUD_InGameRef _asbp_le_voleur)))

(event EventBeginPlay
  (SomebodyHelpMePLZ...|FHideDecal))

(fn ConstructionScript)

(fn FShowDecal
  (Development|SetHiddeninGame (Variables|Default|GetCube) false false)
  (return))

(fn FHideDecal
  (Development|SetHiddeninGame (Variables|Default|GetCube) true false))