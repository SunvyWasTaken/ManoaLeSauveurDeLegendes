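; BP_Cochon is a pig actor that can be kidnapped and dropped elsewhere.
; PickUp hides it, disables collision and calls Kidnapped, which uses the Sphere overlap to send its location as a sound message to BP_Garde guards.
; DropCochon moves and unhides it without re-enabling collision.
; ResetCochon hides its cylinders, point light and FXPasHerbe1 effect.
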(fn ConstructionScript)

(fn PickUp
  ;[1 1 1] Hide the pig and disable collisions
  (Rendering|SetActorHiddenInGame true)
  (Collision|SetActorEnableCollision false)
  (CallFunction|Kidnapped)
  (return))

(fn DropCochon
  (params (Location :type Vector))
  (Transformation|SetActorLocation Location false false)
  (Rendering|SetActorHiddenInGame false)
  (return))

(fn Kidnapped
  ;[1 1 1] Emit a sound at the pig location when it is being kidnapped
  (for _array_element (Collision|GetOverlappingActors (Variables|Default|GetSphere) "/Game/01_Hiro/Blueprint/BP_Garde.BP_Garde_C" :!class /Script/Engine.PrimitiveComponent)
    (Class|BPINoise|MakeSound(Message) _array_element (Transformation|GetActorLocation))
    (Development|PrintString "Kidnapped")
    (return)))

(fn ResetCochon
  ;[1 1 1] Hide all that
  (Development|SetHiddeninGame (Variables|Default|GetCylinder1) true false)
  (return))