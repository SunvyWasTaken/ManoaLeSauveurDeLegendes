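; Player character Hiro for a stealth minigame about stealing pigs past guards and scoring by dropping them in a safe zone.
; Handles movement, sprint that alerts guards within noise range, and overlap-based pig pickup that blocks sprint toggling and slows him until delivery.
; Also drives the HUD, tutorial widgets, camera blends, audio parameters, FX and popup sprites, and exposes spotted, arrested and grass functions, reporting score and game end to the GameMode.
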(event OnComponentBeginOverlap(PickUpRange)
  (params (OverlappedComponent :type Primitive%20Component%20Object%20Reference) (OtherActor :type Actor%20Object%20Reference) (OtherComp :type Primitive%20Component%20Object%20Reference) (OtherBodyIndex :type Integer) (bFromSweep :type Boolean) (SweepResult :type Hit%20Result%20Structure%20%28by%20ref%29))
  ;[0.04394 1 0] Event Collision avec le Cochon
  (bind _asbp_cochon (Utilities|Casting|CastToBP_Cochon OtherActor)) ; Just a lazy way to check if what colided is the pig
  (if (not (Variables|Mechanic|GetbIsPigPickedUp)) ; Check if the pig is not picked up, if it's the case, you can pick him up
    (Variables|Booleans|SetbCanPickUp true)
    (Variables|References|SetBP_Cochon_Ref _asbp_cochon) ; Store the pig's ref when all previous are gud
    (HUD|FShowPickup) ; Show's the pick up interface I gues
  ))

(event OnComponentEndOverlap(PickUpRange)
  (params (OverlappedComponent :type Primitive%20Component%20Object%20Reference) (OtherActor :type Actor%20Object%20Reference) (OtherComp :type Primitive%20Component%20Object%20Reference) (OtherBodyIndex :type Integer))
  ;[0.04394 1 0] Event Collision avec le Cochon
  (if (and (== OtherActor (Variables|References|GetBP_Cochon_Ref)) (not (Variables|Mechanic|GetbIsPigPickedUp))) ; Check if the pig is actually leaving hiro's reach and if Hiro did not picked it up
    (Variables|Booleans|SetbCanPickUp false)
    (Variables|References|SetBP_Cochon_Ref 0) ; get rid of the pig's reference
    (HUD|FHidePickUp)))

(event Custom|HideSprite
  (params (SpriteRef :type Paper%20Sprite%20Actor%20Object%20Reference))
  ;[1 1 1] Hide le sprite
  (Rendering|SetActorHiddenInGame SpriteRef false)
  (Utilities|FlowControl|Delay 2.0)
  (Rendering|SetActorHiddenInGame SpriteRef true))

(event Custom|Running
  ;[1 1 1] Appel les gardes lorsque tu commence à courir.
  (Utilities|FlowControl|DoOnce false
    (:Completed
      (for _array_element (Collision|GetOverlappingActors (Variables|Default|GetRangeNoise) "/Game/01_Hiro/Blueprint/BP_Garde.BP_Garde_C" :!class /Script/Engine.PrimitiveComponent)
        (Class|BPINoise|MakeSound(Message) _array_element (Transformation|GetActorLocation))))))

(event Custom|LetsGo
  (Default|PartyStart (Variables|References|GetGM_HiroLeVoleurRef)))

(event Custom|StartGame
  ;[0 1 0.1145] Begin Play Creation du Widget InGame
  (Input|SetInputModeGameOnly (Game|GetPlayerController 0))
  (Camera|FChangeView false)
  (Utilities|FlowControl|Delay 0.4)
  (bind _returnvalue (UserInterface|CreateWidget "/Game/01_Hiro/HUD/WBP_TutoMove_Hiro.WBP_TutoMove_Hiro_C"))
  (UserInterface|Viewport|AddtoViewport _returnvalue 0)
  (bind _returnvalue_2 (UserInterface|CreateWidget "/Game/01_Hiro/HUD/WBP_HiroLeVoleurDeCochon.WBP_HiroLeVoleurDeCochon_C" (Game|GetPlayerController 0) self))
  (bind _output_get (Variables|References|SetHUD_InGameRef _returnvalue_2))
  (UserInterface|Viewport|AddtoViewport _output_get 0)
  (Sound|FWalkDirt)
  (Effects|Components|ParticleSystem|SetBoolParameter (Variables|Default|GetAudio) "Pig" (Variables|Mechanic|GetbIsPigPickedUp)))

(event EventPickPig
  ;[0 1 0.9831] Evenement lorsque hiro prend le Cochon.
  (if (not (and (Variables|Booleans|GetbIsInSafeZone) (Variables|Mechanic|GetbIsPigPickedUp)))
    (if (and (Variables|Booleans|GetbCanPickUp) (not (Variables|Mechanic|GetbIsPigPickedUp)))
      (Variables|Mechanic|SetbIsPigPickedUp true)
      (Interaction|FPopUp (Variables|SpriteReferences|GetSPR_RamaserRef))
      (Default|PickUp (Variables|References|GetBP_Cochon_Ref))
      (Audio|PlaySound2D "/Game/01_Hiro/Sound/Wav/S_GrabUrCochon.S_GrabUrCochon" 1.3 1.0 0.0 0 0)
      (Mechanic|FSlowMotion)
      (Interaction|FPlaySoundPig)
      (Default|FShowDecal (Variables|References|GetBp_SafeZoneRef))
      (Rendering|SetVisibility (Variables|Default|GetCochonMesh) true false)
      (Effects|Components|ParticleSystem|SetBoolParameter (Variables|Default|GetAudio) "Pig" (Variables|Mechanic|GetbIsPigPickedUp))
      (HUD|FHideSprint)
      (HUD|FHidePickUp)
      (Components|Activation|Activate (Variables|Default|GetFX_PasHerbe1) true)
      (Default|ResetCochon (Variables|References|GetBP_Cochon_Ref))
      (if (Variables|Booleans|GetFistOnBoarding)
        (Utilities|FlowControl|Delay 0.2)
        (bind _returnvalue (UserInterface|CreateWidget "/Game/01_Hiro/HUD/WBP_Objectif_GoSafeZone_Hiro.WBP_Objectif_GoSafeZone_Hiro_C"))
        (UserInterface|Viewport|AddtoViewport _returnvalue 0)
        (Camera|FChangeView true)
        (Variables|Booleans|SetFistOnBoarding false)))
    (else
      (Variables|Booleans|SetbCanPickUp false)
      (Default|DropCochon (Variables|References|GetBP_Cochon_Ref) (- (Transformation|GetActorLocation) "0, 0,50.000000"))
      (Audio|PlaySound2D "/Game/01_Hiro/Sound/Wav/S_DropTheCochon.S_DropTheCochon" 1.0 1.0 0.0 0 0)
      (Variables|References|SetBP_Cochon_Ref 0)
      (Default|FAddScore (Variables|References|GetGM_HiroLeVoleurRef) (Variables|References|GetSpawnerGardeRef) 1)
      (Mechanic|FResetMotion)
      (Interaction|FPopUp (Variables|SpriteReferences|GetSPR_VolerRef))
      (Effects|Components|ParticleSystem|SetTemplate (Variables|Default|GetParticleSystem) "/Game/01_Hiro/VFX/FX/FX_StarEarn.FX_StarEarn")
      (Interaction|FPlaySoundPig)
      (Variables|Mechanic|SetbIsPigPickedUp false)
      (Default|FHideDecal (Variables|References|GetBp_SafeZoneRef))
      (Rendering|SetVisibility (Variables|Default|GetCochonMesh) false false)
      (Effects|Components|ParticleSystem|SetBoolParameter (Variables|Default|GetAudio) "Pig" (Variables|Mechanic|GetbIsPigPickedUp))
      (HUD|FShowSprint)
      (Default|AnimCompteur (Variables|References|GetHUD_InGameRef))
      (Components|Activation|Deactivate (Variables|Default|GetFX_PasHerbe1)))))

(event EventPresseSprint
  ;[0.01576 1 0] Sprint
  ;;[1 1 1] Sprint Pressed
  (if (not (Variables|Mechanic|GetbIsPigPickedUp)) ; Check if the players has the pig. If he doesn't, he can sprint
    (Variables|Booleans|SetbIsRunning true)
    (if (Variables|Mechanic|GetbIsHiroSlow) ; Check if Hiro is slow. If he is, his runspeed is divided by speed reduction
      (Variables|/Script/Engine.CharacterMovementComponent|SetMaxWalkSpeed (Variables|Character|GetCharacterMovement) (/ (Variables|CharacterSpeed|GetRunSpeed) (Variables|CharacterSpeed|GetSpeedReduction)))
      (else
        (Variables|/Script/Engine.CharacterMovementComponent|SetMaxWalkSpeed (Variables|Character|GetCharacterMovement) (Variables|CharacterSpeed|GetRunSpeed))))
    (Sound|FSprintFXon)))

(event EventBeginPlay
  ;[1 1 1] Set la reference du gamemode pour éviter de le cast
  (Game|SetGamePaused true)
  (bind _asgm_hiro_le_voleur (Utilities|Casting|CastToGM_HiroLeVoleur (Game|GetGameMode)))
  (Variables|References|SetGM_HiroLeVoleurRef _asgm_hiro_le_voleur)
  (bind _returnvalue (UserInterface|CreateWidget "/Game/01_Hiro/HUD/WBP_Objectif_GetCochon_Hiro.WBP_Objectif_GetCochon_Hiro_C"))
  (UserInterface|Viewport|AddtoViewport _returnvalue 0))

(event EventReleaseSprint
  (bind _charactermovement (Variables|Character|GetCharacterMovement))
  ;[0.01576 1 0] Sprint
  ;;[1 1 1] EventUnSprint
  (if (not (Variables|Mechanic|GetbIsPigPickedUp))
    (Variables|Booleans|SetbIsRunning false)
    (if (Variables|Mechanic|GetbIsHiroSlow)
      (Variables|/Script/Engine.CharacterMovementComponent|SetMaxWalkSpeed _charactermovement (/ (Variables|CharacterSpeed|GetWalkSpeed) (Variables|CharacterSpeed|GetSpeedReduction)))
      (else
        (Variables|/Script/Engine.CharacterMovementComponent|SetMaxWalkSpeed _charactermovement (Variables|CharacterSpeed|GetWalkSpeed))))
    (Sound|FSprintFXOff)))

(event Input|AxisEvents|InputAxisMoveForwardHiroLeVoleur
  (params (AxisValue :type Float%20%28single-precision%29))
  ;[0 1 0.07112] Déplacement de Hiro.
  (Pawn|Input|AddMovementInput self (Math|Vector|MakeVector 1.0 0.0 0.0) AxisValue false)
  (if (and (Variables|Booleans|GetbIsRunning) (> (Math|Vector|VectorLength (Transformation|GetVelocity)) 0.0))
    (CallFunction|Running)
    (else
      ;[1 1 1] Appel les gardes lorsque tu commence à courir.
      (Utilities|FlowControl|DoOnce false) ; enters at Reset
    )))

(event Input|AxisEvents|InputAxisMoveRightHiroLeVoleur
  (params (AxisValue :type Float%20%28single-precision%29))
  ;[0 1 0.07112] Déplacement de Hiro.
  (Pawn|Input|AddMovementInput self (Math|Vector|MakeVector 0.0 1.0 0.0) AxisValue false)
  (if (and (Variables|Booleans|GetbIsRunning) (> (Math|Vector|VectorLength (Transformation|GetVelocity)) 0.0))
    (CallFunction|Running)
    (else
      ;[1 1 1] Appel les gardes lorsque tu commence à courir.
      (Utilities|FlowControl|DoOnce false) ; enters at Reset
    )))

(fn ConstructionScript
  (Variables|/Script/Engine.CharacterMovementComponent|SetMaxWalkSpeed (Variables|Character|GetCharacterMovement) (Variables|CharacterSpeed|GetWalkSpeed)))

(fn FSpotted
  (Components|Movement|StopMovementImmediately (Variables|Character|GetCharacterMovement))
  (Variables|Mechanic|SetbIsHiroSpotted true)
  (Input|DisableInput (Game|GetPlayerController 0))
  (Interaction|FPopUp (Variables|SpriteReferences|GetSPR_RepereRef))
  (Interaction|FPlaySoundPig)
  (Camera|FChangeView true)
  (return))

(fn FSlowMotion
  (Variables|Mechanic|SetbIsHiroSlow true)
  (Effects|Components|ParticleSystem|SetTemplate (Variables|Default|GetParticleSystem) "/Game/01_Hiro/VFX/FX/FX_Slow.FX_Slow")
  (if (Variables|Booleans|GetbIsRunning)
    (Variables|/Script/Engine.CharacterMovementComponent|SetMaxWalkSpeed (Variables|Character|GetCharacterMovement) (/ (Variables|CharacterSpeed|GetRunSpeed) (Variables|CharacterSpeed|GetSpeedReduction)))
    (else
      (Variables|/Script/Engine.CharacterMovementComponent|SetMaxWalkSpeed (Variables|Character|GetCharacterMovement) (/ (Variables|CharacterSpeed|GetWalkSpeed) (Variables|CharacterSpeed|GetSpeedReduction)))))
  (return))

(fn FResetMotion
  (Variables|Mechanic|SetbIsHiroSlow false)
  (if (not (Variables|Mechanic|GetbIsPigPickedUp))
    (Components|DestroyComponent (Variables|Default|GetParticleSystem))
    (if (Variables|Booleans|GetbIsRunning)
      (Variables|/Script/Engine.CharacterMovementComponent|SetMaxWalkSpeed (Variables|Character|GetCharacterMovement) (Variables|CharacterSpeed|GetRunSpeed))
      (else
        (Variables|/Script/Engine.CharacterMovementComponent|SetMaxWalkSpeed (Variables|Character|GetCharacterMovement) (Variables|CharacterSpeed|GetWalkSpeed))))
    (return)
    (else
      (return))))

(fn FArrested
  (Variables|Booleans|SetbIsbIsHiroArrested true)
  (Default|FEndGame (Variables|References|GetGM_HiroLeVoleurRef))
  (return))

(fn FPopUp
  (params (Sprite :type Paper%20Sprite%20Actor%20Object%20Reference))
  (bind _returnvalue (Transformation|GetActorLocation))
  (bind (_x _y _z) (Math|Vector|BreakVector _returnvalue))
  (Transformation|SetActorLocation Sprite (Math|Vector|MakeVector _x _y (+ _z 8e+01)) false true)
  (Transformation|SetActorScale3D Sprite "0.250000,0.250000,0.250000")
  (CallFunction|HideSprite Sprite)
  (return))

(fn FPlaySoundPig
  (if (Variables|Mechanic|GetbIsPigPickedUp)
    (Audio|PlaySound2D "/Game/01_Hiro/Sound/Cue_Cochon.Cue_Cochon" 1.0 1.0 0.0 0 0))
  (return))

(fn FChangeView
  (params (TopView? :type Boolean))
  (if TopView?
    (Game|Player|SetViewTargetwithBlend (Game|GetPlayerController 0) (Variables|References|GetCameraWorldRef) 1.0 "VTBlend_Linear" 0.0 false)
    (else
      (Game|Player|SetViewTargetwithBlend (Game|GetPlayerController 0) self 1.0 "VTBlend_Linear" 0.0 false)))
  (return))

(fn FHidePickUp
  (Default|HidePickUp (Variables|References|GetHUD_InGameRef))
  (return))

(fn FHideSprint)

(fn FShowPickup
  (Default|ShowPickUp (Variables|References|GetHUD_InGameRef))
  (return))

(fn FShowSprint
  (Default|ShowSprint (Variables|References|GetHUD_InGameRef))
  (return))

(fn FinGrass
  (Components|Activation|Activate (Variables|Default|GetParticleSystem1) false)
  (Variables|Booleans|SetbIsFxOn? true))

(fn FinGrassOff
  (if (Variables|Booleans|GetbIsFxOn?)
    (Components|Activation|Deactivate (Variables|Default|GetParticleSystem1))
    (return)))

(fn FWalkDirt
  (Effects|Components|ParticleSystem|SetBoolParameter (Variables|Default|GetAudio) "Grass" false)
  (return))

(fn FWalkGrass
  (if (Variables|Booleans|GetbFirstTimeBush)
    (Utilities|FlowControl|DoOnce false
      (:Completed
        (Variables|Booleans|SetbFirstTimeBush false)
        (bind _returnvalue (UserInterface|CreateWidget "/Game/01_Hiro/HUD/WBP_TutoDiscretion_Hiro.WBP_TutoDiscretion_Hiro_C"))
        (UserInterface|Viewport|AddtoViewport _returnvalue 0))))
  (Effects|Components|ParticleSystem|SetBoolParameter (Variables|Default|GetAudio) "Grass" true)
  (return))

(fn FSprintFXon
  (Components|Activation|Activate (Variables|Default|GetFX_PasHerbe2) false))

(fn FSprintFXOff
  (Components|Activation|Deactivate (Variables|Default|GetFX_PasHerbe2)))