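; BP_PlatformeCassable is a breakable platform actor, with a box trigger that calls TriggerCassage when BP_TafaiRunner overlaps it.
; TriggerCassage is empty, so the overlap currently breaks nothing.
; Disconnected nodes hold the break sequence: a looping timer on Cassage jitters pitch; after a delay, the timer clears, collision drops, meshes animate, Break activates and the pieces hide.
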(event OnComponentBeginOverlap(BoxTriggerCassage)
  (params (OverlappedComponent :type Primitive%20Component%20Object%20Reference) (OtherActor :type Actor%20Object%20Reference) (OtherComp :type Primitive%20Component%20Object%20Reference) (OtherBodyIndex :type Integer) (bFromSweep :type Boolean) (SweepResult :type Hit%20Result%20Structure%20%28by%20ref%29))
  ;[1 1 1] Trig cassage
  (Utilities|Casting|CastToBP_TafaiRunner OtherActor)
  (CallFunction|TriggerCassage))

(event Custom|TriggerCassage
  ;[1 1 1] Cassage de la plateforme
)

(event Custom|Cassage
  ;[1 1 1] Cassage de la plateforme
  (Transformation|SetActorRotation (Math|Rotator|MakeRotator (Variables|Default|GetRollValue) (+ (Variables|Default|GetPitchValue) (Math|Conversions|ToFloat(Integer) (Math|Random|RandomIntegerinRange -2 2))) (Variables|Default|GetYawValue))))

(event EventBeginPlay)

(event Collision|EventActorBeginOverlap
  (params (OtherActor :type Actor%20Object%20Reference)))

(event EventTick
  (params (DeltaSeconds :type Float%20%28single-precision%29)))

(fn ConstructionScript
  (|CallParentFunction))