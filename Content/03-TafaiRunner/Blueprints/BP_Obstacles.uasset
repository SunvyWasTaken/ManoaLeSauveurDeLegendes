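; BP_Obstacles is a moving rock obstacle in Tafai Runner that drains the player's mana on contact unless they are dashing.
; Any player overlap plays the break particles and sound and hides the rock mesh.
; A looping timer offsets the actor along its direction once activated.
; Stopping clears that timer, hands the obstacle back to its BP_SpawnPlatforms owner and re-shows the mesh, suggesting pooled reuse.
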(event OnComponentBeginOverlap(Box)
  (params (OverlappedComponent :type Primitive%20Component%20Object%20Reference) (OtherActor :type Actor%20Object%20Reference) (OtherComp :type Primitive%20Component%20Object%20Reference) (OtherBodyIndex :type Integer) (bFromSweep :type Boolean) (SweepResult :type Hit%20Result%20Structure%20%28by%20ref%29))
  (bind _asbp_tafai_runner (Utilities|Casting|CastToBP_TafaiRunner OtherActor))
  (bind _output_get (Variables|Default|SetTafaiRef _asbp_tafai_runner))
  (if (Variables|/Game/03-TafaiRunner/Blueprints/BP_TafaiRunner.BP_TafaiRunner_C|GetbIsDashing _output_get)
    _
    (else
      (Default|SuckMana (Variables|Default|GetTafaiRef) (Variables|Default|GetManaToRemoveOnHit))))
  (Components|Activation|Activate (Variables|Default|GetBreakRockSystem) false)
  (Audio|PlaySound2D "/Game/03-TafaiRunner/SFX/SC_break_obstacle.SC_break_obstacle" 1.0 1.0 0.0 0 0)
  (Rendering|SetVisibility (Variables|Default|GetPackABillPirogueRocherTikiHerbe_SM_Rocher) false false))

(event Custom|ActivatePlatform
  (bind _returnvalue (Utilities|Time|SetTimerbyEvent (delegate Custom|Movement) 0.01 true))
  (Variables|Default|SetTimerMovement _returnvalue))

(event Custom|Movement
  (Transformation|AddActorWorldOffset (* (Variables|Default|GetDirectionToGo) (Variables|Default|GetIntensityMovement))))

(event Custom|StopMovement
  (Utilities|Time|ClearandInvalidateTimerbyHandle (Variables|Default|GetTimerMovement))
  (bind _asbp_spawn_platforms (Utilities|Casting|CastToBP_SpawnPlatforms (Components|GetOwner)))
  (Default|RestoreObstacles _asbp_spawn_platforms self)
  (Rendering|SetVisibility (Variables|Default|GetPackABillPirogueRocherTikiHerbe_SM_Rocher) true false))

(fn ConstructionScript)