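; BP_PlatformeCassable_Child is a breakable platform for the TafaiRunner game that collapses after the runner steps on it.
; An overlap with the runner not moving upward starts the break and a rumble sound that fades out.
; A looping timer jitters the pitch around the saved rotation for a configurable delay.
; Collision is then disabled, break animations and effect play, and the platform pieces are hidden shortly after.
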(event OnComponentBeginOverlap(BoxTriggerCassage)
  (params (OverlappedComponent :type Primitive%20Component%20Object%20Reference) (OtherActor :type Actor%20Object%20Reference) (OtherComp :type Primitive%20Component%20Object%20Reference) (OtherBodyIndex :type Integer) (bFromSweep :type Boolean) (SweepResult :type Hit%20Result%20Structure%20%28by%20ref%29))
  ;[1 1 1] Trig cassage
  (bind _asbp_tafai_runner (Utilities|Casting|CastToBP_TafaiRunner OtherActor))
  (if (<= (.z (Transformation|GetVelocity _asbp_tafai_runner)) 0.1)
    (CallFunction|TriggerCassage)
    (CallFunction|TriggerRumble)))

(event Custom|TriggerCassage
  (bind _plateforme (Variables|Default|GetPlateforme))
  ;[1 1 1] Cassage de la plateforme
  (Utilities|SetRotations)
  (bind _returnvalue (Utilities|Time|SetTimerbyEvent (delegate Custom|Cassage) 0.05 true))
  (Variables|Default|SetCassageTimer _returnvalue)
  (Utilities|FlowControl|Delay (Variables|Default|GetDelayAvantCassage))
  (Utilities|Time|ClearandInvalidateTimerbyHandle (Variables|Default|GetCassageTimer))
  (Collision|SetCollisionEnabled _plateforme "NoCollision")
  (Components|Animation|PlayAnimation (Variables|Default|GetPlateforme1) "/Game/03-TafaiRunner/Mesh/Plateformes/A_Break.A_Break" false)
  (Components|Activation|Activate (Variables|Default|GetBreak) false)
  (Utilities|FlowControl|Delay 0.8)
  (Rendering|SetVisibility _plateforme false false))

(event Custom|Cassage
  ;[1 1 1] Cassage de la plateforme
  (Transformation|SetActorRotation (Math|Rotator|MakeRotator (Variables|Default|GetRollValue) (+ (Variables|Default|GetPitchValue) (Math|Conversions|ToFloat(Integer) (Math|Random|RandomIntegerinRange -2 2))) (Variables|Default|GetYawValue))))

(event Custom|trigger_rumble
  (Audio|Components|Audio|Play (Variables|Default|Getrumble) 0.0)
  (Utilities|FlowControl|Delay 0.9)
  (Audio|Components|Audio|FadeOut (Variables|Default|Getrumble) 0.5 0.0 "Linear" :!class /Script/Engine.AudioComponent))

(fn ConstructionScript
  (|CallParentFunction))