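; BP_EndLand_Tafai is the end-of-run land in Tafai Runner, a moving actor that finishes the run when the player reaches it.
; A fast looping timer offsets it along a set direction and intensity.
; It publishes its world position every tick, plus a radius at start, to a Material Parameter Collection.
; Overlapping the StopMove component flags the runner's run as ended, stops the movement timer and calls EndGame on the GameMode.
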(event OnComponentBeginOverlap(StopMove)
  (params (OverlappedComponent :type Primitive%20Component%20Object%20Reference) (OtherActor :type Actor%20Object%20Reference) (OtherComp :type Primitive%20Component%20Object%20Reference) (OtherBodyIndex :type Integer) (bFromSweep :type Boolean) (SweepResult :type Hit%20Result%20Structure%20%28by%20ref%29))
  (bind _asbp_tafai_runner (Utilities|Casting|CastToBP_TafaiRunner OtherActor))
  (Variables|/Game/03-TafaiRunner/Blueprints/BP_TafaiRunner.BP_TafaiRunner_C|SetbEndRun _asbp_tafai_runner true)
  (Utilities|Time|ClearandInvalidateTimerbyHandle (Variables|Default|GetMovementHandle))
  (Default|EndGame (Variables|Default|GetGameModeRef)))

(event Custom|Movement
  (Transformation|AddActorWorldOffset (* (Variables|Default|GetDirectionToGo) (Variables|Default|GetIntensityMovement))))

(event EventBeginPlay
  (bind _returnvalue (Utilities|Time|SetTimerbyEvent (delegate Custom|Movement) 0.01 true))
  (Variables|Default|SetMovementHandle _returnvalue)
  (Rendering|Material|SetScalarParameterValue "/Game/03-TafaiRunner/Materials/MPC_TafaiRunner.MPC_TafaiRunner" "Radius" 5e+02 :!class /Script/Engine.KismetMaterialLibrary)
  (bind _asgm_tafai_runner (Utilities|Casting|CastToGM_TafaiRunner (Game|GetGameMode)))
  (Variables|Default|SetGameModeRef _asgm_tafai_runner))

(event Collision|EventActorBeginOverlap
  (params (OtherActor :type Actor%20Object%20Reference)))

(event EventTick
  (params (DeltaSeconds :type Float%20%28single-precision%29))
  (bind _returnvalue (Transformation|GetActorLocation))
  (Rendering|Material|SetVectorParameterValue "/Game/03-TafaiRunner/Materials/MPC_TafaiRunner.MPC_TafaiRunner" "IslandWorldPosition" (Utilities|Struct|MakeLinearColor (.x _returnvalue) (.y _returnvalue) (.z _returnvalue) 1.0) :!class /Script/Engine.KismetMaterialLibrary))

(fn ConstructionScript)