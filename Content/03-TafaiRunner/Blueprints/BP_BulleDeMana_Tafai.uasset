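; Mana bubble pickup for TafaiRunner that grants a fixed amount of mana and plays a sound when BP_TafaiRunner overlaps its sphere.
; ActivateMana starts a looping timer that offsets the bubble along DirectionToGo by IntensityMovement, without Tick or sweep.
; StopMovement clears the timer and hands the bubble back to its BP_SpawnPlatforms owner through RestoreMana for reuse, or destroys it without such an owner.
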(event OnComponentBeginOverlap(Sphere1)
  (params (OverlappedComponent :type Primitive%20Component%20Object%20Reference) (OtherActor :type Actor%20Object%20Reference) (OtherComp :type Primitive%20Component%20Object%20Reference) (OtherBodyIndex :type Integer) (bFromSweep :type Boolean) (SweepResult :type Hit%20Result%20Structure%20%28by%20ref%29))
  (bind _asbp_tafai_runner (Utilities|Casting|CastToBP_TafaiRunner OtherActor))
  (Default|UpdateMana _asbp_tafai_runner 2e+01)
  (Audio|PlaySound2D "/Game/03-TafaiRunner/SFX/SC_get_mana.SC_get_mana" 1.0 1.0 0.0 0 0))

(event Custom|ActivateMana
  ;[1 1 1] Movement
  (bind _returnvalue (Utilities|Time|SetTimerbyEvent (delegate Custom|Movement) 0.01 true))
  (Variables|Default|SetTimerMovement _returnvalue)
  (Variables|Default|SetbIsMoving true))

(event Custom|Movement
  ;[1 1 1] Movement
  (Transformation|AddActorWorldOffset (* (Variables|Default|GetDirectionToGo) (Variables|Default|GetIntensityMovement))))

(event Custom|StopMovement
  ;[1 1 1] Stop movement and set available
  (Utilities|Time|ClearandInvalidateTimerbyHandle (Variables|Default|GetTimerMovement))
  (bind _asbp_spawn_platforms (Utilities|Casting|CastToBP_SpawnPlatforms (Components|GetOwner))
    (:then
      (Default|RestoreMana _asbp_spawn_platforms self)
      (Variables|Default|SetbIsMoving false))
    (:CastFailed
      (Actor|DestroyActor))))

(event EventBeginPlay)

(event Collision|EventActorBeginOverlap
  (params (OtherActor :type Actor%20Object%20Reference)))

(event EventTick
  (params (DeltaSeconds :type Float%20%28single-precision%29)))

(fn ConstructionScript)