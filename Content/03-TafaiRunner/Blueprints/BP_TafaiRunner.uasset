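; Player character for the Tafai side-view runner, spawning its platform spawner and height-following camera, HUD and tutorial widgets.
; Touch swipes set a Jump, Dash or Down state, gated by onboarding flags, each action costing mana.
; Dash fakes speed by zeroing velocity and gravity while raising global time dilation; Down drops through platforms or fast-falls.
; A looping timer trace drains mana on tagged surfaces, and low landings switch to swimming.
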(event OnComponentBeginOverlap(CapsuleComponent)
  (params (OverlappedComponent :type Primitive%20Component%20Object%20Reference) (OtherActor :type Actor%20Object%20Reference) (OtherComp :type Primitive%20Component%20Object%20Reference) (OtherBodyIndex :type Integer) (bFromSweep :type Boolean) (SweepResult :type Hit%20Result%20Structure%20%28by%20ref%29))
  ;[1 1 1] Regarde sur quel plateforme on est
  (bind _asbp_platforme_parent (Utilities|Casting|CastToBP_PlatformeParent OtherActor)
    (:then
      (Variables|Reference|SetActualPlateformRef _asbp_platforme_parent))
    (:CastFailed
      ;[1 1 1] Sinon quel sphere de mana on touche
      (bind _asbp_bulle_de_mana_tafai (Utilities|Casting|CastToBP_BulleDeMana_Tafai OtherActor)
        (:then
          (Default|StopMovement _asbp_bulle_de_mana_tafai))
        (:CastFailed
          (Utilities|Casting|CastToBP_EndLand_Tafai OtherActor)
          (Variables|Default|SetState "NewEnumerator4"))))))

(event Custom|SuckTheMana
  (bind _returnvalue (Transformation|GetActorLocation))
  ;[1 1 1] Retire du mana si il se trouve sur quelque chose qui a le tag AbsorbeMana
  (bind (_outhit _returnvalue_2) (Collision|LineTraceByChannel _returnvalue (- _returnvalue "0, 0,105.000000") "TraceTypeQuery2" false 0 "None"))
  (if _returnvalue_2
    (if (Actor|ActorHasTag (.HitActor (Collision|BreakHitResult _outhit)) "AbsorbeMana")
      (CallFunction|SuckMana 1.0))))

(event Custom|SuckMana
  (params (ManaToRemove :type Float%20%28single-precision%29))
  ;[1 1 1] Mana absorber par la plateforme
  (CallFunction|RemoveMana ManaToRemove)
  (Audio|PlaySound2D "/Game/03-TafaiRunner/SFX/SC_lose_mana.SC_lose_mana" 1.0 1.0 0.0 0 0))

(event Custom|ShowDash
  ;[1 1 1] Gestion du Tuto
  (Default|ShowDashonBoarding (Variables|Default|GetOnBoardingRef))
  (Variables|Default|SetCanDash? true)
  (Audio|PlaySound2D "/Game/MetaGame/Sounds/S_tap.S_tap" 1.0 1.0 0.0 0 0))

(event Custom|StopDash
  ;[1 1 1] Gestion du Tuto
  (Default|StopAnimationBeingPlayed (Variables|Default|GetOnBoardingRef))
  (Game|SetGamePaused false)
  (Utilities|DashwithDilation))

(event Custom|UnpauseGame
  ;[1 1 1] Gestion du Tuto
  (Game|SetGamePaused false))

(event Custom|ActionMana
  ;[1 1 1] Cout d'action en mana
  (CallFunction|RemoveMana (Variables|Mana|GetActionManaCost)))

(event Custom|CreateHUD
  ;[1 1 1] Créé le hud au moment ou le gm lui dit (a la fin de la cinematique)
  (bind _returnvalue (UserInterface|CreateWidget "/Game/03-TafaiRunner/Widget/WBP_HUD_Tafai.WBP_HUD_Tafai_C"))
  (bind _output_get (Variables|Reference|SetW_HUD_Ref _returnvalue))
  (UserInterface|Viewport|AddtoViewport _output_get 0)
  (bind _returnvalue_2 (UserInterface|CreateWidget "/Game/03-TafaiRunner/Widget/WBP_OnBoarding.WBP_OnBoarding_C"))
  (UserInterface|Viewport|AddtoViewport _returnvalue_2 0)
  (Variables|Default|SetOnBoardingRef _returnvalue_2))

(event Custom|UpdateMana
  (params (ManaToAdd :type Float%20%28single-precision%29))
  ;[1 1 1] Ajoute le mana de la sphere de mana
  (CallFunction|AddMana ManaToAdd))

(event Custom|ShowOnBoardJump
  ;[1 1 1] Gestion du Tuto
  (Default|ShowJumponBoarding (Variables|Default|GetOnBoardingRef))
  (Variables|Default|SetCanJump? true)
  (Audio|PlaySound2D "/Game/MetaGame/Sounds/S_tap.S_tap" 1.0 1.0 0.0 0 0))

(event Custom|StopAnimsOnBoard
  ;[1 1 1] Gestion du Tuto
  (Default|StopAnimationBeingPlayed (Variables|Default|GetOnBoardingRef))
  (Game|SetGamePaused false)
  (Utilities|FlowControl|DoN 1
    (:Exit
      (Variables|Default|SetCanJump? false)
      (Variables|Default|SetCanGoDown false)
      (Variables|Default|SetCanDash? false)
      (Variables|Bool|SetbDashedInAir? false))))

(event Custom|ActivePlateformeDetection
  ;[1 1 1] Retire du mana si il se trouve sur quelque chose qui a le tag AbsorbeMana
  (bind _returnvalue (Utilities|Time|SetTimerbyEvent (delegate Custom|SuckTheMana) 0.1 true))
  (Variables|Default|SetSuckManaHandle _returnvalue))

(event Custom|ShowDownOnboard
  ;[1 1 1] Gestion du Tuto
  (Default|ShowonBoardingDown (Variables|Default|GetOnBoardingRef))
  (Variables|Default|SetCanGoDown true)
  (Audio|PlaySound2D "/Game/MetaGame/Sounds/S_tap.S_tap" 1.0 1.0 0.0 0 0))

(event Custom|ShowAbsorbtion
  ;[1 1 1] Gestion du Tuto
  (bind _returnvalue (UserInterface|CreateWidget "/Game/03-TafaiRunner/Widget/WBP_SuckMana.WBP_SuckMana_C" (Game|GetPlayerController 0)))
  (UserInterface|Viewport|AddtoViewport _returnvalue 0)
  (Audio|PlaySound2D "/Game/MetaGame/Sounds/S_tap.S_tap" 1.0 1.0 0.0 0 0)
  (Variables|Bool|SetbDashedInAir? false))

(event EventBeginPlay
  (bind _returnvalue (Game|SpawnActorfromClass "/Script/Engine.CameraActor" (Math|Transform|MakeTransform (Variables|Default|GetCameraWorldLocation) "0,-90.000000, 0" "1,1,1") "Undefined" self 0))
  (bind _output_get (Variables|Default|SetCameraActorRef _returnvalue))
  ;[1 1 1] BeginPlay
  (Game|Player|SetViewTargetwithBlend (Game|GetPlayerController 0) _output_get 0.0 "VTBlend_Linear" 0.0 false)
  (bind _returnvalue_2 (Game|SpawnActorfromClass "/Game/03-TafaiRunner/Blueprints/BP_SpawnPlatforms.BP_SpawnPlatforms_C" (Math|Transform|MakeTransform (+ (Transformation|GetActorLocation) "2310.000000, 0,-600.000000") "0,180.000000, 0" "1,1,1") "Undefined" self 0))
  (Variables|Reference|SetPlateformSpawnerRef _returnvalue_2)
  (bind _aspc_tafai_runner (Utilities|Casting|CastToPC_TafaiRunner (Game|GetPlayerController 0)))
  (Variables|Reference|SetPC_TafaiRef _aspc_tafai_runner)
  (Variables|Default|SetActualZLocation (.z (Transformation|GetActorLocation)))
  (Variables|Default|SetBaseGravityScaleRef (Variables|/Script/Engine.CharacterMovementComponent|GetGravityScale (Variables|Character|GetCharacterMovement)))
  (CallFunction|ActivePlateformeDetection)
  (CallFunction|AddMana 0.0))

(event EventOnLanded
  (params (Hit :type Hit%20Result%20Structure%20%28by%20ref%29))
  (bind _returnvalue (Transformation|GetActorLocation))
  (bind _charactermovement (Variables|Character|GetCharacterMovement))
  ;[1 1 1] On Landed
  (Variables|Bool|SetbJumped? false)
  (Variables|Bool|SetbDashedInAir? false)
  (Variables|Bool|SetbInAction? false)
  (Variables|Default|SetbIsDownFast false)
  (Variables|/Script/Engine.CharacterMovementComponent|SetGravityScale _charactermovement (Variables|Default|GetBaseGravityScale))
  (Variables|/Script/Engine.CharacterMovementComponent|SetMaxAcceleration _charactermovement (Variables|Default|GetBaseMaxAcceleration))
  (Variables|Default|SetActualZLocation (.z _returnvalue))
  (if (< (.z _returnvalue) 2.8e+02)
    (Variables|Default|SetState "NewEnumerator5")
    (Effects|SpawnEmitteratLocation "/Game/03-TafaiRunner/ParticleSystems/PS_EnterWater.PS_EnterWater" (Transformation|GetActorLocation))
    (Audio|PlaySoundatLocation "/Game/03-TafaiRunner/SFX/S_splash_water.S_splash_water" "0, 0, 0" "0, 0, 0" 0.8 1.0 0.0 0 0 0)
    (else
      (Variables|Default|SetState "NewEnumerator4"))))

(event EventTick
  (params (DeltaSeconds :type Float%20%28single-precision%29))
  (Utilities|SetCameraLocation)
  ;[1 1 1] Debug
  (Development|PrintString (Utilities|String|Append "Dash en l'air : " (Utilities|String|ToString(Boolean) (Variables|Bool|GetbDashedInAir?)) " 
" "Sauter : " (Utilities|String|ToString(Boolean) (Variables|Bool|GetbJumped?)) " 
" "In action ?  " (Utilities|String|ToString(Boolean) (Variables|Bool|GetbInAction?)) " 
" "Z location : " (Utilities|String|ToString(Float) (.z (Transformation|GetActorLocation))) " 
" "Z velocity : " (Utilities|String|ToString(Float) (.z (Transformation|GetVelocity))) " 
" "State : " (Utilities|String|EnumtoString (Variables|Default|GetState))) true true "(R=0.000000,G=0.660000,B=1.000000,A=1.000000)" DeltaSeconds))

(event Input|KeyboardEvents|NumPadZero
  (params (Key :type Key%20Structure))
  ;[1 1 1] Debuging only       SPEEEED BOOOOOST
  (:Pressed
    (Utilities|Time|SetGlobalTimeDilation 1e+01))
  (:Released
    (Utilities|Time|SetGlobalTimeDilation 1.0)))

(event Input|TouchEvents|InputTouch
  (params (Location :type Vector) (FingerIndex :type ETouchIndex%20Enum))
  (bind _returnvalue (CallFunction|ScreenPosition))
  (bind _actualplateformref (Variables|Reference|GetActualPlateformRef))
  (bind _charactermovement (Variables|Character|GetCharacterMovement))
  (:Pressed
    ;[1 1 1] Prend la premiere position du doigt sur l'écran
    (Variables|TouchCoord|SetOldFingerPosition _returnvalue)
    (Variables|Bool|SetbIsPressed? true))
  (:Released
    (Variables|Bool|SetbIsPressed? false))
  (:Moved
    ;[1 1 1] Verifie le mouvement du doigt et si l'action est possible
    (Variables|TouchCoord|SetActualFingerPosition _returnvalue)
    (if (Variables|Bool|GetbIsPressed?)
      (Utilities|SwipeDirection
        (:True
          (if (not (Variables|Bool|GetbInAction?))
            (Variables|Bool|SetbInAction? true :!label _label)
            (CallFunction|ActionMana)
            ;[1 1 1] Fait une action en fonction du mouvement fait
            (switch Utilities|FlowControl|Switch|SwitchonEnum_State (Variables|Default|GetState)
              (:NewEnumerator0
                (if (Variables|Default|GetCanJump?)
                  (Character|Jump)
                  (Audio|PlaySound2D "/Game/03-TafaiRunner/SFX/SC_jump.SC_jump" 1.0 1.0 0.0 0 0)
                  (Variables|Bool|SetbJumped? true)
                  (Effects|SpawnEmitteratLocation "/Game/03-TafaiRunner/ParticleSystems/PS_Saut.PS_Saut" "0, 0, 0")
                  (Utilities|FlowControl|DoN 2
                    (:Exit
                      (CallFunction|StopAnimsonBoard :!label _label_2)))
                  (else
                    (Variables|Default|SetState "NewEnumerator4" :!label _label_3)
                    (Variables|Bool|SetbInAction? false :!label _label_4))))
              (:NewEnumerator1
                (if (Variables|Default|GetCanDash?)
                  (if (< (.z (Transformation|GetActorLocation)) 2.8e+02)
                    (goto _label_4)
                    (elif (Variables|Default|GetOnBoardDash)
                      (Variables|Default|SetOnBoardDash false)
                      (CallFunction|StopDash)
                      (else
                        (Utilities|DashwithDilation)
                        (Utilities|FlowControl|DoOnce false
                          (:Completed
                            (goto _label_2))))))
                  (else
                    (goto _label_3))))
              (:NewEnumerator2
                (if (Variables|Default|GetCanGoDown)
                  (if (< (.z (Transformation|GetActorLocation)) 2.8e+02)
                    (Variables|Bool|SetbInAction? false)
                    (elif (Variables|Default|GetbIsDownFast)
                      (Variables|/Script/Engine.CharacterMovementComponent|SetGravityScale _charactermovement (* (Variables|Default|GetBaseGravityScale) 5.0))
                      (Variables|/Script/Engine.CharacterMovementComponent|SetMaxAcceleration _charactermovement (* (Variables|Default|GetBaseMaxAcceleration) 6.0))
                      (else
                        (Utilities|IsValid _actualplateformref
                          (:Is%20Valid
                            (Default|DisableColision _actualplateformref)
                            (Audio|PlaySound2D "/Game/03-TafaiRunner/SFX/SC_jump.SC_jump" 1.0 1.0 0.0 0 0)
                            (Utilities|FlowControl|DoOnce false
                              (:Completed
                                (goto _label_2))))))))
                  (else
                    (goto _label_3)))))
            (elif (Math|Boolean|ANDBoolean (Utilities|Enum|Equal(Enum) (Variables|Default|GetState) "NewEnumerator1") (Variables|Bool|GetbJumped?) (not (Variables|Bool|GetbDashedInAir?)) (not (Variables|Default|GetbIsDownFast)))
              (Variables|Bool|SetbDashedInAir? true)
              (goto _label)
              (elif (Math|Boolean|ANDBoolean (Utilities|Enum|Equal(Enum) (Variables|Default|GetState) "NewEnumerator2") (Variables|Bool|GetbJumped?) (not (Variables|Default|GetbIsDownFast)) (not (Variables|Bool|GetbDashedInAir?)))
                (Variables|Default|SetbIsDownFast true)
                (goto _label)))))))))

(fn ConstructionScript
  (bind _returnvalue (Transformation|GetActorLocation))
  (Rendering|Material|SetScalarParameterValue "/Game/03-TafaiRunner/Materials/MPC_TafaiRunner.MPC_TafaiRunner" "TafaiRadius" (Variables|OceanCalmer|GetOceanCalmerRadius) :!class /Script/Engine.KismetMaterialLibrary)
  (Rendering|Material|SetScalarParameterValue "/Game/03-TafaiRunner/Materials/MPC_TafaiRunner.MPC_TafaiRunner" "TafaiHardness" (Variables|OceanCalmer|GetOceanCalmerHardness) :!class /Script/Engine.KismetMaterialLibrary)
  (Rendering|Material|SetVectorParameterValue "/Game/03-TafaiRunner/Materials/MPC_TafaiRunner.MPC_TafaiRunner" "TafaiWorldPosition" (Utilities|Struct|MakeLinearColor (.x _returnvalue) (.y _returnvalue) -2.5e+02 1.0) :!class /Script/Engine.KismetMaterialLibrary))

(fn LinetraceCoord
  (bind _returnvalue (Transformation|GetActorLocation))
  (return (+ _returnvalue "0, 0,10.000000") (- _returnvalue "0, 0,5.000000")))

(fn ScreenPosition
  (bind _returnvalue (Game|GetPlayerController 0))
  (bind (_locationx _locationy) (Class|PlayerController|GetInputTouchState _returnvalue "Touch1"))
  (return (Math|Vector2D|MakeVector2D _locationx _locationy)))

(fn RemoveMana
  (params (Remove :type Float%20%28single-precision%29))
  (if (< (- (Variables|Mana|GetMana) Remove) 0.0)
    (Variables|Mana|SetMana 0.0)
    (else
      (Variables|Mana|SetMana (- (Variables|Mana|GetMana) Remove))))
  (Default|UpdateManaBar (Variables|Reference|GetW_HUD_Ref) (Variables|Mana|GetMana) (Variables|Mana|GetMaxMana)))

(fn AddMana
  (params (Add :type Float%20%28single-precision%29))
  (if (> (+ (Variables|Mana|GetMana) Add) 1e+02)
    (Variables|Mana|SetMana 1e+02)
    (else
      (Variables|Mana|SetMana (+ (Variables|Mana|GetMana) Add))))
  (Default|UpdateManaBar (Variables|Reference|GetW_HUD_Ref) (Variables|Mana|GetMana) (Variables|Mana|GetMaxMana)))