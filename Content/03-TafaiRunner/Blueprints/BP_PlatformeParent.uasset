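; BP_PlatformeParent is the parent moving platform of TafaiRunner, with one-way collision for BP_TafaiRunner.
; A looping timer offsets it along DirectionToGo, scaled by IntensityMovement, until StopMovement clears it (if CanBeStop) and returns it to its owning BP_SpawnPlatforms for reuse.
; The UnderCheck overlap disables Cube collision so the runner passes up from below, while DisableColision briefly disables it for dropping through from above.
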(event OnComponentBeginOverlap(UnderCheck)
  (params (OverlappedComponent :type Primitive%20Component%20Object%20Reference) (OtherActor :type Actor%20Object%20Reference) (OtherComp :type Primitive%20Component%20Object%20Reference) (OtherBodyIndex :type Integer) (bFromSweep :type Boolean) (SweepResult :type Hit%20Result%20Structure%20%28by%20ref%29))
  ;[1 1 1] Detect si le perso viens de dessous et disable la collision
  (Utilities|Casting|CastToBP_TafaiRunner OtherActor)
  (Collision|SetCollisionEnabled (Variables|Default|GetCube) "NoCollision"))

(event OnComponentEndOverlap(UnderCheck)
  (params (OverlappedComponent :type Primitive%20Component%20Object%20Reference) (OtherActor :type Actor%20Object%20Reference) (OtherComp :type Primitive%20Component%20Object%20Reference) (OtherBodyIndex :type Integer))
  ;[1 1 1] Detect si le perso viens de dessous et disable la collision
  (Utilities|Casting|CastToBP_TafaiRunner OtherActor)
  (Collision|SetCollisionEnabled (Variables|Default|GetCube) "QueryAndPhysics"))

(event Custom|ActivatePlatform
  ;[1 1 1] Movement
  (bind _returnvalue (Utilities|Time|SetTimerbyEvent (delegate Custom|Movement) 0.01 true))
  (Variables|Default|SetTimerMovement _returnvalue)
  (Variables|Default|SetbIsMoving true))

(event Custom|Movement
  ;[1 1 1] Movement
  (Transformation|AddActorWorldOffset (* (Variables|Default|GetDirectionToGo) (Variables|Default|GetIntensityMovement))))

(event Custom|StopMovement
  ;[1 1 1] Stop movement and set available
  (if (Variables|Default|GetbCanBeStop?)
    (Utilities|Time|ClearandInvalidateTimerbyHandle (Variables|Default|GetTimerMovement))
    (bind _asbp_spawn_platforms (Utilities|Casting|CastToBP_SpawnPlatforms (Components|GetOwner)))
    (Default|RestorePlatformes _asbp_spawn_platforms self)
    (Variables|Default|SetbIsMoving false)))

(event Custom|DisableColision
  ;[1 1 1] Disable la collision pour que le perso traverse du dessus
  (Collision|SetCollisionEnabled (Variables|Default|GetCube) "NoCollision")
  (Utilities|FlowControl|Delay 2.0)
  (Collision|SetCollisionEnabled (Variables|Default|GetCube) "QueryAndPhysics"))

(fn ConstructionScript)