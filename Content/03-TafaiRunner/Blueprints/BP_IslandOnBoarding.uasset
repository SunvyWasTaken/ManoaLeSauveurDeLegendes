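; Tutorial island for TafaiRunner that teaches jump, down, dash and absorption before the endless platforms begin.
; One-shot trigger overlaps tell BP_TafaiRunner to show each prompt, then disable themselves and pause the game.
; The StartGen trigger enables all three movement abilities and calls StartSpawnPlateform on its owning BP_SpawnPlatforms.
; It also feeds a radius and its position into MPC_TafaiRunner to calm the surrounding sea.
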(event OnComponentBeginOverlap(TriggerJumpOnBoard)
  (params (OverlappedComponent :type Primitive%20Component%20Object%20Reference) (OtherActor :type Actor%20Object%20Reference) (OtherComp :type Primitive%20Component%20Object%20Reference) (OtherBodyIndex :type Integer) (bFromSweep :type Boolean) (SweepResult :type Hit%20Result%20Structure%20%28by%20ref%29))
  ;[1 1 1] Show JumpHud
  (CallFunction|ShowJump OtherActor)
  (Collision|SetCollisionEnabled (Variables|Default|GetTriggerJumpOnBoard) "NoCollision")
  (Game|SetGamePaused true))

(event OnComponentBeginOverlap(TriggerDownOnBoard)
  (params (OverlappedComponent :type Primitive%20Component%20Object%20Reference) (OtherActor :type Actor%20Object%20Reference) (OtherComp :type Primitive%20Component%20Object%20Reference) (OtherBodyIndex :type Integer) (bFromSweep :type Boolean) (SweepResult :type Hit%20Result%20Structure%20%28by%20ref%29))
  ;[1 1 1] ShowDownOnboard
  (bind _asbp_tafai_runner (Utilities|Casting|CastToBP_TafaiRunner OtherActor))
  (Utilities|FlowControl|DoOnce false
    (:Completed
      (Default|ShowDownOnboard _asbp_tafai_runner)
      (Collision|SetCollisionEnabled (Variables|Default|GetTriggerDownOnBoard) "NoCollision")
      (Game|SetGamePaused true)
      (Collision|SetCollisionEnabled (Variables|Default|GetPlateforme7) "NoCollision"))))

(event OnComponentBeginOverlap(WaterPlateformTuto)
  (params (OverlappedComponent :type Primitive%20Component%20Object%20Reference) (OtherActor :type Actor%20Object%20Reference) (OtherComp :type Primitive%20Component%20Object%20Reference) (OtherBodyIndex :type Integer) (bFromSweep :type Boolean) (SweepResult :type Hit%20Result%20Structure%20%28by%20ref%29))
  (bind _asbp_tafai_runner (Utilities|Casting|CastToBP_TafaiRunner OtherActor))
  (Utilities|FlowControl|DoOnce false
    (:Completed
      (Default|ShowAbsorbtion _asbp_tafai_runner)
      (Collision|SetCollisionEnabled (Variables|Default|GetWaterPlateformTuto) "NoCollision")
      (Game|SetGamePaused true))))

(event OnComponentBeginOverlap(TriggerDashOnBoard)
  (params (OverlappedComponent :type Primitive%20Component%20Object%20Reference) (OtherActor :type Actor%20Object%20Reference) (OtherComp :type Primitive%20Component%20Object%20Reference) (OtherBodyIndex :type Integer) (bFromSweep :type Boolean) (SweepResult :type Hit%20Result%20Structure%20%28by%20ref%29))
  ;[1 1 1] ShowDash
  (bind _asbp_tafai_runner (Utilities|Casting|CastToBP_TafaiRunner OtherActor))
  (Utilities|FlowControl|DoOnce false
    (:Completed
      (Default|ShowDash _asbp_tafai_runner)
      (Collision|SetCollisionEnabled (Variables|Default|GetTriggerDashOnBoard) "NoCollision")
      (Game|SetGamePaused true))))

(event OnComponentBeginOverlap(StartGen)
  (params (OverlappedComponent :type Primitive%20Component%20Object%20Reference) (OtherActor :type Actor%20Object%20Reference) (OtherComp :type Primitive%20Component%20Object%20Reference) (OtherBodyIndex :type Integer) (bFromSweep :type Boolean) (SweepResult :type Hit%20Result%20Structure%20%28by%20ref%29))
  (bind _asbp_tafai_runner (Utilities|Casting|CastToBP_TafaiRunner OtherActor))
  (Variables|/Game/03-TafaiRunner/Blueprints/BP_TafaiRunner.BP_TafaiRunner_C|SetCanGoDown _asbp_tafai_runner true)
  (Variables|/Game/03-TafaiRunner/Blueprints/BP_TafaiRunner.BP_TafaiRunner_C|SetCanDash? _asbp_tafai_runner true)
  (Variables|/Game/03-TafaiRunner/Blueprints/BP_TafaiRunner.BP_TafaiRunner_C|SetCanJump? _asbp_tafai_runner true)
  (Utilities|FlowControl|DoOnce false
    (:Completed
      (bind _asbp_spawn_platforms (Utilities|Casting|CastToBP_SpawnPlatforms (Components|GetOwner)))
      (Default|StartSpawnPlateform _asbp_spawn_platforms)
      (Collision|SetCollisionEnabled (Variables|Default|GetStartGen) "NoCollision"))))

(event Custom|CustomEvent_0
  (bind _result (Math|Integer|DecrementInt (Variables|Default|GetTimer))
    (:%20%20
      (if (== _result 0)
        _))))

(event EventBeginPlay
  (Utilities|Time|SetTimerbyEvent (delegate Custom|CustomEvent_0) 1.0 true)
  (Rendering|Material|SetScalarParameterValue "/Game/03-TafaiRunner/Materials/MPC_TafaiRunner.MPC_TafaiRunner" "Radius" 5e+02 :!class /Script/Engine.KismetMaterialLibrary))

(event EventTick
  (params (DeltaSeconds :type Float%20%28single-precision%29))
  (bind _returnvalue (Transformation|GetActorLocation))
  ;[1 1 1] Calm the sea around the island
  (Rendering|Material|SetVectorParameterValue "/Game/03-TafaiRunner/Materials/MPC_TafaiRunner.MPC_TafaiRunner" "IslandWorldPosition" (Utilities|Struct|MakeLinearColor (.x _returnvalue) (.y _returnvalue) (.z _returnvalue) 1.0) :!class /Script/Engine.KismetMaterialLibrary))

(fn ConstructionScript
  (|CallParentFunction))

(fn ShowJump
  (params (Object :type Object%20Object%20Reference))
  (bind _asbp_tafai_runner (Utilities|Casting|CastToBP_TafaiRunner Object))
  (Utilities|FlowControl|DoOnce false
    (:Completed
      (Default|ShowonBoardJump _asbp_tafai_runner)
      (return))))