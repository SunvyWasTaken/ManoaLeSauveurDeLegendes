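; Platform spawner for the Tafai runner that pre-spawns hidden pools of normal, mana and breakable platforms, mana bubbles and rocks, plus an onboarding island.
; A looping timer makes a weighted random platform pick, with fallbacks for empty pools, then teleports it to a random height and activates it.
; Normal platforms can carry a rock from the pool or a newly spawned mana bubble.
; Restore events return items to their pools for reuse.
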(event Custom|RestoreObstacles
  (params (Obstacle :type Actor%20Object%20Reference))
  ;[1 1 1] Restore plateformes
  (bind _asbp_obstacles (Utilities|Casting|CastToBP_Obstacles Obstacle))
  (Utilities|Array|Add (Variables|Default|GetRocksAvailables) _asbp_obstacles)
  (Transformation|SetActorLocation _asbp_obstacles "0, 0,-1000.000000" false true))

(event Custom|TP%20Platform%20and%20StartMovementNormal
  ;[1 1 1] Faire TP les plateformes et lancer les movements
  (switch int (Math|Random|RandomIntegerinRange 0 4)
    (:0
      (Utilities|CheckifArrayEmpty (Variables|Plateformes|GetPlateformesNormalesAvailable) (Variables|Plateformes|GetPlateformesManaAvailable) :!label _label
        (:MainEmpty
          (CallFunction|MovementandTPPlatformsMana (Variables|Plateformes|GetPlateformesManaAvailable) :!label _label_2))
        (:MainNotEmpty
          (CallFunction|MovementandTPPlatforms (Variables|Plateformes|GetPlateformesNormalesAvailable) :!label _label_3))))
    (:1
      (goto _label))
    (:2
      (goto _label))
    (:3
      (Utilities|CheckifArrayEmpty (Variables|Plateformes|GetPlateformesManaAvailable) (Variables|Plateformes|GetPlateformesNormalesAvailable)
        (:MainEmpty
          (goto _label_3))
        (:MainNotEmpty
          (goto _label_2))))
    (:4
      (Utilities|CheckifArrayEmpty (Variables|Default|GetPlateformesCassablesAvailables) (Variables|Plateformes|GetPlateformesNormalesAvailable)
        (:MainEmpty
          (goto _label_3))
        (:MainNotEmpty
          (CallFunction|MovementandTPPlatformsCassables (Variables|Default|GetPlateformesCassablesAvailables)))))))

(event Custom|RestorePlatformes
  (params (Plateforme :type Actor%20Object%20Reference%20%28by%20ref%29))
  ;[1 1 1] Restore plateformes
  (bind _asbp_platforme_mana_child (Utilities|Casting|CastToBP_PlatformeMana_Child Plateforme)
    (:then
      (Utilities|Array|Add (Variables|Plateformes|GetPlateformesManaAvailable) _asbp_platforme_mana_child)
      (Utilities|Array|RemoveItem (Variables|Plateformes|GetPlateformesManaInMovement) _asbp_platforme_mana_child))
    (:CastFailed
      (bind _asbp_platforme_normal_child (Utilities|Casting|CastToBP_PlatformeNormal_Child Plateforme)
        (:then
          (Utilities|Array|Add (Variables|Plateformes|GetPlateformesNormalesAvailable) _asbp_platforme_normal_child)
          (Utilities|Array|RemoveItem (Variables|Plateformes|GetPlateformesNormalesInMovement) _asbp_platforme_normal_child))
        (:CastFailed
          (bind _asbp_platforme_cassable_child (Utilities|Casting|CastToBP_PlatformeCassable_Child Plateforme))
          (Utilities|Array|Add (Variables|Default|GetPlateformesCassablesAvailables) _asbp_platforme_cassable_child)
          (Utilities|Array|RemoveItem (Variables|Default|GetPlateformesCassablesMovements) _asbp_platforme_cassable_child))))))

(event Custom|RestoreMana
  (params (Mana :type Actor%20Object%20Reference))
  ;[1 1 1] Restore plateformes
  (bind _asbp_bulle_de_mana_tafai (Utilities|Casting|CastToBP_BulleDeMana_Tafai Mana))
  (Utilities|Array|Add (Variables|Default|GetManaAvailable) _asbp_bulle_de_mana_tafai)
  (Transformation|SetActorLocation _asbp_bulle_de_mana_tafai "0, 0,-1000.000000" false true))

(event Custom|StartSpawnPlateform
  (bind _returnvalue (Utilities|Time|SetTimerbyEvent (delegate Custom|TP%20Platform%20and%20StartMovementNormal) (Variables|VariablesChangeables|GetDelaySpawnPlatformes) true))
  (Variables|Default|SetSpawnPlateformeHandle _returnvalue))

(event Custom|StopPlateformSpawn
  (Utilities|Time|ClearandInvalidateTimerbyHandle (Variables|Default|GetSpawnPlateformeHandle)))

(event EventBeginPlay
  (bind _asgm_tafai_runner (Utilities|Casting|CastToGM_TafaiRunner (Game|GetGameMode)))
  (bind _output_get (Variables|Default|SetGMTafaiRef _asgm_tafai_runner))
  (Default|TransfertInfo _output_get self)
  ;[1 1 1] SpawnPlatformes
  (for _index (range 0 (- (Variables|VariablesChangeables|GetNumberOfNormalToSpawn) 1))
    (bind _returnvalue (Game|SpawnActorfromClass "/Game/03-TafaiRunner/Blueprints/BP_PlatformeNormal_Child.BP_PlatformeNormal_Child_C" (Math|Transform|MakeTransform "0, 0,-5000.000000" "0, 0, 0" "1,1,1") "Undefined" self 0))
    (Utilities|Array|Add (Variables|Plateformes|GetPlateformesNormalesAvailable) _returnvalue))
  (for _index_2 (range 0 (- (Variables|VariablesChangeables|GetNumberOfManaSucklToSpawn) 1))
    (bind _returnvalue_2 (Game|SpawnActorfromClass "/Game/03-TafaiRunner/Blueprints/BP_PlatformeMana_Child.BP_PlatformeMana_Child_C" (Math|Transform|MakeTransform "0, 0,-4950.000000" "0, 0, 0" "1,1,1") "Undefined" self 0))
    (Utilities|Array|Add (Variables|Plateformes|GetPlateformesManaAvailable) _returnvalue_2))
  (for _index_3 (range 0 (- (Variables|VariablesChangeables|GetNumberOfManaToSpawn) 1))
    (bind _returnvalue_3 (Game|SpawnActorfromClass "/Game/03-TafaiRunner/Blueprints/BP_BulleDeMana_Tafai.BP_BulleDeMana_Tafai_C" (Math|Transform|MakeTransform "0, 0,-4950.000000" "0, 0, 0" "1,1,1") "Undefined" self 0))
    (Utilities|Array|Add (Variables|Default|GetManaAvailable) _returnvalue_3)
    (bind _returnvalue_4 (Game|SpawnActorfromClass "/Game/03-TafaiRunner/Blueprints/BP_Obstacles.BP_Obstacles_C" (Math|Transform|MakeTransform "0, 0,-4950.000000" "0, 0, 0" "1,1,1") "Undefined" self 0))
    (Utilities|Array|Add (Variables|Default|GetRocksAvailables) _returnvalue_4))
  (for _index_4 (range 0 (- (Variables|VariablesChangeables|GetNumberOfCassableToSpawn) 1))
    (bind _returnvalue_5 (Game|SpawnActorfromClass "/Game/03-TafaiRunner/Blueprints/BP_PlatformeCassable_Child.BP_PlatformeCassable_Child_C" (Math|Transform|MakeTransform "0, 0,-4950.000000" "0, 0, 0" "1,1,1") "Undefined" 0 0))
    (Utilities|Array|Add (Variables|Default|GetPlateformesCassablesAvailables) _returnvalue_5))
  (bind _returnvalue_6 (Game|SpawnActorfromClass "/Game/03-TafaiRunner/Blueprints/BP_IslandOnBoarding.BP_IslandOnBoarding_C" (Math|Transform|MakeTransform "4710.000000,5210.000000,630.000000" "0, 0, 0" "1,1,1") "Undefined" self 0))
  (Default|ActivatePlatform _returnvalue_6))

(fn ConstructionScript)

(fn MovementandTPPlatforms
  (params (Platform%20Array :type Array%20of%20Actor%20Object%20References))
  (bind _returnvalue (Transformation|GetActorLocation))
  (bind _returnvalue_2 (Transformation|GetActorLocation))
  (bind _returnvalue_3 (Transformation|GetActorLocation))
  ;[1 1 1] On choisis une plateforme aléatoire
  (bind _asbp_platforme_normal_child (Utilities|Casting|CastToBP_PlatformeNormal_Child (Utilities|Array|Get(acopy) Platform%20Array (Math|Random|RandomIntegerinRange 0 (- (Utilities|Array|Length Platform%20Array) 1)))))
  (LocalVariables|SetPlateformeChoisie _asbp_platforme_normal_child)
  ;[1 1 1] On set le niveau de hauteur
  (LocalVariables|SetLvlAttributed (Math|Random|RandomIntegerinRange 0 (Variables|VariablesChangeables|GetNbrMaxDeNiveauHauteur)))
  ;[1 1 1] 1 chance sur 2 pour avoir du mana
  (switch int (Math|Random|RandomIntegerinRange 0 3)
    (:0
      _)
    (:1
      _)
    (:2
      (LocalVariables|SetAvecMana true))
    (:3
      (LocalVariables|SetbRockSpawned true)))
  ;[1 1 1] On remove la disponibilité de la plateforme
  (Utilities|Array|RemoveItem Platform%20Array (LocalVariables|GetPlateformeChoisie))
  ;[1 1 1] On tp la plateforme
  (Transformation|SetActorLocation (LocalVariables|GetPlateformeChoisie) (Math|Vector|MakeVector (+ (.x _returnvalue) 1e+03) (.y _returnvalue) (+ (* (LocalVariables|GetLvlAttributed) 5e+02) (.z _returnvalue))) false true)
  (if (LocalVariables|GetAvecMana)
    (bind _returnvalue_4 (Game|SpawnActorfromClass "/Game/03-TafaiRunner/Blueprints/BP_BulleDeMana_Tafai.BP_BulleDeMana_Tafai_C" (Math|Transform|MakeTransform "0, 0, 0" "0, 0, 0" "1,1,1") "Undefined" 0 0))
    ;[1 1 1] Tp le mana si y'en a
    (Transformation|SetActorLocation _returnvalue_4 (Math|Vector|MakeVector (+ (.x _returnvalue_2) 1e+03) (.y _returnvalue_2) (+ (* (LocalVariables|GetLvlAttributed) 5e+02) (+ (.z _returnvalue_2) 1e+02))) false true)
    ;[1 1 1] Active le mana
    (Default|ActivateMana _returnvalue_4)
    (elif (LocalVariables|GetbRockSpawned)
      (bind _output_get (LocalVariables|SetRockChosen (Utilities|Array|Get(acopy) (Variables|Default|GetRocksAvailables))))
      (Transformation|SetActorLocation _output_get (Math|Vector|MakeVector (+ (.x _returnvalue_3) 1e+03) (.y _returnvalue_3) (+ (* (LocalVariables|GetLvlAttributed) 5e+02) (+ (.z _returnvalue_3) 1e+02))) false true)
      (Default|ActivatePlatform _output_get)
      (Utilities|Array|RemoveItem (Variables|Default|GetRocksAvailables) _output_get)))
  ;[1 1 1] Et on active la plateforme
  (Default|ActivatePlatform (LocalVariables|GetPlateformeChoisie)))

(fn MovementandTPPlatformsMana
  (params (TargetArray :type Array%20of%20Actor%20Object%20References))
  (bind _returnvalue (Transformation|GetActorLocation))
  ;[1 1 1] On choisis une plateforme aléatoire
  (bind _asbp_platforme_mana_child (Utilities|Casting|CastToBP_PlatformeMana_Child (Utilities|Array|Get(acopy) TargetArray (Math|Random|RandomIntegerinRange 0 (- (Utilities|Array|Length TargetArray) 1)))))
  (LocalVariables|SetPlateformeChoisie _asbp_platforme_mana_child)
  ;[1 1 1] Si non, on regarde si le niveau est déjà prit
  (LocalVariables|SetLvlAttributed (Math|Random|RandomIntegerinRange 0 2))
  (Utilities|Array|RemoveItem TargetArray (LocalVariables|GetPlateformeChoisie))
  ;[1 1 1] On tp la plateforme
  (Transformation|SetActorLocation (LocalVariables|GetPlateformeChoisie) (Math|Vector|MakeVector (+ (.x _returnvalue) 1e+03) (.y _returnvalue) (+ (* (LocalVariables|GetLvlAttributed) 5e+02) (.z _returnvalue))) false true)
  ;[1 1 1] On set comme quoi le niveau est occupé
  (Utilities|Array|SetArrayElem (Variables|Plateformes|GetLvlsTaken) (LocalVariables|GetLvlAttributed) true)
  ;[1 1 1] Et on active la plateforme
  (Default|ActivatePlatform (LocalVariables|GetPlateformeChoisie)))

(fn SelectManaOrbe
  (bind _manaavailable (Variables|Default|GetManaAvailable))
  (bind _returnvalue (Utilities|Array|Length _manaavailable))
  (if (> _returnvalue 0) :!label _label
    (bind _output_get (Variables|Default|SetManaToSpawnRef (Utilities|Array|Get(acopy) (Variables|Default|GetManaAvailable) (Math|Random|RandomIntegerinRange 0 (- _returnvalue 1)))))
    (if (Variables|/Game/03-TafaiRunner/Blueprints/BP_BulleDeMana_Tafai.BP_BulleDeMana_Tafai_C|GetbIsMoving _output_get)
      (goto _label)
      (else
        (Utilities|Array|RemoveItem (Variables|Default|GetManaAvailable) _output_get)))))

(fn MovementandTPPlatformsCassables
  (params (TargetArray :type Array%20of%20Actor%20Object%20References))
  (bind _returnvalue (Transformation|GetActorLocation))
  ;[1 1 1] On choisis une plateforme aléatoire
  (bind _asbp_platforme_cassable_child (Utilities|Casting|CastToBP_PlatformeCassable_Child (Utilities|Array|Get(acopy) TargetArray (Math|Random|RandomIntegerinRange 0 (- (Utilities|Array|Length TargetArray) 1)))))
  (LocalVariables|SetPlateformeChoisie _asbp_platforme_cassable_child)
  ;[1 1 1] Si non, on regarde si le niveau est déjà prit
  (LocalVariables|SetLvlAttributed (Math|Random|RandomIntegerinRange 0 2))
  (Utilities|Array|RemoveItem TargetArray (LocalVariables|GetPlateformeChoisie))
  ;[1 1 1] On tp la plateforme
  (Transformation|SetActorLocation (LocalVariables|GetPlateformeChoisie) (Math|Vector|MakeVector (+ (.x _returnvalue) 1e+03) (.y _returnvalue) (+ (* (LocalVariables|GetLvlAttributed) 5e+02) (.z _returnvalue))) false true)
  ;[1 1 1] On set comme quoi le niveau est occupé
  (Utilities|Array|SetArrayElem (Variables|Plateformes|GetLvlsTaken) (LocalVariables|GetLvlAttributed) true)
  ;[1 1 1] Et on active la plateforme
  (Default|ActivatePlatform (LocalVariables|GetPlateformeChoisie)))