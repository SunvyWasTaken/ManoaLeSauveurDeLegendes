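; Game mode for the Tafai runner level, running the round from intro sequence to victory screen.
; After the intro it creates the player's HUD, starts a looping one-second countdown and plays music.
; Countdown thresholds spawn the end land far ahead of the player, then halt the platform spawner registered through TransfertInfo.
; EndGame fades the music and, after a delay, shows the victory menu, scoring Tafai's Mana against star thresholds.
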(event Custom|EndGame
  (Audio|Components|Audio|FadeOut (Variables|Default|Getmusic) 1.0 0.0 "Linear" :!class /Script/Engine.AudioComponent)
  (bind _returnvalue (UserInterface|CreateWidget "/Game/MetaGame/Widgets/WBP_MenuVictoire.WBP_MenuVictoire_C" (Game|GetPlayerController 0) (Math|Float|Truncate (Variables|/Game/03-TafaiRunner/Blueprints/BP_TafaiRunner.BP_TafaiRunner_C|GetMana (Variables|Default|GetTafaiRef))) 25 50 75 0.05))
  (Utilities|FlowControl|Delay 3.0)
  (UserInterface|Viewport|AddtoViewport _returnvalue 0))

(event Custom|GameTimer
  (bind _tafairef (Variables|Default|GetTafaiRef))
  (bind _returnvalue (Transformation|GetActorLocation _tafairef))
  (bind _returnvalue_2 (+ _returnvalue "26000.000000, 0,0.000000"))
  (bind _result (Math|Integer|DecrementInt (Variables|Default|GetTimeRemaining))
    (:%20%20
      (if (== _result 48)
        (Game|SpawnActorfromClass "/Game/03-TafaiRunner/Blueprints/BP_EndLand_Tafai.BP_EndLand_Tafai_C" (Math|Transform|MakeTransform (Math|Vector|MakeVector (.x _returnvalue_2) (.y _returnvalue_2) 1.2e+03) "0, 0, 0" "1,1,1") "Undefined" 0 0)
        (elif (== _result 6)
          (Default|StopPlateformSpawn (Variables|Default|GetSpawnPlateformRef)))))))

(event Custom|TransfertInfo
  (params (Actor :type Actor%20Object%20Reference))
  (bind _asbp_spawn_platforms (Utilities|Casting|CastToBP_SpawnPlatforms Actor))
  (Variables|Default|SetSpawnPlateformRef _asbp_spawn_platforms))

(event EventBeginPlay
  (bind _asbp_tafai_runner (Utilities|Casting|CastToBP_TafaiRunner (Game|GetPlayerCharacter 0)))
  (Variables|Default|SetTafaiRef _asbp_tafai_runner)
  (Sequencer|Player|CreateLevelSequencePlayer 0 (Utilities|Struct|MakeMovieSceneSequencePlaybackSettings true "(Value=0)" 1.0 0.0 false false false false false false false false))
  (Utilities|FlowControl|Delay (Variables|Default|GetIntroDuration))
  (Default|CreateHUD (Variables|Default|GetTafaiRef))
  (Utilities|Time|SetTimerbyEvent (delegate Custom|GameTimer) 1.0 true)
  (Utilities|FlowControl|Delay 2.0)
  (Audio|Components|Audio|Play (Variables|Default|Getmusic) 0.0))

(event EventTick
  (params (DeltaSeconds :type Float%20%28single-precision%29)))

(fn ConstructionScript)