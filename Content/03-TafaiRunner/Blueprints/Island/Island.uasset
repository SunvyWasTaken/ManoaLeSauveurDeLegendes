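; Island actor for Tafai Runner that scrolls past along negative X as moving scenery.
; A fast looping timer offsets it while CanMove is set; past an X limit it stops and teleports back to a fixed start until MoveIsland re-enables it.
; The construction script writes its position, mask radius and hardness to MPC_TafaiRunner to calm the surrounding sea.
; The runtime position update is unconnected, so the mask does not follow the movement.
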(event Custom|MoveIsland
  (Variables|Default|SetbCanMove true))

(event Custom|CustomEvent_0
  (if (Variables|Default|GetbCanMove)
    (Transformation|AddActorWorldOffset "-15.000000, 0, 0")
    (if (< (.x (Transformation|GetActorLocation)) -7.52e+04)
      (Variables|Default|SetbCanMove false)
      (Transformation|SetActorLocation "73860.000000,-16930.000000,190.000000" false false))))

(event EventBeginPlay
  (Utilities|Time|SetTimerbyEvent (delegate Custom|CustomEvent_0) 0.01 true))

(event Collision|EventActorBeginOverlap
  (params (OtherActor :type Actor%20Object%20Reference)))

(event EventTick
  (params (DeltaSeconds :type Float%20%28single-precision%29)))

(fn ConstructionScript
  (bind _returnvalue (Transformation|GetActorLocation))
  (Rendering|Material|SetVectorParameterValue "/Game/03-TafaiRunner/Materials/MPC_TafaiRunner.MPC_TafaiRunner" "IslandWorldPosition" (Utilities|Struct|MakeLinearColor (.x _returnvalue) (.y _returnvalue) (.z _returnvalue) 1.0) :!class /Script/Engine.KismetMaterialLibrary)
  (Rendering|Material|SetScalarParameterValue "/Game/03-TafaiRunner/Materials/MPC_TafaiRunner.MPC_TafaiRunner" "Radius" (Variables|Default|GetMaskRadius) :!class /Script/Engine.KismetMaterialLibrary)
  (Rendering|Material|SetScalarParameterValue "/Game/03-TafaiRunner/Materials/MPC_TafaiRunner.MPC_TafaiRunner" "Hardness" (Variables|Default|GetMaskHardness) :!class /Script/Engine.KismetMaterialLibrary))